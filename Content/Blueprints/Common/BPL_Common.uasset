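; Common Blueprint function library of shared gameplay helpers for game state, party members and world queries.
; Accessors reach the map UI controller and common map object through GameInstance interfaces.
; Story helpers clear event flags, teach skills, sync player level, and add or remove demons such as Hayataro.
; Utilities toggle player input, identify the player, do vector and rotator math, and sphere-trace ground for location, normal and surface type.
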(fn `ApplyNahobinoOpen`
  (`BPL_EventFlag.SetEventFlag` "sflag0004_no_union")
  (`BPL_EventFlag.SetEventFlag` "sflag0001_no_inochigoi")
  (`BPL_GodParameter.GodParameterSkillLearning` 41)
  (`BPL_GodParameter.GodParameterSkillLearning` 21))

(fn `Flatten`
  (params (InVec :type "Vector Structure"))
  (returns (ReturnValue :type "Vector Structure"))
  (return (`KismetMathLibrary.Normal` (`KismetMathLibrary.MakeVector` (.x InVec) (.y InVec)))))

(fn `GetDistance`
  (params (From :type "Vector Structure") (To :type "Vector Structure"))
  (returns (ReturnValue :type "Float (double-precision)"))
  (return (`KismetMathLibrary.Sqrt` (+ (`KismetMathLibrary.Square` (- (.x From) (.x To))) (`KismetMathLibrary.Square` (- (.z From) (.z To))) (`KismetMathLibrary.Square` (- (.y From) (.y To)))))))

(fn `GetMapCommon`
  (returns (rerutn :type "Actor Object Reference"))
  (bind _asbpi_map_common (cast `/Game/Blueprints/Map/BPI_MapCommon` (`GameplayStatics.GetGameInstance` null))
    (:`then`
      (bind _rerutn (`/Game/Blueprints/Map/BPI_MapCommon.BPI_GetMapCommon` _asbpi_map_common))
      (return _rerutn))
    (:`CastFailed`
      (return null))))

(fn `GetMapUICtrl`
  (returns (MapUICtrl :type "Actor Object Reference"))
  (bind _asbpi_project_game_instance (cast `/Game/Blueprints/GameData/BPI_ProjectGameInstance` (`GameplayStatics.GetGameInstance` null))
    (:`then`
      (bind _mapuicommon (`/Game/Blueprints/GameData/BPI_ProjectGameInstance.BPI_GetMapUICtrl` _asbpi_project_game_instance))
      (return _mapuicommon))
    (:`CastFailed`
      (return null))))

(fn `HayataroPartyIn`
  (returns (isEntry :type Boolean) (isBattleIn :type Boolean))
  (bind _returnvalue (`BPL_PartyData.EntryNkmBlank` 152))
  (if (>= _returnvalue 0)
    (bind _returnvalue_2 (`BPL_PartyData.SetNkmBattleUnit` _returnvalue true))
    (return true _returnvalue_2)
    (else
      (return false false))))

(fn `IsPlayer`
  (params (Actor :type "Actor Object Reference"))
  (returns (ReturnValue :type Boolean))
  (bind _aspawn (cast `Pawn` Actor)
    (:`then`
      (return (`Pawn.IsPlayerControlled` _aspawn)))
    (:`CastFailed`
      (return false))))

(fn `MaouPartyIn`
  (params (devilID :type Integer))
  (bind _returnvalue (`BPL_PartyData.EntryMaouBlank` devilID))
  (if (>= _returnvalue 0)
    _))

(fn `RemoveHayataro`
  (locals (lo_HiLevel :type Integer))
  (`BPL_PartyData.RemoveNkmByDevilID` 152))

(fn `RotMaskXY`
  (params (Rotation :type "Rotator Structure"))
  (returns (ReturnValue :type "Rotator Structure"))
  (return (`KismetMathLibrary.MakeRotator` (.yaw Rotation))))

(fn `SetPlayerIgnoreLookInput`
  (params (Ignore :type Boolean))
  (`Controller.SetIgnoreLookInput` (`GameplayStatics.GetPlayerController` null) Ignore))

(fn `SetPlayerIgnoreMoveInput`
  (params (Ignore :type Boolean))
  (`Controller.SetIgnoreMoveInput` (`GameplayStatics.GetPlayerController` null) Ignore))

(fn `SetPlayerLevelFlat`
  (locals (lo_HiLevel :type Integer))
  (`BPL_PartyData.PlayerLevelExpSync`))

(fn `TraceGround`
  (params (Base :type "Vector Structure") (Direction :type "Vector Structure") (Length :type "Float (double-precision)") (Radius :type "Float (double-precision)") (DrawDebugType :type "EDrawDebugTrace Enum" :default "None"))
  (returns (Hit :type Boolean) (Location :type "Vector Structure") (Normal :type "Vector Structure") (Surface :type "EPhysicalSurface Enum"))
  (bind (_outhit _returnvalue) (`KismetSystemLibrary.SphereTraceSingle` :`Start` (- Base (* Direction Length)) :`End` (+ Base (* Direction Radius)) :`Radius` Radius :`TraceChannel` "TraceTypeQuery3" :`DrawDebugType` DrawDebugType))
  (if _returnvalue
    (bind (_bblockinghit _binitialoverlap _time _distance _location _impactpoint _normal _impactnormal _physmat _hitactor _hitcomponent _hitbonename _hititem _elementindex _faceindex _tracestart _traceend) (`GameplayStatics.BreakHitResult` _outhit))
    (if (>= (`KismetMathLibrary.Dot_VectorVector` (- _impactpoint _tracestart) (`local.Direction`)) 0.0)
      (if (not (== _impactpoint (0.0 0.0 0.0)))
        (return true _location _normal (`PhysicalMaterial.SurfaceType` _physmat)))
      (else
        (return false _traceend (0.0 0.0 1.0) "SurfaceType_Default")))))