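; BPL_Camp is a Blueprint function library of helpers for the camp feature, covering player and Nkm (DevilId-based) data.
; It declares builders for added skills, status skills, bad status arrays and endure/weak data, plus queries for next-level experience and whether camp is open.
; All function bodies are empty or return default values, so only the signatures are visible here.
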(fn `GetAddSkill`
  (params (Level :type Integer) (DevilId :type Integer))
  (returns (AddSkill :type "Array of AddGetSkill Structure"))
  (return))

(fn `GetNowLevelNextExp`
  (params (Level :type Integer) (nkmIndex :type Integer))
  (returns (Exp :type Integer))
  (return 0))

(fn `IsCampOpen`
  (returns (IsOpen :type Boolean))
  (return false))

(fn `MakeAddSkill_Nkm`
  (params (devilId :type Integer) (level :type Integer))
  (returns (AddSkillData :type "Array of AddGetSkill Structure"))
  (return))

(fn `MakeAddSkill_Player`
  (params (level :type Integer))
  (returns (AddSkillArray :type "Array of AddGetSkill Structure"))
  (return))

(fn `MakeAddSkillData`
  (params (Level :type Integer) (Id :type Integer))
  (returns (AddSkill :type "Array of StatusAddSkillData Structure"))
  (return))

(fn `MakeBadStatusArray`
  (params (BadStatus :type Integer))
  (returns (BadStatusArray :type "Array of E_BAD_STATUS Enum"))
  (return))

(fn `MakeEndureWeadData`
  (params (DevilId :type Integer))
  (returns (`Return Value M En Weak` :type "Array of EndureWeakData Structure"))
  (return))

(fn `MakeStatusSkillData`
  (params (Array :type "Array of Integer (by ref)") (SkillPropaty :type "Array of Integer (by ref)"))
  (returns (SkillData :type "Array of StatusSkillData Structure"))
  (return))