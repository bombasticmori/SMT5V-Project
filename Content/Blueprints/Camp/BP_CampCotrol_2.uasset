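; BP_CampCotrol_2 is a camp controller child Blueprint that is mostly a stub.
; Its open, close, return-to-title and player-lock events are empty, as is the asset-loaded callback.
; GetIsCampOpen always returns false, while CheckCampOpenFlag returns the parent's result.
; BeginPlay, Tick and Destroyed only forward to the parent.
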(event `self.ReceiveBeginPlay`
  (`parent.ReceiveBeginPlay`))

(event `self.ReceiveTick`
  (params (DeltaSeconds :type "Float (single-precision)"))
  (`parent.ReceiveTick` DeltaSeconds))

(event `OnLoaded_20B106F442986DC0ACBDAAA873BBBE3A`
  (params (Loaded :type "Object Class Reference")))

(event `CampClose`)

(event `self.ReceiveDestroyed`
  (`parent.ReceiveDestroyed`))

(event `CampReturnTitle`)

(event `OpenCamp`)

(event `PlayerLock`
  (params (IsLock :type Boolean)))

(fn `CheckCampOpenFlag`
  (returns (ReturnValue :type Boolean))
  (bind _returnvalue (`parent.CheckCampOpenFlag`))
  (return _returnvalue))

(fn `GetIsCampOpen`
  (returns (IsCampOpen :type Boolean))
  (return false))

(fn `UserConstructionScript`)