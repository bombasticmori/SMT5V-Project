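; Status screen UI controller for the camp menu, also covering simple status, skill inheritance and fusion result views.
; BPI_ functions form the external surface for start, tick, visibility and inherit UI control.
; Helper functions are declared for skill, condition and biography page ticks, mouse slots and scrolling, button help and skill swap.
; All are empty stubs returning defaults; only BeginPlay and EndPlay do anything, calling their parents.
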(event `self.ReceiveBeginPlay`
  (`parent.ReceiveBeginPlay`))

(event `self.ReceiveEndPlay`
  (params (EndPlayReason :type "EEndPlayReason Enum" :default "Destroyed"))
  (`parent.ReceiveEndPlay` EndPlayReason))

(event `private_AnimStart`)

(event `private_InheritAnimStart`
  (params (Duration :type "Float (double-precision)")))

(fn `BindFunc_OnClickedFaceBtnLR`
  (params (move :type Integer)))

(fn `BindFunc_OnClickedFaceIcon`
  (params (move :type Integer)))

(fn `BindFunc_OnClickedParentSlot`
  (params (Index :type Integer)))

(fn `BindFunc_OnClickedRightSlot`
  (params (Index :type Integer)))

(fn `BindFunc_OnHoveredParentSlot`
  (params (Index :type Integer)))

(fn `BindFunc_OnHoveredRightSlot`
  (params (Index :type Integer)))

(fn `BindFunc_OnMovedParentScrollBarByMouse`
  (params (NewOffset :type Integer)))

(fn `BindFunc_OnMovedRightScrollBarByMouse`
  (params (NewOffset :type Integer)))

(fn `BPI_ChangeBtnHelpStatus_StatusUI`
  (params (Visibility :type Boolean))
  (returns (Success :type Boolean))
  (return false))

(fn `BPI_ChangeStatus`
  (returns (dummy :type Boolean))
  (return false))

(fn `BPI_CheckMouseHoverList`
  (returns (Main :type Boolean) (Sub :type Boolean))
  (return false false))

(fn `BPI_ClearMouseMediator`
  (returns (Success :type Boolean))
  (return false))

(fn `BPI_Close_SimpleStatus`
  (params (Immediate :type Boolean))
  (returns (dummy :type Boolean))
  (return false))

(fn `BPI_CloseInheritUI`
  (params (CloseUI :type Boolean) (ReturnCamera :type Boolean) (Immediate :type Boolean))
  (returns (dummy :type Boolean))
  (return false))

(fn `BPI_GetHoverIndex`
  (returns (Main :type Integer) (Sub :type Integer))
  (return 0 0))

(fn `BPI_Init_SimpleStatus`
  (params (StatusData :type "Object Object Reference") (WidgetPriority :type "E_WIDGET_PRIO Enum" :default "E_WIDGET_PRIO_DEFAULT"))
  (returns (success :type Boolean))
  (return false))

(fn `BPI_InitInheritUI`
  (params (CharaChanger :type "Object Object Reference") (UIStatusCtrlDataObjUnite :type "Object Object Reference"))
  (returns (Success :type Boolean))
  (return false))

(fn `BPI_IsComplete`
  (returns (IsComplete :type Boolean))
  (return false))

(fn `BPI_IsEndAnimation_InheritStatus`
  (returns (IsEnd :type Boolean))
  (return false))

(fn `BPI_IsEndAnimation_SimpleStatus`
  (returns (IsEnd :type Boolean))
  (return false))

(fn `BPI_Open_SimpleStatus`
  (params (Immediate :type Boolean))
  (returns (dummy :type Boolean))
  (return false))

(fn `BPI_RestartResultCtrl_FromMessage`
  (returns (dummy :type Boolean))
  (return false))

(fn `BPI_SetMouseMediator`
  (params (MouseMediator :type "Object Object Reference"))
  (returns (Success :type Boolean))
  (return false))

(fn `BPI_SetTaskBeforeViewEnd`
  (params (Runner :type "Object Object Reference"))
  (returns (Success :type Boolean))
  (return false))

(fn `BPI_SetVisibility`
  (params (Visibility :type "ESlateVisibility Enum" :default "Visible"))
  (returns (Success :type Boolean))
  (return false))

(fn `BPI_ShowFusionResultUI`
  (returns (dummy :type Boolean))
  (return false))

(fn `BPI_ShowInheritUI`
  (params (ParentTop :type Integer) (FirstCursorIndex :type Integer) (ChildTop :type Integer) (UseCostWindow :type Boolean))
  (returns (dummy :type Boolean))
  (return false))

(fn `BPI_ShowResistancesInheritResultUI`
  (returns (dummy :type Boolean))
  (return false))

(fn `BPI_StartCtrl`
  (params (DataObj :type "UIStatusCtrlDataObjBase Object Reference") (CtrlType :type "E_UI_STATUS_CTRL_TYPE Enum" :default "E_UI_STATUS_CTRL_TYPE_BTL_ENEMY") (StatusCharaChanger :type "/Game/Blueprints/Camp/Status/BPI_StatusCharaChanger Interface") (WidgetPriority :type "E_WIDGET_PRIO Enum" :default "E_WIDGET_PRIO_DEFAULT"))
  (returns (Success :type Boolean))
  (return false))

(fn `BPI_TickEvent`
  (params (DeltaSeconds :type "Float (double-precision)"))
  (returns (StatusEnd :type Boolean))
  (return false))

(fn `BPI_TickFunc_InheritResult`
  (returns (Decide :type Boolean) (Cancel :type Boolean))
  (return false false))

(fn `BPI_TickFunc_InheritStatus`
  (params (deltaTime :type "Float (double-precision)"))
  (returns (dummy :type Boolean))
  (return false))

(fn `BPI_UpdateInheritUI`
  (params (ParentTop :type Integer) (ParentCurrent :type Integer) (ChildTop :type Integer) (ChildCategory :type Integer) (ChildCurrent :type Integer))
  (returns (dummy :type Boolean))
  (return false))

(fn `ButtonHelpIn`
  (params (InSkipAnim :type Boolean) (PageType :type "E_UI_STATUS_PAGE_TYPE Enum" :default "E_UI_STATUS_PAGE_TYPE_SKILL") (InCtrlType :type "E_UI_STATUS_CTRL_TYPE Enum" :default "E_UI_STATUS_CTRL_TYPE_BTL_ENEMY")))

(fn `ButtonHelpOut`
  (params (SkipAnimation :type Boolean)))

(fn `Calc Move Index by Wheel`
  (params (InOffset :type Integer) (InMove :type Integer))
  (returns (CursorDataIndex :type Integer) (ScrollStack :type Integer) (CurosrMoved :type Boolean))
  (return 0 0 false))

(fn `Change Button Help Page Change`
  (params (PageType :type "E_UI_STATUS_PAGE_TYPE Enum" :default "E_UI_STATUS_PAGE_TYPE_SKILL") (CtrlType :type "E_UI_STATUS_CTRL_TYPE Enum" :default "E_UI_STATUS_CTRL_TYPE_BTL_ENEMY") (ForceChange :type Boolean)))

(fn `ChangeCost`)

(fn `CheckOpenFlag`
  (params (OpenFlag :type Integer) (Status :type "E_UI_STATUS_OPEN Enum" :default "E_UI_STATUS_OPEN_RACE"))
  (returns (Open :type Boolean))
  (return false))

(fn `CloseCommonWindow`)

(fn `CloseHelpWindow`
  (params (Immediate :type Boolean)))

(fn `CloseUI`)

(fn `CommonTickFunc`
  (params (InputNum :type Integer)))

(fn `CreateStatusWidget`)

(fn `DataStep`
  (params (InMove :type Integer))
  (returns (Moved :type Integer))
  (return 0))

(fn `EndViewStatus`)

(fn `FuncBiographyTick`
  (params (EnableChangeNewOld :type Boolean))
  (returns (Pushed :type Boolean))
  (return false))

(fn `FuncConditionTick`
  (params (EnableChangeNewOld :type Boolean))
  (returns (Pushed :type Boolean))
  (return false))

(fn `FuncHideUITick`)

(fn `FuncSkillTick`
  (params (EnableSkillSwap :type Boolean) (EnableChangeNewOld :type Boolean)))

(fn `FuncTWindowTick`)

(fn `GetCostColor`
  (params (Difference :type Integer))
  (returns (ReturnValue :type "LinearColor Structure"))
  (return))

(fn `GetEnableMouseCtrl`
  (returns (enable :type Boolean))
  (return false))

(fn `GetHoldInputButton`
  (returns (InputNum :type Integer) (Repeat :type Boolean))
  (return 0 false))

(fn `GetInputButton`
  (params (EnableA :type Boolean) (EnableX :type Boolean))
  (returns (InputNum :type Integer) (Repeat :type Boolean))
  (return 0 false))

(fn `GetIsComplete`
  (returns (IsComplete :type Boolean))
  (return false))

(fn `GetWithTitle`
  (returns (ReturnValue :type Boolean))
  (return false))

(fn `IsActiveBibleSkillSwap`
  (returns (ReturnValue :type Boolean))
  (return false))

(fn `IsActivePartySkillSwap`
  (returns (ReturnValue :type Boolean))
  (return false))

(fn `IsEnableButtonL`
  (params (IsTrigger :type Boolean))
  (returns (ReturnValue :type Boolean))
  (return false))

(fn `IsEnableButtonR`
  (params (IsTrigger :type Boolean))
  (returns (ReturnValue :type Boolean))
  (return false))

(fn `IsHolding`
  (returns (ReturnValue :type Boolean))
  (return false))

(fn `MyMakkaWindowClose`
  (params (inShowTotalWindow :type Boolean) (inAnimation :type Boolean)))

(fn `NewInit`
  (params (UIStatusData :type "UIStatusCtrlDataObjBase Object Reference (by ref)") (ControlType :type "E_UI_STATUS_CTRL_TYPE Enum" :default "E_UI_STATUS_CTRL_TYPE_BTL_ENEMY") (StatusCharaChanger :type "/Game/Blueprints/Camp/Status/BPI_StatusCharaChanger Interface (by ref)")))

(fn `NewTickFunc`
  (returns (StatusEnd :type Boolean))
  (return false))

(fn `OpenCommonWindow`)

(fn `ResetCursorPos`
  (params (PageType :type "E_UI_STATUS_PAGE_TYPE Enum" :default "E_UI_STATUS_PAGE_TYPE_SKILL")))

(fn `SetHelpWindow`
  (params (InputPin :type "UIStatusCtrlDataObjBase Object Reference")))

(fn `SkillPageChangeCursorButtonHelp`)

(fn `SlotType`
  (returns (MovableSkill :type Boolean) (SwitchableKamui :type Boolean))
  (return false false))

(fn `StartViewStatus`
  (returns (Success :type Boolean))
  (return false))

(fn `UpdateAnalyzeNewIcon`)

(fn `UpdateButtonHelp`)

(fn `UserConstructionScript`)