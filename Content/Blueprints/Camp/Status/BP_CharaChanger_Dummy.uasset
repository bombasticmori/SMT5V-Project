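; BP_CharaChanger_Dummy is a no-op stand-in for a character changer in the camp status screen.
; Its events for view start and end, initialization, character change, battle setup and pre-request are empty.
; Its functions for voice calls, rotation locking, preparation checks, initialization and init delay just return false, so it loads no models and holds no state.
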(event `/Game/Blueprints/Camp/Status/BPI_StatusCharaChanger.ViewStart`)

(event `/Game/Blueprints/Camp/Status/BPI_StatusCharaChanger.ViewEnd`)

(event `/Game/Blueprints/Camp/Status/BPI_StatusCharaChanger.Init`
  (params (SpawnPos :type "Transform Structure") (Type :type "E_UI_STATUS_CTRL_TYPE Enum" :default "E_UI_STATUS_CTRL_TYPE_BTL_ENEMY")))

(event `/Game/Blueprints/Camp/Status/BPI_StatusCharaChanger.ChangeChara`
  (params (DevilID :type Integer) (IsUnknown :type Boolean)))

(event `/Game/Blueprints/Camp/Status/BPI_StatusCharaChanger.Init_Battle`
  (params (SpawnPos :type "Transform Structure") (Type :type "E_UI_STATUS_CTRL_TYPE Enum" :default "E_UI_STATUS_CTRL_TYPE_BTL_ENEMY") (StatusCtrlDataBtl :type "Object Object Reference") (useAnalyzeItem :type Boolean)))

(event `/Game/Blueprints/Camp/Status/BPI_StatusCharaChanger.PreRequest`
  (params (DevilID :type Integer)))

(fn `CallVoice`
  (params (VoiceType :type "EDevilVoiceType Enum" :default "EDevilVoiceType_None"))
  (returns (dummy :type Boolean))
  (return false))

(fn `DisableRotation`
  (params (IsDisable :type Boolean))
  (returns (NoUse :type Boolean))
  (return false))

(fn `IsEndPreparation`
  (params (DevilID :type Integer))
  (returns (IsEnd :type Boolean))
  (return false))

(fn `NewInit`
  (params (DataObject :type "Object Object Reference") (SpawnTransform :type "Transform Structure") (WithModelLoad :type Boolean) (WithModelSpawn :type Boolean))
  (returns (Success :type Boolean))
  (return false))

(fn `NewInit_Battle`
  (params (StatusCtrlDataBtl :type "Object Object Reference") (BattleParty :type "Object Object Reference") (Type :type "E_UI_STATUS_CTRL_TYPE Enum" :default "E_UI_STATUS_CTRL_TYPE_BTL_ENEMY") (useAnalyzeItem :type Boolean))
  (returns (Dummy :type Boolean))
  (return false))

(fn `SetDelayInInit`
  (params (Num :type Integer))
  (returns (Dummy :type Boolean))
  (return false))

(fn `UserConstructionScript`)