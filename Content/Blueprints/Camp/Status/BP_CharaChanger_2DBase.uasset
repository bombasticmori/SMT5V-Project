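; Base Blueprint for the camp status character changer, defining the interface for displaying and switching devil models.
; Nearly every event and function is an empty stub or returns a default; only lifecycle events call their parent.
; The declared hooks cover async model loading and spawning, camera framing, materials, motion, IK, rotation input, voice, and camp or battle initialization, with no logic implemented here.
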(event `self.ReceiveBeginPlay`
  (`parent.ReceiveBeginPlay`))

(event `self.ReceiveTick`
  (params (DeltaSeconds :type "Float (single-precision)"))
  (`parent.ReceiveTick` DeltaSeconds))

(event `OnLoaded_F558972E4A9D79E3856B3ABB1474FD1D`
  (params (Loaded :type "Object Class Reference")))

(event `OnLoaded_79EC33A541A43AF01F7DA795713A1D41`
  (params (Loaded :type "Object Object Reference")))

(event `/Game/Blueprints/Camp/Status/BPI_StatusCharaChanger.ViewStart`)

(event `/Game/Blueprints/Camp/Status/BPI_StatusCharaChanger.ViewEnd`)

(event `/Game/Blueprints/Camp/Status/BPI_StatusCharaChanger.Init`
  (params (SpawnPos :type "Transform Structure") (Type :type "E_UI_STATUS_CTRL_TYPE Enum" :default "E_UI_STATUS_CTRL_TYPE_BTL_ENEMY")))

(event `/Game/Blueprints/Camp/Status/BPI_StatusCharaChanger.ChangeChara`
  (params (DevilID :type Integer) (IsUnknown :type Boolean)))

(event `self.ReceiveDestroyed`
  (`parent.ReceiveDestroyed`))

(event `/Game/Blueprints/Camp/Status/BPI_StatusCharaChanger.Init_Battle`
  (params (SpawnPos :type "Transform Structure") (Type :type "E_UI_STATUS_CTRL_TYPE Enum" :default "E_UI_STATUS_CTRL_TYPE_BTL_ENEMY") (StatusCtrlDataBtl :type "Object Object Reference") (useAnalyzeItem :type Boolean)))

(event `/Game/Blueprints/Camp/Status/BPI_StatusCharaChanger.PreRequest`
  (params (DevilID :type Integer)))

(event `self.ReceiveEndPlay`
  (params (EndPlayReason :type "EEndPlayReason Enum" :default "Destroyed"))
  (`parent.ReceiveEndPlay` EndPlayReason))

(event `private_LoadModel`)

(event `private_ActivateTextureStreamingArea`)

(event `private_MotionReset`)

(fn `CallVoice`
  (params (VoiceType :type "EDevilVoiceType Enum" :default "EDevilVoiceType_None"))
  (returns (dummy :type Boolean))
  (return false))

(fn `CharaChangeGC`)

(fn `CheckLoadedModel`
  (returns (Complete :type Boolean) (Loaded :type Boolean) (Spawned :type Boolean) (DevilID :type Integer))
  (return false false false 0))

(fn `ConstLoadModelClassListMax`
  (returns (num :type Integer))
  (return 0))

(fn `ConstSpawnMax`
  (returns (Value :type Integer))
  (return 0))

(fn `DestroyDevilModelAll`)

(fn `DisableRotation`
  (params (IsDisable :type Boolean))
  (returns (NoUse :type Boolean))
  (return false))

(fn `FocusNowCurrentActor`
  (params (Target :type "/Game/Blueprints/Character/Base/CharaBase Object Reference") (DevilID :type Integer)))

(fn `GetDevilCameraCenter`
  (params (ST_StCameraSetUp :type "/Game/Blueprints/Camp/Status/ST_StCameraSetUp Structure (by ref)"))
  (returns (ReturnValue :type "Vector Structure"))
  (return (0.0 0.0 0.0)))

(fn `GetDevilCameraData`
  (params (DevilID :type Integer))
  (returns (ReturnValue :type "/Game/Blueprints/Camp/Status/ST_StCameraSetUp Structure"))
  (return))

(fn `GetDevilCameraDistance`
  (params (ST_StCameraSetUp :type "/Game/Blueprints/Camp/Status/ST_StCameraSetUp Structure (by ref)"))
  (returns (ReturnValue :type "Float (double-precision)"))
  (return 0.0))

(fn `GetDevilCameraRotation`
  (params (ST_StCameraSetUp :type "/Game/Blueprints/Camp/Status/ST_StCameraSetUp Structure (by ref)"))
  (returns (OutputPin :type "Rotator Structure"))
  (return))

(fn `GetDevilCameraRowName`
  (params (ID :type Integer))
  (returns (ExtensionPart :type String))
  (return ""))

(fn `GetDevilIDForAsset`
  (params (InDevilID :type Integer))
  (returns (OutDevilID :type Integer))
  (return 0))

(fn `GetDevilYaw`
  (returns (Yaw :type "Float (double-precision)"))
  (return 0.0))

(fn `GetModelClassReference`
  (params (ID :type Integer))
  (returns (Pawn :type "CustomPawn Soft Class Reference"))
  (return null))

(fn `GetNearlyNum`
  (params (LoopNum :type Integer))
  (returns (ReturnValue :type Integer))
  (return 0))

(fn `GetSpawnDelay`
  (params (step :type Integer))
  (returns (ret :type Integer))
  (return 0))

(fn `GetSpawnEarlyDelay`
  (params (step :type Integer))
  (returns (ret :type Integer))
  (return 0))

(fn `GetSpawnNeedMax`
  (params (InputPin :type "UIStatusCtrlDataObjBase Object Reference"))
  (returns (ReturnValue :type Integer))
  (return 0))

(fn `HideActor`)

(fn `IsEndPreparation`
  (params (DevilID :type Integer))
  (returns (IsEnd :type Boolean))
  (return false))

(fn `NeutralSpawnTransform`
  (returns (m_DefaultTransform :type "Transform Structure"))
  (return))

(fn `NewInit`
  (params (DataObject :type "Object Object Reference") (SpawnTransform :type "Transform Structure") (WithModelLoad :type Boolean) (WithModelSpawn :type Boolean))
  (returns (Success :type Boolean))
  (return false))

(fn `NewInit_Battle`
  (params (StatusCtrlDataBtl :type "Object Object Reference") (BattleParty :type "Object Object Reference") (Type :type "E_UI_STATUS_CTRL_TYPE Enum" :default "E_UI_STATUS_CTRL_TYPE_BTL_ENEMY") (useAnalyzeItem :type Boolean))
  (returns (Dummy :type Boolean))
  (return false))

(fn `PlayDevilMotion`
  (params (CharaBase :type "/Game/Blueprints/Character/Base/CharaBase Object Reference") (DevilID :type Integer)))

(fn `PreparePreSpawnList`)

(fn `PreSpawnTransform`
  (returns (ReturnValue :type "Transform Structure"))
  (return))

(fn `ProcessInputRotate`
  (params (DeltaSeconds :type "Float (double-precision)")))

(fn `ResizeClassList`)

(fn `ScaleCorrect`
  (params (InputPin :type "Actor Object Reference")))

(fn `SetDelayInInit`
  (params (Num :type Integer))
  (returns (Dummy :type Boolean))
  (return false))

(fn `SetDevilMaterial`
  (params (CharaBase :type "/Game/Blueprints/Character/Base/CharaBase Object Reference") (devilId :type Integer)))

(fn `SetDevilMaterialForRotate`
  (params (CharaBase :type "CustomPawn Object Reference") (devilId :type Integer)))

(fn `SetIK`
  (params (target :type "CustomPawn Object Reference") (DevilId :type Integer)))

(fn `SetMaterialFunc`
  (params (Material :type "Object Soft Object Reference") (Mesh :type "PrimitiveComponent Object Reference") (ElementIndex :type Integer)))

(fn `SetModelVisibility`
  (params (Target :type "/Game/Blueprints/Character/Base/CharaBase Object Reference") (DevilID :type Integer)))

(fn `SetMotionTable`
  (params (CharaBase :type "/Game/Blueprints/Character/Base/CharaBase Object Reference") (DevilId :type Integer)))

(fn `SetSelfTickEnable`
  (params (bEnabled :type Boolean)))

(fn `UserConstructionScript`)