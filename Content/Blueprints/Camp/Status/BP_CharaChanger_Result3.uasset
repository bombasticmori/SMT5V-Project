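; Child Blueprint of a character changer under Camp/Status, apparently the Result3 variant for showing devil models.
; Its overrides for devil rotation material, devil motion, self tick toggling, nearest-number lookup and spawn-need maximum all just forward to the parent.
; The construction script also only calls the parent, and the event graph holds only disabled default events, so the graphs add no logic of their own.
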(fn `GetNearlyNum`
  (params (LoopNum :type Integer))
  (returns (ReturnValue :type Integer))
  (return (`parent.GetNearlyNum` LoopNum)))

(fn `GetSpawnNeedMax`
  (params (InputPin :type "UIStatusCtrlDataObjBase Object Reference"))
  (returns (ReturnValue :type Integer))
  (return (`parent.GetSpawnNeedMax` InputPin)))

(fn `PlayDevilMotion`
  (params (CharaBase :type "/Game/Blueprints/Character/Base/CharaBase Object Reference") (DevilID :type Integer))
  (`parent.PlayDevilMotion` CharaBase DevilID))

(fn `SetDevilMaterialForRotate`
  (params (CharaBase :type "CustomPawn Object Reference") (devilId :type Integer))
  (`parent.SetDevilMaterialForRotate` CharaBase devilId))

(fn `SetSelfTickEnable`
  (params (bEnabled :type Boolean))
  (`parent.SetSelfTickEnable` bEnabled))

(fn `UserConstructionScript`
  (`parent.UserConstructionScript`))