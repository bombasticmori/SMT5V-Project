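; BP_CharaChanger_Battle2 is a stubbed character changer for the camp status screen, with a battle-oriented API.
; It declares events and functions for initialization, devil spawning and switching, battle member visibility, voices and status camera framing.
; All bodies are empty or return false, zero or nothing, except Tick, which only forwards to its parent, so the file itself holds no working logic.
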(event `self.ReceiveTick`
  (params (DeltaSeconds :type "Float (single-precision)"))
  (`parent.ReceiveTick` DeltaSeconds))

(event `OnLoaded_CDB3BABB4D9D1D885E2ECFAFCDC9FA47`
  (params (Loaded :type "Object Class Reference")))

(event `/Game/Blueprints/Camp/Status/BPI_StatusCharaChanger.PreRequest`
  (params (DevilID :type Integer)))

(event `/Game/Blueprints/Camp/Status/BPI_StatusCharaChanger.Init_Battle`
  (params (SpawnPos :type "Transform Structure") (Type :type "E_UI_STATUS_CTRL_TYPE Enum" :default "E_UI_STATUS_CTRL_TYPE_BTL_ENEMY") (StatusCtrlDataBtl :type "Object Object Reference") (useAnalyzeItem :type Boolean)))

(event `/Game/Blueprints/Camp/Status/BPI_StatusCharaChanger.Init`
  (params (SpawnPos :type "Transform Structure") (Type :type "E_UI_STATUS_CTRL_TYPE Enum" :default "E_UI_STATUS_CTRL_TYPE_BTL_ENEMY")))

(event `SpawnStockDevil`)

(event `/Game/Blueprints/Camp/Status/BPI_StatusCharaChanger.ChangeChara`
  (params (DevilID :type Integer) (IsUnknown :type Boolean)))

(event `/Game/Blueprints/Camp/Status/BPI_StatusCharaChanger.ViewEnd`)

(event `/Game/Blueprints/Camp/Status/BPI_StatusCharaChanger.ViewStart`)

(fn `CalcBaseLocation`
  (params (ActorForwardVector :type "Vector Structure (by ref)") (ActorTransform :type "Transform Structure (by ref)")))

(fn `CalcCamera`
  (params (ActorTransform :type "Transform Structure (by ref)"))
  (returns (Eye :type "Vector Structure") (Look :type "Vector Structure"))
  (return (0.0 0.0 0.0) (0.0 0.0 0.0)))

(fn `CallVoice`
  (params (VoiceType :type "EDevilVoiceType Enum" :default "EDevilVoiceType_None"))
  (returns (dummy :type Boolean))
  (return false))

(fn `CameraReset`
  (params (EnemyID :type Integer) (ActorForwardVector :type "Vector Structure (by ref)") (ActorTransform :type "Transform Structure (by ref)") (CameraScale :type "Float (double-precision)")))

(fn `CheckIsChangedRequest`
  (returns (NoChange :type Boolean))
  (return false))

(fn `DestroyDevilModel`
  (returns (destroyed :type Boolean))
  (return false))

(fn `DisableRotation`
  (params (IsDisable :type Boolean))
  (returns (NoUse :type Boolean))
  (return false))

(fn `GetEyeOffset`
  (returns (EyeOffset :type "Vector Structure"))
  (return (0.0 0.0 0.0)))

(fn `GetLookOffset`
  (returns (LookOffset :type "Vector Structure"))
  (return (0.0 0.0 0.0)))

(fn `GetNearlyNum`
  (params (InputPin :type Integer))
  (returns (ReturnValue :type Integer))
  (return 0))

(fn `GetSocketPos`
  (params (Object :type "Actor Object Reference"))
  (returns (Transform :type "Vector Structure"))
  (return (0.0 0.0 0.0)))

(fn `GetTargetFaceLocation`
  (params (ActorTransform :type "Transform Structure (by ref)"))
  (returns (Location :type "Vector Structure"))
  (return (0.0 0.0 0.0)))

(fn `HideAllBattleMember`)

(fn `IsEndPreparation`
  (params (DevilID :type Integer))
  (returns (IsEnd :type Boolean))
  (return false))

(fn `ModifyEyeFromCameraScale`
  (params (InEye :type "Vector Structure") (InLook :type "Vector Structure") (InCameraScale :type "Float (double-precision)"))
  (returns (OutEye :type "Vector Structure"))
  (return (0.0 0.0 0.0)))

(fn `NeedEnemyCameraData`
  (returns (ReturnValue :type Boolean))
  (return false))

(fn `NeedToFinalize`
  (returns (IsNeedToFinalize :type Boolean))
  (return false))

(fn `NewInit`
  (params (DataObject :type "Object Object Reference") (SpawnTransform :type "Transform Structure") (WithModelLoad :type Boolean) (WithModelSpawn :type Boolean))
  (returns (Success :type Boolean))
  (return false))

(fn `NewInit_Battle`
  (params (StatusCtrlDataBtl :type "Object Object Reference") (BattleParty :type "Object Object Reference") (Type :type "E_UI_STATUS_CTRL_TYPE Enum" :default "E_UI_STATUS_CTRL_TYPE_BTL_ENEMY") (useAnalyzeItem :type Boolean))
  (returns (Dummy :type Boolean))
  (return false))

(fn `SetBattleStatusData`
  (params (EnemyID :type Integer))
  (returns (BattleCameraData :type "/Game/Blueprints/Camp/Status/ST_StBattleCameraSetUp Structure"))
  (return))

(fn `SetDelayInInit`
  (params (Num :type Integer))
  (returns (Dummy :type Boolean))
  (return false))

(fn `SetTalkCameraOffsetTable`
  (params (DevilID :type Integer) (IsEnemy :type Boolean))
  (returns (CameraOffset :type "/Game/Blueprints/Camp/Status/ST_TalkCameraOffset Structure"))
  (return))

(fn `SetTargetChara`
  (params (InActor :type "Actor Object Reference")))

(fn `SetTracedTransform`
  (params (InChara :type "/Game/Blueprints/Character/Base/CharaBase Object Reference") (InTransform :type "Transform Structure")))

(fn `UpdateVisibilityForBattleMember`
  (params (PartyIndex :type Integer)))

(fn `UserConstructionScript`)