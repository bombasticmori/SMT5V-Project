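; Base Blueprint for the character model changer in the camp status screen, apparently for displaying player and devil models.
; It declares an interface for model spawning and swapping, camera, lighting, post-process, materials, silhouette, motion, rotation and voice, with camp and battle init variants.
; Nearly every function and event is an empty stub returning defaults, and BeginPlay, Tick and Destroyed only call the parent.
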(event `self.ReceiveBeginPlay`
  (`parent.ReceiveBeginPlay`))

(event `self.ReceiveTick`
  (params (DeltaSeconds :type "Float (single-precision)"))
  (`parent.ReceiveTick` DeltaSeconds))

(event `OnLoaded_76280045409E72DBF890BEAF8DDCCCE4`
  (params (Loaded :type "Object Class Reference")))

(event `/Game/Blueprints/Camp/Status/BPI_StatusCharaChanger.ViewStart`)

(event `/Game/Blueprints/Camp/Status/BPI_StatusCharaChanger.ViewEnd`)

(event `/Game/Blueprints/Camp/Status/BPI_StatusCharaChanger.ChangeChara`
  (params (DevilID :type Integer) (IsUnknown :type Boolean)))

(event `self.ReceiveDestroyed`
  (`parent.ReceiveDestroyed`))

(event `Private_SpawnDevilModel`)

(event `/Game/Blueprints/Camp/Status/BPI_StatusCharaChanger.PreRequest`
  (params (DevilID :type Integer)))

(event `/Game/Blueprints/Camp/Status/BPI_StatusCharaChanger.Init_Battle`
  (params (SpawnPos :type "Transform Structure") (Type :type "E_UI_STATUS_CTRL_TYPE Enum" :default "E_UI_STATUS_CTRL_TYPE_BTL_ENEMY") (StatusCtrlDataBtl :type "Object Object Reference") (useAnalyzeItem :type Boolean)))

(event `/Game/Blueprints/Camp/Status/BPI_StatusCharaChanger.Init`
  (params (SpawnPos :type "Transform Structure") (Type :type "E_UI_STATUS_CTRL_TYPE Enum" :default "E_UI_STATUS_CTRL_TYPE_BTL_ENEMY")))

(fn `CallVoice`
  (params (VoiceType :type "EDevilVoiceType Enum" :default "EDevilVoiceType_None"))
  (returns (dummy :type Boolean))
  (return false))

(fn `CameraReset`
  (returns (NoUse :type Boolean))
  (return false))

(fn `CheckIsChangedRequest`
  (returns (NoChange :type Boolean))
  (return false))

(fn `DestroyDevilModel`
  (returns (destroyed :type Boolean))
  (return false))

(fn `DisableRotation`
  (params (IsDisable :type Boolean))
  (returns (NoUse :type Boolean))
  (return false))

(fn `GetDevilCameraData`
  (params (SoftClassReference :type "Object Soft Class Reference (by ref)"))
  (returns (ReturnValue :type "/Game/Blueprints/Camp/Status/ST_StCameraSetUp Structure") (spot_intensity :type "Float (double-precision)"))
  (return (struct) 0.0))

(fn `GetDevilIDForAsset`
  (params (InDevilID :type Integer))
  (returns (OutDevilID :type Integer))
  (return 0))

(fn `GetDevilSpawnTransform`
  (returns (m_DefaultTransform :type "Transform Structure") (`Rotation X (Roll)` :type "Float (double-precision)"))
  (return (struct) 0.0))

(fn `GetModelClassReference`
  (params (ID :type Integer) (IsPlayer :type Boolean))
  (returns (Pawn :type "CustomPawn Soft Class Reference"))
  (return null))

(fn `GetSelfTransform`
  (returns (SelfTransform :type "Transform Structure"))
  (return))

(fn `GetSocketPos`
  (params (Object :type "Actor Object Reference"))
  (returns (Transform :type "Vector Structure"))
  (return (0.0 0.0 0.0)))

(fn `IsEndPreparation`
  (params (DevilID :type Integer))
  (returns (IsEnd :type Boolean))
  (return false))

(fn `IsNPCModel`
  (params (InputPin :type Integer))
  (returns (ReturnValue :type Boolean))
  (return false))

(fn `IsTao`
  (params (Id :type Integer))
  (returns (Ret :type Boolean))
  (return false))

(fn `ModifyCameraTableData`
  (params (InCameraData :type "/Game/Blueprints/Camp/Status/ST_StCameraSetUp Structure (by ref)"))
  (returns (OutCameraData :type "/Game/Blueprints/Camp/Status/ST_StCameraSetUp Structure"))
  (return))

(fn `NeedToFinalize`
  (returns (IsNeedToFinalize :type Boolean))
  (return false))

(fn `NewInit`
  (params (DataObject :type "Object Object Reference") (SpawnTransform :type "Transform Structure") (WithModelLoad :type Boolean) (WithModelSpawn :type Boolean))
  (returns (Success :type Boolean))
  (return false))

(fn `NewInit_Battle`
  (params (StatusCtrlDataBtl :type "Object Object Reference") (BattleParty :type "Object Object Reference") (Type :type "E_UI_STATUS_CTRL_TYPE Enum" :default "E_UI_STATUS_CTRL_TYPE_BTL_ENEMY") (useAnalyzeItem :type Boolean))
  (returns (Dummy :type Boolean))
  (return false))

(fn `ProcessInputMotion`)

(fn `ProcessInputRotate`
  (params (DeltaSeconds :type "Float (double-precision)")))

(fn `ResetLight`
  (returns (NoUse :type Boolean))
  (return false))

(fn `ResetPostProcess`
  (returns (NoUse :type Boolean))
  (return false))

(fn `ScaleCorrect`
  (params (InputPin :type "Actor Object Reference")))

(fn `Set Material Func`
  (params (Material :type "Object Soft Object Reference") (Mesh :type "PrimitiveComponent Object Reference") (ElementIndex :type Integer)))

(fn `SetDelayInInit`
  (params (Num :type Integer))
  (returns (Dummy :type Boolean))
  (return false))

(fn `SetDevilMaterial`
  (params (InCharaBase :type "/Game/Blueprints/Character/Base/CharaBase Object Reference") (InDevilId :type Integer))
  (returns (NoUse :type Boolean))
  (return false))

(fn `SetDevilMotion`
  (params (InCharaBase :type "/Game/Blueprints/Character/Base/CharaBase Object Reference") (InDevilId :type Integer))
  (returns (NoUse :type Boolean))
  (return false))

(fn `SetLight`
  (returns (NoUse :type Boolean))
  (return false))

(fn `SetLOD`
  (params (DevilID :type Integer) (InCharaBase :type "/Game/Blueprints/Character/Base/CharaBase Object Reference")))

(fn `SetPlayerMaterial`
  (params (InCharaBase :type "/Game/Blueprints/Character/Base/CharaBase Object Reference"))
  (returns (NoUse :type Boolean))
  (return false))

(fn `SetSelfTransform`
  (returns (NoUse :type Boolean))
  (return false))

(fn `SetSilhouette`
  (params (IsSilhouette :type Boolean))
  (returns (NoUse :type Boolean))
  (return false))

(fn `UpdatePostProcess`
  (returns (NoUse :type Boolean))
  (return false))

(fn `UserConstructionScript`)