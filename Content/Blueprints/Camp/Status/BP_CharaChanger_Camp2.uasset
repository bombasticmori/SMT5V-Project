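; BP_CharaChanger_Camp2 is a child character-changer Blueprint under Camp/Status, apparently for displaying demons on the camp status screen.
; Its overrides for camera row name, motion table setup, asset ID lookup and demon material pass straight through to the parent.
; LoadMotionTable is the exception, with an empty body that returns without loading anything or calling the parent.
; The event graph holds only disabled placeholder events, and construction just runs the parent script.
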(fn `GetDevilCameraRowName`
  (params (ID :type Integer))
  (returns (ExtensionPart :type String))
  (return (`parent.GetDevilCameraRowName` ID)))

(fn `GetDevilIDForAsset`
  (params (InDevilID :type Integer))
  (returns (OutDevilID :type Integer))
  (return (`parent.GetDevilIDForAsset` InDevilID)))

(fn `LoadMotionTable`
  (params (Reference :type "Object Soft Object Reference") (alreadyLoadedTable :type "CharaMotionTable Object Reference"))
  (returns (return :type "CharaMotionTable Object Reference"))
  (return null))

(fn `SetDevilMaterial`
  (params (CharaBase :type "/Game/Blueprints/Character/Base/CharaBase Object Reference") (devilId :type Integer))
  (`parent.SetDevilMaterial` CharaBase devilId))

(fn `SetMotionTable`
  (params (CharaBase :type "/Game/Blueprints/Character/Base/CharaBase Object Reference") (DevilId :type Integer))
  (`parent.SetMotionTable` CharaBase DevilId))

(fn `UserConstructionScript`
  (`parent.UserConstructionScript`))