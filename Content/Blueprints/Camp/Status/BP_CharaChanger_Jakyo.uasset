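; Jakyo variant of the camp status character changer, a child Blueprint for displaying characters and devils with their materials, lighting, camera and post-process.
; Overrides for silhouette, devil material, camera table, transform, lighting and post-process only forward to the parent.
; The one behavioral difference visible here is UpdatePostProcess_Silhouette, left empty without a parent call.
; BeginPlay, overlap and Tick events are disabled stubs.
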(fn `GetSelfTransform`
  (returns (SelfTransform :type "Transform Structure"))
  (return (`parent.GetSelfTransform`)))

(fn `ModifyCameraTableData`
  (params (InCameraData :type "/Game/Blueprints/Camp/Status/ST_StCameraSetUp Structure (by ref)"))
  (`parent.ModifyCameraTableData` InCameraData))

(fn `ResetLight`
  (returns (NoUse :type Boolean))
  (bind _nouse (`parent.ResetLight`))
  (return _nouse))

(fn `ResetPostProcess`
  (returns (NoUse :type Boolean))
  (bind _nouse (`parent.ResetPostProcess`))
  (return _nouse))

(fn `SetDevilMaterial`
  (params (InCharaBase :type "/Game/Blueprints/Character/Base/CharaBase Object Reference") (InDevilId :type Integer))
  (returns (NoUse :type Boolean))
  (bind _nouse (`parent.SetDevilMaterial` InCharaBase InDevilId))
  (return _nouse))

(fn `SetLight`
  (returns (NoUse :type Boolean))
  (bind _nouse (`parent.SetLight`))
  (return _nouse))

(fn `SetSilhouette`
  (params (IsSilhouette :type Boolean))
  (returns (NoUse :type Boolean))
  (bind _nouse (`parent.SetSilhouette` IsSilhouette))
  (return _nouse))

(fn `UpdatePostProcess`
  (returns (NoUse :type Boolean))
  (bind _nouse (`parent.UpdatePostProcess`))
  (return _nouse))

(fn `UpdatePostProcess_Silhouette`
  (params (SilhouetteWeight :type "Float (double-precision)")))

(fn `UserConstructionScript`
  (`parent.UserConstructionScript`))