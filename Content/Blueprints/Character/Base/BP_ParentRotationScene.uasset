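; Scene component that, each tick, matches its world rotation to one of its ancestor components, chosen by ParentIndex clamped to the parent chain.
; When that ancestor is valid, it copies the ancestor's world rotation directly.
; Only when the ancestor is invalid does it add a world rotation built from RelativeRotate's roll, pitch and yaw around axes read from that same ancestor.
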(event `self.ReceiveTick`
  (params (DeltaSeconds :type "Float (single-precision)"))
  (bind _parents (`self.GetParentComponents`))
  (bind _output (`|GetArrayItem` _parents (`KismetMathLibrary.Clamp` (`self.ParentIndex`) 0 (`KismetArrayLibrary.Array_LastIndex` _parents))))
  (bind _returnvalue (`self.K2_GetComponentRotation` _output))
  (bind (_x _y _z) (`KismetMathLibrary.GetAxes` _returnvalue))
  (if (`KismetSystemLibrary.IsValid` _output)
    (`self.K2_SetWorldRotation` _returnvalue)
    (else
      (`self.K2_AddWorldRotation` (`KismetMathLibrary.ComposeRotators` (`KismetMathLibrary.ComposeRotators` (`KismetMathLibrary.RotatorFromAxisAndAngle` _x (.roll (`self.RelativeRotate`))) (`KismetMathLibrary.RotatorFromAxisAndAngle` _y (.pitch (`self.RelativeRotate`)))) (`KismetMathLibrary.RotatorFromAxisAndAngle` _z (.yaw (`self.RelativeRotate`))))))))