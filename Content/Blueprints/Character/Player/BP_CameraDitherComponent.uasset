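; Player camera component that dither-masks meshes and foliage obstructing the follow camera.
; While dithering, each tick fades masked meshes, traces for blockers, masks hits and writes a hit location to a material parameter collection for the shaders.
; Disabling dither unmasks meshes, and ToggleDitherState also swaps the camera boom's probe channel.
; Temporary toggles save and restore the state, with an immediate variant forcing a manual tick.
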(event `self.ReceiveBeginPlay`
  (`self.AddTickPrerequisiteActor` (`self.GetOwner`)))

(event `self.ReceiveTick`
  (params (DeltaSeconds :type "Float (single-precision)"))
  (if (`self.Dither`) :!label _label
    (`self.FadeInMaskedMeshes` DeltaSeconds)
    (bind (_hitresults _returnvalue) (`self.TraceForMaskingObjects`))
    (if _returnvalue
      (`self.MaskHitMeshes` _hitresults)
      (`self.Mask Foliage`)
      (`self.DebugTraceForDitherArea` _returnvalue)
      (`KismetMaterialLibrary.SetVectorParameterValue` "/Game/Design/Map/Daath/LargeMap/Celestial/Material/MPC_DaathColor.MPC_DaathColor" "HitLocation" (`KismetMathLibrary.Conv_VectorToLinearColor` (`self.CalculateHitLocation`))))
    (else
      (if (`KismetArrayLibrary.Array_IsValidIndex` (`self.MaskedMeshes`))
        (`self.UnmaskMeshes`))
      (if (`KismetArrayLibrary.Array_IsValidIndex` (`self.FadeMeshes`))
        _
        (else
          _))
      (`self.SetComponentTickEnabled` true))))

(event `ManualTick`
  (goto _label))

(fn `BP CalcHitlocation`
  (returns (ReturnValue :type "Vector Structure"))
  (return (+ (* (`SceneComponent.GetForwardVector` (`self.m_CameraComponent`)) (* (- (+ (+ (`self.m_LineWidth`) (`self.m_FallOff`)) (`self.MaskStartOffset`)) (`CapsuleComponent.GetScaledCapsuleRadius` (`self.m_CapsuleComponent`))) -1.0)) (`SceneComponent.K2_GetComponentLocation` (`self.m_CameraBoom`)))))

(fn `BP Trace For Masking Objects`
  (returns (ReturnValue :type Boolean) (OutHits :type "Array of HitResult Structure"))
  (bind _m_cameracomponent (`self.m_CameraComponent`))
  (bind _m_tracewidth (`self.m_TraceWidth`))
  (bind _returnvalue (`SceneComponent.GetForwardVector` _m_cameracomponent))
  (bind _output_get (set `self.m_StartTraceLoc` (+ (* _returnvalue (* _m_tracewidth -1.414214)) (* (`SceneComponent.GetUpVector` (`self.m_CapsuleComponent`)) (`self.m_TraceHeightOffset`)))))
  (bind _output_get_2 (set `self.m_EndTraceLoc` (`SceneComponent.K2_GetComponentLocation` _m_cameracomponent)))
  (bind _output_get_3 (set `self.m_TraceSize` (`KismetMathLibrary.MakeVector` _m_tracewidth _m_tracewidth (`self.m_TraceHeight`))))
  (bind _outhits (`KismetSystemLibrary.BoxTraceMulti` :`Start` _output_get :`End` _output_get_2 :`HalfSize` _output_get_3 :`Orientation` (`KismetMathLibrary.Conv_VectorToRotator` (`KismetMathLibrary.MakeVector` (.x _returnvalue) (.y _returnvalue))) :`TraceChannel` (`self.m_TraceChannel`) :`DrawDebugType` (`self.m_TraceVisibility`)))
  (return (`KismetArrayLibrary.Array_IsValidIndex` _outhits) _outhits))

(fn `BPI_TempToggleDitherState_Immediate`
  (params (ForceDitherOff :type Boolean))
  (returns (dummy :type Boolean))
  (`self.TempToggleDitherState_Immediate` ForceDitherOff)
  (return false))

(fn `DebugTraceForDitherArea`
  (params (IsDithering :type Boolean))
  (if (and (== (`self.DitherVisibility`) 1) IsDithering)
    (`KismetSystemLibrary.SphereTraceMulti` :`Start` (`self.CalculateHitLocation`) :`End` (`self.m_EndTraceLoc`) :`Radius` (+ (`self.m_LineWidth`) (`self.m_FallOff`)) :`TraceChannel` (`self.m_TraceChannel`) :`DrawDebugType` "ForOneFrame")))

(fn `Initialize Dither Component`
  (params (CameraBoom :type "SpringArmComponent Object Reference") (CapsuleComponent :type "CapsuleComponent Object Reference") (FollowCamera :type "CameraComponent Object Reference"))
  (set `self.m_CameraBoom` CameraBoom)
  (set `self.m_CapsuleComponent` CapsuleComponent)
  (set `self.m_CameraComponent` FollowCamera))

(fn `Mask Foliage`
  (`self.MaskExuldedFoliages`))

(fn `Set Trace Collisions`
  (params (TraceHeight :type "Float (double-precision)") (TraceWidth :type "Float (double-precision)") (TraceHeightOffset :type "Float (double-precision)"))
  (bind _m_linewidth (`self.m_LineWidth`))
  (bind _output_get (set `self.m_TraceHeight` TraceHeight))
  (`BPL_DebugMenuAdmin.SetParamDataFromPathName` "MapDebug/CameraDither/CameraCollision/TraceHeight" (`KismetMathLibrary.FTrunc` _output_get) 0 200)
  (bind _output_get_2 (set `self.m_TraceWidth` TraceWidth))
  (`BPL_DebugMenuAdmin.SetParamDataFromPathName` "MapDebug/CameraDither/CameraCollision/TraceWidth" (`KismetMathLibrary.FTrunc` _output_get_2) 0 200)
  (bind _output_get_3 (set `self.m_TraceHeightOffset` TraceHeightOffset))
  (`BPL_DebugMenuAdmin.SetParamDataFromPathName` "MapDebug/CameraDither/CameraCollision/TraceHeightOffset" 0 0 200)
  (set `self.m_TraceSize` (`KismetMathLibrary.MakeVector` _m_linewidth _m_linewidth _output_get)))

(fn `SetVariables`
  (bind _returnvalue (`KismetMaterialLibrary.GetScalarParameterValue` "/Game/Design/Map/Daath/LargeMap/Celestial/Material/MPC_DaathColor.MPC_DaathColor" "LineWidth"))
  (set `self.m_LineWidth` _returnvalue)
  (bind _returnvalue_2 (`KismetMaterialLibrary.GetScalarParameterValue` "/Game/Design/Map/Daath/LargeMap/Celestial/Material/MPC_DaathColor.MPC_DaathColor" "FallOff"))
  (set `self.m_FallOff` _returnvalue_2))

(fn `TempToggleDitherState`
  (params (ForceDitherOff :type Boolean))
  (bind _tempditherstate (`self.TempDitherState`))
  (set `self.FadeTime` (`self.PresetFadeTime`))
  (if ForceDitherOff
    (if (!= (not (`self.Dither`)) ForceDitherOff)
      (set `self.TempDitherState` (`self.Dither`))
      (set `self.Dither` false))
    (else
      (set `self.Dither` _tempditherstate)
      (if _tempditherstate
        (if (== (`GameplayStatics.GetPlayerPawn` 0) (`self.GetOwner`))
          (`self.SetComponentTickEnabled` true))))))

(fn `TempToggleDitherState_Immediate`
  (params (ForceDitherOff :type Boolean))
  (bind _dither (`self.Dither`))
  (bind _tempditherstate (`self.TempDitherState`))
  (if ForceDitherOff
    (if (!= (not _dither) ForceDitherOff)
      (set `self.TempDitherState` _dither)
      (set `self.Dither` false)
      (set `self.FadeTime` 0.0)
      (`self.ManualTick`))
    (else
      (set `self.Dither` _tempditherstate)
      (if _tempditherstate
        (if (== (`GameplayStatics.GetPlayerPawn` 0) (`self.GetOwner`))
          (`self.SetComponentTickEnabled` true)
          (set `self.FadeTime` (`self.PresetFadeTime`))
          (`self.ManualTick`))))))

(fn `ToggleDitherState`
  (params (NewDitherState :type Boolean))
  (set `self.TempDitherState` NewDitherState)
  (bind _output_get (set `self.Dither` NewDitherState))
  (set `self.FadeTime` (`self.PresetFadeTime`))
  (set `SpringArmComponent.ProbeChannel` (select `int` (`KismetMathLibrary.Conv_BoolToInt` _output_get) :`0` "ECC_GameTraceChannel8" :`1` "ECC_Camera" :!type "ECollisionChannel Enum") (`self.m_CameraBoom`))
  (if _output_get
    (if (== (`self.GetOwner`) (`GameplayStatics.GetPlayerPawn` 0))
      (`self.SetComponentTickEnabled` true))))