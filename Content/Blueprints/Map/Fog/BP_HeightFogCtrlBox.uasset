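; BP_HeightFogCtrlBox is a map Blueprint that, by its name, serves as a height fog control box.
; BeginPlay, EndPlay and actor overlap events only forward to the parent implementation.
; Fade, activation, current-box switching and environment reset events are empty stubs, as are the priority-box lookup and holder get-or-spawn functions.
; The file itself contains no fog or fade logic.
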(event `self.ReceiveBeginPlay`
  (`parent.ReceiveBeginPlay`))

(event `self.ReceiveActorBeginOverlap`
  (params (OtherActor :type "Actor Object Reference"))
  (`parent.ReceiveActorBeginOverlap` OtherActor))

(event `TL_Fade__FinishedFunc`)

(event `TL_Fade__UpdateFunc`)

(event `StopFade`)

(event `/Game/Blueprints/Map/Daath/EnvCtrl/BPI_EnvCtrl.BPI_EnvReset`)

(event `self.ReceiveActorEndOverlap`
  (params (OtherActor :type "Actor Object Reference"))
  (`parent.ReceiveActorEndOverlap` OtherActor))

(event `SetToCurrent`)

(event `UnsetFromCurrent`)

(event `StartFadeIn`)

(event `StartFadeOut`)

(event `self.ReceiveEndPlay`
  (params (EndPlayReason :type "EEndPlayReason Enum" :default "Destroyed"))
  (`parent.ReceiveEndPlay` EndPlayReason))

(event `ActivateFogCtrl`)

(event `DeactivateFogCtrl`)

(fn `FindHighestPriorityHittingCtrlBox`
  (returns (Result :type "/Game/Blueprints/Map/Fog/BP_HeightFogCtrlBox Object Reference"))
  (return null))

(fn `GetOrSpawnCtrlHolder`
  (return))

(fn `UserConstructionScript`)