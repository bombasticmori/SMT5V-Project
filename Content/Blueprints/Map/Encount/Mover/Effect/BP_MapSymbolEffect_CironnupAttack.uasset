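; Map symbol effect Blueprint for the Cironnup attack, part of the map encounter mover effects.
; BeginPlay and Tick only forward to the parent class, and the overlap and destroyed events are empty.
; Arrow-named functions for location history, return check, encounter collision and hit effect are stubs that do nothing or return zero or false, so this asset adds no working logic of its own.
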(event `self.ReceiveBeginPlay`
  (`parent.ReceiveBeginPlay`))

(event `self.ReceiveTick`
  (params (DeltaSeconds :type "Float (single-precision)"))
  (`parent.ReceiveTick` DeltaSeconds))

(event `OnComponentBeginOverlap`
  (params (OverlappedComponent :type "PrimitiveComponent Object Reference") (OtherActor :type "Actor Object Reference") (OtherComp :type "PrimitiveComponent Object Reference") (OtherBodyIndex :type Integer) (bFromSweep :type Boolean) (SweepResult :type "HitResult Structure (by ref)")))

(event `OnDestroyed_`
  (params (DestroyedActor :type "Actor Object Reference")))

(fn `CheckArrowReturn`
  (returns (Return :type Boolean))
  (return false))

(fn `CheckCollisionViewDebug`
  (returns (View :type Boolean))
  (return false))

(fn `GetArrowLateLocation`
  (returns (Location :type "Vector Structure"))
  (return (0.0 0.0 0.0)))

(fn `GetArrowLocation`
  (returns (Location :type "Vector Structure"))
  (return (0.0 0.0 0.0)))

(fn `InitArrowHistory`)

(fn `SetEncountCollisionLocation`)

(fn `SpawnHitEffect`
  (params (Location :type "Vector Structure")))

(fn `UpdateArrowHistory`)

(fn `UserConstructionScript`)