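; BP_LoadBossRushField is an actor Blueprint that outlines loading and switching of Boss Rush battle fields.
; It declares level load, unload, visibility and field-data functions, with handling for a first and second field.
; BPI-prefixed interface entry points cover readying, finishing, switching and querying fields.
; All bodies here are empty or return defaults, apart from parent BeginPlay and EndPlay calls.
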(event `self.ReceiveBeginPlay`
  (`parent.ReceiveBeginPlay`))

(event `LoadLevel`
  (params (LevelVisible :type Boolean) (SecondLevel :type Boolean)))

(event `UnloadLevel`)

(event `self.ReceiveEndPlay`
  (params (EndPlayReason :type "EEndPlayReason Enum" :default "Destroyed"))
  (`parent.ReceiveEndPlay` EndPlayReason))

(event `/Game/Blueprints/Map/Encount/LoadBossRushField/BPI_LoadBossRushField.BPI_ReadyBossRushField`
  (params (BattleFieldID :type Integer)))

(event `/Game/Blueprints/Map/Encount/LoadBossRushField/BPI_LoadBossRushField.BPI_FinishBossRushFieldAll`
  (params (UnloadBossRushLevel :type Boolean) (ShowBattleHideLevel :type Boolean)))

(event `SetVisible_BattleHideLevel`
  (params (Visible :type Boolean)))

(event `/Game/Blueprints/Map/Encount/LoadBossRushField/BPI_LoadBossRushField.BPI_LoadSecondBossRushField`
  (params (BattleFieldID :type Integer)))

(event `/Game/Blueprints/Map/Encount/LoadBossRushField/BPI_LoadBossRushField.BPI_ChangeBossRushField_FirstOrSecond`
  (params (SecondLevel :type Boolean)))

(fn `BPI_CheckLoadedBossRushField`
  (params (SecondLevel :type Boolean))
  (returns (Loaded :type Boolean))
  (return false))

(fn `BPI_CheckVisibleBossRushField`
  (params (SecondLevel :type Boolean))
  (returns (Visible :type Boolean))
  (return false))

(fn `BPI_Completed_FinishBossRushField`
  (returns (Completed :type Boolean))
  (return false))

(fn `BPI_Completed_ReadyBossRushField`
  (returns (Completed :type Boolean))
  (return false))

(fn `BPI_GetBattleFieldID`
  (returns (BattleFieldID :type Integer))
  (return 0))

(fn `BPI_GetBossRushFieldPos`
  (returns (EncountPos :type "Transform Structure") (LevelPos :type "Transform Structure"))
  (return))

(fn `CheckLevelLoaded`
  (params (SecondLevel :type Boolean))
  (returns (Loaded :type Boolean))
  (return false))

(fn `CheckLevelVisible`
  (params (SecondLevel :type Boolean))
  (returns (Visible :type Boolean))
  (return false))

(fn `GetBattleFieldData`
  (params (SecondLevel :type Boolean))
  (returns (LevelAssetIDs :type "Array of PrimaryAssetId Structure") (LevelTransform :type "Transform Structure") (EncountTransform :type "Transform Structure") (BattleFieldTable :type "/Game/Blueprints/BattleField/Table/BattleFieldTableItem_ST Structure"))
  (return))

(fn `ResetSecondLevelInfo`)

(fn `UserConstructionScript`)