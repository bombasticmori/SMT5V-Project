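; BP_EncountAreaSpawner is an actor Blueprint in the map encounter-area system, with an interface for tracing and spawning encounter symbols.
; It declares events for spawning, deleting and debug-spawning symbols, plus helpers for components, logging and success queries.
; All of these are empty stubs, with GetSuccsess always returning false.
; BeginPlay, EndPlay and the construction script only call the parent, and Tick and overlap are disabled.
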(event `self.ReceiveBeginPlay`
  (`parent.ReceiveBeginPlay`))

(event `OnLoaded_E5E0B1E74B354A4530CE2ABDF1028360`
  (params (Loaded :type "Object Class Reference")))

(event `_EvtDis_EndInit`
  (params (Success :type Boolean)))

(event `TraceAndSpawnSymbol`
  (params (Delay :type "Float (double-precision)") (IsEffect :type Boolean) (AngleManual :type Boolean) (Angle :type "Float (double-precision)") (IgnorePause :type Boolean) (Index :type Integer) (NotCalcAngle :type Boolean) (SpawnMotion :type Boolean)))

(event `SpawnSymbol`)

(event `DeleteSpawn`)

(event `Debug_TraceAndSpawnSymbol`
  (params (DevilID :type Integer) (BlankIndex :type Integer)))

(event `self.ReceiveEndPlay`
  (params (EndPlayReason :type "EEndPlayReason Enum" :default "Destroyed"))
  (`parent.ReceiveEndPlay` EndPlayReason))

(fn `AddExComponent`)

(fn `FailLog`
  (params (Reason :type String)))

(fn `FirstReturn`)

(fn `GetSuccsess`
  (returns (Sucsess :type Boolean))
  (return false))

(fn `PrintSpawn`)

(fn `UserConstructionScript`
  (`parent.UserConstructionScript`))