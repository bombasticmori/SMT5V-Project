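; Dungeon spline variant of an encounter area, defined as a child Blueprint that takes its behavior from its parent class.
; BeginPlay, construction and the functions for spline selection, reversal, fly checks, view and spawn points only forward to the parent.
; CalcBoxPosSize is the exception, with an empty body and no parent call.
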(event `self.ReceiveBeginPlay`
  (`parent.ReceiveBeginPlay`))

(fn `BPI_GetSymbolSpline`
  (returns (Spline :type "SplineComponent Object Reference"))
  (bind _spline (`parent.BPI_GetSymbolSpline`))
  (return _spline))

(fn `CalcBoxPosSize`)

(fn `CalcSpawnPointList`
  (params (LineTrace :type Boolean))
  (returns (SpawnPointList :type "Array of Transform Structure"))
  (bind _spawnpointlist (`parent.CalcSpawnPointList` LineTrace))
  (return _spawnpointlist))

(fn `ChangeOptionSpline`
  (params (Index :type Integer))
  (`parent.ChangeOptionSpline` Index))

(fn `CheckFly`
  (returns (IsFly :type Boolean))
  (return (`parent.CheckFly`)))

(fn `CheckSplineReverse`
  (returns (Reverse :type Boolean))
  (return (`parent.CheckSplineReverse`)))

(fn `GetBaseSpline`
  (returns (Spline :type "SplineComponent Object Reference"))
  (return (`parent.GetBaseSpline`)))

(fn `GetOptionSplineIndex`
  (returns (Index :type Integer))
  (return (`parent.GetOptionSplineIndex`)))

(fn `GetOptionSplines`
  (returns (OptionSplines :type "Array of /Game/Blueprints/Map/Encount/EncountArea/BP_EncountArea_OptionSpline Object Reference"))
  (bind _optionsplines (`parent.GetOptionSplines`))
  (return _optionsplines))

(fn `GetSpawnSplinePoint`
  (returns (SplinePoints :type "Array of Integer"))
  (return (`parent.GetSpawnSplinePoint`)))

(fn `GetSpline`
  (returns (Spline :type "SplineComponent Object Reference"))
  (return (`parent.GetSpline`)))

(fn `SetSplineReverse`
  (params (Reverse :type Boolean))
  (`parent.SetSplineReverse` Reverse))

(fn `SetView`
  (params (IsView :type Boolean))
  (returns (NewParam :type Boolean))
  (bind _newparam (`parent.SetView` IsView))
  (return _newparam))

(fn `UserConstructionScript`
  (`parent.UserConstructionScript`))