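; Room Guardian encounter gimmick Blueprint for map encounter areas, containing only stub logic.
; BeginPlay, Tick and the construction script just call the parent.
; Hooks for spawn, summon, return, give-up, reset, area data, wait points and route-node visibility are empty.
; Discovery, spawn-area and give-up checks always return false, and the main symbol component lookup reports invalid.
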(event `self.ReceiveBeginPlay`
  (`parent.ReceiveBeginPlay`))

(event `self.ReceiveTick`
  (params (DeltaSeconds :type "Float (single-precision)"))
  (`parent.ReceiveTick` DeltaSeconds))

(event `ProcSpawnHit`)

(event `ProcSummon`)

(event `ProcReturnHit`)

(event `Reset`)

(event `EvtDis_ImmediateryBeforeRespawn_`
  (params (BlankIndex :type Integer)))

(event `GiveupFromStopTime`)

(event `ProcGiveupHit`)

(fn `CalcNextWaitPoint`
  (returns (Point :type "/Game/Blueprints/Map/Encount/EncountArea/Struct/EncountRoomGuardian_SpawnPoint Structure"))
  (return))

(fn `ChangeMainAreaData`)

(fn `ChangeSummonAreaData`)

(fn `CheckDiscovery`
  (returns (Discovery :type Boolean))
  (return false))

(fn `CheckDiscoveryArea`
  (returns (AreaIN :type Boolean))
  (return false))

(fn `CheckGiveupArea`
  (returns (AreaIN :type Boolean))
  (return false))

(fn `CheckSpawnArea`
  (returns (AreaIN :type Boolean))
  (return false))

(fn `GetMainSymbolComponent`
  (returns (Valid :type Boolean) (Comp :type "/Game/Blueprints/Map/Encount/Mover/MapSymbolBaseCompornent Object Reference"))
  (return false null))

(fn `HideRouteNode`)

(fn `Init`)

(fn `UserConstructionScript`
  (`parent.UserConstructionScript`))

(fn `ViewRouteNode`)