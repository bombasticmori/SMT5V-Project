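; BP_MapSymbol_MatchSplineMove is an encounter-area map symbol Blueprint, named for spline-matched movement of encounter symbols.
; It declares functions for spline location and distance, position records, respawn offsets, respawn and return waits, and area checks.
; All of these, plus the battle-start event, are empty or return defaults here; BeginPlay and Tick only call the parent.
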(event `self.ReceiveBeginPlay`
  (`parent.ReceiveBeginPlay`))

(event `self.ReceiveTick`
  (params (DeltaSeconds :type "Float (single-precision)"))
  (`parent.ReceiveTick` DeltaSeconds))

(event `CallStartBattle_Core`)

(fn `AddSplineDistance`
  (params (Distance1 :type "Float (double-precision)") (Distance2 :type "Float (double-precision)") (SplineComp :type "SplineComponent Object Reference"))
  (returns (OutDistance :type "Float (double-precision)"))
  (return 0.0))

(fn `AllRespawn`)

(fn `AllReturn`)

(fn `CalcAreaIN`)

(fn `CalcRespawnAddSplinePos`
  (params (EncountAreaIndex :type Integer) (SymbolIndex :type Integer)))

(fn `ConvertIndex_FromEncountAreaIndex`
  (params (EncountAreaIndex :type Integer) (SymbolIndex :type Integer))
  (returns (Index :type Integer))
  (return 0))

(fn `GetSplineLocation`
  (params (Spline :type "SplineComponent Object Reference") (Distance :type "Float (double-precision)"))
  (returns (Location :type "Vector Structure") (Reverse :type Boolean))
  (return (0.0 0.0 0.0) false))

(fn `InitSplinePosRecord`)

(fn `UpdateSplinePosRecord`)

(fn `UserConstructionScript`)

(fn `WaitAllReturn`
  (returns (AllReturn :type Boolean))
  (return false))

(fn `WaitOnceReturn`
  (returns (OneReturn :type Boolean) (EncountAreaIndex :type Integer) (SymbolIndex :type Integer))
  (return false 0 0))