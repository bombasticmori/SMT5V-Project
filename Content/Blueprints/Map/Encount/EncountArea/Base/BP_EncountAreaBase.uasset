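; Base Blueprint for map encounter areas that spawn, return and respawn devil symbols and start their battles; almost all bodies are empty stubs.
; Its functions cover area in/out checks, box, spline or generator spawn points with traces, and random encounter picks including Mitama and Magatsuhi variants.
; Further hooks handle route nodes, chain encounters, dead-symbol saving, time attack and room guardians.
; BPI functions, some suffixed cpp, expose control and queries externally.
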(event `self.ReceiveBeginPlay`
  (`parent.ReceiveBeginPlay`))

(event `self.ReceiveTick`
  (params (DeltaSeconds :type "Float (single-precision)"))
  (`parent.ReceiveTick` DeltaSeconds))

(event `Timeline_Giv__FinishedFunc`)

(event `Timeline_Giv__UpdateFunc`)

(event `SpawnAllSymbols_Core`)

(event `SpawnSymbolOne_Core`
  (params (Index :type Integer) (IsManualPos :type Boolean) (ManualPos :type "Transform Structure")))

(event `ReSpawnAllSymbols_Core`)

(event `ReqSpawnSymbol`
  (params (BlankIndex :type Integer) (Location :type "Vector Structure")))

(event `OnSpawnDevil`
  (params (Devil :type "CustomPawn Object Reference") (This :type "/Game/Blueprints/Map/Encount/EncountArea/Calc/BP_EncountAreaSpawner Object Reference")))

(event `OnDestroyedSymbol`
  (params (DestroyedActor :type "Actor Object Reference")))

(event `EvtDis_SpawnEnd_`
  (params (This :type "/Game/Blueprints/Map/Encount/EncountArea/Calc/BP_EncountAreaSpawner Object Reference")))

(event `EvtDis_Dead_`
  (params (Symbol :type "Actor Object Reference") (Save :type Boolean)))

(event `CalcWallCheck_WhenSpawn`)

(event `BeginOverlap_SpawnHit`
  (params (OverlappedComponent :type "PrimitiveComponent Object Reference") (OtherActor :type "Actor Object Reference") (OtherComp :type "PrimitiveComponent Object Reference") (OtherBodyIndex :type Integer) (bFromSweep :type Boolean) (SweepResult :type "HitResult Structure (by ref)")))

(event `InitOverlap`)

(event `EndOverlap_SpawnHit`
  (params (OverlappedComponent :type "PrimitiveComponent Object Reference") (OtherActor :type "Actor Object Reference") (OtherComp :type "PrimitiveComponent Object Reference") (OtherBodyIndex :type Integer)))

(event `BeginingSpawn`)

(event `OnOtherDiscoveryHit`)

(event `Reb`)

(event `Giv`)

(event `_View`)

(event `Giv_Out`)

(event `Tick_SymbolSpawn`)

(event `Tick_SymbolReturn`)

(event `_SpawnHit`)

(event `_ReturnHit`)

(event `Manual_SymbolSpawn`)

(event `Manual_SymbolReturn`)

(event `OnOtherDiscoveryHit_Out`)

(event `self.BPI_CalcSpawnSymbol_cpp`)

(event `self.BPI_CalcReturnSymbol_cpp`)

(event `/Game/Blueprints/Map/Encount/EncountArea/Interface/BPI_EncountArea.BPI_EncountBattleStart`
  (params (SymbolPawn :type "Pawn Object Reference")))

(event `Evt_SilentMoon`)

(event `CallStartBattle`)

(event `CallStartBattle_Core`)

(event `EndMapInit_イベント_0`)

(event `CallEndBattle_Core`
  (params (BtlEndType :type "E_BTL_END Enum" :default "E_BTL_END_NONE") (ChainEncountNum :type Integer)))

(event `/Game/Blueprints/Map/Encount/EncountArea/Interface/BPI_EncountArea.BPI_EncountArea_ReSpawnSymbolAll`)

(event `/Game/Blueprints/Map/Encount/EncountArea/Interface/BPI_EncountArea.BPI_EncountArea_DestroySymbolAll`
  (params (Respawn :type Boolean)))

(event `EvtDis_EncountReset_`)

(event `/Game/Blueprints/Map/Encount/EncountArea/Interface/BPI_EncountArea.BPI_Summon_ForRoomGuardian`)

(event `self.ReceiveEndPlay`
  (params (EndPlayReason :type "EEndPlayReason Enum" :default "Destroyed"))
  (`parent.ReceiveEndPlay` EndPlayReason))

(event `Init_RoomGuardian`)

(event `/Game/Blueprints/Map/Encount/EncountArea/Interface/BPI_EncountArea.BPI_RecalcFlag_ForMapSymbols`)

(event `KillSymbol_ForBattle`
  (params (SymbolIndex :type Integer)))

(event `CallEndBattle`
  (params (BattleEnd :type "E_BTL_END Enum" :default "E_BTL_END_NONE") (ChainEncountNum :type Integer)))

(event `/Game/Blueprints/Map/Gimic/Common/Interface/BPI_MapGimmickAffectedByTimeStop.BPI_SetStopTime`
  (params (StopTime :type Boolean)))

(fn `ActorsToLocations`
  (params (Actors :type "Array of Actor Object Reference (by ref)"))
  (returns (Locations :type "Array of Vector Structure"))
  (return))

(fn `AddSpawner`
  (params (Spawner :type "/Game/Blueprints/Map/Encount/EncountArea/Calc/BP_EncountAreaSpawner Object Reference")))

(fn `BPI_ActSymbolWhenPause_FromOutside`
  (params (OutsideID :type Integer))
  (returns (NewParam :type Boolean))
  (return false))

(fn `BPI_AreaIn_cpp`
  (returns (ReturnValue :type Boolean))
  (return false))

(fn `BPI_AreaOut_cpp`
  (returns (ReturnValue :type Boolean))
  (return false))

(fn `BPI_ChangeReturnPoint`
  (params (Index :type Integer) (ReturnPoint :type "Vector Structure"))
  (returns (NewParam :type Boolean))
  (return false))

(fn `BPI_ChangeSplineLocationZ`
  (params (SymbolLocation :type "Vector Structure") (SymbolHalfHeight :type "Float (double-precision)"))
  (returns (NewParam :type Boolean))
  (return false))

(fn `BPI_CheckAreaIN`
  (returns (AreaIN :type Boolean))
  (return false))

(fn `BPI_CheckAreaIn_cpp`
  (returns (ReturnValue :type Boolean))
  (return false))

(fn `BPI_CheckDaathSpawnType_cpp`
  (returns (ReturnValue :type Boolean))
  (return false))

(fn `BPI_CheckEncountAreaGenerator`
  (returns (Generator :type Boolean))
  (return false))

(fn `BPI_CheckEncountAreaOverlap`
  (returns (Overlap :type Boolean))
  (return false))

(fn `BPI_CheckGenerator_cpp`
  (returns (ReturnValue :type Boolean))
  (return false))

(fn `BPI_CheckGiveupHitList`
  (returns (Hit :type Boolean))
  (return false))

(fn `BPI_CheckIgnorePause_cpp`
  (returns (ReturnValue :type Boolean))
  (return false))

(fn `BPI_CheckLastBattleArea`
  (returns (Last :type Boolean))
  (return false))

(fn `BPI_CheckMagatsukaEncountArea`
  (returns (Magatsuka :type Boolean))
  (return false))

(fn `BPI_CheckOtherDiscoveryHit`
  (returns (Overlap :type Boolean))
  (return false))

(fn `BPI_CheckRoomGuardian_cpp`
  (returns (ReturnValue :type Boolean))
  (return false))

(fn `BPI_CheckTimeAttack_cpp`
  (returns (ReturnValue :type Boolean))
  (return false))

(fn `BPI_CheckViewSymbol`
  (returns (View :type Boolean))
  (return false))

(fn `BPI_DestroySymbol`
  (params (Pawn :type "Pawn Object Reference"))
  (returns (NewParam :type Boolean))
  (return false))

(fn `BPI_Discovery_FromOutside`
  (params (OutsideID :type Integer))
  (returns (NewParam :type Boolean))
  (return false))

(fn `BPI_GetDeadSaveID`
  (returns (DeadSaveID :type Integer))
  (return 0))

(fn `BPI_GetEncountArea_RouteNodeList`
  (returns (NodeList :type "Array of MapSymbolRouteNode Structure"))
  (return))

(fn `BPI_GetEncountArea_RouteNodeSpace`
  (returns (Space :type "Float (double-precision)"))
  (return 0.0))

(fn `BPI_GetEncountAreaBox`
  (returns (BoxPos :type "Transform Structure") (BoxSize :type "Vector Structure") (AddPoints :type "Array of Vector Structure"))
  (return (struct) (0.0 0.0 0.0)))

(fn `BPI_GetEncountComeAreaInfo`
  (returns (Transform :type "Transform Structure") (HitSize :type "Vector Structure"))
  (return (struct) (0.0 0.0 0.0)))

(fn `BPI_GetNowSymbolNum_cpp`
  (returns (ReturnValue :type Integer))
  (return 0))

(fn `BPI_GetSafeZoneID`
  (returns (ManualSafeZoneID :type Boolean) (SafeZoneID :type Integer))
  (return false 0))

(fn `BPI_GetSymbolInfo`
  (params (Index :type Integer))
  (return))

(fn `BPI_GetSymbolList`
  (params (IgnorePawn :type "Pawn Object Reference"))
  (returns (PawnList :type "Array of Pawn Object Reference"))
  (return))

(fn `BPI_GetSymbolSpline`
  (returns (Spline :type "SplineComponent Object Reference"))
  (return null))

(fn `BPI_GiveUpSymbol_FromOutside`
  (params (OutsideID :type Integer))
  (returns (NewParam :type Boolean))
  (return false))

(fn `BPI_InComeArea`
  (params (Pos :type "Vector Structure") (AddHitSize :type "Float (double-precision)"))
  (returns (In :type Boolean))
  (return false))

(fn `BPI_InHitArea`
  (params (Pos :type "Vector Structure") (AddHitSize :type "Float (double-precision)"))
  (returns (IN :type Boolean))
  (return false))

(fn `BPI_NotOutHit`
  (returns (NotOut :type Boolean))
  (return false))

(fn `BPI_ProcGenerator_cpp`
  (params (DeltaTime :type "Float (double-precision)"))
  (returns (ReturnValue :type Boolean))
  (return false))

(fn `BPI_ProcTimeAttack_cpp`
  (returns (ReturnValue :type Boolean))
  (return false))

(fn `BPI_RebornSymbol_FromOutside`
  (params (OutsideID :type Integer))
  (returns (NewParam :type Boolean))
  (return false))

(fn `BPI_ResetSymbolSpawn`
  (returns (NewParam :type Boolean))
  (return false))

(fn `BPI_ReturnSymbol_FromOutside`
  (params (OutsideID :type Integer))
  (returns (NewParam :type Boolean))
  (return false))

(fn `BPI_ReturnSymbols`
  (params (Effect :type Boolean))
  (returns (NewParam :type Boolean))
  (return false))

(fn `BPI_SetChainEncountList`
  (params (Components :type "Array of ActorComponent Object Reference (by ref)"))
  (returns (NewParam :type Boolean))
  (return false))

(fn `BPI_SetMagatsuhiDevilAll`
  (params (Magatsuhi :type Boolean))
  (returns (NewParam :type Boolean))
  (return false))

(fn `BPI_SetSpawnSymbolEffect`
  (params (EffectON :type Boolean))
  (returns (NewParam1 :type Boolean))
  (return false))

(fn `BPI_SpawnSymbol`
  (params (Index :type Integer) (IsManualPos :type Boolean) (ManualPos :type "Transform Structure"))
  (returns (NewParam :type Boolean))
  (return false))

(fn `BPI_SpawnSymbol_FromOutside`
  (params (OutsideID :type Integer))
  (returns (NewParam :type Boolean))
  (return false))

(fn `BPI_SpawnSymbols`
  (returns (Success :type Boolean))
  (return false))

(fn `BPI_StopSpawn_FromIndex`
  (params (Index :type Integer))
  (returns (NewParam :type Boolean))
  (return false))

(fn `BPI_StopSymbolRespawn`
  (params (Pawn :type "Pawn Object Reference") (Stop :type Boolean))
  (returns (NewParam1 :type Boolean))
  (return false))

(fn `BPI_SummonSymbol`
  (returns (Success :type Boolean))
  (return false))

(fn `BPI_TimeAttackEncountAreaEnd`
  (params (Effect :type Boolean) (CheckMission :type Boolean) (MissionID :type Integer))
  (returns (NewParam :type Boolean))
  (return false))

(fn `BPI_TimeAttackEncountAreaStart`
  (params (CheckMission :type Boolean) (MissionID :type Integer))
  (returns (NewParam :type Boolean))
  (return false))

(fn `BPI_UpdateOptionSpline`
  (returns (NewParam :type Boolean))
  (return false))

(fn `CalcAreaIn`)

(fn `CalcBlankSpawnIndex`)

(fn `CalcBoxPosSize_ForSpline`)

(fn `CalcDefaultParam`)

(fn `CalcEncount_ForTimeAttack`)

(fn `CalcEncountID`
  (params (ManualSeed :type Boolean) (Seed :type Integer) (CheckMitama :type Boolean) (OnceCalc :type Boolean)))

(fn `CalcMagatsuhiDevil`)

(fn `CalcMitama`
  (returns (MitamaType :type "E_MITAMA_ENCOUNT Enum"))
  (return "E_MITAMA_ENCOUNT_NONE"))

(fn `CalcMitamaAll`)

(fn `CalcNotSpawn_WhenLevelDiffEscape`
  (params (SymbolID :type Integer))
  (returns (Spawn :type Boolean))
  (return false))

(fn `CalcSpawnPoint_Generator`
  (params (LineTrace :type Boolean)))

(fn `CalcSpawnPointList`
  (params (LineTrace :type Boolean))
  (returns (SpawnPointList :type "Array of Transform Structure"))
  (return))

(fn `CalcSpawnPointList_Box`
  (params (Box :type "Vector Structure") (LineTrace :type Boolean)))

(fn `CalcSpawnPointList_Spline`
  (params (Spline :type "SplineComponent Object Reference") (LineTrace :type Boolean)))

(fn `CalcTimeAttackMissionSaveID`)

(fn `CanSpawn_WhenGeneratorActive`
  (returns (CanSpawn :type Boolean))
  (return false))

(fn `ChainDeadTeam`
  (params (Effect :type Boolean)))

(fn `ChangeOptionSpline`
  (params (Index :type Integer)))

(fn `ChangeReturnPoint`
  (params (Index :type Integer) (ReturnPos :type "Vector Structure")))

(fn `CheckAreaIN`
  (returns (AreaIN :type Boolean))
  (return false))

(fn `CheckCanSpawnSymbol`
  (params (Pos :type "Vector Structure") (DevilID :type Integer))
  (returns (Can :type Boolean) (SpawnerRadius :type "Float (double-precision)"))
  (return false 0.0))

(fn `CheckCoasterRiding`
  (returns (CoasterRiding :type Boolean))
  (return false))

(fn `CheckDevilBlock`
  (params (Start :type "Vector Structure") (End :type "Vector Structure"))
  (returns (Free :type Boolean))
  (return false))

(fn `CheckFloatingIK_OFF`
  (params (SpawnListIndex :type Integer))
  (returns (FloatingIK_OFF :type Boolean))
  (return false))

(fn `CheckFly`
  (returns (IsFly :type Boolean))
  (return false))

(fn `CheckGeneratorAreaIn`
  (returns (AreaIn :type Boolean))
  (return false))

(fn `CheckImmediateUpdateFloatingIK_WhenCameraIn`
  (params (SpawnListIndex :type Integer))
  (returns (ImmediateUpdateFloatingIK :type Boolean))
  (return false))

(fn `CheckLevelDiff`
  (params (SymbolID :type Integer))
  (returns (LevelDiff :type Boolean))
  (return false))

(fn `CheckMitamaGroup`
  (params (DevilId :type Integer))
  (returns (Mitama :type Boolean))
  (return false))

(fn `CheckNowDiscovery`
  (returns (Exist :type Boolean))
  (return false))

(fn `CheckRouteNodeRange`
  (params (Location :type "Vector Structure"))
  (returns (OK :type Boolean))
  (return false))

(fn `CheckSpawnable_ForTimeAttack`
  (returns (Spawnable :type Boolean))
  (return false))

(fn `CheckSplineReverse`
  (returns (Reverse :type Boolean))
  (return false))

(fn `CheckStartEndFlag`
  (params (PackID :type Integer))
  (returns (OK :type Boolean))
  (return false))

(fn `CheckViewSymbolBox`
  (returns (IN :type Boolean))
  (return false))

(fn `ClearChainEncount`)

(fn `DebugEncountArea`
  (params (DevilID :type Integer)))

(fn `DestroyDebugCylinder`)

(fn `DestroyNeedless`)

(fn `DiscoveryAll`)

(fn `EndSpawnSymbol`
  (params (IsEffect :type Boolean) (IsIgnoreCome :type Boolean) (IgnorePawn :type "Pawn Object Reference") (ReqRespawn :type Boolean) (IsEffect_WhenNotNormalAct :type Boolean)))

(fn `ExtractInt_FromStr`
  (params (Str :type String))
  (returns (Int :type Integer))
  (return 0))

(fn `FailLog`
  (params (Reason :type String)))

(fn `GeneratorAreaIn`)

(fn `GeneratorAreaOut`)

(fn `GetBaseSpline`
  (returns (Spline :type "SplineComponent Object Reference"))
  (return null))

(fn `GetBlankSpawnIndex`
  (returns (Index :type Integer))
  (return 0))

(fn `GetComeRangeSize`
  (returns (ComeSize :type "Vector Structure"))
  (return (0.0 0.0 0.0)))

(fn `GetDeadSaveID`
  (returns (DeadSaveID :type Integer))
  (return 0))

(fn `GetDeadSymbolNum`
  (returns (Num :type Integer))
  (return 0))

(fn `GetDefaultParam`
  (returns (DefaultParam :type "/Game/Blueprints/Map/Encount/EncountArea/Struct/EncountArea_Default Structure") (Success :type Boolean))
  (return (struct) false))

(fn `GetEncountPack`
  (params (ArrayIndex :type Integer) (MitamaType :type "E_MITAMA_ENCOUNT Enum" :default "E_MITAMA_ENCOUNT_NONE"))
  (returns (Pack :type "PackEncount Structure") (PackId :type Integer))
  (return (struct) 0))

(fn `GetMoverData`
  (params (Pos :type "Vector Structure") (ReSpawn :type Boolean))
  (returns (MoverData :type "/Game/Blueprints/Map/Encount/Mover/SymbolMoverData Structure"))
  (return))

(fn `GetOptionSplineIndex`
  (returns (Index :type Integer))
  (return 0))

(fn `GetOptionSplines`
  (returns (OptionSplines :type "Array of /Game/Blueprints/Map/Encount/EncountArea/BP_EncountArea_OptionSpline Object Reference"))
  (return))

(fn `GetRandomEncountId`
  (params (ArrayIndex :type Integer) (MitamaType :type "E_MITAMA_ENCOUNT Enum" :default "E_MITAMA_ENCOUNT_NONE"))
  (returns (EncountId :type Integer))
  (return 0))

(fn `GetRandomEncountId_FromIndex`
  (params (Index :type Integer) (ArrayIndex :type Integer))
  (returns (EncountId :type Integer))
  (return 0))

(fn `GetRandomSpawnPos`
  (returns (Transform :type "Transform Structure"))
  (return))

(fn `GetRate`
  (params (TotalRate :type "Float (double-precision)") (Num :type Integer))
  (returns (Rate :type "Float (double-precision)"))
  (return 0.0))

(fn `GetReqSpawnSymbolNum`
  (returns (Num :type Integer))
  (return 0))

(fn `GetRouteNodeData`
  (params (X :type Integer) (Y :type Integer))
  (returns (Node :type "MapSymbolRouteNode Structure"))
  (return))

(fn `GetRouteNodeIndex`
  (params (X :type Integer) (Y :type Integer))
  (returns (Index :type Integer))
  (return 0))

(fn `GetSpawnSplinePoint`
  (returns (SplinePoints :type "Array of Integer"))
  (return))

(fn `GetSpawnSymbolNum`
  (returns (Num :type Integer))
  (return 0))

(fn `GetSpline`
  (returns (Spline :type "SplineComponent Object Reference"))
  (return null))

(fn `GetSplineKey_FromPos`
  (params (Pos :type "Vector Structure"))
  (returns (Key :type Integer))
  (return 0))

(fn `GetSymbolComponent`
  (params (Pawn :type "Actor Object Reference"))
  (returns (Valid :type Boolean) (Comp :type "/Game/Blueprints/Map/Encount/Mover/MapSymbolBaseCompornent Object Reference"))
  (return false null))

(fn `GetSymbolID`
  (params (EncountID :type Integer) (ArrayIndex :type Integer) (MitamaType :type "E_MITAMA_ENCOUNT Enum" :default "E_MITAMA_ENCOUNT_NONE"))
  (returns (SymbolId :type Integer))
  (return 0))

(fn `GetSymbolParam`
  (params (DevilID :type Integer))
  (returns (Param :type "/Game/Blueprints/Map/Encount/Mover/ParamTable/MapSymbolParam Structure"))
  (return))

(fn `GiveupAll`)

(fn `HideRouteNode`)

(fn `InitComeRange`)

(fn `InitCompData`)

(fn `InitRouteNode`)

(fn `ModifySymbolID`
  (params (EncountID :type Integer) (BlankIndex :type Integer)))

(fn `ProcSpawnOrReturn`)

(fn `Reborn`
  (params (exec :type Boolean) (Save :type Boolean)))

(fn `RecordActPattern`
  (params (Pawn :type "Actor Object Reference") (Index :type Integer)))

(fn `SaveSplineCompInfo`)

(fn `SetAreaIN_ForMatchSpline`
  (params (AreaIN_ForMatchSpline :type Boolean)))

(fn `SetDeadSymbol`
  (params (Index :type Integer) (Dead :type Boolean)))

(fn `SetSpawnSymbolEntry`
  (params (Index :type Integer) (Entry :type Boolean)))

(fn `SetSplineReverse`
  (params (Reverse :type Boolean)))

(fn `SetStopSpawnSymbol`
  (params (Index :type Integer) (StopSpawn :type Boolean)))

(fn `SetView`
  (params (IsView :type Boolean))
  (returns (NewParam :type Boolean))
  (return false))

(fn `ShowDaathSpawnHit`
  (params (Show :type Boolean)))

(fn `ShowSymbolDebugMemo`)

(fn `SpawnAreaIN`
  (params (IsSpawnEffectOFF :type Boolean) (IgnorePauseSpawn :type Boolean) (IsSummon :type Boolean) (OtherHit :type Boolean)))

(fn `SpawnAreaOut`
  (params (IsReturnEffectOFF :type Boolean)))

(fn `SpawnDebugCylinder`
  (params (Radius :type "Float (double-precision)") (HalfHeight :type "Float (double-precision)") (SideNum :type Integer) (Offset :type "Vector Structure") (Color :type "LinearColor Structure") (MeshView :type Boolean)))

(fn `SphereTrace`
  (params (Start :type "Vector Structure") (End :type "Vector Structure") (Radius :type "Float (double-precision)"))
  (returns (ReturnValue :type Boolean))
  (return false))

(fn `TraceSpawnPoint`
  (params (SpawnPoint :type "Vector Structure"))
  (returns (OutSpawnPoint :type "Transform Structure") (Success :type Boolean))
  (return (struct) false))

(fn `UpdateGeneratorActive`
  (params (DeltaSec :type "Float (double-precision)")))

(fn `UpdateSplineCompInfo`)

(fn `UserConstructionScript`
  (`parent.UserConstructionScript`))

(fn `ViewRouteNode`)