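; Base Blueprint for Magatsuka encounter areas, a variant of the parent encounter area on the map.
; It declares empty events and functions for area setup, discovery, symbol spawning, all-dead and all-reborn, plus parameter table setup.
; Spawn, route node, IK, flight and encounter pack queries simply forward to the parent.
; The unfixed spawn count returns zero and the Magatsuka spawn point calculation is an empty stub.
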(event `MagatsukaDiscovery`
  (params (Discovery :type Boolean)))

(event `InitMagatsukaArea`
  (params (EncountPackIndex :type "Array of /Game/Blueprints/Map/Gimic/Daath/Struct/MagatsukaSymbolPoint Structure (by ref)") (NoEncount :type Boolean) (RouteNodeSpace :type "Float (double-precision)") (RouteNode_LimitHeight :type "Float (double-precision)") (RouteNode_LimitSlope :type "Float (double-precision)") (MagatsukaCenter :type Boolean) (DevilLocationList :type "Array of Vector2D Structure (by ref)") (SafeZoneID :type Integer) (ManualSafeZone :type Boolean) (AttackAlongWall :type Boolean) (SecondActPatterns :type "Array of /Game/Blueprints/Map/Encount/Mover/SymbolActPattern Structure (by ref)")))

(event `AllDead`)

(event `/Game/Blueprints/Map/Encount/EncountArea/Base/BP_EncountAreaBase.InitRouteNode`
  (`parent.InitRouteNode`))

(event `MagatsukaSpawnOneSymbol`)

(event `AllReborn`)

(fn `BPI_CheckEncountAreaOverlap`
  (returns (Overlap :type Boolean))
  (bind _overlap (`parent.BPI_CheckEncountAreaOverlap`))
  (return _overlap))

(fn `BPI_CheckMagatsukaEncountArea`
  (returns (Magatsuka :type Boolean))
  (bind _magatsuka (`parent.BPI_CheckMagatsukaEncountArea`))
  (return _magatsuka))

(fn `CalcSpawnPointList`
  (params (LineTrace :type Boolean))
  (returns (SpawnPointList :type "Array of Transform Structure"))
  (bind _spawnpointlist (`parent.CalcSpawnPointList` LineTrace))
  (return _spawnpointlist))

(fn `CalcSpawnPointList_Magatsuka`
  (params (SpawnNum :type Integer))
  (returns (SpawnPoint :type "Array of Transform Structure"))
  (return))

(fn `CheckFloatingIK_OFF`
  (params (SpawnListIndex :type Integer))
  (returns (FloatingIK_OFF :type Boolean))
  (return (`parent.CheckFloatingIK_OFF` SpawnListIndex)))

(fn `CheckFly`
  (returns (IsFly :type Boolean))
  (return (`parent.CheckFly`)))

(fn `CheckImmediateUpdateFloatingIK_WhenCameraIn`
  (params (SpawnListIndex :type Integer))
  (returns (ImmediateUpdateFloatingIK :type Boolean))
  (return (`parent.CheckImmediateUpdateFloatingIK_WhenCameraIn` SpawnListIndex)))

(fn `CheckRouteNodeRange`
  (params (Location :type "Vector Structure"))
  (returns (OK :type Boolean))
  (return (`parent.CheckRouteNodeRange` Location)))

(fn `GetEncountPack`
  (params (ArrayIndex :type Integer) (MitamaType :type "E_MITAMA_ENCOUNT Enum" :default "E_MITAMA_ENCOUNT_NONE"))
  (returns (Pack :type "PackEncount Structure") (PackId :type Integer))
  (bind (_pack _packid) (`parent.GetEncountPack` ArrayIndex MitamaType))
  (return _pack _packid))

(fn `GetMoverData`
  (params (Pos :type "Vector Structure") (ReSpawn :type Boolean))
  (returns (MoverData :type "/Game/Blueprints/Map/Encount/Mover/SymbolMoverData Structure"))
  (bind _moverdata (`parent.GetMoverData` Pos ReSpawn))
  (return _moverdata))

(fn `GetRandomEncountId`
  (params (ArrayIndex :type Integer) (MitamaType :type "E_MITAMA_ENCOUNT Enum" :default "E_MITAMA_ENCOUNT_NONE"))
  (returns (EncountId :type Integer))
  (return (`parent.GetRandomEncountId` ArrayIndex MitamaType)))

(fn `GetUnfixSpawnNum`
  (returns (Num :type Integer))
  (return 0))

(fn `InitMagatsukaParamTable`)

(fn `UserConstructionScript`
  (`parent.UserConstructionScript`))