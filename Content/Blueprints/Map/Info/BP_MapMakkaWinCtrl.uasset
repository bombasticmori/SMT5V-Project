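; BP_MapMakkaWinCtrl is a stub Blueprint controller, named for the map's Makka window.
; It exposes interface events and functions for opening, locking and advancing Makka and Miitsu map windows, plus area name show/hide.
; All of these are empty or return false; only BeginPlay and Tick do anything, forwarding to the parent class.
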(event `self.ReceiveBeginPlay`
  (`parent.ReceiveBeginPlay`))

(event `self.ReceiveTick`
  (params (DeltaSeconds :type "Float (single-precision)"))
  (`parent.ReceiveTick` DeltaSeconds))

(event `Tick_Miitsu`)

(event `/Game/Blueprints/Map/Info/BPI_MapMakkaWinCtrl.BPI_OpenMapMiitsuWin`
  (params (PrevMiitsu :type Integer) (AddMiitsu :type Integer)))

(event `/Game/Blueprints/Map/Info/BPI_MapMakkaWinCtrl.BPI_SetPrevMiitsu_MiitsuWindow`
  (params (PrevMiitsu :type Integer)))

(event `/Game/Blueprints/Map/Info/BPI_MapMakkaWinCtrl.BPI_OpenMapMiitsuWin_ManualNext`
  (params (PrevMiitsu :type Integer) (AddMiitsu :type Integer)))

(event `/Game/Blueprints/Map/Info/BPI_MapMakkaWinCtrl.BPI_OpenMapMakkaWin`
  (params (PrevMakka :type Integer) (AddMakka :type Integer)))

(event `/Game/Blueprints/Map/Info/BPI_MapMakkaWinCtrl.BPI_SetPrevMakka_MakkaWindow`
  (params (PrevMakka :type Integer)))

(event `/Game/Blueprints/Map/Info/BPI_MapMakkaWinCtrl.BPI_SetLock_MapMakkaWin`
  (params (Lock :type Boolean) (ReturnAreaName :type Boolean)))

(fn `BPI_CheckActive`
  (returns (Active :type Boolean))
  (return false))

(fn `BPI_CheckActive_Miitsu`
  (returns (Active :type Boolean))
  (return false))

(fn `BPI_CheckNext_MapMiitsuWin`
  (returns (Next :type Boolean))
  (return false))

(fn `BPI_CheckNext_MimanMiitsu`
  (returns (Next :type Boolean))
  (return false))

(fn `BPI_NextMapMiitsuWin`
  (returns (Success :type Boolean))
  (return false))

(fn `HideAreaName`)

(fn `ShowAreaName`)

(fn `UserConstructionScript`)