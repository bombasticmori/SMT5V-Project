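; Garden map manager for free camera mode, left as a thin child Blueprint whose behavior comes from its parent class.
; Tick and the request, enable, disable and UI toggle functions only forward to the parent.
; The delay events and helpers for pawn lookup, input speeds, level visibility, nav collision and actor cleanup are empty stubs, with getters returning empty or default values.
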(event `self.ReceiveTick`
  (params (DeltaSeconds :type "Float (single-precision)"))
  (`parent.ReceiveTick` DeltaSeconds))

(event `DelayEnableCamera`)

(event `DelayDisableCamera`)

(event `DelayWaitPlayerStop`)

(fn `AddNaviCollision`)

(fn `CheckDebugValues`)

(fn `DeleteNaviCollision`)

(fn `DestroyFreeCameraActors`
  (returns (DestroySuccess :type Boolean))
  (return false))

(fn `DisableFreeCamera`
  (`parent.DisableFreeCamera`))

(fn `EnableFreeCamera`
  (`parent.EnableFreeCamera`))

(fn `Get FC Pawn`
  (returns (SpectatorPawn :type "SpectatorPawn Object Reference"))
  (return null))

(fn `GetInputSpeed`
  (returns (`Default Camera Movement Speed` :type "Float (double-precision)") (`Dash Camera Movement Speed` :type "Float (double-precision)") (`Sneak Camera Movement Speed` :type "Float (double-precision)") (`Default Turn Input Scale` :type "Float (double-precision)") (`Dash Turn Input Scale` :type "Float (double-precision)") (`Sneak Turn Input Scale` :type "Float (double-precision)") (`Mouse Turn Input Max` :type "Float (double-precision)"))
  (return 0.0 0.0 0.0 0.0 0.0 0.0 0.0))

(fn `RequestEndFreeCamera`
  (`parent.RequestEndFreeCamera`))

(fn `RequestStartFreeCamera`
  (`parent.RequestStartFreeCamera`))

(fn `Set Visibility Free Camera Unload Level`
  (params (`Should be Visible` :type Boolean)))

(fn `SetInputSpeed`
  (params (`Default Camera Movement Speed` :type "Float (double-precision)") (`Dash Camera Movement Speed` :type "Float (double-precision)") (`Sneak Camera Movement Speed` :type "Float (double-precision)") (`Default Turn Input Scale` :type "Float (double-precision)") (`Dash Turn Input Scale` :type "Float (double-precision)") (`Sneak Turn Input Scale` :type "Float (double-precision)") (`Mouse Turn Input Max` :type "Float (double-precision)")))

(fn `ToggleFreeCameraUI`
  (`parent.ToggleFreeCameraUI`))