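; Controller Blueprint for a free camera in the Garden map, with input hooks for moving, looking, dashing, attack, cancel and automap.
; Input events and functions for speed, turn scale, mouse clamping, input shaping and reset are empty stubs or return zero.
; BeginPlay and EndPlay only forward to the parent.
; InitFreeCamera returns the parent's result, but its parent call is disconnected from execution and never runs.
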(event `self.ReceiveBeginPlay`
  (`parent.ReceiveBeginPlay`))

(event `ActPadEvt_Map_Dash_R_K2Node_ActionPadEvent_6`
  (params (Key :type "Key Structure")))

(event `ActPadEvt_Map_Dash_R_K2Node_ActionPadEvent_5`
  (params (Key :type "Key Structure")))

(event `ActPadEvt_Map_Dash_K2Node_ActionPadEvent_4`
  (params (Key :type "Key Structure")))

(event `ActPadEvt_Map_Dash_K2Node_ActionPadEvent_3`
  (params (Key :type "Key Structure")))

(event `ActPadEvt_Utl_Cancel_K2Node_ActionPadEvent_2`
  (params (Key :type "Key Structure")))

(event `ActPadEvt_Map_Attack_K2Node_ActionPadEvent_1`
  (params (Key :type "Key Structure")))

(event `ActPadEvt_Map_AutoMap_K2Node_ActionPadEvent_0`
  (params (Key :type "Key Structure")))

(event `InpAxisEvt_LookRight_K2Node_InputAxisEvent_4`
  (params (AxisValue :type "Float (double-precision)")))

(event `InpAxisEvt_Garden_MoveUp_K2Node_InputAxisEvent_5`
  (params (AxisValue :type "Float (double-precision)")))

(event `InpAxisEvt_Garden_MoveRight_K2Node_InputAxisEvent_6`
  (params (AxisValue :type "Float (double-precision)")))

(event `InpAxisEvt_LookUp_K2Node_InputAxisEvent_3`
  (params (AxisValue :type "Float (double-precision)")))

(event `InpAxisEvt_MoveForward_K2Node_InputAxisEvent_2`
  (params (AxisValue :type "Float (double-precision)")))

(event `InpAxisEvt_MoveRight_K2Node_InputAxisEvent_0`
  (params (AxisValue :type "Float (double-precision)")))

(event `InpAxisEvt_LookRight_Mouse_K2Node_InputAxisEvent_9`
  (params (AxisValue :type "Float (double-precision)")))

(event `InpAxisEvt_LookUp_Mouse_K2Node_InputAxisEvent_8`
  (params (AxisValue :type "Float (double-precision)")))

(event `self.ReceiveEndPlay`
  (params (EndPlayReason :type "EEndPlayReason Enum" :default "Destroyed"))
  (`parent.ReceiveEndPlay` EndPlayReason))

(fn `Clamp Mouse Max`
  (params (Value :type "Float (double-precision)"))
  (returns (ReturnValue :type "Float (double-precision)"))
  (return 0.0))

(fn `InitFreeCamera`
  (returns (ReturnValue :type Boolean))
  (bind _returnvalue (`parent.InitFreeCamera`))
  (return _returnvalue))

(fn `ModifyInput_DPAD`
  (params (RawInput :type "Float (double-precision)"))
  (returns (ModifiedInput :type "Float (double-precision)"))
  (return 0.0))

(fn `ModifyInput_KM_STICK`
  (params (RawInput :type "Float (double-precision)"))
  (returns (ModifiedInput :type "Float (double-precision)"))
  (return 0.0))

(fn `ResetFreeCamera`)

(fn `Set Input Speed`
  (params (`Default Camera Movement Speed` :type "Float (double-precision)") (`Dash Camera Movement Speed` :type "Float (double-precision)") (`Sneak Camera Movement Speed` :type "Float (double-precision)") (`Default Turn Input Scale` :type "Float (double-precision)") (`Dash Turn Input Scale` :type "Float (double-precision)") (`Sneak Turn Input Scale` :type "Float (double-precision)") (MouseMax :type "Float (double-precision)")))

(fn `Set Turn InputSpeed`
  (params (`Input Scale` :type "Float (double-precision)")))

(fn `UserConstructionScript`)