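; BP_GardenEventMissionBase is a base Blueprint for Garden map event missions and quests, with every event and function left as a stub.
; It declares hooks for quest lifecycle, mission acceptance, actor warping and look-at, plus BI-prefixed calls for script spawning, screen fades and active-area checks.
; Functions with results return false, and BeginPlay, Tick and overlap events are disabled, so the graphs contain no gameplay logic.
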(event `/Game/Blueprints/Event/Script/BPI_EventScript.CheckActive`)

(event `/Game/Blueprints/Event/Script/BPI_EventScript.DestroyKeyFree`)

(event `/Game/Blueprints/Event/Script/BPI_EventScript.PlayDeadMotion`
  (params (Active :type Boolean)))

(event `/Game/Blueprints/Event/Script/BPI_EventScript.BI_ChangeMaterialAlice`)

(event `/Game/Blueprints/Event/Script/BPI_EventScript.BI_RecalcOverlap`)

(event `StartQuest`)

(event `/Game/Blueprints/Event/Script/BPI_EventScript.CallDeactivate`)

(event `ActivateQuest`
  (params (`Quest Devil Ref` :type "/Game/Blueprints/Character/Base/DevilBase Object Reference (by ref)")))

(event `EndQuest`)

(event `ReadyQuest`)

(fn `AcceptMission`
  (params (missionId :type Integer)))

(fn `BI_CheckActiveArea`
  (returns (IsActive :type Boolean))
  (return false))

(fn `BI_DeleteScript`
  (returns (NoUse :type Boolean))
  (return false))

(fn `BI_FadeInBlack`
  (params (Time :type "Float (double-precision)"))
  (returns (ret :type Boolean))
  (return false))

(fn `BI_FadeInWhite`
  (params (Time :type "Float (double-precision)"))
  (returns (ret :type Boolean))
  (return false))

(fn `BI_FadeOutBlack`
  (params (Time :type "Float (double-precision)"))
  (returns (ret :type Boolean))
  (return false))

(fn `BI_FadeOutWhite`
  (params (Time :type "Float (double-precision)"))
  (returns (ret :type Boolean))
  (return false))

(fn `BI_SetInvalidWindow`
  (params (Invalid :type Boolean))
  (returns (NoUse :type Boolean))
  (return false))

(fn `BI_SpawnScript`
  (returns (NoUse :type Boolean))
  (return false))

(fn `ForceSpawnScript`
  (returns (NoUse :type Boolean))
  (return false))

(fn `IsQuestTalkDone`
  (returns (IsFinished :type Boolean))
  (return false))

(fn `SetLookAtPlayerForActors`
  (params (Enable :type Boolean)))

(fn `SpawnReflesh`
  (returns (NoUse :type Boolean))
  (return false))

(fn `TryForceAcceptQuestByDevilID`
  (params (DevilID :type Integer))
  (returns (IsSuccessful :type Boolean))
  (return false))

(fn `UserConstructionScript`
  (`parent.UserConstructionScript`))

(fn `Warp Actor`
  (params (TargetLocation :type "Vector Structure") (TargetRotation :type "Rotator Structure") (WarpActor :type "Actor Object Reference (by ref)")))