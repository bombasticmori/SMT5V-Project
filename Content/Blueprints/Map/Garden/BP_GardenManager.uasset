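; Garden map manager Blueprint whose interface covers devil spawning, talks, quests, tributes and a free camera mode.
; It holds almost no logic of its own: initialization, teardown, readiness checks, tick, delayed and single devil spawning, and devil type lookup only forward to the parent class.
; All other events and functions are empty stubs or return defaults such as false, zero or none.
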(event `self.ReceiveTick`
  (params (DeltaSeconds :type "Float (single-precision)"))
  (`parent.ReceiveTick` DeltaSeconds))

(event `OnLoaded_E1F8C9284D257424E847A29EA321E822`
  (params (Loaded :type "Object Object Reference")))

(event `/Game/Blueprints/Map/Garden/BPI_GardenManager.SetVisibilityPlayerTalkGodray`
  (params (bNewVisibility :type Boolean)))

(event `/Game/Blueprints/Map/Garden/BPI_GardenManager.PlayWalkingMotion`)

(event `/Game/Blueprints/Map/Garden/BPI_GardenManager.SetFreeCameraMode`
  (params (IsFreeCameraMode :type Boolean)))

(event `/Game/Blueprints/Map/Garden/BPI_GardenManager.TryActivateTribute`)

(event `/Game/Blueprints/Map/Garden/BPI_GardenManager.EnableFreeCamera`)

(event `/Game/Blueprints/Map/Garden/BPI_GardenManager.SetGardenTributeTarget`
  (params (TributeTarget :type "Actor Object Reference")))

(event `/Game/Blueprints/Map/Garden/BPI_GardenManager.EndGardenDevilTalk`)

(event `/Game/Blueprints/Map/Garden/BPI_GardenManager.Set Visibility Garden Devils`
  (params (Visibility :type Boolean) (ExcludedDevilID :type Integer)))

(event `/Game/Blueprints/Map/Garden/BPI_GardenManager.StartGardenDevilTalk`
  (params (DevilChara :type "Actor Object Reference") (DevilID :type Integer) (IdleMotionID :type "E_CHARA_MOTION_ID Enum" :default "NONE") (IsHitoshura :type Boolean)))

(event `/Game/Blueprints/Map/Garden/BPI_GardenManager.StartGardenResult`
  (params (GardenResultData :type "GardenResultData Structure")))

(event `/Game/Blueprints/Map/Garden/BPI_GardenManager.UpdatePlayerMapIcon`)

(event `/Game/Blueprints/Map/Garden/BPI_GardenManager.StartPlayerTalkTutorial`
  (params (GardenPlayer :type "Actor Object Reference")))

(event `/Game/Blueprints/Map/Garden/BPI_GardenManager.RespawnGardenDevils`
  (params (ExcludedDevilID :type Integer)))

(event `/Game/Blueprints/Map/Garden/BPI_GardenManager.RepickGardenDevils`)

(event `GetValidPhaseData`)

(event `self.CheckGardenReady`
  (`parent.CheckGardenReady`))

(event `Activate Garden Quest`)

(event `SetGardenBGM`
  (params (Asset :type "Object Soft Object Reference")))

(event `self.SpawnDevilsDelayed`
  (`parent.SpawnDevilsDelayed`))

(event `SetFreeCameraPlayerCollision`
  (params (bFreeCameraMode :type Boolean)))

(fn `Check Player Movement Stopped`
  (returns (ReturnValue :type Boolean))
  (return false))

(fn `CheckDespawnGardenQuestFinished`
  (returns (IsDespawnFinished :type Boolean))
  (return false))

(fn `CheckGardenMoveFinished`
  (returns (IsMoveFinished :type Boolean))
  (return false))

(fn `CheckGardenQuestAccepted`
  (returns (IsQuestAccepted :type Boolean))
  (return false))

(fn `CheckGardenQuestFinished`
  (returns (IsQuestFinished :type Boolean))
  (return false))

(fn `CheckGardenResultFinished`
  (returns (IsResultFinished :type Boolean))
  (return false))

(fn `CheckManagerInitializationDone`
  (returns (ReturnValue :type Boolean))
  (bind _returnvalue (`parent.CheckManagerInitializationDone`))
  (return _returnvalue))

(fn `CheckMessageLoadDone`
  (returns (AllMessageLoadDone :type Boolean))
  (return false))

(fn `CheckReplacementCharaID`
  (params (DevilID :type Integer))
  (returns (ReplacementID :type Integer) (HasReplacement :type Boolean))
  (return 0 false))

(fn `CheckValidGardenQuest`
  (params (DevilID :type Integer))
  (returns (IsValid :type Boolean))
  (return false))

(fn `CheckValidTributeTarget`
  (returns (IsValid :type Boolean))
  (return false))

(fn `DebugInitFreeCameraDevilCollision`)

(fn `DebugSetGardenDevilMessage`
  (params (DevilID :type Integer) (`Chat Msg Type` :type "E_GARDEN_MSG_USE_TYPE Enum" :default "MSG_NONE") (`Chat Msg Index` :type Integer)))

(fn `DebugSetParty`)

(fn `DebugSpawnDevils`)

(fn `DespawnGardenQuestSublevel`
  (returns (UnloadSuccess :type Boolean))
  (return false))

(fn `DestroyGardenDevil`
  (params (DevilID :type Integer)))

(fn `DestroyManager`
  (`parent.DestroyManager`))

(fn `FindDevilType`
  (params (GardenDevilID :type Integer))
  (returns (ReturnValue :type "GardenDevilInfo Structure"))
  (bind _returnvalue (`parent.FindDevilType` GardenDevilID))
  (return _returnvalue))

(fn `GardenSpawnDevils`)

(fn `Get Garden Table Rows`)

(fn `GetAdjustRate`
  (params (DevilID :type Integer))
  (returns (Rate :type "Float (double-precision)"))
  (return 0.0))

(fn `GetDevilMsgData`
  (params (DevilID :type Integer))
  (returns (UniqueDevilMsgData :type "GardenUniqueDevilMsgData Structure") (SpeechTypeMsgData :type "GardenSpeechTypeMsgData Structure") (SoftUniqueDevilMsgAsset :type "ScriptMessageAsset Soft Object Reference") (SoftSpeechTypeMsgAsset :type "ScriptMessageAsset Soft Object Reference") (CurrentGardenArea :type "E_RYUKETSU_GARDEN_TYPE Enum") (`Valid Phases` :type "Array of Byte"))
  (return (struct) (struct) null null "E_NONE"))

(fn `GetFCManager`
  (returns (`FC Manager` :type "ActorComponent Object Reference"))
  (return null))

(fn `GetFreeCameraMS`
  (returns (`Default Camera Movement Speed` :type "Float (double-precision)") (`Dash Camera Movement Speed` :type "Float (double-precision)") (`Sneak Camera Movement Speed` :type "Float (double-precision)") (`Default Turn Input Scale` :type "Float (double-precision)") (`Dash Turn Input Scale` :type "Float (double-precision)") (`Sneak Turn Input Scale` :type "Float (double-precision)") (`Mouse Turn Input Max` :type "Float (double-precision)"))
  (return 0.0 0.0 0.0 0.0 0.0 0.0 0.0))

(fn `GetFreeCameraPawn`
  (returns (`FC Pawn` :type "SpectatorPawn Object Reference"))
  (return null))

(fn `GetGardenCollisionScale`
  (params (DevilID :type Integer))
  (returns (CollisionVal :type "GardenTalkCollision Structure") (Found :type Boolean))
  (return (struct) false))

(fn `GetGardenTalkHeight`
  (params (DevilID :type Integer))
  (returns (CameraParam :type "GardenTalkHeightOverride Structure") (Found :type Boolean))
  (return (struct) false))

(fn `GetUsedSPTList`
  (returns (UsedSPTDataList :type "Array of GardenSPTData Structure"))
  (return))

(fn `IncrementMessageCheck`
  (returns (dummy :type Boolean))
  (return false))

(fn `Init Garden Talk Params`
  (params (GardenDevilInfo :type "GardenDevilInfo Structure (by ref)") (UsedAnimation :type "E_GARDEN_SPAWN_ANIMATION Enum" :default "E_STAND") (GardenDevil :type "/Game/Blueprints/Map/Garden/BP_GardenDevil Object Reference") (GardenTalk :type "/Game/Blueprints/Map/Garden/BP_GardenTalk Object Reference") (DevilID :type Integer)))

(fn `InitializeManager`
  (params (FreeCameraDisableLevel :type Name))
  (`parent.InitializeManager` FreeCameraDisableLevel))

(fn `IsFreeCameraCollisionSwitchFinished`
  (returns (IsFinished :type Boolean))
  (return false))

(fn `IsPlayerTalkFinished`
  (returns (IsFinished :type Boolean))
  (return false))

(fn `IsRespawning`
  (returns (RespawnFlag :type Boolean))
  (return false))

(fn `NeedsCollisionAdjust`
  (params (DevilID :type Integer))
  (returns (NeedsAdjust :type Boolean) (AdjustType :type "E_GARDEN_FC_DEVIL_COL_TYPE Enum"))
  (return false "E_TYPE_A"))

(fn `Re-PickGardenDevil`)

(fn `Route Flag Check`
  (params (Index :type Integer))
  (returns (ReturnValue :type Boolean))
  (return false))

(fn `Set Devil Free Camera Collision Mode`
  (params (IsFreeCameraMode :type Boolean)))

(fn `Set Visibility All Devils`
  (params (Visibility :type Boolean) (Devil_ID :type Integer)))

(fn `SetArea`)

(fn `SetDebugSpawnFlag`
  (params (DebugSpawnOff :type Boolean))
  (returns (dummy :type Boolean))
  (return false))

(fn `SetFreeCameraMS`
  (params (`Default Camera Movement Speed` :type "Float (double-precision)") (`Dash Camera Movement Speed` :type "Float (double-precision)") (`Sneak Camera Movement Speed` :type "Float (double-precision)") (`Default Turn Input Scale` :type "Float (double-precision)") (`Dash Turn Input Scale` :type "Float (double-precision)") (`Sneak Turn Input Scale` :type "Float (double-precision)") (`Mouse Turn Input Max` :type "Float (double-precision)"))
  (returns (dummy :type Boolean))
  (return false))

(fn `SetMessageTalkFlag`
  (params (SpeechType :type "E_TALK_TONE_TYPE Enum" :default "E_NONE") (ChatMsgType :type "E_GARDEN_MSG_USE_TYPE Enum" :default "MSG_NONE") (DevilID :type Integer) (ChatMsgIndex :type Integer))
  (returns (dummy :type Boolean))
  (return false))

(fn `SetUsedSPTList`
  (params (`New SPTData` :type "Array of GardenSPTData Structure (by ref)"))
  (returns (dummy :type Boolean))
  (return false))

(fn `SpawnDespawnGardenDevils`
  (params (IsSpawn :type Boolean) (DevilID :type Integer)))

(fn `SpawnGardenDevil`
  (params (GardenDevilSpawnInfo :type "GardenDevilSpawnInfo Structure") (DevilID :type Integer))
  (returns (ReturnValue :type "GardenDevil Object Reference"))
  (bind _returnvalue (`parent.SpawnGardenDevil` GardenDevilSpawnInfo DevilID))
  (return _returnvalue))

(fn `SpawnGardenQuestSubLevel`
  (params (DevilID :type Integer) (QuestDevil :type "Actor Object Reference"))
  (returns (SpawnSuccess :type Boolean))
  (return false))

(fn `SpawnQuestSublevel`
  (params (DevilID :type Integer) (`Quest Devil Ref` :type "/Game/Blueprints/Character/Base/DevilBase Object Reference (by ref)"))
  (returns (Success :type Boolean))
  (return false))

(fn `Tick Hit`)

(fn `TutorialSpawnDevils`)

(fn `UserConstructionScript`)