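; BP_GardenDevil is the devil actor for the Garden map, a child Blueprint with hooks for model loading, talk, sit/stand motion, visibility and free-camera collision.
; Tick, spawn, despawn, destruction and chat-message lookup only forward to the parent class.
; All other events and functions are empty or return false or zero, so this file holds no garden-specific logic of its own.
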(event `self.ReceiveTick`
  (params (DeltaSeconds :type "Float (single-precision)"))
  (`parent.ReceiveTick` DeltaSeconds))

(event `TempHidden_Timeline__FinishedFunc`)

(event `TempHidden_Timeline__UpdateFunc`)

(event `OnLoaded_88315CEC420B99FA256673AB6B5A7A82`
  (params (Loaded :type "Object Object Reference")))

(event `OnLoaded_75CF795F4744832BD1C3369CD666C789`
  (params (Loaded :type "Object Object Reference")))

(event `OnLoaded_C0F1829F4565B66D977F73BC6B382242`
  (params (Loaded :type "Object Object Reference")))

(event `OnLoaded_1639E30C4B4CCAF79551B5A08F03B037`
  (params (Loaded :type "Object Class Reference")))

(event `OnLoaded_A44684DC43BA922C34C4FEAE23D429F5`
  (params (Loaded :type "Object Object Reference")))

(event `OnLoaded_E976BEF349CDA0EF713853B96104BDA7`
  (params (Loaded :type "Object Object Reference")))

(event `self.SpawnDevil`
  (`parent.SpawnDevil`))

(event `self.ReceiveDestroyed`
  (`parent.ReceiveDestroyed`))

(event `LoadModelAndStart`)

(event `/Game/Blueprints/Map/Garden/BPI_GardenDevil.TempHidden_Garden`)

(fn `Check Flags`)

(fn `Check Is Devil Shown`
  (returns (DevilIsVisible :type Boolean))
  (return false))

(fn `Despawn`
  (`parent.Despawn`))

(fn `GetDevilFreeCameraDistance`
  (params (SoftClassReference :type "Object Soft Class Reference (by ref)"))
  (returns (ReturnValue :type "Float (double-precision)"))
  (return 0.0))

(fn `GetUsedChatMsg`
  (returns (ReturnValue :type "GardenRespawnChatInfo Structure"))
  (bind _returnvalue (`parent.GetUsedChatMsg`))
  (return _returnvalue))

(fn `InitFreeCameraCollision`)

(fn `IsMessageInitDone`
  (returns (InitDone :type Boolean))
  (return false))

(fn `Replace Material Check`
  (params (`Devil ClassAssetID` :type "Object Soft Class Reference (by ref)")))

(fn `Set Garden Camera Param`)

(fn `Set Garden Talk`
  (params (GardenTalk :type "/Game/Blueprints/Map/Garden/BP_GardenTalk Object Reference") (IsSitting :type Boolean) (IsLarge :type Boolean) (SpotScale :type Boolean)))

(fn `Set Icon Talk`
  (params (`Speech Type` :type "E_TALK_TONE_TYPE Enum" :default "E_NONE") (`Chat Msg Type` :type "E_GARDEN_MSG_USE_TYPE Enum" :default "MSG_NONE") (`Chat Msg Index` :type Integer)))

(fn `SetCanBeHiddenFlag`
  (params (CanBeHidden :type Boolean)))

(fn `SetFreeCameraCollision`
  (params (SetFreeCameraMode :type Boolean)))

(fn `SetGardenBoundsScale`)

(fn `SetSitMotion`)

(fn `SetStandingMotion`)

(fn `SetVisibility`
  (params (Enabled :type Boolean)))

(fn `UserConstructionScript`)