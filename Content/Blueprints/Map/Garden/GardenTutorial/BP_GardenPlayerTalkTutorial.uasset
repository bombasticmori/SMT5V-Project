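; Garden map tutorial quest Blueprint, named for a player talk step, with CheckActive, QuestExecute and ReadyQuest events that only call their parent versions.
; It declares a MovePlayer timeline with a stop event track, asynchronous load callbacks, a WalkToBenchStop event and a SetVisibility function, all with empty bodies.
; BeginPlay, overlap and Tick are disabled, so any working behavior comes from the parent class.
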(event `MovePlayer__FinishedFunc`)

(event `MovePlayer__UpdateFunc`)

(event `MovePlayer__StopTrack__EventFunc`)

(event `OnLoaded_8C5F64BC4F1BBF199F45C4BC90E798EE`
  (params (Loaded :type "Object Object Reference")))

(event `OnLoaded_8C5F64BC4F1BBF199F45C4BC1BFC419A`
  (params (Loaded :type "Object Object Reference")))

(event `OnLoaded_8C5F64BC4F1BBF199F45C4BC3FAAC91D`
  (params (Loaded :type "Object Object Reference")))

(event `OnLoaded_0E38A2EA4724D2AEB4E20FBD9F97EF82`
  (params (Loaded :type "Object Object Reference")))

(event `/Game/Blueprints/Event/Script/BPI_EventScript.CheckActive`
  (`parent.CheckActive`))

(event `/Game/Blueprints/Event/Script/BP_EventMissionBaseCommon.QuestExecute`
  (`parent.QuestExecute`))

(event `self.ReadyQuest`
  (`parent.ReadyQuest`))

(event `WalkToBenchStop`)

(fn `Set Visibility`
  (params (Show :type Boolean)))

(fn `UserConstructionScript`
  (`parent.UserConstructionScript`))