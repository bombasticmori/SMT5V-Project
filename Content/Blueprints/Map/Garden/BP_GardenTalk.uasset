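; BP_GardenTalk is a Garden map Blueprint whose interface covers talking to devils: chat messages, voice and motion, tributes, trophy counters and map icons.
; Its quest, message-window and map-event hooks suggest a quest-style talk event that starts from a given devil, camera parameter and icon offset.
; All logic here is stubbed: BeginPlay and Tick only call the parent, while everything else is empty or returns default values.
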(event `self.ReceiveBeginPlay`
  (`parent.ReceiveBeginPlay`))

(event `self.ReceiveTick`
  (params (DeltaSeconds :type "Float (single-precision)"))
  (`parent.ReceiveTick` DeltaSeconds))

(event `OnLoaded_43A715774CD3016AB2BC1599E4691F66`
  (params (Loaded :type "Object Class Reference")))

(event `EvtDrawCommonMsgTextLabel`
  (params (ScriptMessageAsset :type "ScriptMessageAsset Object Reference") (Label :type Name) (SpeakingActor :type "Actor Object Reference")))

(event `EvtDrawCommonMsgTextIndex`
  (params (ScriptMessageAsset :type "ScriptMessageAsset Object Reference") (Index :type Integer) (SpeakingActor :type "Actor Object Reference")))

(event `EvtOpenCommonMsgWindow`)

(event `EvtCloseCommonMsgWindow`)

(event `StartQuest`)

(event `ReadyQuest`)

(event `AreaIn`)

(event `AreaOut`)

(event `Deactivate`)

(event `EndQuest`)

(event `ActionIn`)

(event `ActionOut`)

(event `SetInvalidWindow`
  (params (Invalid :type Boolean)))

(event `CheckActive`)

(event `CallDeactivate`)

(event `EndMission`)

(event `QuestExecute`)

(event `Play Devil Voice`
  (params (DevilVoiceType :type "EDevilVoiceType Enum" :default "EDevilVoiceType_None")))

(event `TributeMessage`)

(fn `ActivateBase`)

(fn `Add Tribute Points`
  (params (DevilID :type Integer) (IsRare :type Boolean)))

(fn `Change Map Icon`)

(fn `Check Debug Override Chat Message`
  (returns (m_UsedChatIndex :type Integer) (ReturnValue :type "GardenChatMsgData Structure"))
  (return 0))

(fn `Check Debug Override Item Message`)

(fn `Check Debug Override Powerup Message`)

(fn `Check Tribute`
  (returns (CanGiveTribute :type Boolean))
  (return false))

(fn `Check Tribute Button`
  (returns (IsButton :type Boolean))
  (return false))

(fn `CheckRespawn_PickChatMsg`
  (params (RespawnFlag :type Boolean) (CurrentGardenArea :type "Byte (by ref)") (ValidPhases :type "Array of Byte (by ref)"))
  (returns (Success :type Boolean) (SPTDataList :type "Array of GardenSPTData Structure"))
  (return false))

(fn `DeactivateBase`)

(fn `Do Trophy Counter Process`
  (params (GardenTrophyType :type "E_GARDEN_TROPHY_COUNTER_TYPE Enum" :default "E_TRIBUTE")))

(fn `Draw Common Msg Text Label No Delay`
  (params (ScriptMessageAsset :type "ScriptMessageAsset Object Reference") (Label :type Name) (ExecutionText :type Boolean) (ShowPageIconAfterCompleted :type Boolean)))

(fn `EndMapEvent`
  (returns (Dummy :type Boolean))
  (return false))

(fn `EndMapEvent_0`
  (returns (Dummy :type Boolean))
  (return false))

(fn `FadeInMapEvent`
  (returns (Delay :type "Float (double-precision)"))
  (return 0.0))

(fn `FadeOutMapEvent`
  (returns (Delay :type "Float (double-precision)"))
  (return 0.0))

(fn `GetActive`
  (returns (IsActive :type Boolean))
  (return false))

(fn `Initialize Map Icon`
  (params (IconOffset :type "Vector Structure")))

(fn `InitializeMessage`
  (params (GardenUniqueDevilMsgData :type "GardenUniqueDevilMsgData Structure (by ref)") (GardenSpeechTypeMsgData :type "GardenSpeechTypeMsgData Structure (by ref)") (DevilID :type Integer) (CurrentGardenArea :type "E_RYUKETSU_GARDEN_TYPE Enum (by ref)") (ValidPhases :type "Array of Byte (by ref)") (UniqueMessageAsset :type "ScriptMessageAsset Object Reference") (SpeechTypeMessageAsset :type "ScriptMessageAsset Object Reference"))
  (returns (Success :type Boolean))
  (return false))

(fn `IsPlayerLooking`
  (returns (IsLooking :type Boolean))
  (return false))

(fn `PlayMsgDataVoiceMotion`
  (params (GardenMsgData :type "GardenMsgData Structure (by ref)")))

(fn `RefreshMsgFlagStatus`)

(fn `Set Chara Name by ID`
  (params (`Script Message` :type "ScriptMessageAsset Object Reference") (DevilID :type Integer) (MessageID :type Integer)))

(fn `SetChatMessageIcon`
  (params (`L Chat Msg Type` :type "E_GARDEN_MSG_USE_TYPE Enum" :default "MSG_NONE") (`L Raw Chat Msg Index` :type Integer) (`L isInit` :type Boolean)))

(fn `SetDevilAndStart`
  (params (GardenUniqueDevilMsgData :type "GardenUniqueDevilMsgData Structure (by ref)") (GardenSpeechTypeMsgData :type "GardenSpeechTypeMsgData Structure (by ref)") (CurrentGardenArea :type "E_RYUKETSU_GARDEN_TYPE Enum (by ref)") (`Valid Phases` :type "Array of Byte (by ref)") (DevilBase :type "/Game/Blueprints/Character/Base/DevilBase Object Reference") (Unique :type "ScriptMessageAsset Object Reference") (SpeechType :type "ScriptMessageAsset Object Reference") (DevilID :type Integer) (IconOffset :type "Vector Structure") (GardenTalkCameraParam :type "GardenTalkCameraParam Structure")))

(fn `SetDevilAndStart_New`
  (params (DevilBase :type "/Game/Blueprints/Character/Base/DevilBase Object Reference") (IconOffset :type "Vector Structure") (GardenTalkCameraParam :type "GardenTalkCameraParam Structure")))

(fn `SetEndMapEventParam`
  (returns (Dummy :type Boolean))
  (return false))

(fn `SetMessageEventFlag`
  (params (EventFlag :type Boolean)))

(fn `SetMessageProgramValue`
  (params (InIndex :type Integer) (`Program String` :type String)))

(fn `SetMessageTagValue`
  (params (Index :type Integer) (Value :type Integer)))

(fn `SetPlayerLookAt`
  (params (Enable :type Boolean)))

(fn `StartMapEvent`
  (params (PlayerVisible :type Boolean) (NoStopPrioBGM :type Boolean) (PlayerCameraEnable :type Boolean))
  (returns (Dummy :type Boolean))
  (return false))

(fn `StartMapEvent_0`
  (params (PlayerVisible :type Boolean) (NoStopPrioBGM :type Boolean) (PlayerCameraEnable :type Boolean))
  (returns (Dummy :type Boolean))
  (return false))

(fn `StartWithErrors`
  (params (DevilBase :type "/Game/Blueprints/Character/Base/DevilBase Object Reference") (DevilID :type Integer) (`Icon Offset` :type "Vector Structure") (`Garden Talk Camera Param` :type "GardenTalkCameraParam Structure")))

(fn `Stop Voice Component`)

(fn `Unset Devil Garden Talk Flag`
  (params (FlagType :type "E_GARDEN_TALK_TYPE Enum" :default "E_TRUST")))

(fn `UserConstructionScript`)