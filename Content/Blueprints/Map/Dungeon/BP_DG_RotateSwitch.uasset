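; BP_DG_RotateSwitch is a dungeon switch actor, apparently for rotating a room when hit.
; Its BeginPlay, Tick, hit action, EndPlay and construction script only forward to the parent.
; Functions outline a camera state sequence (ease-in, rotating, falling, ease-out), player hiding and falling, skip input, minimap icon and room-rotator hookup.
; All of these, plus the rotate start/finish events, are empty or return defaults here.
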(event `self.ReceiveBeginPlay`
  (`parent.ReceiveBeginPlay`))

(event `self.ReceiveTick`
  (params (DeltaSeconds :type "Float (single-precision)"))
  (`parent.ReceiveTick` DeltaSeconds))

(event `/Game/Blueprints/Map/Hit/Base/BPI_MapEventHit.EventHitAction`
  (`parent.EventHitAction`))

(event `DG_RoomRotatableInterface.OnRotateFinished`
  (params (isSkipped :type Boolean)))

(event `DG_RoomRotatableInterface.OnRotateStarted`)

(event `Init`)

(event `self.ReceiveEndPlay`
  (params (EndPlayReason :type "EEndPlayReason Enum" :default "Destroyed"))
  (`parent.ReceiveEndPlay` EndPlayReason))

(event `InitIconEndBattle`
  (params (BtlEndType :type "E_BTL_END Enum" :default "E_BTL_END_NONE") (ChainEncountNum :type Integer)))

(fn `BPI_SetDataId`
  (params (DataId :type Integer))
  (returns (Dummy :type Boolean))
  (return false))

(fn `CheckSkipInput`
  (returns (skip :type Boolean))
  (return false))

(fn `GetCameraComponentToUse`
  (returns (CameraComponent :type "CameraComponent Object Reference"))
  (return null))

(fn `GetRoomRotator`
  (returns (ReturnValue :type "DG_RoomRotator Object Reference"))
  (return null))

(fn `HidePlayer`)

(fn `ResetViewPitch`)

(fn `SetCameraState`
  (params (NewState :type "E_DG_ROOM_ROTATOR_CAMERA_STATE Enum" :default "E_IDLE")))

(fn `SetDeviceVisibility`
  (params (Visibility :type Boolean)))

(fn `SetMinimapIconTableRow`
  (params (Index :type Integer))
  (returns (OutRow :type "MinimapIconTableRow Structure") (NeedToAddMore :type Boolean))
  (return (struct) false))

(fn `SetRoomRotator`
  (params (RoomRotator :type "DG_RoomRotator Object Reference"))
  (returns (ReturnValue :type Boolean))
  (return false))

(fn `SetViewPitch`)

(fn `ShowButtonHelp`)

(fn `SkipRotate`
  (returns (CanSkip :type Boolean))
  (return false))

(fn `StartEaseInCamera`)

(fn `StartEaseOut`)

(fn `StartFallCamera`)

(fn `StartFallPlayer`)

(fn `StartRotate`)

(fn `SwitchCamera`)

(fn `ToKeyFreeCamera`)

(fn `Update Camera Rotating`
  (params (DeltaTime :type "Float (double-precision)")))

(fn `UpdateCameraEaseIn`)

(fn `UpdateCameraEaseOut`
  (params (DeltaTime :type "Float (double-precision)")))

(fn `UpdateCameraFalling`
  (params (DeltaTime :type "Float (double-precision)")))

(fn `UpdateCameraIdle`)

(fn `UpdatePlayerRotating`
  (params (DeltaSeconds :type "Float (double-precision)")))

(fn `UserConstructionScript`
  (`parent.UserConstructionScript`))