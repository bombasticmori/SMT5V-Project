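; BP_DG_ShooterManager is a dungeon map actor that, by its name and functions, manages shooters that launch or move the player along splines.
; It declares spline-arrival and player start/stop move events, plus functions for initial side and upward speed, move speed with acceleration, start notification and cancel.
; All are empty or return zero or false, and lifecycle events only call the parent, so this Blueprint adds no behavior of its own.
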(event `self.ReceiveBeginPlay`
  (`parent.ReceiveBeginPlay`))

(event `self.ReceiveTick`
  (params (DeltaSeconds :type "Float (single-precision)"))
  (`parent.ReceiveTick` DeltaSeconds))

(event `OnArriveSplineEnd`
  (params (ThisComponent :type "/Game/Blueprints/Map/Move/BPC_CharaSplineMover Object Reference")))

(event `StartPlayerMove`)

(event `StopPlayerMove`
  (params (SplineMover :type "/Game/Blueprints/Map/Move/BPC_CharaSplineMover Object Reference")))

(fn `CalcInitialSpeedSide`
  (params (Shooter :type "/Game/Blueprints/Map/Dungeon/BP_DG_Shooter Object Reference") (Location :type "Vector Structure"))
  (returns (InitialSpeed :type "Float (double-precision)"))
  (return 0.0))

(fn `CalcInitialSpeedUp`
  (params (Shooter :type "/Game/Blueprints/Map/Dungeon/BP_DG_Shooter Object Reference") (Location :type "Vector Structure"))
  (returns (InitialSpeed :type "Float (double-precision)"))
  (return 0.0))

(fn `GetSpeed`
  (params (Shooter :type "/Game/Blueprints/Map/Dungeon/BP_DG_Shooter Object Reference"))
  (returns (MoveSpeed :type "Float (double-precision)") (Acceleration :type "Float (double-precision)"))
  (return 0.0 0.0))

(fn `NotifyCancel`
  (returns (dummy :type Boolean))
  (return false))

(fn `NotifyStartMove`
  (params (Shooter :type "/Game/Blueprints/Map/Dungeon/BP_DG_Shooter Object Reference")))

(fn `UserConstructionScript`
  (`parent.UserConstructionScript`))