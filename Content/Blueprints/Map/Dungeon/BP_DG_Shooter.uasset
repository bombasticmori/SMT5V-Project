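; BP_DG_Shooter is a dungeon map actor, by name a shooter, built as a child Blueprint with no logic of its own.
; BeginPlay, the hit action event and the construction script only forward to the parent; overlap and Tick are disabled.
; Functions for pausing, effects, timer-based states, spline access, data setup and minimap icons are empty stubs or return defaults.
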(event `self.ReceiveBeginPlay`
  (`parent.ReceiveBeginPlay`))

(event `/Game/Blueprints/Map/Hit/Base/BPI_MapEventHit.EventHitAction`
  (`parent.EventHitAction`))

(fn `ActivateEffect`
  (returns (Dummy :type Boolean))
  (return false))

(fn `BPI_SetDataId`
  (params (DataId :type Integer))
  (returns (Dummy :type Boolean))
  (return false))

(fn `DeactivateEffect`
  (returns (Dummy :type Boolean))
  (return false))

(fn `EnterState`
  (params (NextState :type "/Game/Blueprints/Map/Dungeon/E_DG_SHOOTER_STATE Enum" :default "NewEnumerator0")))

(fn `GetIsUp`
  (returns (IsUp :type Boolean))
  (return false))

(fn `GetSpline`
  (returns (Spline :type "SplineComponent Object Reference"))
  (return null))

(fn `GetStateFromTimer`
  (params (Timer :type "Float (double-precision)"))
  (returns (State :type "/Game/Blueprints/Map/Dungeon/E_DG_SHOOTER_STATE Enum"))
  (return "NewEnumerator0"))

(fn `Init`
  (params (Manager :type "/Game/Blueprints/Map/Dungeon/BP_DG_ShooterManager Object Reference")))

(fn `LeaveState`
  (params (PrevState :type "/Game/Blueprints/Map/Dungeon/E_DG_SHOOTER_STATE Enum" :default "NewEnumerator0")))

(fn `SetDefaultData`)

(fn `SetMinimapIconTableRow`
  (params (Index :type Integer))
  (returns (OutRow :type "MinimapIconTableRow Structure") (NeedToAddMore :type Boolean))
  (return (struct) false))

(fn `SetPause`)

(fn `SetUnpause`)

(fn `Update`
  (params (MapTimer :type "Float (double-precision)")))

(fn `UserConstructionScript`
  (`parent.UserConstructionScript`))