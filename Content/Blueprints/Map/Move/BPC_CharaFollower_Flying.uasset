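; Flying variant of the character follower component, used for map movement.
; Tick, state, motion, position, velocity and warp logic all pass straight through to the parent follower.
; Ground-specific overrides are neutralized: slope, fall, on-ground, trace size, stop distance and dash effect are empty or return zero.
; Ground-type, give-up-following, turning, loop-motion and gimmick obstacle checks all return false.
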(event `self.ReceiveBeginPlay`
  (`parent.ReceiveBeginPlay`))

(event `self.ReceiveTick`
  (params (DeltaSeconds :type "Float (single-precision)"))
  (`parent.ReceiveTick` DeltaSeconds))

(event `OnLoaded_6E8E0874402C10BA5673C0B97FB96BD6`
  (params (Loaded :type "Object Object Reference")))

(event `self.Tick_DecideMotion`
  (`parent.Tick_DecideMotion`))

(event `self.PlayIdleMotion`
  (`parent.PlayIdleMotion`))

(event `self.Tick_DecideNextPos`
  (`parent.Tick_DecideNextPos`))

(event `self.Tick_DecideTargetRotate`
  (`parent.Tick_DecideTargetRotate`))

(event `self.Tick_DecideTargetPos`
  (`parent.Tick_DecideTargetPos`))

(event `self.Tick_DecideState`
  (`parent.Tick_DecideState`))

(event `self.Tick_DecideVelocity`
  (`parent.Tick_DecideVelocity`))

(event `/Game/Blueprints/Map/Move/BPI_CharaFollower.BPI_TeleportNaviLocationAndRotation`
  (params (Location :type "Vector Structure") (Rotation :type "Rotator Structure") (StopUntilPlayerMove :type Boolean))
  (`parent.BPI_TeleportNaviLocationAndRotation` Location Rotation StopUntilPlayerMove))

(event `self.Tick_CalcWarp`
  (`parent.Tick_CalcWarp`))

(fn `AfterWarp`
  (`parent.AfterWarp`))

(fn `BPI_WarpNaviDevilBasePos`
  (params (CalcOnGround :type Boolean))
  (returns (NewParam :type Boolean))
  (bind _newparam (`parent.BPI_WarpNaviDevilBasePos` CalcOnGround))
  (return _newparam))

(fn `CalcFall_ForGroundType`
  (params (InLocation :type "Vector Structure"))
  (returns (OutLocation :type "Vector Structure"))
  (return (0.0 0.0 0.0)))

(fn `CalcGiveupFollowing_ForGroundType`
  (returns (Giveup :type Boolean))
  (return false))

(fn `CalcMovingTraceSize`
  (returns (OffsetZ :type "Float (double-precision)") (Radius :type "Float (double-precision)") (HalfHeight :type "Float (double-precision)"))
  (return 0.0 0.0 0.0))

(fn `CalcOnGround`
  (params (InLocation :type "Vector Structure"))
  (returns (OutLocation :type "Vector Structure"))
  (return (0.0 0.0 0.0)))

(fn `CalcSlopeNormal`)

(fn `CanTurningWhenGimmickStopping`
  (returns (CanTurn :type Boolean))
  (return false))

(fn `ChangeFollowerState`
  (params (State :type "/Game/Blueprints/Map/Move/E_CharaFollowerState Enum" :default "NewEnumerator0") (TargetActor :type "Actor Object Reference"))
  (`parent.ChangeFollowerState` State TargetActor))

(fn `CheckGroundType`
  (returns (GroundType :type Boolean))
  (return false))

(fn `CheckLoopMotion`
  (returns (Loop :type Boolean))
  (return false))

(fn `GetFionnRunMotion`
  (returns (MotionID :type "E_CHARA_MOTION_ID Enum"))
  (return (`parent.GetFionnRunMotion`)))

(fn `GetStopDistance`
  (returns (Distance :type "Float (double-precision)"))
  (return 0.0))

(fn `IsCheckObstacle_WhenGotoGimmick`
  (returns (CheckObstacle_WhenGotoGimmick :type Boolean))
  (return false))

(fn `IsTurningTypeWhileWalking`
  (returns (IsWalking :type Boolean))
  (return false))

(fn `ResetMoveParam`
  (`parent.ResetMoveParam`))

(fn `UpdateDashEffect`)