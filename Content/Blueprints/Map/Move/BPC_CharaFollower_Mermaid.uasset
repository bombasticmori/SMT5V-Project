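; Follower component for the Mermaid character on the map, a child of a shared follower Blueprint that supplies its behavior.
; Tick stages for state, position, rotation, velocity and motion, plus warp, dive and most trace functions, simply forward to the parent.
; Other overrides are empty or return false and zero defaults, including visibility calculation, effects, post-dive view, motion checks and several ground searches, with no Mermaid-specific logic.
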(event `self.ReceiveBeginPlay`
  (`parent.ReceiveBeginPlay`))

(event `self.ReceiveTick`
  (params (DeltaSeconds :type "Float (single-precision)"))
  (`parent.ReceiveTick` DeltaSeconds))

(event `self.Tick_DecideNextPos`
  (`parent.Tick_DecideNextPos`))

(event `self.Tick_DecideTargetRotate`
  (`parent.Tick_DecideTargetRotate`))

(event `self.PlayIdleMotion`
  (`parent.PlayIdleMotion`))

(event `self.Tick_DecideMotion`
  (`parent.Tick_DecideMotion`))

(event `self.Tick_DecideVelocity`
  (`parent.Tick_DecideVelocity`))

(event `self.Tick_DecideTargetPos`
  (`parent.Tick_DecideTargetPos`))

(event `self.Tick_DecideState`
  (`parent.Tick_DecideState`))

(event `Tick_CalcVisible`)

(event `self.Hide_ForSomeReason`
  (params (Hide :type Boolean) (Reason :type "/Game/Blueprints/Map/Move/E_NaviDevilHideReason Enum" :default "NewEnumerator0"))
  (`parent.Hide_ForSomeReason` Hide Reason))

(event `/Game/Blueprints/Map/Move/BPI_CharaFollower.BPI_ChangeDecalAnimNotify`
  (params (Decal :type "DecalComponent Object Reference") (Visible :type Boolean))
  (`parent.BPI_ChangeDecalAnimNotify` Decal Visible))

(event `/Game/Blueprints/Map/Move/BPI_CharaFollower.BPI_ProcMermaid_WhenFoundCoaster`
  (`parent.BPI_ProcMermaid_WhenFoundCoaster`))

(event `ReadyView_AfterDive`)

(event `/Game/Blueprints/Map/Move/BPI_CharaFollower.BPI_DiveMermaid`
  (`parent.BPI_DiveMermaid`))

(fn `AfterWarp`
  (`parent.AfterWarp`))

(fn `BPI_WarpNaviDevilBasePos`
  (params (CalcOnGround :type Boolean))
  (returns (NewParam :type Boolean))
  (bind _newparam (`parent.BPI_WarpNaviDevilBasePos` CalcOnGround))
  (return _newparam))

(fn `CapsureTrace`
  (params (Start :type "Vector Structure") (End :type "Vector Structure") (Radius :type "Float (double-precision)") (HalfHeight :type "Float (double-precision)") (DrawDebugType :type "EDrawDebugTrace Enum" :default "None"))
  (returns (OutHit :type "HitResult Structure") (Hit :type Boolean) (HitNPC :type Boolean))
  (bind (_outhit _hit _hitnpc) (`parent.CapsureTrace` Start End Radius HalfHeight DrawDebugType))
  (return _outhit _hit _hitnpc))

(fn `ChangeFollowerState`
  (params (State :type "/Game/Blueprints/Map/Move/E_CharaFollowerState Enum" :default "NewEnumerator0") (TargetActor :type "Actor Object Reference"))
  (`parent.ChangeFollowerState` State TargetActor))

(fn `CheckFireEffect_WhenCameraOutside`
  (params (Hide :type Boolean) (Reason :type "/Game/Blueprints/Map/Move/E_NaviDevilHideReason Enum" :default "NewEnumerator0"))
  (returns (NewVisible :type Boolean))
  (return false))

(fn `CheckFlatGround`
  (params (Location :type "Vector Structure") (CheckPlayerToThis :type Boolean) (SearchGround :type Boolean))
  (returns (Enable :type Boolean) (OutLocation :type "Vector Structure"))
  (return false (0.0 0.0 0.0)))

(fn `CheckLoopMotion`
  (returns (Loop :type Boolean))
  (return false))

(fn `CheckMovableMotion`
  (returns (Movable :type Boolean))
  (return false))

(fn `GetAroundLocation`
  (params (BaseLocation :type "Vector Structure") (BaseDir :type "Vector Structure") (Distance :type "Float (double-precision)") (LocationNum :type Integer))
  (returns (LocationList :type "Array of Vector Structure"))
  (return))

(fn `GetNaviBasePosition`
  (returns (Location :type "Vector Structure") (Rotation :type "Rotator Structure"))
  (bind (_location _rotation) (`parent.GetNaviBasePosition`))
  (return _location _rotation))

(fn `InitEffect`)

(fn `LineTrace`
  (params (Start :type "Vector Structure") (End :type "Vector Structure") (DrawDebugType :type "EDrawDebugTrace Enum" :default "None"))
  (returns (OutHit :type "HitResult Structure") (Hit :type Boolean))
  (bind (_outhit _hit) (`parent.LineTrace` Start End DrawDebugType))
  (return _outhit _hit))

(fn `LineTrace_GroundAndNPC`
  (params (Start :type "Vector Structure") (End :type "Vector Structure") (DrawDebugType :type "EDrawDebugTrace Enum" :default "None"))
  (returns (OutHit :type "HitResult Structure") (Hit :type Boolean))
  (return (struct) false))

(fn `OnActived_IdleEffect`
  (params (Comp :type "ActorComponent Object Reference") (Reset :type Boolean)))

(fn `TraceGround`
  (params (NextPos :type "Vector Structure"))
  (returns (OutPos :type "Vector Structure") (Hit :type Boolean))
  (bind (_outpos _hit) (`parent.TraceGround` NextPos))
  (return _outpos _hit))

(fn `TraceGround_ForMermaidMove`
  (params (In_NowPos :type "Vector Structure") (In_NextPos :type "Vector Structure") (In_TargetPos :type "Vector Structure"))
  (returns (ResultPos :type "Vector Structure") (HitGround :type Boolean) (GroundNormal :type "Vector Structure") (HitWater :type Boolean))
  (return (0.0 0.0 0.0) false (0.0 0.0 0.0) false))

(fn `UpdateEffect`)