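; Character follower component for the navi devil companion, covering following, warping, gimmick guidance, coaster riding and mermaid diving.
; Its interface outlines a staged tick (state, target, velocity, position, rotation, motion, camera, warp) plus trace helpers for ground, walls and climbing.
; Only BeginPlay, Tick and EndPlay do anything, each calling its parent.
; All other events and functions here are empty stubs or return default values.
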(event `self.ReceiveBeginPlay`
  (`parent.ReceiveBeginPlay`))

(event `self.ReceiveTick`
  (params (DeltaSeconds :type "Float (single-precision)"))
  (`parent.ReceiveTick` DeltaSeconds))

(event `Tick_CalcCamera`)

(event `Tick_ProcMove`)

(event `OnSystemFinished_イベント_0`
  (params (PSystem :type "ParticleSystemComponent Object Reference")))

(event `Tick_CalcWarp`)

(event `OnEndMoveEffect`
  (params (PSystem :type "ParticleSystemComponent Object Reference")))

(event `EvtDis_StoppedTarget_Event`
  (params (Target :type "Actor Object Reference") (This :type "/Game/Blueprints/Map/Move/BPC_CharaFollower Object Reference")))

(event `EvtDis_LeaveTarget_Event`
  (params (Target :type "Actor Object Reference") (This :type "/Game/Blueprints/Map/Move/BPC_CharaFollower Object Reference")))

(event `EndGimmickEffect`
  (params (Immediately :type Boolean)))

(event `StartGimmickEffect`)

(event `EndMoveEffect`)

(event `StartMoveEffect`)

(event `self.ReceiveEndPlay`
  (params (EndPlayReason :type "EEndPlayReason Enum" :default "Destroyed"))
  (`parent.ReceiveEndPlay` EndPlayReason))

(event `SettingMeshOffset`)

(event `/Game/Blueprints/Map/Move/BPI_CharaFollower.BPI_SetVisibility`
  (params (Visible :type Boolean)))

(event `Tick_DecideVelocity`)

(event `Tick_DecideTargetPos`)

(event `TickDebug`)

(event `Tick_DecideTargetRotate`)

(event `/Game/Blueprints/Map/Move/BPI_CharaFollower.BPI_DiveMermaid`)

(event `Tick_DecideNextPos`)

(event `/Game/Blueprints/Map/Move/BPI_CharaFollower.BPI_ProcMermaid_WhenFoundCoaster`)

(event `Tick_DecideMotion`)

(event `/Game/Blueprints/Map/Move/BPI_CharaFollower.BPI_ChangeDecalAnimNotify`
  (params (Decal :type "DecalComponent Object Reference") (Visible :type Boolean)))

(event `PlayIdleMotion`)

(event `Hide_ForSomeReason`
  (params (Hide :type Boolean) (Reason :type "/Game/Blueprints/Map/Move/E_NaviDevilHideReason Enum" :default "NewEnumerator0")))

(event `Tick_DecideState`)

(event `/Game/Blueprints/Map/Move/BPI_CharaFollower.BPI_TeleportNaviLocationAndRotation`
  (params (Location :type "Vector Structure") (Rotation :type "Rotator Structure") (StopUntilPlayerMove :type Boolean)))

(event `/Game/Blueprints/Map/Move/BPI_CharaFollower.BPI_RideCoaster_ForNaviDevil`)

(event `/Game/Blueprints/Map/Move/BPI_CharaFollower.BPI_GetOffCoaster_ForNaviDevl`)

(event `Tick_FromEventNaviDevil`)

(event `/Game/Blueprints/Map/Move/BPI_CharaFollower.BPI_SetVisible_NaviGimmickEffect`
  (params (Visible :type Boolean)))

(event `/Game/Blueprints/Map/Move/BPI_CharaFollower.BPI_SetVisible_NaviMoveEffect`
  (params (Visible :type Boolean)))

(event `Test_MovingTraceScale`
  (params (Scale :type "Float (double-precision)")))

(fn `AddHitCount`)

(fn `AddTargetActor`
  (params (Target :type "Actor Object Reference") (IsCoaster :type Boolean) (Gimmick :type "Actor Object Reference")))

(fn `AfterWarp`)

(fn `BoxTrace`
  (params (Start :type "Vector Structure") (End :type "Vector Structure") (HalfSize :type "Vector Structure") (Orientation :type "Rotator Structure") (DrawDebugType :type "EDrawDebugTrace Enum" :default "None"))
  (returns (OutHit :type "HitResult Structure") (Hit :type Boolean) (HitNPC :type Boolean))
  (return (struct) false false))

(fn `BPI_WarpNaviDevilBasePos`
  (params (CalcOnGround :type Boolean))
  (returns (NewParam :type Boolean))
  (return false))

(fn `CalcDir_AlongWall`
  (params (Hit :type "HitResult Structure (by ref)"))
  (returns (Dir :type "Vector Structure"))
  (return (0.0 0.0 0.0)))

(fn `CalcGimmickRoute`)

(fn `CalcRecordGimmickDistance`
  (returns (Warp :type Boolean))
  (return false))

(fn `CapsureTrace`
  (params (Start :type "Vector Structure") (End :type "Vector Structure") (Radius :type "Float (double-precision)") (HalfHeight :type "Float (double-precision)") (DrawDebugType :type "EDrawDebugTrace Enum" :default "None"))
  (returns (OutHit :type "HitResult Structure") (Hit :type Boolean) (HitNPC :type Boolean))
  (return (struct) false false))

(fn `ChangeFollowerState`
  (params (State :type "/Game/Blueprints/Map/Move/E_CharaFollowerState Enum" :default "NewEnumerator0") (TargetActor :type "Actor Object Reference")))

(fn `CheckEnableChangeMotion`
  (returns (Enable :type Boolean))
  (return false))

(fn `CheckFrontNavi_ThanPlayer`
  (returns (FrontNavi :type Boolean))
  (return false))

(fn `CheckIdleMotion_AfterGimmickMotion`
  (returns (Enable :type Boolean))
  (return false))

(fn `CheckInsideCamera`
  (returns (Inside :type Boolean))
  (return false))

(fn `CheckMermaidDivingHit`
  (returns (Diving :type Boolean))
  (return false))

(fn `ClearHitCount`)

(fn `CompareDistance`
  (params (Pos1 :type "Vector Structure") (Pos2 :type "Vector Structure") (FlatDistance :type "Float (double-precision)") (HeightDistance :type "Float (double-precision)"))
  (returns (Inner :type Boolean))
  (return false))

(fn `ConvertCapsuleTraceLocation`
  (params (Start :type "Vector Structure") (Target :type "Vector Structure") (HitLocation :type "Vector Structure"))
  (returns (Margin :type "Vector Structure"))
  (return (0.0 0.0 0.0)))

(fn `DebugLog`
  (params (InString :type String)))

(fn `GetFionnRunMotion`
  (returns (MotionID :type "E_CHARA_MOTION_ID Enum"))
  (return "NONE"))

(fn `GetGimmickMotionID`
  (returns (MotionID :type "E_CHARA_MOTION_ID Enum"))
  (return "NONE"))

(fn `GetIdleMotionID`
  (returns (MotionID :type "E_CHARA_MOTION_ID Enum"))
  (return "NONE"))

(fn `GetMotionBlendTime`
  (returns (BlendTime :type "Float (double-precision)"))
  (return 0.0))

(fn `GetNaviBasePosition`
  (returns (Location :type "Vector Structure") (Rotation :type "Rotator Structure"))
  (return (0.0 0.0 0.0)))

(fn `GetNaviParam`
  (returns (Param :type "/Game/Blueprints/Map/Gimic/Daath/Struct/NaviDevilParam_st Structure"))
  (return))

(fn `GetNaviWarpPosition`
  (returns (Location :type "Vector Structure") (Rotation :type "Rotator Structure"))
  (return (0.0 0.0 0.0)))

(fn `GetNaviWarpPosition_ForGimmick`
  (returns (Location :type "Vector Structure") (Rotation :type "Rotator Structure"))
  (return (0.0 0.0 0.0)))

(fn `GetRunMotionID`
  (returns (MotionID :type "E_CHARA_MOTION_ID Enum"))
  (return "NONE"))

(fn `IsCheckGotoGimmickMoving`
  (returns (CheckGotoGimmickMoving :type Boolean))
  (return false))

(fn `LineTrace`
  (params (Start :type "Vector Structure") (End :type "Vector Structure") (DrawDebugType :type "EDrawDebugTrace Enum" :default "None"))
  (returns (OutHit :type "HitResult Structure") (Hit :type Boolean))
  (return (struct) false))

(fn `PlayerLook`
  (params (Look :type Boolean)))

(fn `RemoveTargetActor`
  (params (Target :type "Actor Object Reference")))

(fn `ResetMoveParam`)

(fn `SetFromLoad`
  (params (FromLoad :type Boolean)))

(fn `SetURO`
  (params (URO :type Boolean)))

(fn `TickSound`)

(fn `Trace_CanClimb`
  (params (StartPos :type "Vector Structure") (Move :type "Vector Structure") (Upper :type "Float (double-precision)"))
  (returns (CanClimb :type Boolean) (DetourRight :type Boolean) (Normal :type "Vector Structure"))
  (return false false (0.0 0.0 0.0)))

(fn `TraceGround`
  (params (NextPos :type "Vector Structure"))
  (returns (OutPos :type "Vector Structure") (Hit :type Boolean))
  (return (0.0 0.0 0.0) false))

(fn `UpdateHitCount`)

(fn `UpdateNaviScale`)

(fn `UpdatePerticle`)