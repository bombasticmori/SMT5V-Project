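; Gate A actor Blueprint for the konton chaos dungeon in the Daath map, with almost no logic of its own.
; BeginPlay and the construction script only call the parent.
; A DoorOpen timeline exists with empty update and finished handlers.
; Functions for loop sound, closing checks, overlapping devils, data ID and minimap icon rows are stubs, either empty or returning false.
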(event `self.ReceiveBeginPlay`
  (`parent.ReceiveBeginPlay`))

(event `Door Open__FinishedFunc`)

(event `Door Open__UpdateFunc`)

(fn `BPI_SetDataId`
  (params (DataId :type Integer))
  (returns (Dummy :type Boolean))
  (return false))

(fn `IsShouldClose`
  (returns (IsShouldClose :type Boolean))
  (return false))

(fn `MoveOverlappingDevil`)

(fn `ResetLoopSE`)

(fn `SetMinimapIconTableRow`
  (params (Index :type Integer))
  (returns (OutRow :type "MinimapIconTableRow Structure") (NeedToAddMore :type Boolean))
  (return (struct) false))

(fn `SwitchLoopSE`
  (params (NewSE :type "AtomComponent Object Reference (by ref)")))

(fn `UserConstructionScript`
  (`parent.UserConstructionScript`))