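; Gate A part for the Daath wheel dungeon map, set up as a skeleton Blueprint with no gate logic of its own.
; BeginPlay, EndPlay and the construction script only forward to the parent.
; Door, rotation, init, loop sound, minimap icon and room rotator hooks are empty or return default values.
; Overlap and Tick events are disabled.
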(event `self.ReceiveBeginPlay`
  (`parent.ReceiveBeginPlay`))

(event `Door Open__FinishedFunc`)

(event `Door Open__UpdateFunc`)

(event `DG_RoomRotatableInterface.OnRotateFinished`
  (params (isSkipped :type Boolean)))

(event `DG_RoomRotatableInterface.OnRotateStarted`)

(event `Init`)

(event `self.ReceiveEndPlay`
  (params (EndPlayReason :type "EEndPlayReason Enum" :default "Destroyed"))
  (`parent.ReceiveEndPlay` EndPlayReason))

(event `InitIconEndBattle`
  (params (BtlEndType :type "E_BTL_END Enum" :default "E_BTL_END_NONE") (ChainEncountNum :type Integer)))

(fn `BPI_SetDataId`
  (params (DataId :type Integer))
  (returns (Dummy :type Boolean))
  (return false))

(fn `GetRoomRotator`
  (returns (ReturnValue :type "DG_RoomRotator Object Reference"))
  (return null))

(fn `IsInOriginalState`
  (returns (original :type Boolean))
  (return false))

(fn `IsPlayerOverlap`
  (params (OtherActor :type "Actor Object Reference (by ref)"))
  (returns (IsPlayer :type Boolean))
  (return false))

(fn `IsShouldClose`
  (returns (IsShouldClose :type Boolean))
  (return false))

(fn `MoveOverlappingDevil`)

(fn `ResetLoopSE`)

(fn `SetMinimapIconTableRow`
  (params (Index :type Integer))
  (returns (OutRow :type "MinimapIconTableRow Structure") (NeedToAddMore :type Boolean))
  (return (struct) false))

(fn `SetRoomRotator`
  (params (RoomRotator :type "DG_RoomRotator Object Reference"))
  (returns (ReturnValue :type Boolean))
  (return false))

(fn `SwitchLoopSE`
  (params (NewSE :type "AtomComponent Object Reference (by ref)")))

(fn `UserConstructionScript`
  (`parent.UserConstructionScript`))