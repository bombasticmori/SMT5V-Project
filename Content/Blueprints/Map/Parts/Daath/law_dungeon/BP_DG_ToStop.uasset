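; BP_DG_ToStop is a Daath law-dungeon map part Blueprint, apparently a skeleton with little logic of its own.
; BeginPlay, EndPlay, the hit action and the construction script only forward to the parent class.
; The StopRateTimeLine callbacks and the effect, particle and model-link functions are empty.
; The data ID and minimap icon functions just return false, and overlap and Tick are disabled.
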(event `self.ReceiveBeginPlay`
  (`parent.ReceiveBeginPlay`))

(event `StopRateTimeLine__FinishedFunc`)

(event `StopRateTimeLine__UpdateFunc`)

(event `/Game/Blueprints/Map/Hit/Base/BPI_MapEventHit.EventHitAction`
  (`parent.EventHitAction`))

(event `self.ReceiveEndPlay`
  (params (EndPlayReason :type "EEndPlayReason Enum" :default "Destroyed"))
  (`parent.ReceiveEndPlay` EndPlayReason))

(fn `BPI_SetDataId`
  (params (DataId :type Integer))
  (returns (Dummy :type Boolean))
  (return false))

(fn `ChangeEffectParam`)

(fn `LinkModel`)

(fn `SetMinimapIconTableRow`
  (params (Index :type Integer))
  (returns (OutRow :type "MinimapIconTableRow Structure") (NeedToAddMore :type Boolean))
  (return (struct) false))

(fn `StopParticles`)

(fn `UserConstructionScript`
  (`parent.UserConstructionScript`))