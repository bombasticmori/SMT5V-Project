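; Event variant of the Navi Devil map gimmick in Daath, built as a mostly empty Blueprint shell.
; BeginPlay, EndPlay, construction, quest execution, activation check and deactivation only forward to the parent class.
; Battle-end, found-gimmick, navi tick and Pixie IK events are empty.
; Encounter, item lottery, Magatsuhi, Mitama, message, save and info functions are stubs that do nothing or return empty defaults.
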(event `self.ReceiveBeginPlay`
  (`parent.ReceiveBeginPlay`))

(event `/Game/Blueprints/Event/Script/BP_EventMissionBaseCommon.QuestExecute`
  (`parent.QuestExecute`))

(event `/Game/Blueprints/Event/Script/BPI_EventScript.CheckActive`
  (`parent.CheckActive`))

(event `/Game/Blueprints/Event/Script/BPI_EventScript.CallDeactivate`
  (`parent.CallDeactivate`))

(event `Evt_EndBattle`
  (params (BtlEndType :type "E_BTL_END Enum" :default "E_BTL_END_NONE") (ChainEncountNum :type Integer)))

(event `OnDestroyed_`
  (params (DestroyedActor :type "Actor Object Reference")))

(event `self.ReceiveEndPlay`
  (params (EndPlayReason :type "EEndPlayReason Enum" :default "Destroyed"))
  (`parent.ReceiveEndPlay` EndPlayReason))

(event `OnDestroyed_イベント_0`
  (params (DestroyedActor :type "Actor Object Reference")))

(event `EvtDis_EndFoundGimmick_`)

(event `Event_EndStep`)

(event `EvtDis_EndFadeOut_FoundGimmick_`)

(event `StartNaviTick`)

(event `EndNaviTick`)

(event `SetPixieUpdateIK`
  (params (Update :type Boolean)))

(fn `CalcChainEncountInfo`
  (returns (Info :type "ChainEncountInfo Structure"))
  (return))

(fn `CalcMagatsuhi`
  (params (PackData :type "PackEncount Structure") (`EnemyIDｓ` :type "Array of Integer (by ref)"))
  (returns (Magatsuhi :type Boolean))
  (return false))

(fn `CalcMitama`
  (params (PackData :type "PackEncount Structure"))
  (returns (MitamaType :type "E_MITAMA_ENCOUNT Enum") (OutPackData :type "PackEncount Structure"))
  (return "E_MITAMA_ENCOUNT_NONE"))

(fn `DebugLog`
  (params (Str :type String)))

(fn `GetEncountID`
  (returns (EncountID :type Integer) (PackData :type "PackEncount Structure"))
  (return 0))

(fn `GetGazeTargetSocket`
  (returns (Socket :type Name))
  (return "None"))

(fn `GetMsgAsset`
  (params (NaviType :type "E_NAVI_DEVIL Enum" :default "E_NAVI_DEVIL_NONE"))
  (returns (MsgAsset :type "ScriptMessageAsset Object Reference"))
  (return null))

(fn `GodInfo`)

(fn `ItemInfo`
  (params (HaveOver :type Boolean)))

(fn `Lot_ItemOrEncount`
  (returns (ItemGet :type Boolean))
  (return false))

(fn `LotItem`
  (returns (IsItem :type Boolean) (IsMakka :type Boolean) (ItemID :type Integer) (Num :type Integer) (OnFlag :type Integer))
  (return false false 0 0 0))

(fn `MakkaInfo`)

(fn `OnlySaveLog`)

(fn `SaveUniqueGimmick`)

(fn `UserConstructionScript`
  (`parent.UserConstructionScript`))