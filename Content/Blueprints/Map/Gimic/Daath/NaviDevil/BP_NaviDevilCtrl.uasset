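; Blueprint controller for navi devils in the Daath map gimmicks, covering devil changes, clearing, respawn around events and navi gimmick existence.
; It is a thin child layer: the main events and gimmick list and category queries forward to the parent class.
; Its other functions, including ID and follower lookup, debug lot, save-data and random existence calculations, are empty or return defaults, as are the asset-load callbacks.
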(event `self.ReceiveBeginPlay`
  (`parent.ReceiveBeginPlay`))

(event `OnLoaded_F534CB9742FFFC92B833D3BD952FF069`
  (params (Loaded :type "Object Class Reference")))

(event `OnLoaded_083605C14B145B1030BE4097BDE8E3D0`
  (params (Loaded :type "Object Class Reference")))

(event `OnLoaded_72AB99394720690AD3F6F58B43FE2369`
  (params (Loaded :type "Object Class Reference")))

(event `OnLoaded_FF2000D2461D357E27EC05B853646995`
  (params (Loaded :type "Object Class Reference")))

(event `OnLoaded_DE4EC22B4917FCFEC9C46FAB87D29F96`
  (params (Loaded :type "Object Class Reference")))

(event `self.ClearNaviDevil`
  (`parent.ClearNaviDevil`))

(event `self.ChangeNaviDevil_FromEnum`
  (params (NaviDevil :type "E_NAVI_DEVIL Enum" :default "E_NAVI_DEVIL_NONE") (CalcOnGround :type Boolean))
  (`parent.ChangeNaviDevil_FromEnum` NaviDevil CalcOnGround))

(event `self.ChangeNaviDevil_FromPawn`
  (params (Pawn :type "Pawn Object Reference") (NaviDevil :type "E_NAVI_DEVIL Enum" :default "E_NAVI_DEVIL_NONE"))
  (`parent.ChangeNaviDevil_FromPawn` Pawn NaviDevil))

(event `ClearNaviDevil_Once`)

(event `self.CalcNaviGimmickExist_Other`
  (`parent.CalcNaviGimmickExist_Other`))

(event `self.RespawnNaviDevil_AfterEvent`
  (`parent.RespawnNaviDevil_AfterEvent`))

(event `self.DestroyNaviDevil_BeforeEvent`
  (`parent.DestroyNaviDevil_BeforeEvent`))

(fn `CalcNaviGimmickExist_Core`
  (params (NaviDevilGimmickInfo :type "NaviDevilGimmickActors Structure (by ref)") (Index :type Integer)))

(fn `CalcNaviGimmickExist_ForSaveData`)

(fn `CalcNaviGimmickExist_FromCategory`
  (params (CategoryList :type "Array of Integer (by ref)"))
  (returns (NewParam :type Boolean))
  (bind _newparam (`parent.CalcNaviGimmickExist_FromCategory` CategoryList))
  (return _newparam))

(fn `CalcNaviGimmickExist_Random`
  (params (Gimmicks :type "Array of Actor Object Reference (by ref)")))

(fn `CheckDebugLot`
  (returns (CanLot :type Boolean))
  (return false))

(fn `DestroyNPCCollision`)

(fn `GetDevilID_FromEnum`
  (params (naviDevil :type "E_NAVI_DEVIL Enum" :default "E_NAVI_DEVIL_NONE"))
  (returns (DevilID :type Integer))
  (return 0))

(fn `GetFollowerComp_Soft`
  (params (NaviDevil :type "E_NAVI_DEVIL Enum" :default "E_NAVI_DEVIL_NONE"))
  (returns (Comp :type "/Game/Blueprints/Map/Move/BPC_CharaFollower Soft Class Reference"))
  (return null))

(fn `GetGimmickInfoList`
  (returns (List :type "Array of NaviDevilGimmickActors Structure"))
  (bind _list (`parent.GetGimmickInfoList`))
  (return _list))

(fn `InitNaviGimmickInfo`)

(fn `UserConstructionScript`
  (`parent.UserConstructionScript`))