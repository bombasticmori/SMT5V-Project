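; Navi Devil gimmick variant for the Daath map that, judging by its name, marks a spot where the navigator pause is ignored.
; BeginPlay, construction and hit in/out events forward to the parent class.
; The other active events and functions, covering overlap, warp, tutorials, icons, save and navi queries, are empty stubs returning false, zero or nothing.
; The interface therefore reports that no gimmick can exist, leaving the actor largely inert apart from inherited hit handling.
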(event `self.ReceiveBeginPlay`
  (`parent.ReceiveBeginPlay`))

(event `OnLoaded_A2400B66439F28435BD53BB0D9184B44`
  (params (Loaded :type "Object Object Reference")))

(event `OnLoaded_3040A93845BE129A9498D9B94AC20E0D`
  (params (Loaded :type "Object Object Reference")))

(event `/Game/Blueprints/Map/Hit/Base/BPI_MapEventHit.EventHitIN`
  (`parent.EventHitIN`))

(event `/Game/Blueprints/Map/Hit/Base/BPI_MapEventHit.EventHitOUT`
  (`parent.EventHitOUT`))

(event `/Game/Blueprints/Map/Gimic/Daath/NaviDevil/BPI_NaviDevilGimmick.BPI_SetNaviGimmickActive`
  (params (Active :type Boolean)))

(event `/Game/Blueprints/Map/Gimic/Daath/NaviDevil/BPI_NaviDevilGimmick.BPI_SetNaviGimmickDebugView`
  (params (View :type Boolean)))

(event `EvtDis_BeginOverlap_`)

(event `EvtDis_EndOverlap_`)

(event `EvtDis_GoalGimmick_`
  (params (Target :type "Actor Object Reference") (This :type "/Game/Blueprints/Map/Move/BPC_CharaFollower Object Reference")))

(event `EvtDis_LeaveTarget_`
  (params (Target :type "Actor Object Reference") (This :type "/Game/Blueprints/Map/Move/BPC_CharaFollower Object Reference")))

(event `EvtDis_EndEvent_`)

(event `Evt_WarpBasePos`
  (params (Target :type "Actor Object Reference") (This :type "/Game/Blueprints/Map/Move/BPC_CharaFollower Object Reference")))

(event `BeginOverlap_FollowHit`)

(event `EndOverlap_FollowHit`)

(fn `BPI_CanExistNaviGimmick`
  (returns (CanExist :type Boolean))
  (return false))

(fn `BPI_GetNaviGimmickCategory`
  (returns (Category :type Integer))
  (return 0))

(fn `BPI_GetNaviGimmickExistNum`
  (returns (Num :type Integer))
  (return 0))

(fn `BPI_GetNaviGimmickSaveID`
  (returns (SaveID :type Integer))
  (return 0))

(fn `BPI_IsCheckGotoGimmickMoving`
  (returns (CheckGotoGimmickMoving :type Boolean))
  (return false))

(fn `BPI_IsCheckObstacle_WhenGotoGimmick`
  (returns (CheckObstacle_WhenGotoGimmick :type Boolean))
  (return false))

(fn `CalcExistNum`)

(fn `CalcSave`)

(fn `CalcSmallSpace`)

(fn `CallInnerMovedTutorial`)

(fn `CallInnerTutorial`)

(fn `CallOuterTutorial`)

(fn `CheckIgnoreBox`
  (returns (Lock :type Boolean))
  (return false))

(fn `DebugText`)

(fn `GetAroundLocation`
  (params (BaseLocation :type "Vector Structure") (BaseDir :type "Vector Structure") (Distance :type "Float (double-precision)") (LocationNum :type Integer))
  (returns (LocationList :type "Array of Vector Structure"))
  (return))

(fn `GetNaviMovePoint`
  (returns (Actor :type "Actor Object Reference"))
  (return null))

(fn `GetNaviParam`
  (returns (Param :type "/Game/Blueprints/Map/Gimic/Daath/Struct/NaviDevilParam_st Structure"))
  (return))

(fn `HideIcon`)

(fn `LineTrace`
  (params (Start :type "Vector Structure") (End :type "Vector Structure") (DrawDebugType :type "EDrawDebugTrace Enum" :default "None"))
  (returns (OutHit :type "HitResult Structure") (Hit :type Boolean))
  (return (struct) false))

(fn `ShowIcon`)

(fn `UserConstructionScript`
  (`parent.UserConstructionScript`))