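; Map gimmick Blueprint for an Aogami debris object in the Daath area, with show/hide, hit action and an after-piece-pickup event.
; Declares timelines for effect and camera-inside handling, async load callbacks, and getters for soft mesh, animation, gaze target and minimap icon.
; Nearly every body is empty or returns a default; only BeginPlay, Tick, EndPlay, EventHitAction and construction forward to the parent.
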(event `self.ReceiveBeginPlay`
  (`parent.ReceiveBeginPlay`))

(event `self.ReceiveTick`
  (params (DeltaSeconds :type "Float (single-precision)"))
  (`parent.ReceiveTick` DeltaSeconds))

(event `Timeline_Effect__FinishedFunc`)

(event `Timeline_Effect__UpdateFunc`)

(event `Timeline_CameraInside__FinishedFunc`)

(event `Timeline_CameraInside__UpdateFunc`)

(event `OnLoaded_645CA1794707F3B15888D8A495502D64`
  (params (Loaded :type "Object Object Reference")))

(event `OnLoaded_FD85D9D9479AABDFF8A378A10D8634C9`
  (params (Loaded :type "Object Object Reference")))

(event `OnLoaded_30E44BF94D36DD156FBDACB35A7C1D51`
  (params (Loaded :type "Object Object Reference")))

(event `OnLoaded_2937499042F992BF312A6EBF58C3E12B`
  (params (Loaded :type "Object Object Reference")))

(event `OnLoaded_675A044649F76ED9C782B286CB195269`
  (params (Loaded :type "Object Object Reference")))

(event `EvtDis_Show_`)

(event `EvtDis_Hide_`)

(event `UpdateActive`)

(event `/Game/Blueprints/Map/Gimic/Common/Interface/BPI_MapGimmick.BPI_ShowGimmick`
  (params (HideReason :type "/Game/Blueprints/Map/Gimic/Common/Enum/E_MapGimmickHideReason Enum" :default "NewEnumerator0")))

(event `/Game/Blueprints/Map/Gimic/Common/Interface/BPI_MapGimmick.BPI_HideGimmick`
  (params (HideReason :type "/Game/Blueprints/Map/Gimic/Common/Enum/E_MapGimmickHideReason Enum" :default "NewEnumerator0")))

(event `self.ReceiveEndPlay`
  (params (EndPlayReason :type "EEndPlayReason Enum" :default "Destroyed"))
  (`parent.ReceiveEndPlay` EndPlayReason))

(event `/Game/Blueprints/Map/Hit/Base/BPI_MapEventHit.EventHitAction`
  (`parent.EventHitAction`))

(event `AfterGetPiece`)

(event `SetMeshVisibility`
  (params (Visible :type Boolean)))

(event `SetEffectVisible`
  (params (Visible :type Boolean) (Anim :type Boolean)))

(event `/Game/Blueprints/Map/Gimic/Daath/Interface/BPI_AogamiDebris.BPI_AogamiDebrisCameraInside`
  (params (CameraPos :type "Vector Structure")))

(fn `DebugTextView`
  (params (View :type Boolean)))

(fn `GetAnimation_Soft`
  (returns (Anim :type "AnimSequence Soft Object Reference"))
  (return null))

(fn `GetDefaultScale`
  (returns (Scale :type "Float (double-precision)"))
  (return 0.0))

(fn `GetGazeTargetLocation`
  (returns (ReturnValue :type "Vector Structure"))
  (return (0.0 0.0 0.0)))

(fn `GetGazeTargetType`
  (returns (ReturnValue :type "EGazeTargetType Enum"))
  (return "Dummy"))

(fn `GetSkeletalMesh_Soft`
  (returns (Mesh :type "SkeletalMesh Soft Object Reference"))
  (return null))

(fn `SetMinimapIconTableRow`
  (params (Index :type Integer))
  (returns (OutRow :type "MinimapIconTableRow Structure") (NeedToAddMore :type Boolean))
  (return (struct) false))

(fn `SettingScale`)

(fn `UserConstructionScript`
  (`parent.UserConstructionScript`))