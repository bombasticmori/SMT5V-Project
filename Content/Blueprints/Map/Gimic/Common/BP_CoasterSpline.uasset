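; BP_CoasterSpline is a map gimmick for a coaster spline that, judging by its names, carries the player between start and end gimmicks.
; Spline move, show and activation, open state, chain opening and gimmick getters only forward to the parent class.
; Camera, spline math, save ID, skip and timeline handlers are empty or return defaults, so this graph holds no logic of its own.
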(event `self.ReceiveBeginPlay`
  (`parent.ReceiveBeginPlay`))

(event `Timeline_ActiveSpline__FinishedFunc`)

(event `Timeline_ActiveSpline__UpdateFunc`)

(event `Timeline_ShowSpline__FinishedFunc`)

(event `Timeline_ShowSpline__UpdateFunc`)

(event `タイムライン_0__FinishedFunc`)

(event `タイムライン_0__UpdateFunc`)

(event `タイムライン_1__FinishedFunc`)

(event `タイムライン_1__UpdateFunc`)

(event `TimeLine_RideCamera__FinishedFunc`)

(event `TimeLine_RideCamera__UpdateFunc`)

(event `OnArriveSplineEnd`
  (params (ThisComponent :type "/Game/Blueprints/Map/Move/BPC_CharaSplineMover Object Reference")))

(event `self.MoveSpline`
  (params (FromStartGimmick :type Boolean))
  (`parent.MoveSpline` FromStartGimmick))

(event `self.ActiveSplineAnim`
  (params (Active :type Boolean) (Anim :type Boolean))
  (`parent.ActiveSplineAnim` Active Anim))

(event `EvtDis_Stop_`
  (params (ThisComponent :type "/Game/Blueprints/Map/Move/BPC_CharaSplineMover Object Reference")))

(event `self.ShowSpline`
  (params (Show :type Boolean) (Anim :type Boolean))
  (`parent.ShowSpline` Show Anim))

(event `EvtDis_EndActiveSpline_IN`)

(event `_EndActiveSpline_OUT`)

(event `PlayerStartPositionSetting`)

(event `Stop_PlayerStartPositionSetting`)

(event `OnEvtDis_MapStart`)

(event `/Game/Blueprints/Map/Gimic/Common/Interface/BPI_CoasterSpline.BPI_UpdateCoasterFlag`)

(event `ProcSkip`)

(event `MovePlayerEventTrigger`)

(event `OnEndFadeOut_ForSkip`)

(fn `BPI_GetGlobalSaveID`
  (returns (SaveID :type Integer))
  (return 0))

(fn `BPI_GetIsOpen`
  (returns (StartGimmickOpen :type Boolean) (EndGimmickOpen :type Boolean))
  (return false false))

(fn `CalcAddSplinePoint`)

(fn `CalcCoasterCameraPos`
  (returns (Location :type "Vector Structure") (Rotate :type "Rotator Structure") (FOV :type "Float (double-precision)"))
  (return (0.0 0.0 0.0) (struct) 0.0))

(fn `CalcOpen`
  (`parent.CalcOpen`))

(fn `CalcPlayerCameraRot`
  (params (PrevCameraRot :type "Rotator Structure") (PrevPlayerRot :type "Rotator Structure") (NextPlayerRot :type "Rotator Structure"))
  (returns (NextPlayerCameraRot :type "Rotator Structure"))
  (return))

(fn `CalcSaveID`)

(fn `CalcSplineForMove`)

(fn `ChainOpen`
  (`parent.ChainOpen`))

(fn `DebugOpen`
  (params (Open :type Boolean)))

(fn `GetEndGimmick`
  (returns (Actor :type "Actor Object Reference"))
  (return (`parent.GetEndGimmick`)))

(fn `GetGlobalSaveID`
  (returns (SaveID :type Integer))
  (return 0))

(fn `GetNaviComponent`
  (returns (Valid :type Boolean) (Comp :type "ActorComponent Object Reference"))
  (return false null))

(fn `GetSpline`
  (returns (Spline :type "SplineComponent Object Reference"))
  (return null))

(fn `GetSplineForward`
  (params (Distance :type "Float (double-precision)") (Reverse :type Boolean))
  (returns (Forward :type "Vector Structure"))
  (return (0.0 0.0 0.0)))

(fn `GetSplineMeshs`
  (returns (SplineMeshs :type "Array of SplineMeshComponent Object Reference"))
  (return))

(fn `GetSplineUpVec`
  (params (Distance :type "Float (double-precision)"))
  (returns (UpVec :type "Vector Structure"))
  (return (0.0 0.0 0.0)))

(fn `GetStartGimmick`
  (returns (Actor :type "Actor Object Reference"))
  (return (`parent.GetStartGimmick`)))

(fn `MakeDMI`)

(fn `SetOpen`
  (params (Open :type Boolean) (StartGimmick :type Boolean) (EndGimmick :type Boolean) (UpdateIcon :type Boolean) (UpdateNaviDeactive :type Boolean) (UpdateChain :type Boolean))
  (`parent.SetOpen` Open StartGimmick EndGimmick UpdateIcon UpdateNaviDeactive UpdateChain))

(fn `TraseGround`
  (params (Pos :type "Vector Structure"))
  (returns (OutPos :type "Vector Structure"))
  (return (0.0 0.0 0.0)))

(fn `UserConstructionScript`
  (`parent.UserConstructionScript`))