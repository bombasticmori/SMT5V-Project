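; Chest piece map gimmick, apparently a collectible that grants items, Makka, Magatsuhi, God Points or HP/MP recovery.
; Its interface declares overlap, collection effects, info display, particle and decal fades, limit checks, reborn, Silent Moon and room-rotation hooks.
; Nearly all bodies are empty or return defaults, so the file shows the structure without the logic.
; Only BeginPlay, the hit action and the construction script do anything, forwarding to the parent.
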(event `self.ReceiveBeginPlay`
  (`parent.ReceiveBeginPlay`))

(event `タイムライン_1__FinishedFunc`)

(event `タイムライン_1__UpdateFunc`)

(event `Timeline_DecalFadeIn__FinishedFunc`)

(event `Timeline_DecalFadeIn__UpdateFunc`)

(event `OnLoaded_000CEC1647E4F09283905AA617AF2AAC`
  (params (Loaded :type "Object Class Reference")))

(event `GetItemPiece`
  (params (Get :type Boolean) (Info :type Boolean)))

(event `GetMakkaPiece`
  (params (Get :type Boolean) (Info :type Boolean)))

(event `OpenNotHaveItemInfo`)

(event `/Game/Blueprints/Map/Hit/Base/BPI_MapEventHit.EventHitAction`
  (`parent.EventHitAction`))

(event `OverlapPiece`)

(event `StartCollectEffect`)

(event `EndCollectEffect`)

(event `EvtDis_Show_`)

(event `EvtDis_Hide_`)

(event `EvtDis_EndInfo_Event`)

(event `EvtDis_EndNotInfo_Event`)

(event `CallUnPause_`)

(event `WaitSilentMoon`)

(event `SilentMoon`)

(event `DecalFadeOut`)

(event `DecalFadeIn`)

(event `GetMagatsuhiPiece`)

(event `/Game/Blueprints/Map/Gimic/Common/Interface/BPI_MapGimmick.BPI_ShowGimmick`
  (params (HideReason :type "/Game/Blueprints/Map/Gimic/Common/Enum/E_MapGimmickHideReason Enum" :default "NewEnumerator0")))

(event `/Game/Blueprints/Map/Gimic/Common/Interface/BPI_MapGimmick.BPI_HideGimmick`
  (params (HideReason :type "/Game/Blueprints/Map/Gimic/Common/Enum/E_MapGimmickHideReason Enum" :default "NewEnumerator0")))

(event `GetMpCurePiece`)

(event `GetHpCurePiece`)

(event `GetGodPointPiece`
  (params (Get :type Boolean) (Info :type Boolean)))

(event `DG_RoomRotatableInterface.OnRotateStarted`)

(event `DG_RoomRotatableInterface.OnRotateFinished`
  (params (isSkipped :type Boolean)))

(event `/Game/Blueprints/Map/Gimic/Common/Interface/BPI_MapGimmickAffectedByTimeStop.BPI_SetStopTime`
  (params (StopTime :type Boolean)))

(event `ParticleStopCheck`)

(fn `CheckHaveLimitOver`
  (params (PieceData :type "PieceData Structure"))
  (returns (LimitOver :type Boolean) (GetNum :type Integer))
  (return false 0))

(fn `CureHp`)

(fn `CureMp`)

(fn `EndPiece`)

(fn `GetNkmHPMPMax`
  (params (NkmIndex :type Integer))
  (returns (HPMax :type Integer) (MPMax :type Integer))
  (return 0 0))

(fn `GetPlayerHPMPMax`
  (params (playerType :type "E_PLAYER_TYPE Enum" :default "E_PLAYER_BOY"))
  (returns (HPMax :type Integer) (MPMax :type Integer))
  (return 0 0))

(fn `GetRoomRotator`
  (returns (ReturnValue :type "DG_RoomRotator Object Reference"))
  (return null))

(fn `GetTargetLocation`
  (returns (Location :type "Vector Structure"))
  (return (0.0 0.0 0.0)))

(fn `InitDecal`)

(fn `InitEffect`)

(fn `RebornPiece`)

(fn `SetPieceData`
  (params (PieceData :type "PieceData Structure")))

(fn `SetRoomRotator`
  (params (RoomRotator :type "DG_RoomRotator Object Reference"))
  (returns (ReturnValue :type Boolean))
  (return false))

(fn `ShowDecal`
  (params (Show :type Boolean) (Execution :type Boolean)))

(fn `ShowLineParticle`
  (params (Show :type Boolean)))

(fn `ShowMainParticle`
  (params (Show :type Boolean)))

(fn `SpawnCureEffect`
  (params (PieceType :type "E_PIECE_TYPE Enum" :default "E_PIECE_TYPE_ITEM")))

(fn `Stop_MovePiece`)

(fn `TriggerSilentMoon`)

(fn `UserConstructionScript`
  (`parent.UserConstructionScript`))