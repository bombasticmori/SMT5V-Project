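; BP_Ryuketsu is a map gimmick Blueprint in the common gimmick set, with no logic of its own in its graphs.
; BeginPlay, the construction script and the show/hide gimmick interface events only forward to the parent class.
; The map exit and return object hide/show events are empty and make no parent call.
; Overlap and Tick are disabled placeholder nodes.
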(event `self.ReceiveBeginPlay`
  (`parent.ReceiveBeginPlay`))

(event `/Game/Blueprints/Map/Gimic/Common/Interface/BPI_MapGimmick.BPI_ShowGimmick`
  (params (HideReason :type "/Game/Blueprints/Map/Gimic/Common/Enum/E_MapGimmickHideReason Enum" :default "NewEnumerator0"))
  (`parent.BPI_ShowGimmick` HideReason))

(event `/Game/Blueprints/Map/Gimic/Common/Interface/BPI_MapGimmick.BPI_HideGimmick`
  (params (HideReason :type "/Game/Blueprints/Map/Gimic/Common/Enum/E_MapGimmickHideReason Enum" :default "NewEnumerator0"))
  (`parent.BPI_HideGimmick` HideReason))

(event `Evt_HideObjects_WhenExitMap`)

(event `Evt_ShowObjects_WhenReturnMap`)

(fn `UserConstructionScript`
  (`parent.UserConstructionScript`))