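; BP_MapRelic is a relic gimmick actor for the map, with hooks for appearance, display, save, gaze targeting and minimap icons.
; Lifecycle and hit events only forward to the parent class.
; Show, hide, result and active-update events are empty, and the functions return empty or default values such as a Dummy gaze type, so this graph adds no behavior of its own.
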(event `self.ReceiveBeginPlay`
  (`parent.ReceiveBeginPlay`))

(event `self.ReceiveTick`
  (params (DeltaSeconds :type "Float (single-precision)"))
  (`parent.ReceiveTick` DeltaSeconds))

(event `EvtDis_Show_`)

(event `EvtDis_Hide_`)

(event `EvtDis_Result_`
  (params (Success :type Boolean)))

(event `/Game/Blueprints/Map/Hit/Base/BPI_MapEventHit.EventHitIN`
  (`parent.EventHitIN`))

(event `/Game/Blueprints/Map/Gimic/Common/Interface/BPI_MapGimmick.BPI_ShowGimmick`
  (params (HideReason :type "/Game/Blueprints/Map/Gimic/Common/Enum/E_MapGimmickHideReason Enum" :default "NewEnumerator0")))

(event `/Game/Blueprints/Map/Gimic/Common/Interface/BPI_MapGimmick.BPI_HideGimmick`
  (params (HideReason :type "/Game/Blueprints/Map/Gimic/Common/Enum/E_MapGimmickHideReason Enum" :default "NewEnumerator0")))

(event `UpdateActive`)

(event `/Game/Blueprints/Map/Hit/Base/BPI_MapEventHit.EventHitAction`
  (`parent.EventHitAction`))

(event `self.ReceiveEndPlay`
  (params (EndPlayReason :type "EEndPlayReason Enum" :default "Destroyed"))
  (`parent.ReceiveEndPlay` EndPlayReason))

(fn `CalcSave`)

(fn `DebugTextView`
  (params (View :type Boolean)))

(fn `GetGazeTargetLocation`
  (returns (ReturnValue :type "Vector Structure"))
  (return (0.0 0.0 0.0)))

(fn `GetGazeTargetType`
  (returns (ReturnValue :type "EGazeTargetType Enum"))
  (return "Dummy"))

(fn `GetParticle`
  (returns (ParticleSystem :type "ParticleSystemComponent Object Reference"))
  (return null))

(fn `GetRealSaveID`
  (returns (SaveID :type Integer))
  (return 0))

(fn `GetRelicAppearance`
  (returns (RelicApearance :type "/Game/Blueprints/Map/Gimic/Common/Sub/BP_RelicAppearanceBase Object Reference"))
  (return null))

(fn `GetStaticMesh`
  (returns (StaticMesh :type "StaticMeshComponent Object Reference"))
  (return null))

(fn `SetMinimapIconTableRow`
  (params (Index :type Integer))
  (returns (OutRow :type "MinimapIconTableRow Structure") (NeedToAddMore :type Boolean))
  (return (struct) false))

(fn `UserConstructionScript`
  (`parent.UserConstructionScript`))