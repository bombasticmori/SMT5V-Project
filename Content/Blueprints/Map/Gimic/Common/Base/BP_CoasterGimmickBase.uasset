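; BP_CoasterGimmickBase is the base Blueprint for coaster gimmicks on the map, serving as a common interface with no logic of its own.
; It declares empty events for initialization, discovery and mesh open/animation parameters.
; Stub functions cover ride relay, icon opening and ID calculation, view and active checks (both returning false), other-gimmick lookup and dynamic material creation, presumably for child Blueprints to override.
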(event `SetMeshParam`
  (params (Open :type Boolean) (Animation :type Boolean)))

(event `FoundGimmick`)

(event `Init`)

(fn `CalcIconDataID`)

(fn `CheckActive`
  (returns (Active :type Boolean))
  (return false))

(fn `CheckView`
  (returns (View :type Boolean))
  (return false))

(fn `GetOtherGimmick`
  (returns (Gimmick :type "/Game/Blueprints/Map/Gimic/Common/Base/BP_CoasterGimmickBase Object Reference"))
  (return null))

(fn `MakeDMI`)

(fn `OpenIcon`)

(fn `ProcRelay`
  (params (RideOn :type Boolean)))

(fn `UserConstructionScript`
  (`parent.UserConstructionScript`))