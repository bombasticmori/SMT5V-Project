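; Base Blueprint for Ryuketsu map gimmicks, serving as a common skeleton with almost no logic of its own.
; BeginPlay, the hit events and the construction script only forward to the parent class.
; Hooks for show/hide, Ryuketsu call, Aogami talk, data calculation, distance view and map-init end are empty stubs, while the index and minimap-icon functions return default values.
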(event `self.ReceiveBeginPlay`
  (`parent.ReceiveBeginPlay`))

(event `OnLoaded_209DEC174BEC1F7CBA8DC19645F38F65`
  (params (Loaded :type "Object Object Reference")))

(event `/Game/Blueprints/Map/Gimic/Common/Interface/BPI_MapGimmick.BPI_ShowGimmick`
  (params (HideReason :type "/Game/Blueprints/Map/Gimic/Common/Enum/E_MapGimmickHideReason Enum" :default "NewEnumerator0")))

(event `/Game/Blueprints/Map/Gimic/Common/Interface/BPI_MapGimmick.BPI_HideGimmick`
  (params (HideReason :type "/Game/Blueprints/Map/Gimic/Common/Enum/E_MapGimmickHideReason Enum" :default "NewEnumerator0")))

(event `/Game/Blueprints/Map/Hit/Base/BPI_MapEventHit.EventHitAction`
  (`parent.EventHitAction`))

(event `/Game/Blueprints/Map/Hit/Base/BPI_MapEventHit.EventHitIN`
  (`parent.EventHitIN`))

(event `/Game/Blueprints/Map/Gimic/Common/Interface/BPI_Ryuketsu.BPI_CallRyuketsu`)

(event `Evt_AogamiTalk`)

(event `CalcRyuketsuData`)

(event `EndMapInit_イベント_0`)

(fn `BPI_GetRyuketsuIndex`
  (returns (RyuketsuIndex :type Integer))
  (return 0))

(fn `ProcDistanceView`)

(fn `SetMinimapIconTableRow`
  (params (Index :type Integer))
  (returns (OutRow :type "MinimapIconTableRow Structure") (NeedToAddMore :type Boolean))
  (return (struct) false))

(fn `UserConstructionScript`
  (`parent.UserConstructionScript`))