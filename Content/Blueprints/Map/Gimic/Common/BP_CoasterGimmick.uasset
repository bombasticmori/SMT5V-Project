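; BP_CoasterGimmick is a map gimmick Blueprint, named for a coaster, that as shown is mostly a skeleton over its parent class.
; BeginPlay, Init, hit, found, mesh-parameter, relay, icon and active-check overrides only forward to the parent.
; Spline-move, show/hide, timeline and load events are empty, while existence, start, navigation and minimap queries return false or zero defaults.
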(event `self.ReceiveBeginPlay`
  (`parent.ReceiveBeginPlay`))

(event `タイムライン_0__FinishedFunc`)

(event `タイムライン_0__UpdateFunc`)

(event `OnLoaded_F3C8ACCB48DFF75596E91DAE0009CFD9`
  (params (Loaded :type "Object Object Reference")))

(event `/Game/Blueprints/Map/Hit/Base/BPI_MapEventHit.EventHitAction`
  (`parent.EventHitAction`))

(event `OnEvtDis_EndMoveSpline`)

(event `self.Init`
  (`parent.Init`))

(event `/Game/Blueprints/Map/Gimic/Common/Interface/BPI_MapGimmick.BPI_ShowGimmick`
  (params (HideReason :type "/Game/Blueprints/Map/Gimic/Common/Enum/E_MapGimmickHideReason Enum" :default "NewEnumerator0")))

(event `/Game/Blueprints/Map/Gimic/Common/Interface/BPI_MapGimmick.BPI_HideGimmick`
  (params (HideReason :type "/Game/Blueprints/Map/Gimic/Common/Enum/E_MapGimmickHideReason Enum" :default "NewEnumerator0")))

(event `EvtDis_Hide_`)

(event `EvtDis_Show_WalkedIn_`
  (params (WalkedIn :type Boolean)))

(event `_EvtDis_EndShowSpline_`)

(event `self.FoundGimmick`
  (`parent.FoundGimmick`))

(event `self.SetMeshParam`
  (params (Open :type Boolean) (Animation :type Boolean))
  (`parent.SetMeshParam` Open Animation))

(event `OnEvtDis_StartMoveSpline`)

(event `OnEvtDis_CallVisible`
  (params (Visible :type Boolean)))

(event `/Game/Blueprints/Map/Gimic/Common/Interface/BPI_CoasterGimmick.BPI_CallAfterNaviFound`)

(fn `BPI_CheckActive_WhenFlag`
  (returns (Active :type Boolean))
  (return false))

(fn `BPI_CheckExist`
  (returns (Exist :type Boolean))
  (return false))

(fn `BPI_GetMinimapDataID`
  (returns (DataID :type Integer))
  (return 0))

(fn `BPI_SetDataId`
  (params (DataId :type Integer))
  (returns (Dummy :type Boolean))
  (return false))

(fn `CalcIconDataID`
  (`parent.CalcIconDataID`))

(fn `CalcNaviPosition`
  (returns (NaviPosition :type "Vector Structure"))
  (return (0.0 0.0 0.0)))

(fn `CheckActive`
  (returns (Active :type Boolean))
  (return (`parent.CheckActive`)))

(fn `CheckExist`
  (returns (Exist :type Boolean))
  (return false))

(fn `CheckNaviPositionEnable`
  (params (Index :type Integer))
  (returns (Enable :type Boolean))
  (return false))

(fn `CheckStartGimmick`
  (returns (StartGimmick :type Boolean))
  (return false))

(fn `GetMinimapDataID`
  (returns (DataID :type Integer))
  (return 0))

(fn `OpenIcon`
  (`parent.OpenIcon`))

(fn `ProcRelay`
  (params (RideOn :type Boolean))
  (`parent.ProcRelay` RideOn))

(fn `SetMinimapIconTableRow`
  (params (Index :type Integer))
  (returns (OutRow :type "MinimapIconTableRow Structure") (NeedToAddMore :type Boolean))
  (return (struct) false))

(fn `UserConstructionScript`
  (`parent.UserConstructionScript`))