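; BP_FindItem is a map gimmick Blueprint, apparently for a findable item, that leaves nearly all behavior to its parent class.
; BeginPlay, EventHitAction, construction and FlagCh simply forward to the parent.
; CheckExist always returns false, while the hide, show, end-action and custom events are empty stubs with no parent call.
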(event `self.ReceiveBeginPlay`
  (`parent.ReceiveBeginPlay`))

(event `CustomEvent`)

(event `/Game/Blueprints/Map/Hit/Base/BPI_MapEventHit.EventHitAction`
  (`parent.EventHitAction`))

(event `/Game/Blueprints/Map/Gimic/Common/Interface/BPI_MapGimmick.BPI_HideGimmick`
  (params (HideReason :type "/Game/Blueprints/Map/Gimic/Common/Enum/E_MapGimmickHideReason Enum" :default "NewEnumerator0")))

(event `/Game/Blueprints/Map/Gimic/Common/Interface/BPI_MapGimmick.BPI_ShowGimmick`
  (params (HideReason :type "/Game/Blueprints/Map/Gimic/Common/Enum/E_MapGimmickHideReason Enum" :default "NewEnumerator0")))

(event `EvtDis_Hide_`)

(event `EvtDis_Show_`)

(event `OnEndAction`)

(fn `CheckExist`
  (returns (Exist :type Boolean))
  (return false))

(fn `FlagCh`
  (returns (OK :type Boolean))
  (return (`parent.FlagCh`)))

(fn `UserConstructionScript`
  (`parent.UserConstructionScript`))