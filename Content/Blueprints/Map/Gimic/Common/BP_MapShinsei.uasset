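; BP_MapShinsei is a common map gimmick Blueprint whose function and event bodies are almost entirely empty.
; It declares hooks for show/hide, hit action, particles, a material timeline, movement end, saving, gaze targeting and minimap icons.
; BeginPlay, EndPlay, EventHitAction and construction only call the parent.
; Query functions return fixed defaults: not existing, zero gaze location, Dummy gaze type and no additional minimap icons.
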(event `self.ReceiveBeginPlay`
  (`parent.ReceiveBeginPlay`))

(event `Timeline_Material__FinishedFunc`)

(event `Timeline_Material__UpdateFunc`)

(event `OnSystemFinished_`
  (params (PSystem :type "ParticleSystemComponent Object Reference")))

(event `EvtDis_Hide_`)

(event `OnDestroyed_イベント_0`
  (params (DestroyedActor :type "Actor Object Reference")))

(event `/Game/Blueprints/Map/Gimic/Common/Interface/BPI_MapGimmick.BPI_ShowGimmick`
  (params (HideReason :type "/Game/Blueprints/Map/Gimic/Common/Enum/E_MapGimmickHideReason Enum" :default "NewEnumerator0")))

(event `/Game/Blueprints/Map/Gimic/Common/Interface/BPI_MapGimmick.BPI_HideGimmick`
  (params (HideReason :type "/Game/Blueprints/Map/Gimic/Common/Enum/E_MapGimmickHideReason Enum" :default "NewEnumerator0")))

(event `CallTaskEnd_`)

(event `AnimOut`)

(event `self.ReceiveEndPlay`
  (params (EndPlayReason :type "EEndPlayReason Enum" :default "Destroyed"))
  (`parent.ReceiveEndPlay` EndPlayReason))

(event `/Game/Blueprints/Map/Hit/Base/BPI_MapEventHit.EventHitAction`
  (`parent.EventHitAction`))

(event `ProcMiitsuGetEvent`)

(event `MoveEnd`)

(event `EvtDis_Show_WalkedIn_`
  (params (WalkedIn :type Boolean)))

(fn `CalcSave`)

(fn `CheckExist`
  (returns (Exist :type Boolean))
  (return false))

(fn `GetGazeTargetLocation`
  (returns (ReturnValue :type "Vector Structure"))
  (return (0.0 0.0 0.0)))

(fn `GetGazeTargetType`
  (returns (ReturnValue :type "EGazeTargetType Enum"))
  (return "Dummy"))

(fn `SetMinimapIconTableRow`
  (params (Index :type Integer))
  (returns (OutRow :type "MinimapIconTableRow Structure") (NeedToAddMore :type Boolean))
  (return (struct) false))

(fn `ShowParticle`
  (params (Show :type Boolean) (WalkedIn :type Boolean)))

(fn `UserConstructionScript`
  (`parent.UserConstructionScript`))