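; Top-down map camera Blueprint, with hooks for start and finish, movement input, tracing, button help, field visibility, and LOD and console variable overrides.
; Tick, OnStartTop and OnFinishTop only forward to the parent class.
; Every function here is an empty stub or returns zero or false, so this graph adds no camera behavior of its own.
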(event `self.ReceiveTick`
  (params (DeltaSeconds :type "Float (single-precision)"))
  (`parent.ReceiveTick` DeltaSeconds))

(event `self.OnStartTop`
  (`parent.OnStartTop`))

(event `self.OnFinishTop`
  (`parent.OnFinishTop`))

(fn `ApplyConsoleVariables`)

(fn `ApplyConsoleVariables_debug`)

(fn `ApplyTransitionDebugParam`)

(fn `Deactivate`)

(fn `FieldVisibilityOnFinish`)

(fn `FieldVisibilityOnStart`)

(fn `GetBlendExp`
  (returns (BlendExp :type "Float (double-precision)"))
  (return 0.0))

(fn `GetBlendTime`
  (returns (Seconds :type "Float (double-precision)"))
  (return 0.0))

(fn `GetConsoleVariables`)

(fn `GetDefaultFOVY`
  (returns (Height :type "Float (double-precision)"))
  (return 0.0))

(fn `GetDefaultHeight`
  (returns (Height :type "Float (double-precision)"))
  (return 0.0))

(fn `GetHeightDistanceMin`
  (returns (Height :type "Float (double-precision)"))
  (return 0.0))

(fn `GetHorizontalDistanceLimit`
  (returns (Limit :type "Float (double-precision)"))
  (return 0.0))

(fn `GetHorizontalDistanceModifier`
  (returns (Modifier :type "Float (double-precision)"))
  (return 0.0))

(fn `GetHorizontalSpeed`
  (returns (Speed :type "Float (double-precision)"))
  (return 0.0))

(fn `GetStartHeight`
  (returns (Height :type "Float (double-precision)"))
  (return 0.0))

(fn `Init Camera Param`)

(fn `IsNorthUp`
  (returns (IsNorthUp :type Boolean))
  (return false))

(fn `OpenButtonHelp`)

(fn `ProcessInput`
  (params (DeltaSeconds :type "Float (double-precision)")))

(fn `ProcessInput_ActorHorizontal`
  (params (DeltaSeconds :type "Float (double-precision)") (ForceUpdate :type Boolean)))

(fn `ProcessInput_Height`
  (params (DeltaSeconds :type "Float (double-precision)")))

(fn `ProcessInput_Horizontal`
  (params (DeltaSeconds :type "Float (double-precision)")))

(fn `ProcessInput_Target`
  (params (DeltaSeconds :type "Float (double-precision)")))

(fn `ProcessInputInconHelp`)

(fn `ResetConsoleVariables`)

(fn `ResetFoliageLOD`)

(fn `ResetLOD`)

(fn `SetFoliageLOD`)

(fn `SetLOD`)

(fn `Start`)

(fn `TryTrace`
  (params (PrevLocation :type "Vector Structure") (NextLocation :type "Vector Structure"))
  (returns (OutNext :type "Vector Structure") (CanMove :type Boolean))
  (return (0.0 0.0 0.0) false))

(fn `UpdateButtonHelp`
  (params (IconShowing :type Boolean)))

(fn `UserConstructionScript`)