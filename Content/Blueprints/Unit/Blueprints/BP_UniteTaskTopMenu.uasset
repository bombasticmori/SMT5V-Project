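; Top-menu task Blueprint for the Unite task system, shaped to build and navigate a selectable menu list.
; InitTask, RunTask and EndTask only forward to the parent class.
; Menu functions for creation, next/previous lookup, labels, open checks and new-item display are stubs returning fixed defaults.
; BeginPlay and Tick are disabled, so the asset holds no menu logic of its own.
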(fn `CheckNewDisp`
  (params (InSelectMenu :type "/Game/Blueprints/Unit/Enums/E_UniteMenu Enum" :default "NewEnumerator5"))
  (returns (bOutDisp :type Boolean))
  (return false))

(fn `CreateMenu`
  (params (Menu :type "/Game/Blueprints/Unit/Enums/E_UniteMenu Enum" :default "NewEnumerator5") (bNext :type Boolean) (bPrev :type Boolean))
  (returns (bOk :type Boolean))
  (return false))

(fn `CreateMenuList`
  (params (Menu :type "/Game/Blueprints/Unit/Enums/E_UniteMenu Enum" :default "NewEnumerator5") (bNext :type Boolean) (bPrev :type Boolean))
  (returns (OutSelectMenu :type "/Game/Blueprints/Unit/Enums/E_UniteMenu Enum") (OutMenuList :type "Array of /Game/Blueprints/Unit/Enums/E_UniteMenu Enum"))
  (return "NewEnumerator5"))

(fn `CreateMenuUI`
  (params (SelectMenu :type "/Game/Blueprints/Unit/Enums/E_UniteMenu Enum" :default "NewEnumerator5") (MenuList :type "Array of /Game/Blueprints/Unit/Enums/E_UniteMenu Enum (by ref)"))
  (returns (bOk :type Boolean))
  (return false))

(fn `EndTask`
  (returns (OutParam :type Integer))
  (bind _outparam (`parent.EndTask`))
  (return _outparam))

(fn `FindMenuList`
  (params (InSelectMenu :type "/Game/Blueprints/Unit/Enums/E_UniteMenu Enum" :default "NewEnumerator5"))
  (returns (OutSelectMenu :type "/Game/Blueprints/Unit/Enums/E_UniteMenu Enum") (OutMenuList :type "Array of /Game/Blueprints/Unit/Enums/E_UniteMenu Enum"))
  (return "NewEnumerator5"))

(fn `FindMenuListNext`
  (params (InSelectMenu :type "/Game/Blueprints/Unit/Enums/E_UniteMenu Enum" :default "NewEnumerator5"))
  (returns (OutSelectMenu :type "/Game/Blueprints/Unit/Enums/E_UniteMenu Enum") (OutMenuList :type "Array of /Game/Blueprints/Unit/Enums/E_UniteMenu Enum"))
  (return "NewEnumerator5"))

(fn `FindMenuListPrev`
  (params (InSelectMenu :type "/Game/Blueprints/Unit/Enums/E_UniteMenu Enum" :default "NewEnumerator5"))
  (returns (OutSelectMenu :type "/Game/Blueprints/Unit/Enums/E_UniteMenu Enum") (OutMenuList :type "Array of /Game/Blueprints/Unit/Enums/E_UniteMenu Enum"))
  (return "NewEnumerator5"))

(fn `GetMenuTextLabel`
  (params (Menu :type "/Game/Blueprints/Unit/Enums/E_UniteMenu Enum" :default "NewEnumerator5"))
  (returns (MenuName :type Name) (MenuInfo :type Name))
  (return "None" "None"))

(fn `GetSelectMenu`
  (returns (OutSelectMenu :type "/Game/Blueprints/Unit/Enums/E_UniteMenu Enum"))
  (return "NewEnumerator5"))

(fn `InitTask`
  (params (InParam :type Integer) (InParam2 :type Integer))
  (returns (OutParam :type Integer))
  (bind _outparam (`parent.InitTask` InParam InParam2))
  (return _outparam))

(fn `IsOpenMenu`
  (params (Menu :type "/Game/Blueprints/Unit/Enums/E_UniteMenu Enum" :default "NewEnumerator5"))
  (returns (bOpen :type Boolean))
  (return false))

(fn `RunTask`
  (params (DeltaSeconds :type "Float (double-precision)"))
  (returns (bDecision :type Boolean) (bCancel :type Boolean) (OutParam :type Integer))
  (bind (_bdecision _bcancel _outparam) (`parent.RunTask` DeltaSeconds))
  (return _bdecision _bcancel _outparam))