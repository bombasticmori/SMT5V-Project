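; BP_UniteMenuCtrl is a menu controller Blueprint that exposes an interface for menus, windows, messages and yes/no prompts.
; InitCtrl only forwards to its parent implementation, and the BeginPlay and Tick events are disabled.
; Every interface function here is a stub returning false or zero, so this Blueprint itself opens nothing and reports no input.
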(fn `IGetMenuCursorPos`
  (returns (CursorPos :type Integer))
  (return 0))

(fn `IIsOpenMenu`
  (returns (bOpen :type Boolean))
  (return false))

(fn `IIsOpenWindow`
  (returns (bOpen :type Boolean))
  (return false))

(fn `InitCtrl`
  (params (ScriptAsset :type "ScriptMessageAsset Object Reference"))
  (returns (bOK :type Boolean))
  (bind _bok (`parent.InitCtrl` ScriptAsset))
  (return _bok))

(fn `IRequestCloseMenu`
  (params (bWindowClose :type Boolean) (bWindowExcution :type Boolean))
  (returns (bOk :type Boolean))
  (return false))

(fn `IRequestCloseMessage`
  (params (bExcution :type Boolean))
  (returns (bOk :type Boolean))
  (return false))

(fn `IRequestMenu`
  (params (MenuName :type "Array of Name (by ref)") (MenuCursorPos :type Integer) (MenuNewIocn :type "Array of Boolean (by ref)") (bMenuWaitMsg :type Boolean) (WindowMessage :type Name) (bWindowExcution :type Boolean) (bWindowSystemMsg :type Boolean))
  (returns (bOk :type Boolean))
  (return false))

(fn `IRequestMenuMultiMsg`
  (params (MenuName :type "Array of Name (by ref)") (MenuCursorPos :type Integer) (MenuNewIocn :type "Array of Boolean (by ref)") (bMenuWaitMsg :type Boolean) (WindowMessageList :type "Array of Name (by ref)") (bWindowExcution :type Boolean) (bWindowSystemMsg :type Boolean))
  (returns (bOk :type Boolean))
  (return false))

(fn `IRequestMenuTagValue`
  (params (MenuName :type "Array of Name (by ref)") (MenuCursorPos :type Integer) (MenuNewIocn :type "Array of Boolean (by ref)") (bMenuWaitMsg :type Boolean) (WindowMessage :type Name) (WindowTagInfo :type "Array of /Game/Blueprints/Facility/Blueprints/FacilityMsgTagInfo Structure (by ref)") (bWindowExcution :type Boolean) (bWindowSystemMsg :type Boolean))
  (returns (bOk :type Boolean))
  (return false))

(fn `IRequestMenuYesNo`
  (params (WindowMessage :type Name) (bWindowExcution :type Boolean) (bWindowSystemMsg :type Boolean))
  (returns (bOk :type Boolean))
  (return false))

(fn `IRequestMenuYesNoTagValue`
  (params (WindowMessage :type Name) (WindowTagInfo :type "Array of /Game/Blueprints/Facility/Blueprints/FacilityMsgTagInfo Structure (by ref)") (bWindowExcution :type Boolean) (bWindowSystemMsg :type Boolean))
  (returns (bOk :type Boolean))
  (return false))

(fn `IRequestMessage`
  (params (Label :type Name) (bExecution :type Boolean) (bNextIcon :type Boolean) (bSystemMsg :type Boolean))
  (returns (bOk :type Boolean))
  (return false))

(fn `IRequestMessageTagValue`
  (params (Label :type Name) (TagInfo :type "Array of /Game/Blueprints/Facility/Blueprints/FacilityMsgTagInfo Structure (by ref)") (bExecution :type Boolean) (bNextIcon :type Boolean) (bSystemMsg :type Boolean))
  (returns (bOk :type Boolean))
  (return false))

(fn `IUpdateMenuInput`
  (params (bPlayActionSE :type Boolean) (bPlayCancelSE :type Boolean) (bPlayCursorSE :type Boolean) (bPlayMessageSE :type Boolean))
  (returns (bAction :type Boolean) (bCancel :type Boolean) (bMoveCursor :type Boolean) (bSkipMessage :type Boolean))
  (return false false false false))

(fn `IUpdateMessageInput`
  (params (bPlaySE :type Boolean))
  (returns (bRunningMsg :type Boolean) (bCompleteMsg :type Boolean) (bReqCompleteMsg :type Boolean) (bReqNextPage :type Boolean) (bMW_Off :type Boolean))
  (return false false false false false))