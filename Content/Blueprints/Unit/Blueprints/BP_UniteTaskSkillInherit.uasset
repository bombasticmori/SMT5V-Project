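; Unite task Blueprint for a skill-inherit step, apparently part of unit fusion, with a defence affinity (Aishou) variant, currently only a skeleton.
; InitTask, RunTask, EndTask and EndPlay simply forward to the parent class.
; UI open/close, input checks, mouse slot and scrollbar handlers, cost, help and effect functions are empty stubs or return false or nothing, so no inheritance logic runs here.
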(event `self.ReceiveEndPlay`
  (params (EndPlayReason :type "EEndPlayReason Enum" :default "Destroyed"))
  (`parent.ReceiveEndPlay` EndPlayReason))

(fn `CloseCmnHelp`)

(fn `CloseUI`
  (params (Immediate :type Boolean)))

(fn `EndTask`
  (returns (OutParam :type Integer))
  (bind _outparam (`parent.EndTask`))
  (return _outparam))

(fn `GetUICtrl`
  (returns (InheritUICtrl :type "/Game/Blueprints/Camp/Status/BPI_InheritStatusUICtrl Interface"))
  (return null))

(fn `InitTask`
  (params (InParam :type Integer) (InParam2 :type Integer))
  (returns (OutParam :type Integer))
  (bind _outparam (`parent.InitTask` InParam InParam2))
  (return _outparam))

(fn `IsEndUIAnim`
  (returns (bEnd :type Boolean))
  (return false))

(fn `IsKeyCheckBase`
  (params (ActionMapping :type "E_ACTION_MAPPING_TYPE Enum" :default "E_ACTION_MAPPING_ACTION") (bAbleKeyPepeat :type Boolean))
  (returns (bInput :type Boolean))
  (return false))

(fn `IsKeyPepeatDown`
  (returns (bOutAble :type Boolean))
  (return false))

(fn `IsKeyPepeatUp`
  (returns (bOutAble :type Boolean))
  (return false))

(fn `IsPlayNextEffect`
  (returns (bPlay :type Boolean))
  (return false))

(fn `OnClickedParentSlot`
  (params (Index :type Integer)))

(fn `OnClickedRightSlot`
  (params (Index :type Integer)))

(fn `OnHoveredParentSlot`
  (params (Index :type Integer)))

(fn `OnHoveredRightSlot`
  (params (Index :type Integer)))

(fn `OnMovedParentScrollBarbyMouse`
  (params (NewOffset :type Integer)))

(fn `OnMovedRightScrollBarbyMouse`
  (params (NewOffset :type Integer)))

(fn `OpenUI`)

(fn `OpenUIForDefenceAishou`)

(fn `ReqeuestErrorMessage`)

(fn `RestartCmnHelp`)

(fn `RunDefenceAishou`
  (returns (bOutDecison :type Boolean) (bOutCancel :type Boolean))
  (return false false))

(fn `RunSkillInherit`
  (returns (bOutDecison :type Boolean) (bOutCancel :type Boolean))
  (return false false))

(fn `RunTask`
  (params (DeltaSeconds :type "Float (double-precision)"))
  (returns (bDecision :type Boolean) (bCancel :type Boolean) (OutParam :type Integer))
  (bind (_bdecision _bcancel _outparam) (`parent.RunTask` DeltaSeconds))
  (return _bdecision _bcancel _outparam))

(fn `SetButtonHelp`
  (params (InType :type Integer)))

(fn `SetMouseMediator`)

(fn `SetUniteCost`
  (params (Cost :type Integer)))

(fn `StartNextEffcet`)

(fn `StartPreUiClose`)

(fn `UpdateDefenceInput`
  (returns (bNext :type Boolean) (bBack :type Boolean) (update :type Boolean))
  (return false false false))

(fn `UpdateInput`
  (returns (bNext :type Boolean) (bBack :type Boolean) (update :type Boolean) (bError :type Boolean))
  (return false false false false))

(fn `UpdatePreUiCloseTime`
  (params (InTime :type "Float (double-precision)")))

(fn `UpdateStatusCheckInput`
  (returns (bNext :type Boolean) (bBack :type Boolean) (update :type Boolean))
  (return false false false))

(fn `UpdateUI`)