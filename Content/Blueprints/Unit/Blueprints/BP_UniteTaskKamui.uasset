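; BP_UniteTaskKamui is a unit task Blueprint for Kamui, currently a skeleton with no logic of its own.
; InitTask, RunTask and EndTask forward to the parent implementations, with RunTask returning the parent's Decision, Cancel and OutParam.
; BeginPlay and EndPlay also defer to the parent, Tick is disabled, and the StartKamuiCtrl and OnLoaded events are empty.
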(event `self.ReceiveBeginPlay`
  (`parent.ReceiveBeginPlay`))

(event `OnLoaded_CB8A5FED401A6359C8785C9125C7A90C`
  (params (Loaded :type "Object Class Reference")))

(event `self.ReceiveEndPlay`
  (params (EndPlayReason :type "EEndPlayReason Enum" :default "Destroyed"))
  (`parent.ReceiveEndPlay` EndPlayReason))

(event `StartKamuiCtrl`)

(fn `EndTask`
  (returns (OutParam :type Integer))
  (bind _outparam (`parent.EndTask`))
  (return _outparam))

(fn `InitTask`
  (params (InParam :type Integer) (InParam2 :type Integer))
  (returns (OutParam :type Integer))
  (bind _outparam (`parent.InitTask` InParam InParam2))
  (return _outparam))

(fn `RunTask`
  (params (DeltaSeconds :type "Float (double-precision)"))
  (returns (bDecision :type Boolean) (bCancel :type Boolean) (OutParam :type Integer))
  (bind (_bdecision _bcancel _outparam) (`parent.RunTask` DeltaSeconds))
  (return _bdecision _bcancel _outparam))