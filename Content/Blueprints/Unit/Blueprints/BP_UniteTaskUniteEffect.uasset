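; BP_UniteTaskUniteEffect is a task Blueprint that, by its names, covers the effect sequence for uniting up to four source devils into a result devil.
; InitTask, RunTask and EndTask only forward to the parent task.
; SetParam (devils and an Accident value), SetLevelLocation, and the events for loading, starting, waiting on and unloading the event level are empty stubs, so this file holds no effect logic.
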(event `LoadEventLevel`)

(event `UnloadEventLevel`)

(event `StartUniteEvent`)

(event `WaitUniteEvLoad`)

(event `WaitUniteEvLoad2`)

(fn `EndTask`
  (returns (OutParam :type Integer))
  (bind _outparam (`parent.EndTask`))
  (return _outparam))

(fn `InitTask`
  (params (InParam :type Integer) (InParam2 :type Integer))
  (returns (OutParam :type Integer))
  (bind _outparam (`parent.InitTask` InParam InParam2))
  (return _outparam))

(fn `RunTask`
  (params (DeltaSeconds :type "Float (double-precision)"))
  (returns (bDecision :type Boolean) (bCancel :type Boolean) (OutParam :type Integer))
  (bind (_bdecision _bcancel _outparam) (`parent.RunTask` DeltaSeconds))
  (return _bdecision _bcancel _outparam))

(fn `SetLevelLocation`
  (params (EventLevelLocation :type "Vector Structure")))

(fn `SetParam`
  (params (ResultDevil :type Integer) (SourceDevil_1 :type Integer) (SourceDevil_2 :type Integer) (SourceDevil_3 :type Integer) (SourceDevil_4 :type Integer) (bAccident :type Boolean)))