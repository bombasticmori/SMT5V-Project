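; BP_UniteCtrl is the controller skeleton for the Unite (fusion) facility, covering menus, camera views, BGM, tutorial and skill inheritance.
; Its interface is a flow state machine (FlowChange, FlowUpdate, Init/Run/End per screen) spanning top menu, search, double and special unite, Bible and others.
; BPI functions expose inherit-list input and UI controller getters.
; All bodies are empty or return defaults, except BeginPlay, Tick and EndPlay, which call the parent.
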(event `self.ReceiveBeginPlay`
  (`parent.ReceiveBeginPlay`))

(event `self.ReceiveTick`
  (params (DeltaSeconds :type "Float (single-precision)"))
  (`parent.ReceiveTick` DeltaSeconds))

(event `self.ReceiveEndPlay`
  (params (EndPlayReason :type "EEndPlayReason Enum" :default "Destroyed"))
  (`parent.ReceiveEndPlay` EndPlayReason))

(event `Evt_FadeEnd`)

(event `Evt_CallEnd`)

(event `Evt_ExitFadeOut`)

(event `Evt_Exit`)

(event `Evt_StartTutorial`)

(event `Evt_EndTutorial`)

(event `CameraChange_SophiaView`
  (params (view :type Boolean)))

(event `CameraChange_PlayerView`
  (params (view :type Boolean)))

(event `FirstGazeSet`
  (params (First :type Boolean)))

(fn `AddUniteMember`
  (params (bCheckAccident :type Boolean)))

(fn `BPI_GetSophia`
  (returns (Pawn :type "Pawn Object Reference"))
  (return null))

(fn `BPI_UniteGetInheritUICtrl`
  (returns (InheritUICtrl :type "/Game/Blueprints/Camp/Status/BPI_InheritStatusUICtrl Interface"))
  (return null))

(fn `BPI_UniteIheritSetStatusUIBtnHelpStatus`
  (params (Visibility :type Boolean))
  (returns (Success :type Boolean))
  (return false))

(fn `BPI_UniteInheritCancelButton`
  (returns (Result :type "E_SKILLINHERIT_RESULT Enum"))
  (return "E_SKILLINHERIT_RESULT_NONE"))

(fn `BPI_UniteInheritClickedSlot`
  (params (isMain :type Boolean) (index :type Integer))
  (returns (moveResult :type "E_SKILLINHERIT_RESULT Enum") (decisionResult :type "E_SKILLINHERIT_RESULT Enum"))
  (return "E_SKILLINHERIT_RESULT_NONE" "E_SKILLINHERIT_RESULT_NONE"))

(fn `BPI_UniteInheritDecisionButton`
  (returns (Result :type "E_SKILLINHERIT_RESULT Enum"))
  (return "E_SKILLINHERIT_RESULT_NONE"))

(fn `BPI_UniteInheritDraggedScrollBar`
  (params (IsMain :type Boolean) (NewTopPos :type Integer))
  (returns (TopMoved :type Boolean) (CursorMoved :type Boolean) (IsCurrentList :type Boolean))
  (return false false false))

(fn `BPI_UniteInheritEndButton`
  (returns (Result :type "E_SKILLINHERIT_RESULT Enum"))
  (return "E_SKILLINHERIT_RESULT_NONE"))

(fn `BPI_UniteInheritGetListPos`
  (returns (OutParentTop :type Integer) (OutParentCurrent :type Integer) (OutChildTop :type Integer) (OutChildCategory :type Integer) (OutChildCurrent :type Integer))
  (return 0 0 0 0 0))

(fn `BPI_UniteInheritHoveredSlot`
  (params (isMain :type Boolean) (index :type Integer))
  (returns (Result :type "E_SKILLINHERIT_RESULT Enum"))
  (return "E_SKILLINHERIT_RESULT_NONE"))

(fn `BPI_UniteInheritIsAbleKeyPepeatDown`
  (returns (bAble :type Boolean))
  (return false))

(fn `BPI_UniteInheritIsAbleKeyPepeatUp`
  (returns (bAble :type Boolean))
  (return false))

(fn `BPI_UniteInheritScrollDown`
  (returns (Result :type "E_SKILLINHERIT_RESULT Enum"))
  (return "E_SKILLINHERIT_RESULT_NONE"))

(fn `BPI_UniteInheritScrollPageDown`
  (returns (Result :type "E_SKILLINHERIT_RESULT Enum"))
  (return "E_SKILLINHERIT_RESULT_NONE"))

(fn `BPI_UniteInheritScrollPageUp`
  (returns (Result :type "E_SKILLINHERIT_RESULT Enum"))
  (return "E_SKILLINHERIT_RESULT_NONE"))

(fn `BPI_UniteInheritScrollUp`
  (returns (Result :type "E_SKILLINHERIT_RESULT Enum"))
  (return "E_SKILLINHERIT_RESULT_NONE"))

(fn `BPI_UniteInheritSetUIVisibility`
  (params (Visibility :type "ESlateVisibility Enum" :default "Visible"))
  (returns (Success :type Boolean))
  (return false))

(fn `BPI_UniteInheritWheelDown`
  (params (MainHover :type Boolean) (Sub :type Boolean) (HoverPos :type Integer))
  (returns (TopMoved :type Boolean) (CursorMoved :type Boolean) (IsCurrentList :type Boolean))
  (return false false false))

(fn `BPI_UniteInheritWheelUp`
  (params (MainHover :type Boolean) (SubHover :type Boolean) (HoverPos :type Integer))
  (returns (TopMoved :type Boolean) (CursorMoved :type Boolean) (IsCurrentList :type Boolean))
  (return false false false))

(fn `BPI_UniteUpdateInheritUI`
  (returns (bOk :type Boolean))
  (return false))

(fn `CloseLocationName`
  (params (PlayAnim :type Boolean)))

(fn `EntryBookForFusionEvent`)

(fn `FlowChange`
  (params (Flow :type "/Game/Blueprints/Unit/Enums/E_UniteFlow Enum" :default "NewEnumerator14")))

(fn `FlowDataInit`)

(fn `FlowEnd`
  (params (Flow :type "/Game/Blueprints/Unit/Enums/E_UniteFlow Enum" :default "NewEnumerator14")))

(fn `FlowEnd_BibleBrowse`)

(fn `FlowEnd_BibleRewrite`)

(fn `FlowEnd_Enter`)

(fn `FlowEnd_Exit`)

(fn `FlowEnd_Kamui`)

(fn `FlowEnd_OpenInfo`)

(fn `FlowEnd_PartyInfo`)

(fn `FlowEnd_TopMenu`)

(fn `FlowEnd_Tutorial`)

(fn `FlowEnd_UniteDouble`)

(fn `FlowEnd_UniteDoubleEx`)

(fn `FlowEnd_UniteSearch`)

(fn `FlowEnd_UniteSpecial`)

(fn `FlowEnd_Utsusemi`)

(fn `FlowInit_BibleBrowse`)

(fn `FlowInit_BibleRewrite`)

(fn `FlowInit_Enter`)

(fn `FlowInit_Exit`)

(fn `FlowInit_Kamui`)

(fn `FlowInit_OpenInfo`)

(fn `FlowInit_PartyInfo`)

(fn `FlowInit_TopMenu`
  (params (Menu :type "/Game/Blueprints/Unit/Enums/E_UniteMenu Enum" :default "NewEnumerator5")))

(fn `FlowInit_Tutorial`)

(fn `FlowInit_UniteDouble`)

(fn `FlowInit_UniteDoubleEｘ`)

(fn `FlowInit_UniteSearch`
  (params (bUseDevilBook :type Boolean)))

(fn `FlowInit_UniteSpecial`)

(fn `FlowInit_Utsusemi`)

(fn `FlowRun`
  (params (Flow :type "/Game/Blueprints/Unit/Enums/E_UniteFlow Enum" :default "NewEnumerator14") (DeltaSeconds :type "Float (double-precision)"))
  (returns (NextFlow :type "/Game/Blueprints/Unit/Enums/E_UniteFlow Enum"))
  (return "NewEnumerator14"))

(fn `FlowRun_BibleBrowse`
  (params (DeltaSeconds :type "Float (double-precision)"))
  (returns (NextFlow :type "/Game/Blueprints/Unit/Enums/E_UniteFlow Enum"))
  (return "NewEnumerator14"))

(fn `FlowRun_BibleRewrite`
  (params (DeltaSeconds :type "Float (double-precision)"))
  (returns (NextFlow :type "/Game/Blueprints/Unit/Enums/E_UniteFlow Enum"))
  (return "NewEnumerator14"))

(fn `FlowRun_Enter`
  (params (DeltaSeconds :type "Float (double-precision)"))
  (returns (NextFlow :type "/Game/Blueprints/Unit/Enums/E_UniteFlow Enum"))
  (return "NewEnumerator14"))

(fn `FlowRun_Exit`
  (params (DeltaSeconds :type "Float (double-precision)"))
  (returns (NextFlow :type "/Game/Blueprints/Unit/Enums/E_UniteFlow Enum"))
  (return "NewEnumerator14"))

(fn `FlowRun_Kamui`
  (params (DeltaSeconds :type "Float (double-precision)"))
  (returns (NextFlow :type "/Game/Blueprints/Unit/Enums/E_UniteFlow Enum"))
  (return "NewEnumerator14"))

(fn `FlowRun_OpenInfo`
  (params (DeltaSeconds :type "Float (double-precision)"))
  (returns (NextFlow :type "/Game/Blueprints/Unit/Enums/E_UniteFlow Enum"))
  (return "NewEnumerator14"))

(fn `FlowRun_PartyInfo`
  (params (DeltaSeconds :type "Float (double-precision)"))
  (returns (NextFlow :type "/Game/Blueprints/Unit/Enums/E_UniteFlow Enum"))
  (return "NewEnumerator14"))

(fn `FlowRun_TopMenu`
  (params (DeltaSeconds :type "Float (double-precision)"))
  (returns (NextFlow :type "/Game/Blueprints/Unit/Enums/E_UniteFlow Enum"))
  (return "NewEnumerator14"))

(fn `FlowRun_Tutorial`
  (params (DeltaSeconds :type "Float (double-precision)"))
  (returns (NextFlow :type "/Game/Blueprints/Unit/Enums/E_UniteFlow Enum"))
  (return "NewEnumerator14"))

(fn `FlowRun_UniteDouble`
  (params (DeltaSeconds :type "Float (double-precision)"))
  (returns (NextFlow :type "/Game/Blueprints/Unit/Enums/E_UniteFlow Enum"))
  (return "NewEnumerator14"))

(fn `FlowRun_UniteDoubleEx`
  (params (DeltaSeconds :type "Float (double-precision)"))
  (returns (NextFlow :type "/Game/Blueprints/Unit/Enums/E_UniteFlow Enum"))
  (return "NewEnumerator14"))

(fn `FlowRun_UniteSearch`
  (params (DeltaSeconds :type "Float (double-precision)"))
  (returns (NextFlow :type "/Game/Blueprints/Unit/Enums/E_UniteFlow Enum"))
  (return "NewEnumerator14"))

(fn `FlowRun_UniteSpecial`
  (params (DeltaSeconds :type "Float (double-precision)"))
  (returns (NextFlow :type "/Game/Blueprints/Unit/Enums/E_UniteFlow Enum"))
  (return "NewEnumerator14"))

(fn `FlowRun_Utsusemi`
  (params (DeltaSeconds :type "Float (double-precision)"))
  (returns (NextFlow :type "/Game/Blueprints/Unit/Enums/E_UniteFlow Enum"))
  (return "NewEnumerator14"))

(fn `FlowUpdate`
  (params (DeltaSeconds :type "Float (double-precision)")))

(fn `GetEnterMessage`
  (returns (label :type Name))
  (return "None"))

(fn `InUniteBGM`)

(fn `OpenLocationName`
  (params (PlayAnim :type Boolean)))

(fn `OutUniteBGM`)

(fn `SetCamera`
  (params (InBlendTime :type "Float (double-precision)") (Type :type Integer)))

(fn `SetViewPlayer`
  (params (bView :type Boolean)))

(fn `SetViewSophia`
  (params (bView :type Boolean)))

(fn `StartSearchExAsync`)

(fn `UniteBgCtrl`
  (returns (bDisp :type Boolean))
  (return false))

(fn `UniteGetCharaPanelCtrl`
  (returns (ICharaPanel :type "/Game/Blueprints/UI/PartyPanel/BPI_UniteCharaPanelCrtl Interface"))
  (return null))

(fn `UniteGetMenuCtrl`
  (returns (IMenuCtrl :type "/Game/Blueprints/Unit/Blueprints/BPI_UniteMenuCtrl Interface"))
  (return null))

(fn `UniteGetSkillPanelCtrl`
  (returns (ISkillPanel :type "/Game/Blueprints/UI/Camp/Skill/BPI_CampSkillCtrl Interface"))
  (return null))

(fn `UniteIsPlayEventTutorial`
  (returns (bPlay :type Boolean))
  (return false))

(fn `UniteIsPlayFlash`
  (returns (bPlay :type Boolean))
  (return false))

(fn `UniteStartEventTutorial`
  (returns (bStart :type Boolean))
  (return false))

(fn `UniteStartFlash`
  (returns (bOh :type Boolean))
  (return false))

(fn `UserConstructionScript`)