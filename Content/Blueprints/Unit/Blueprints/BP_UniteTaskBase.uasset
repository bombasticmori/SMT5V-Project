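; BP_UniteTaskBase is a base Blueprint for Unite tasks, defining a shared interface with no behavior of its own.
; It declares an InitTask, RunTask and EndTask lifecycle, with RunTask taking delta time and returning Decision, Cancel and an output parameter.
; Stub hooks cover Unite flash, event tutorials, and getters for inherit, skill panel, party panel and menu controllers.
; Every function is empty or returns default values, presumably for child Blueprints to override.
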(fn `EndTask`
  (returns (OutParam :type Integer))
  (return 0))

(fn `GetInheritCtrl`
  (returns (BPIUniteIneritCtrl :type "/Game/Blueprints/Unit/Blueprints/BPI_UniteInheritCtrl Interface"))
  (return null))

(fn `GetMenuCtrl`
  (returns (OutIMenuCtrl :type "/Game/Blueprints/Unit/Blueprints/BPI_UniteMenuCtrl Interface"))
  (return null))

(fn `GetPartyPanelCtrl`
  (returns (CharaPanel :type "/Game/Blueprints/UI/PartyPanel/BPI_UniteCharaPanelCrtl Interface"))
  (return null))

(fn `GetSkillPanelCtrl`
  (returns (SkillPanel :type "/Game/Blueprints/UI/Camp/Skill/BPI_CampSkillCtrl Interface"))
  (return null))

(fn `InitTask`
  (params (InParam :type Integer) (InParam2 :type Integer))
  (returns (OutParam :type Integer))
  (return 0))

(fn `IsPlayEventTutorial`
  (returns (bPlay :type Boolean))
  (return false))

(fn `IsUniteFlash`
  (returns (bPlay :type Boolean))
  (return false))

(fn `RunTask`
  (params (DeltaSeconds :type "Float (double-precision)"))
  (returns (bDecision :type Boolean) (bCancel :type Boolean) (OutParam :type Integer))
  (return false false 0))

(fn `StartEventTutorial`)

(fn `StartUniteFlash`)