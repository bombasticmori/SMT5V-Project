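; BP_UniteTaskTutorial is a task Blueprint for a tutorial menu and window, currently only a skeleton.
; InitTask, RunTask and EndTask forward directly to the parent class and return its results.
; The menu, list navigation, label and tutorial-state functions are stubs returning fixed defaults such as false, "None" or a single enum value.
; BeginPlay and Tick are disabled, so the asset adds no behavior of its own.
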(fn `CreateMenuList`
  (params (Menu :type "/Game/Blueprints/Unit/Enums/E_UniteTutorialMenu Enum" :default "NewEnumerator28") (bNext :type Boolean) (bPrev :type Boolean))
  (returns (OutSelectMenu :type "/Game/Blueprints/Unit/Enums/E_UniteTutorialMenu Enum") (OutMenuList :type "Array of /Game/Blueprints/Unit/Enums/E_UniteTutorialMenu Enum"))
  (return "NewEnumerator28"))

(fn `CreateMenuUI`
  (params (SelectMenu :type "/Game/Blueprints/Unit/Enums/E_UniteTutorialMenu Enum" :default "NewEnumerator28") (MenuList :type "Array of /Game/Blueprints/Unit/Enums/E_UniteTutorialMenu Enum (by ref)"))
  (returns (bOk :type Boolean))
  (return false))

(fn `EndTask`
  (returns (OutParam :type Integer))
  (bind _outparam (`parent.EndTask`))
  (return _outparam))

(fn `FindMenuList`
  (params (InSelectMenu :type "/Game/Blueprints/Unit/Enums/E_UniteTutorialMenu Enum" :default "NewEnumerator28"))
  (returns (OutSelectMenu :type "/Game/Blueprints/Unit/Enums/E_UniteTutorialMenu Enum") (OutMenuList :type "Array of /Game/Blueprints/Unit/Enums/E_UniteTutorialMenu Enum"))
  (return "NewEnumerator28"))

(fn `FindMenuListNext`
  (params (InSelectMenu :type "/Game/Blueprints/Unit/Enums/E_UniteTutorialMenu Enum" :default "NewEnumerator28"))
  (returns (OutSelectMenu :type "/Game/Blueprints/Unit/Enums/E_UniteTutorialMenu Enum") (OutMenuList :type "Array of /Game/Blueprints/Unit/Enums/E_UniteTutorialMenu Enum"))
  (return "NewEnumerator28"))

(fn `FindMenuListPrev`
  (params (InSelectMenu :type "/Game/Blueprints/Unit/Enums/E_UniteTutorialMenu Enum" :default "NewEnumerator28"))
  (returns (OutSelectMenu :type "/Game/Blueprints/Unit/Enums/E_UniteTutorialMenu Enum") (OutMenuList :type "Array of /Game/Blueprints/Unit/Enums/E_UniteTutorialMenu Enum"))
  (return "NewEnumerator28"))

(fn `GetForwardMsgLabel`
  (params (Menu :type "/Game/Blueprints/Unit/Enums/E_UniteTutorialMenu Enum" :default "NewEnumerator28"))
  (returns (MenuName :type Name))
  (return "None"))

(fn `GetMenuMsgLabel`
  (params (Menu :type "/Game/Blueprints/Unit/Enums/E_UniteTutorialMenu Enum" :default "NewEnumerator28"))
  (returns (MsgName :type Name))
  (return "None"))

(fn `GetMenuTitleLabel`
  (params (Menu :type "/Game/Blueprints/Unit/Enums/E_UniteTutorialMenu Enum" :default "NewEnumerator28"))
  (returns (MenuName :type Name))
  (return "None"))

(fn `GetTutorialType`
  (params (Menu :type "/Game/Blueprints/Unit/Enums/E_UniteTutorialMenu Enum" :default "NewEnumerator28"))
  (returns (OutTutoType :type "E_TUTORIAL_WINDOW_MESSAGE_TYPE Enum"))
  (return "DASH"))

(fn `InitTask`
  (params (InParam :type Integer) (InParam2 :type Integer))
  (returns (OutParam :type Integer))
  (bind _outparam (`parent.InitTask` InParam InParam2))
  (return _outparam))

(fn `IsNewDisp`
  (params (InSelectMenu :type "/Game/Blueprints/Unit/Enums/E_UniteTutorialMenu Enum" :default "NewEnumerator28"))
  (returns (bOutDisp :type Boolean))
  (return false))

(fn `IsOpenMenu`
  (params (Menu :type "/Game/Blueprints/Unit/Enums/E_UniteTutorialMenu Enum" :default "NewEnumerator28"))
  (returns (bOpen :type Boolean))
  (return false))

(fn `IsUserOpenTurorial`
  (returns (bOpen :type Boolean))
  (return false))

(fn `RunTask`
  (params (DeltaSeconds :type "Float (double-precision)"))
  (returns (bDecision :type Boolean) (bCancel :type Boolean) (OutParam :type Integer))
  (bind (_bdecision _bcancel _outparam) (`parent.RunTask` DeltaSeconds))
  (return _bdecision _bcancel _outparam))

(fn `UpdateMenu`
  (returns (bNext :type Boolean) (bPrev :type Boolean))
  (return false false))

(fn `UpdateTutorialWindow`
  (returns (bNext :type Boolean) (bPrev :type Boolean))
  (return false false))