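; Project Game Instance that exposes a wide interface surface for map, encounter, battle, event, UI and level-loading calls.
; Nearly all of these events and functions are empty stubs returning default values.
; The only working logic forwards to the parent class: first-time game init plus getters for battle main, event base, system and save messages, difficulty text, device notification assets and warp-point textures.
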(event `/Game/Blueprints/Common/Character/BPI_PlayerManager.BPI_SetDeactiveLocation`
  (params (PlayerType :type "/Game/Blueprints/Common/Character/E_PLAYER_MANAGER_TYPE Enum" :default "NewEnumerator0") (Location :type "Transform Structure")))

(event `/Game/Blueprints/Common/Character/BPI_PlayerManager.BPI_SetActive`
  (params (PlayerType :type "/Game/Blueprints/Common/Character/E_PLAYER_MANAGER_TYPE Enum" :default "NewEnumerator0") (Active :type Boolean)))

(event `/Game/Blueprints/Common/Character/BPI_PlayerManager.BPI_SetContlrolActivePawn`
  (params (Pawn :type "/Game/Blueprints/Character/Base/PlayerBase Object Reference") (Type :type "/Game/Blueprints/Common/Character/E_PLAYER_MANAGER_TYPE Enum" :default "NewEnumerator0")))

(event `/Game/Blueprints/UI/BPI_UIManager.BPI_SetMapCharaPanelCtrlUI`
  (params (InActor :type "Actor Object Reference")))

(event `/Game/Blueprints/Map/BPI_MapCommon.BPI_SpawnEncountActor`
  (params (EnemyIdList :type "Array of Integer (by ref)") (EncountId :type Integer) (SpawnTransform :type "Transform Structure") (EncountPawn :type "Actor Object Reference") (SymbolEncountType :type "E_BTL_SYMBOL_ENCOUNT Enum" :default "E_BTL_SYMBOL_ENCOUNT_NORMAL") (ManualWhenNotEscape :type Boolean) (HitMapAttack :type Boolean) (ChainEncountInfo :type "ChainEncountInfo Structure") (Magatsuhi :type Boolean)))

(event `/Game/Blueprints/Map/BPI_MapCommon.BPI_ReturnFromBtl`)

(event `/Game/Blueprints/Map/BPI_MapCommon.BPI_SetEncountOff`)

(event `/Game/Blueprints/Map/BPI_MapCommon.BPI_SetEncountON`)

(event `/Game/Blueprints/Map/BPI_MapCommon.BPI_MapPlayerStop`
  (params (Stop :type Boolean) (Hidden :type Boolean)))

(event `/Game/Blueprints/Map/BPI_MapCommon.BPI_LoadMap`
  (params (inFadeCancel :type Boolean)))

(event `/Game/Blueprints/Map/BPI_MapCommon.BPI_AddSpawnEnemyCount`)

(event `/Game/Blueprints/Map/BPI_MapCommon.BPI_DebugChangeChar`
  (params (Type :type "/Game/Blueprints/Map/Common/E_MAP_PLAYER_TYPE Enum" :default "NewEnumerator0")))

(event `/Game/Blueprints/Map/BPI_MapCommon.BPI_DebugMesWindow`
  (params (MesType :type "/Game/Blueprints/Map/Debug/E_MAP_DEBUG_MES_TYPE Enum" :default "NewEnumerator1")))

(event `/Game/Blueprints/Map/BPI_MapCommon.BPI_MapPause`
  (params (PlayerMoveEnable :type Boolean) (PlayerCameraEnable :type Boolean) (PlayerVisible :type Boolean) (MoonTimeEnable :type Boolean) (SymbolEnable :type Boolean) (AllMapStop :type Boolean) (AllObjectHidden :type Boolean) (TopCamera :type Boolean)))

(event `/Game/Blueprints/Map/BPI_MapCommon.BPI_MapStart`
  (params (MissionCheckDisable :type Boolean) (StartSymbolAIDisable :type Boolean) (ReturnPlayerPosition :type Boolean) (UI_Immediate :type Boolean)))

(event `/Game/Blueprints/Map/BPI_MapCommon.BPI_CallEventEncount`
  (params (EventEncountID :type Integer) (SpawnTransform :type "Transform Structure") (NextEventID :type Integer) (NowEventID :type Integer) (Manual :type Boolean)))

(event `/Game/Blueprints/Map/BPI_MapCommon.BPI_PlayerOFF`)

(event `/Game/Blueprints/Map/BPI_MapCommon.BPI_PlayerON`)

(event `/Game/Blueprints/Map/BPI_MapCommon.BPI_CallKokubouEvent`
  (params (EventId :type Integer) (RestarPoint :type "Actor Object Reference") (BattlePoint :type "Actor Object Reference")))

(event `/Game/Blueprints/Map/BPI_MapCommon.BPI_OpenSkyTerminal`)

(event `/Game/Blueprints/Map/BPI_MapCommon.BPI_MapAttackEnd`
  (params (Enable :type Boolean)))

(event `/Game/Blueprints/Map/BPI_MapCommon.BPI_ForceSafeEncount`
  (params (Enable :type Boolean)))

(event `/Game/Blueprints/Map/BPI_MapCommon.BPI_HeroChange`
  (params (IsFade :type Boolean) (Hero :type "/Game/Blueprints/Map/Common/E_MAP_PLAYER_TYPE Enum" :default "NewEnumerator0")))

(event `/Game/Blueprints/Map/BPI_MapCommon.MapInit`)

(event `/Game/Blueprints/Map/BPI_MapCommon.SetEventBattleActor`
  (params (BTLActor :type "Array of /Game/Blueprints/Map/Struct/EventBattleListStruct Structure (by ref)") (PlayerPos :type "Transform Structure")))

(event `/Game/Blueprints/Map/BPI_MapCommon.BPI_SetEncountActor`
  (params (actor :type "Actor Object Reference")))

(event `/Game/Blueprints/Map/BPI_MapCommon.BPI_CallMapEvent`
  (params (MapEventID_ :type Integer) (ReStartPoint :type "Actor Object Reference") (BattlePoint :type "Actor Object Reference") (InitFade :type Boolean) (WaitEvent :type Boolean)))

(event `/Game/Blueprints/Map/BPI_MapCommon.BPI_CallEncountForMagatsuka`
  (params (EncountID :type Integer) (EnemyList :type "Array of Integer (by ref)") (SafeZoneID :type Integer) (ManualSafeZone :type Boolean) (EncountType :type "E_BTL_SYMBOL_ENCOUNT Enum" :default "E_BTL_SYMBOL_ENCOUNT_NORMAL") (HitMapAttack :type Boolean)))

(event `/Game/Blueprints/Map/BPI_MapCommon.BPI_ReturnMapFromOutside`
  (params (AutoSave :type Boolean) (ReturnPlayerPosition :type Boolean) (UI_Immediate :type Boolean)))

(event `/Game/Blueprints/Map/BPI_MapCommon.EnvChange_Play`
  (params (Next :type "/Game/Blueprints/Map/Daath/ST_LightParam Structure") (Prev :type "/Game/Blueprints/Map/Daath/ST_LightParam Structure")))

(event `/Game/Blueprints/Map/BPI_MapCommon.EnvChange_Reverse`)

(event `/Game/Blueprints/Map/BPI_MapCommon.BPI_ChangeArea`
  (params (NextAreaID :type Integer) (WarpPoint :type Integer) (FadeInTime :type "Float (single-precision)")))

(event `/Game/Blueprints/Map/BPI_MapCommon.BPI_CallEncountForNaviDevil`
  (params (EncountID :type Integer) (EnemyList :type "Array of Integer (by ref)") (SafeZoneID :type Integer) (ManualSafeZone :type Boolean) (ChainEncountInfo :type "ChainEncountInfo Structure") (Magatsuhi :type Boolean) (PlayerFirst :type Boolean)))

(event `/Game/Blueprints/Map/BPI_MapCommon.BPI_EntryNaviDevillGimmick`
  (params (Actor :type "Actor Object Reference")))

(event `/Game/Blueprints/Map/BPI_MapCommon.BPI_MapStart_SimpleEventEnable`)

(event `/Game/Blueprints/Map/BPI_MapCommon.EnvChangeMagatuka_Play`
  (params (Alpha :type "Float (single-precision)")))

(event `/Game/Blueprints/Map/BPI_MapCommon.ResetEventBattleActor`)

(event `/Game/Blueprints/Map/BPI_MapCommon.BPI_EndTakara_ForSimpleEvent`
  (params (TakaraID :type Integer)))

(event `/Game/Blueprints/Map/BPI_MapCommon.BPI_ShowObjects_WhenReturnMap`)

(event `/Game/Blueprints/Map/BPI_MapCommon.BPI_HideObjects_WhenExitMap`)

(event `/Game/Blueprints/Map/BPI_MapCommon.Env_ChangeSpecial_Play`
  (params (Index :type Integer) (alpha :type "Float (single-precision)")))

(event `/Game/Blueprints/Map/BPI_MapCommon.BPI_TokyoLargeMapAddIconTalk`
  (params (ActorLocation :type "Vector Structure") (InactiveFlag :type Name) (Owner :type "Actor Object Reference")))

(event `/Game/Blueprints/Map/BPI_MapCommon.BPI_TokyoLargeMapDeleteIcon`
  (params (Owner :type "Actor Object Reference")))

(event `/Game/Blueprints/Map/BPI_MapCommon.BPI_CallEncountForDebug`
  (params (EncountID :type Integer) (EnemyList :type "Array of Integer (by ref)") (SafeZoneID :type Integer) (ManualSafeZone :type Boolean) (EncountType :type "E_BTL_SYMBOL_ENCOUNT Enum" :default "E_BTL_SYMBOL_ENCOUNT_NORMAL")))

(event `/Game/Blueprints/Map/BPI_MapCommon.BPI_CallEventEncount_ForUniqueSymbol`
  (params (EventEncountID :type Integer) (SpawnTransform :type "Transform Structure") (ManualWhenNotEscape :type Boolean) (HitMapAttack :type Boolean) (EncountType :type "E_BTL_SYMBOL_ENCOUNT Enum" :default "E_BTL_SYMBOL_ENCOUNT_NORMAL")))

(event `/Game/Blueprints/Map/BPI_MapCommon.BPI_CallEventEncountForMagatsuka`
  (params (EventEncountID :type Integer) (SafeZoeID :type Integer) (ManualSafeZone :type Boolean) (HitMapAttack :type Boolean)))

(event `/Game/Blueprints/Map/BPI_MapCommon.BPI_NaviGimmickTutorial_ForInner`)

(event `/Game/Blueprints/Map/BPI_MapCommon.BPI_NaviGimmickTutorial_ForOuter`)

(event `/Game/Blueprints/Map/BPI_MapCommon.BPI_PreSystemLoad`
  (params (MapID :type Integer) (Enum :type "/Game/Blueprints/Common/Map/LevelCtrl/E_MAP_SYSTEMRESIDENT_ID Enum" :default "NewEnumerator0")))

(event `/Game/Blueprints/Map/BPI_MapCommon.BPI_EndMagatsuka_ForSimpleEvent`)

(event `/Game/Blueprints/Map/BPI_MapCommon.BPI_TokyoLargeMapShowPlace`
  (params (DataId :type Integer)))

(event `/Game/Blueprints/Map/BPI_MapCommon.BPI_TokyoLargeMapHidePlace`
  (params (DataId :type Integer)))

(event `/Game/Blueprints/Map/BPI_MapCommon.BPI_GardenLoad`
  (params (WarpPoint :type Integer) (FadeInTime :type "Float (single-precision)")))

(event `/Game/Blueprints/Map/BPI_MapCommon.BPI_GardenUnload`
  (params (FadeInTime :type "Float (single-precision)")))

(event `/Game/Blueprints/Map/BPI_MapCommon.BPI Tokyo Large Map Add Icon Mission`
  (params (ActorLocation :type "Vector Structure") (MissionId :type Integer) (Owner :type "Actor Object Reference")))

(event `/Game/Blueprints/Map/BPI_MapCommon.BPI_CallEventEncount_BossRush`
  (params (EventEncountID :type Integer) (NextEventID :type Integer) (NowEventID :type Integer) (Manual :type Boolean) (ChallengeMode :type Boolean)))

(event `/Game/Blueprints/Map/BPI_MapCommon.BPI_RequestNaviDevilVisible`
  (params (Visible :type Boolean)))

(event `/Game/Blueprints/Map/BPI_MapCommon.EnvChange_Immediate`)

(event `/Game/Blueprints/Map/BPI_MapCommon.BPI_LoadMapBridgeMode`
  (params (NextMapId :type Integer) (NextAreaId :type Integer) (FadeCancel :type Boolean)))

(event `/Game/Blueprints/Map/BPI_MapCommon.BPI_SetMapCommon`
  (params (actor :type "Actor Object Reference")))

(event `/Game/Blueprints/Battle/FrameWork/Actors/BPI_ExternalBattle.BI_SetBattleMain`
  (params (battleMain :type "Actor Object Reference")))

(event `/Game/Blueprints/Common/AssetTable/BPI_CharaBaseTable.BI_SetCharaTable`
  (params (CharaTable :type "Object Object Reference")))

(event `/Game/Blueprints/Map/BPI_MapCommon.BPI_SetEventReserv`
  (params (MapEventID :type Integer)))

(event `/Game/Blueprints/Map/BPI_MapCommon.SetNextMapAssetList`
  (params (LevelList :type "Array of PrimaryAssetId Structure (by ref)") (NameList :type "Array of Name (by ref)") (MapID :type Integer) (AreaID :type Integer)))

(event `/Game/Blueprints/Map/BPI_MapCommon.SetNextMapLoadStart`
  (params (Enable :type Boolean)))

(event `/Game/Blueprints/Map/BPI_MapCommon.SetNextMapLoadEnd`
  (params (Enable :type Boolean)))

(event `/Game/Blueprints/Map/BPI_MapCommon.DeleteNextMapAssetList`)

(event `/Game/Blueprints/Map/BPI_MapCommon.SetNextMapStartList`
  (params (LevelList :type "Array of PrimaryAssetId Structure (by ref)") (LevelNameList :type "Array of Name (by ref)") (MapID :type Integer) (AreaID :type Integer)))

(event `/Game/Blueprints/Map/BPI_MapCommon.SetMapStartLoadFlag`
  (params (enable :type Boolean)))

(event `/Game/Blueprints/Map/BPI_MapCommon.SetLoadLevelGame`
  (params (enable :type Boolean)))

(event `self.GameFirstInitEvent`
  (`parent.GameFirstInitEvent`))

(event `/Game/Blueprints/Common/Character/BPI_PlayerManager.BPI_SetGamePlayer`
  (params (In :type "Array of Pawn Object Reference (by ref)")))

(event `OnDestroyed_イベント_0`
  (params (DestroyedActor :type "Actor Object Reference")))

(event `/Game/Blueprints/Map/BPI_MapCommon.StartDebugGameTrace`
  (params (IsEnable :type Boolean)))

(event `/Game/Blueprints/Map/BPI_MapCommon.SetJsonData`
  (params (Json :type "JsonDataCtrl Object Reference")))

(event `/Game/Blueprints/Map/BPI_MapCommon.SetJsonFile`
  (params (Json :type String)))

(event `/Game/Blueprints/Common/AssetTable/BPI_DevilAssetTable.BI_SetDevilAssetTable`
  (params (CharaTable :type "Object Object Reference")))

(event `/Game/Blueprints/Map/BPI_MapCommon.JsonCounterAdd`
  (params (EncountAdd :type Integer) (MagatukaNum :type Integer)))

(event `/Game/Blueprints/Map/BPI_MapCommon.BI_SetMapChange`
  (params (IsMapChange :type Boolean) (WarpPoint :type Integer) (FromEvent :type Integer) (OtherMapReturn :type Integer)))

(event `/Game/Blueprints/Gamedata/BPI_ProjectGameInstance.BPI_SetMapUICtrl`
  (params (MapUICommon :type "Actor Object Reference")))

(event `/Game/Blueprints/Gamedata/BPI_ProjectGameInstance.BPI_SetPreloadLevelList`
  (params (PreloadLevelList :type "Array of PrimaryAssetId Structure (by ref)")))

(event `/Game/Blueprints/Gamedata/BPI_ProjectGameInstance.BPI_ClearPreloadLevelList`)

(fn `AutomationEventEnd`)

(fn `AutomationEventStart`)

(fn `BattleEnd`)

(fn `BattleStart`
  (params (desc :type "BtlDescData Structure") (PrevBattleBGM :type "SoundAtomCue Object Reference")))

(fn `BI_CheckEncountOn`
  (returns (EncountOn :type Boolean))
  (return false))

(fn `BI_GetBattleMain`
  (returns (retValue :type "Actor Object Reference"))
  (return null))

(fn `BI_GetCharaTable`
  (returns (instance :type "Object Object Reference"))
  (return null))

(fn `BI_GetDaathIntensityEff`
  (returns (Intensity :type "LinearColor Structure"))
  (return))

(fn `BI_GetDevilAssetTable`
  (returns (instance :type "Object Object Reference"))
  (return null))

(fn `BI_IsEventView`
  (returns (IsEventView :type Boolean))
  (return false))

(fn `BPI_AddEncountAreaList`
  (params (EncountArea :type "Actor Object Reference"))
  (returns (NewParam :type Boolean))
  (return false))

(fn `BPI_AddMagatsukaDiscoveryCnt`
  (params (Add :type Integer))
  (returns (NewParam1 :type Boolean))
  (return false))

(fn `BPI_CategoryWindowCtrl`
  (returns (outActor :type "Actor Object Reference"))
  (return null))

(fn `BPI_CheckAActionLock`
  (returns (Lock :type Boolean) (AActionActor :type "Actor Object Reference"))
  (return false null))

(fn `BPI_CheckAfterLoaded`
  (returns (AfterLoaded :type Boolean))
  (return false))

(fn `BPI_CheckAgratField`
  (returns (Inside :type Boolean))
  (return false))

(fn `BPI_CheckHide_WhenBattleOrEvent`
  (returns (Hide :type Boolean))
  (return false))

(fn `BPI_CheckLoadMap`
  (returns (LoadMap :type Boolean))
  (return false))

(fn `BPI_CheckMagatsukaDiscoveryCnt`
  (returns (Discovery :type Boolean))
  (return false))

(fn `BPI_CheckMapEnableCamera`
  (returns (IsPause :type Boolean))
  (return false))

(fn `BPI_CheckMapPause`
  (returns (IsPause :type Boolean))
  (return false))

(fn `BPI_CheckSymbolPause`
  (returns (Pause :type Boolean))
  (return false))

(fn `BPI_GetActive`
  (params (PlayerType :type "/Game/Blueprints/Common/Character/E_PLAYER_MANAGER_TYPE Enum" :default "NewEnumerator0"))
  (returns (IsActive :type Boolean))
  (return false))

(fn `BPI_GetBossRushFieldCtrl`
  (returns (Actor :type "Actor Object Reference"))
  (return null))

(fn `BPI_GetBuddyPawn`
  (returns (Pawn :type "Pawn Object Reference"))
  (return null))

(fn `BPI_GetButtonHelpCtrl2`
  (returns (outActor :type "Actor Object Reference"))
  (return null))

(fn `BPI_GetCommonHelpWindowCtrl`
  (returns (OutActor :type "/Game/Blueprints/UI/CommonWindow/CommonHelpWindow/BPI_CommonHelpWindowCtrl Interface"))
  (return null))

(fn `BPI_GetCommonUI_EventCtrl`
  (returns (outActor :type "Actor Object Reference"))
  (return null))

(fn `BPI_GetCommonWindowCtrl`
  (returns (OutActor :type "/Game/Blueprints/UI/CommonWindow/BPI_CommonWindowCtrl Interface") (Success :type Boolean))
  (return null false))

(fn `BPI_GetContlrolActivePawn`
  (returns (Pawn :type "/Game/Blueprints/Character/Base/PlayerBase Object Reference") (Type :type "/Game/Blueprints/Common/Character/E_PLAYER_MANAGER_TYPE Enum"))
  (return null "NewEnumerator0"))

(fn `BPI_GetDaathLightType`
  (returns (LightType :type "/Game/Blueprints/Map/Daath/DaathTypeList Enum"))
  (return "NewEnumerator0"))

(fn `BPI_GetDeactiveLocation`
  (params (PlayerType :type "/Game/Blueprints/Common/Character/E_PLAYER_MANAGER_TYPE Enum" :default "NewEnumerator0"))
  (returns (Location :type "Transform Structure"))
  (return))

(fn `BPI_GetDialogWindowCtrl`
  (returns (OutActor :type "/Game/Blueprints/UI/CommonWindow/Dialog/BPI_DialogCtrl Interface"))
  (return null))

(fn `BPI_GetDLCAnnouncer`
  (returns (outActor :type "Actor Object Reference"))
  (return null))

(fn `BPI_GetDlcCheck`
  (returns (DlcTableData :type "DlcTableData Object Reference"))
  (return null))

(fn `BPI_GetEncountAreaAll`
  (returns (Actors :type "Array of Actor Object Reference"))
  (return))

(fn `BPI_GetEncountScene`
  (returns (EncountScene :type "Actor Object Reference"))
  (return null))

(fn `BPI_GetEventBase`
  (returns (return :type "EventBase Object Reference"))
  (return null))

(fn `BPI_GetEventReserv`
  (returns (MapEventID :type Integer))
  (return 0))

(fn `BPI_GetGamePlayer`
  (returns (list :type "Array of Pawn Object Reference"))
  (return))

(fn `BPI_GetInfoWindowCtrl`
  (returns (OutActor :type "/Game/Blueprints/UI/CommonWindow/InfoWindow/BPI_InfoWindowCtrl Interface"))
  (return null))

(fn `BPI_GetItemWindowCtrl`
  (returns (OutActor :type "/Game/Blueprints/UI/CommonWindow/ItemWindow/BPI_ItemWindowCtrl Interface"))
  (return null))

(fn `BPI_GetMagatsuhiGaugeCtrl`
  (returns (outActor :type "Actor Object Reference"))
  (return null))

(fn `BPI_GetMakkaWindowCtrl2`
  (returns (outActor :type "Actor Object Reference"))
  (return null))

(fn `BPI_GetMapButtonHelpType`
  (returns (out :type "E_BTN_HELP_SET Enum"))
  (return "E_BTN_HELP_SET_DUMMY"))

(fn `BPI_GetMapCharaPanelCtrlUI`
  (returns (OutActor :type "/Game/Blueprints/UI/PartyPanel/BPI_MapCharaPanelCtrl Interface") (IsValid :type Boolean))
  (return null false))

(fn `BPI_GetMapCommon`
  (returns (rerutn :type "Actor Object Reference"))
  (return null))

(fn `BPI_GetMapGimmickTrigger`
  (returns (Actor :type "Actor Object Reference"))
  (return null))

(fn `BPI_GetMapTimer`
  (returns (MapTimer :type "Float (double-precision)"))
  (return 0.0))

(fn `BPI_GetMapUICtrl`
  (returns (MapUICommon :type "Actor Object Reference"))
  (return null))

(fn `BPI_GetMiitsuWindowCtrl`
  (returns (outActor :type "Actor Object Reference"))
  (return null))

(fn `BPI_GetMsgCtrl`
  (returns (OutActor :type "Actor Object Reference"))
  (return null))

(fn `BPI_GetNaviDevilCtrl`
  (returns (Actor :type "Actor Object Reference"))
  (return null))

(fn `BPI_GetNaviDevilPawn`
  (returns (Pawn :type "Pawn Object Reference"))
  (return null))

(fn `BPI_GetOptionFieldBrightnessCtrl`
  (returns (Component :type "ActorComponent Object Reference"))
  (return null))

(fn `BPI_GetPreloadLevelList`
  (returns (PreloadLevelList :type "Array of PrimaryAssetId Structure"))
  (return))

(fn `BPI_GetScreenFadeWidget`
  (returns (Obj :type "Object Object Reference"))
  (return null))

(fn `BPI_GetSkillSearchWindowCtrl`
  (returns (outActor :type "Actor Object Reference"))
  (return null))

(fn `BPI_GetSortWindowCtrl2`
  (returns (outActor :type "Actor Object Reference"))
  (return null))

(fn `BPI_GetTutorialWIndowCtrl2`
  (returns (outActor :type "Actor Object Reference"))
  (return null))

(fn `BPI_GetUIManager`
  (returns (UIManager :type "ProjectUIManager Object Reference"))
  (return null))

(fn `BPI_IgnoreEstomaEffectPause`
  (params (Ignore :type Boolean))
  (returns (NewParam :type Boolean))
  (return false))

(fn `BPI_IsEventPlay`
  (returns (IsPlay :type Boolean))
  (return false))

(fn `BPI_IsScreenShot`
  (returns (return :type Boolean))
  (return false))

(fn `BPI_IsSpawnedUiCtrlActors`
  (returns (Complete :type Boolean))
  (return false))

(fn `BPI_IsSpawnSymbol`
  (returns (NewParam :type Boolean))
  (return false))

(fn `BPI_IsStatusMode`
  (returns (IsStatusMode :type Boolean))
  (return false))

(fn `BPI_IsTokyoLargeMap`
  (returns (IsTokyoLargeMap :type Boolean))
  (return false))

(fn `BPI_LocationWindowCtrl`
  (returns (OutActor :type "Actor Object Reference"))
  (return null))

(fn `BPI_MakeUpLessEvent`
  (returns (retValue :type Boolean))
  (return false))

(fn `BPI_MapTopCameraOnFinishTop`
  (returns (dummy :type Boolean))
  (return false))

(fn `BPI_MapTopCameraOnStartTop`
  (returns (dummy :type Boolean))
  (return false))

(fn `BPI_MoonAgeCtrl`
  (returns (outActor :type "Actor Object Reference"))
  (return null))

(fn `BPI_RegisterMagatsuka`
  (params (Actor :type "Actor Object Reference"))
  (returns (NewParam1 :type Boolean))
  (return false))

(fn `BPI_RemoveEncountAreaList`
  (params (EncountArea :type "Actor Object Reference"))
  (returns (NewParam :type Boolean))
  (return false))

(fn `BPI_ScreeTransitionCtrl`
  (returns (outActor :type "Actor Object Reference"))
  (return null))

(fn `BPI_SetAActionLock`
  (params (Lock :type Boolean) (AActionActor :type "Actor Object Reference"))
  (returns (NewParam1 :type Boolean))
  (return false))

(fn `BPI_SetAgratField`
  (params (Inside :type Boolean))
  (returns (NewParam :type Boolean))
  (return false))

(fn `BPI_SetBossRushFieldCtrl`
  (params (Actor :type "Actor Object Reference"))
  (returns (NewParam :type Boolean))
  (return false))

(fn `BPI_SetDebugOverrideBattleMapDarkID`
  (params (MapDarkID :type Integer))
  (returns (NoUse :type Boolean))
  (return false))

(fn `BPI_SetEncountScene`
  (params (EncountScene :type "Actor Object Reference"))
  (returns (NewParam :type Boolean))
  (return false))

(fn `BPI_SetEventBase`
  (params (base :type "EventBase Object Reference"))
  (returns (NoUse :type Boolean))
  (return false))

(fn `BPI_SetLevelVisibilityEnabled`
  (params (Enable :type Boolean))
  (returns (dummy :type Boolean))
  (return false))

(fn `BPI_SetNaviDevilPawn`
  (params (Pawn :type "Pawn Object Reference"))
  (returns (NewParam1 :type Boolean))
  (return false))

(fn `BPI_SetStatusMode`
  (params (IsStatusMode :type Boolean))
  (returns (NoUse :type Boolean))
  (return false))

(fn `BPI_ShowMapButtonHelp`
  (returns (dummy :type Boolean))
  (return false))

(fn `BPI_UnregisterMagatsuka`
  (params (Actor :type "Actor Object Reference"))
  (returns (NewParam :type Boolean))
  (return false))

(fn `BPI_UpdateLevelVisibility`
  (params (NewLocation :type "Vector Structure"))
  (returns (Updated :type Boolean))
  (return false))

(fn `BPI_UpdateOptionFieldBrightness`
  (returns (NewParam :type Boolean))
  (return false))

(fn `BPI_UpdateUniqueSymbolBGM`
  (returns (NewParam :type Boolean))
  (return false))

(fn `EncountStart`
  (params (EnemyIdList :type "Array of Integer (by ref)") (EncountId :type Integer) (SpawnTransform :type "Transform Structure") (EncountPawn :type "Actor Object Reference") (SymbolEncountType :type "E_BTL_SYMBOL_ENCOUNT Enum" :default "E_BTL_SYMBOL_ENCOUNT_NORMAL") (ManualWhenNotEscape :type Boolean) (HitMapAttack :type Boolean) (ChainEncountInfo :type "ChainEncountInfo Structure") (Magatsuhi :type Boolean)))

(fn `GetBattleMain`
  (returns (ReturnValue :type "Actor Object Reference"))
  (bind _returnvalue (`parent.GetBattleMain`))
  (return _returnvalue))

(fn `GetcurrentLevelCustom`
  (returns (Enable :type Boolean))
  (return false))

(fn `GetDebugGameTrace`
  (returns (IsEnable :type Boolean))
  (return false))

(fn `GetDeviceNotifySoundAssets`
  (returns (Cue :type "SoundAtomCue Object Reference"))
  (bind _cue (`parent.GetDeviceNotifySoundAssets`))
  (return _cue))

(fn `GetDeviceNotifyViewAssets`
  (returns (OutMaterial :type "MaterialInterface Object Reference") (OutFont :type "Font Object Reference"))
  (bind (_outmaterial _outfont) (`parent.GetDeviceNotifyViewAssets`))
  (return _outmaterial _outfont))

(fn `GetDifficultyMessage`
  (returns (ReturnValue :type "ScriptMessageAsset Object Reference"))
  (bind _returnvalue (`parent.GetDifficultyMessage`))
  (return _returnvalue))

(fn `GetEventBase`
  (returns (ReturnValue :type "EventBase Object Reference"))
  (bind _returnvalue (`parent.GetEventBase`))
  (return _returnvalue))

(fn `GetEventBattleActor`
  (returns (List :type "Array of Actor Object Reference"))
  (return))

(fn `GetGShopCamera`
  (returns (cam :type "CameraActor Object Reference"))
  (return null))

(fn `GetIsBattle`
  (returns (IsBattle :type Boolean))
  (return false))

(fn `GetJsonData`
  (returns (Json :type "JsonDataCtrl Object Reference"))
  (return null))

(fn `GetJsonFileName`
  (returns (FileName :type String))
  (return ""))

(fn `GetLoadMap`
  (returns (IsLoadMap :type Boolean))
  (return false))

(fn `GetMapChange`
  (returns (IsMapChange :type Boolean) (m_WarpPoint :type Integer) (m_FromEvent :type Integer) (m_OtherMapReturn :type Integer))
  (return false 0 0 0))

(fn `GetMapCommon`
  (returns (return :type "Actor Object Reference"))
  (return null))

(fn `GetMapStartLoadFlag`
  (returns (enable :type Boolean))
  (return false))

(fn `GetNextMapAssetList`
  (returns (LevelList :type "Array of /Game/Blueprints/Common/Map/Sublevel/Struct/LoadOnlyResident_ST Structure"))
  (return))

(fn `GetNextMapStartList`
  (returns (return :type "/Game/Blueprints/Common/Map/Sublevel/Struct/LoadOnlyResident_ST Structure"))
  (return))

(fn `GetSavingWidget`
  (returns (Widget :type Boolean))
  (return false))

(fn `GetSonySaveMessage`
  (returns (ReturnValue :type "ScriptMessageAsset Object Reference"))
  (bind _returnvalue (`parent.GetSonySaveMessage`))
  (return _returnvalue))

(fn `GetSystemMessage`
  (returns (ReturnValue :type "ScriptMessageAsset Object Reference"))
  (bind _returnvalue (`parent.GetSystemMessage`))
  (return _returnvalue))

(fn `GetTextureBoostMapWarpPoint`
  (params (MapWarpPoints :type "Array of MapWarpPoint Object Reference (by ref)"))
  (returns (ReturnValue :type "MapWarpPoint Object Reference"))
  (bind _returnvalue (`parent.GetTextureBoostMapWarpPoint` MapWarpPoints))
  (return _returnvalue))

(fn `IsBattleEnd`
  (returns (retValue :type Boolean))
  (return false))

(fn `IsEventHitOff`
  (returns (Enable :type Boolean))
  (return false))

(fn `IsLoadLevelGame`
  (returns (Enable :type Boolean))
  (return false))

(fn `IsNextMapLoadEnd`
  (returns (return :type Boolean))
  (return false))

(fn `IsNextMapLoadStart`
  (returns (return :type Boolean))
  (return false))

(fn `JsonCounterGet`
  (returns (EncountNum :type Integer) (Magatukanum :type Integer))
  (return 0 0))

(fn `RegisterMinimapIconTableAll`)

(fn `ReturnMapCamera`
  (params (FainalCameraPos :type "Transform Structure") (SetBtlResultCameraPos_0 :type "Transform Structure")))

(fn `ReturnMapFromBtl`)

(fn `SetKeyFreeEvent`
  (params (Actor :type "Actor Object Reference")))

(fn `SetLoadMap`
  (params (IsLoadMap :type Boolean)))

(fn `SetMapBEffectParamType`
  (params (Next :type "/Game/Blueprints/Map/Dungeon/MapBEffectParamType Enum" :default "NewEnumerator0")))

(fn `SetMapChange`
  (params (IsMapChange :type Boolean) (m_WarpPoint :type Integer) (m_FromEvent :type Integer) (m_OtherMapReturn :type Integer)))

(fn `SetMapCommon`
  (params (Actor :type "Actor Object Reference")))

(fn `StopKeyFreeEvent`)