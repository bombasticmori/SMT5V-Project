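; ProjectGameMode is a game mode Blueprint that outlines game startup, map and area streaming, garden levels and level changes, with nearly all logic left as empty stubs.
; Only BeginPlay, Tick, EndPlay, PreloadMap and the console auto-pause and reactivation events do anything, forwarding to the parent class.
; Map loading, debug trace and other events have empty bodies, and query functions return false or zero.
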(event `self.ReceiveBeginPlay`
  (`parent.ReceiveBeginPlay`))

(event `self.ReceiveTick`
  (params (DeltaSeconds :type "Float (single-precision)"))
  (`parent.ReceiveTick` DeltaSeconds))

(event `OnLoaded_A7E7758C4A4D3C8A1981CA8D45CB3767`
  (params (Loaded :type "Object Class Reference")))

(event `OnLoaded_A5C472BF496F2067C4FFFBB5841704CC`
  (params (Loaded :type "Object Class Reference")))

(event `/Game/Blueprints/Gamedata/BPI_GameMode.SetDaathAreaLock`
  (params (Lock :type Boolean)))

(event `/Game/Blueprints/Gamedata/BPI_GameMode.DaathSublevelManagerInit`)

(event `/Game/Blueprints/Gamedata/BPI_GameMode.DebugTraceStart`)

(event `/Game/Blueprints/Gamedata/BPI_GameMode.DebugTraceStop`)

(event `/Game/Blueprints/Gamedata/BPI_GameMode.DebugTraceView_Player`)

(event `/Game/Blueprints/Gamedata/BPI_GameMode.DebugTraceActivePos`
  (params (Action :type "/Game/Blueprints/Map/Debug/DebugTrace/DebugTrace_St_Action Structure")))

(event `/Game/Blueprints/Gamedata/BPI_GameMode.DebugTraceViewOFF`)

(event `GameLoadStart`)

(event `PlayerLoadStart`)

(event `MapLoadStart`)

(event `MapInitStart`)

(event `GamePlayStart`)

(event `GameInit`)

(event `/Game/Blueprints/Gamedata/BPI_GameMode.InitFadeCancel`)

(event `OtherSubLevelLoad`)

(event `/Game/Blueprints/Gamedata/BPI_GameMode.InitPause`)

(event `OnAllresidentLoadEnd`)

(event `Tick_ReadyMapInitStart`)

(event `/Game/Blueprints/Gamedata/BPI_GameMode.MapStartLoad`)

(event `/Game/Blueprints/Gamedata/BPI_GameMode.MapAllResidentDelete`
  (params (NextMap :type Integer) (NextArea :type Integer)))

(event `AllresidentLoadEnd_イベント_0`)

(event `/Game/Blueprints/Gamedata/BPI_GameMode.MapAreaLoad`
  (params (Map :type Integer) (Area :type Integer) (LoadAfterView :type Boolean)))

(event `/Game/Blueprints/Gamedata/BPI_GameMode.MapAreaUnload`
  (params (map :type Integer) (Area :type Integer)))

(event `/Game/Blueprints/Gamedata/BPI_GameMode.MapAreaView`
  (params (Map :type Integer) (Area :type Integer)))

(event `/Game/Blueprints/Gamedata/BPI_GameMode.MapUnResidentLoad`
  (params (MapID :type Integer) (AreaID :type Integer) (LoadAfterView :type Boolean)))

(event `/Game/Blueprints/Gamedata/BPI_GameMode.MapUnResidentUnLoad`
  (params (MapId :type Integer)))

(event `/Game/Blueprints/Gamedata/BPI_GameMode.MapUnResidentView`
  (params (MapID :type Integer)))

(event `/Game/Blueprints/Gamedata/BPI_GameMode.StartNextMapBGLoad`
  (params (MapID :type Integer) (AreaID :type Integer)))

(event `/Game/Blueprints/Gamedata/BPI_GameMode.MapOpenLevel`
  (params (old_mapID :type Integer) (Old_AreaID :type Integer) (New_MapID :type Integer) (New_AreaId :type Integer)))

(event `/Game/Blueprints/Gamedata/BPI_GameMode.MapInitEnd`)

(event `/Game/Blueprints/Gamedata/BPI_GameMode.NextMapBGUnLoad`)

(event `/Game/Blueprints/Gamedata/BPI_GameMode.MapSystemBKLoad`
  (params (MapID :type Integer) (Type :type "/Game/Blueprints/Common/Map/LevelCtrl/E_MAP_SYSTEMRESIDENT_ID Enum" :default "NewEnumerator0")))

(event `/Game/Blueprints/Gamedata/BPI_GameMode.MapSystemBKUnLoad`
  (params (MapID :type Integer) (Type :type "/Game/Blueprints/Common/Map/LevelCtrl/E_MAP_SYSTEMRESIDENT_ID Enum" :default "NewEnumerator0")))

(event `/Game/Blueprints/Gamedata/BPI_GameMode.MapSystemBKView`
  (params (MapID :type Integer) (Type :type "/Game/Blueprints/Common/Map/LevelCtrl/E_MAP_SYSTEMRESIDENT_ID Enum" :default "NewEnumerator0")))

(event `/Game/Blueprints/Gamedata/BPI_GameMode.MapSystem_StreamOnlyUnLoad`
  (params (MapId :type Integer) (type :type "/Game/Blueprints/Common/Map/LevelCtrl/E_MAP_SYSTEMRESIDENT_ID Enum" :default "NewEnumerator0")))

(event `/Game/Blueprints/Gamedata/BPI_GameMode.MapSystem_StreamOnlyLoad`
  (params (MapID :type Integer) (Type :type "/Game/Blueprints/Common/Map/LevelCtrl/E_MAP_SYSTEMRESIDENT_ID Enum" :default "NewEnumerator0")))

(event `/Game/Blueprints/Gamedata/BPI_GameMode.LevelChange`
  (params (UnLoad :type "PrimaryAssetId Structure") (Load :type "PrimaryAssetId Structure")))

(event `/Game/Blueprints/Gamedata/BPI_GameMode.EndLoadUnResident`)

(event `/Game/Blueprints/Gamedata/BPI_GameMode.MapSystemBKHide`
  (params (MapID :type Integer) (Type :type "/Game/Blueprints/Common/Map/LevelCtrl/E_MAP_SYSTEMRESIDENT_ID Enum" :default "NewEnumerator0")))

(event `/Game/Blueprints/Gamedata/BPI_GameMode.MapAreaChange`
  (params (MapId :type Integer) (CurrentAreaId :type Integer) (NewAreaId :type Integer) (LoadAfterView :type Boolean)))

(event `/Game/Blueprints/Gamedata/BPI_GameMode.StartGardenUnload`
  (params (MapID :type Integer)))

(event `/Game/Blueprints/Gamedata/BPI_GameMode.StartGardenLoad`
  (params (MapID :type Integer) (WarpPoint :type Integer) (LoadAfterView :type Boolean)))

(event `self.ReceiveEndPlay`
  (params (EndPlayReason :type "EEndPlayReason Enum" :default "Destroyed"))
  (`parent.ReceiveEndPlay` EndPlayReason))

(event `/Game/Blueprints/Gamedata/BPI_GameMode.ForceTraport`)

(event `self.PreloadMap`
  (params (mapId :type Integer) (AreaId :type Integer))
  (`parent.PreloadMap` mapId AreaId))

(event `EndAreaInit_`)

(event `self.CallAutoPause_ForConsumer`
  (`parent.CallAutoPause_ForConsumer`))

(event `self.CallReactivatedApp_ForConsumer`
  (`parent.CallReactivatedApp_ForConsumer`))

(event `OnDestroyed_AutoPause`
  (params (DestroyedActor :type "Actor Object Reference")))

(fn `ApplyMissionMapBGM`
  (returns (dummy :type Boolean))
  (return false))

(fn `GetGardenWarpPoint`
  (returns (WarpPoint :type Integer))
  (return 0))

(fn `IsBGLoadMapArea`
  (returns (emd :type Boolean))
  (return false))

(fn `IsGameStart`
  (returns (enable :type Boolean))
  (return false))

(fn `IsGardenLoaded`
  (returns (end :type Boolean))
  (return false))

(fn `IsGardenOpen`
  (params (MapID :type Integer))
  (returns (IsGardenOpen :type Boolean))
  (return false))

(fn `IsInGardenLevel`
  (returns (IsInGardenLevel :type Boolean))
  (return false))

(fn `IsLoadMapArea`
  (returns (end :type Boolean))
  (return false))

(fn `IsLoadMapUnResident`
  (params (MapID :type Integer))
  (returns (LoadAfterView :type Boolean))
  (return false))

(fn `IsMapEventPlaying`
  (returns (IsMapEventPlaying :type Boolean))
  (return false))

(fn `IsMapSystemBKLoadEnd`
  (params (MapID :type Integer) (type :type "/Game/Blueprints/Common/Map/LevelCtrl/E_MAP_SYSTEMRESIDENT_ID Enum" :default "NewEnumerator0"))
  (returns (end :type Boolean))
  (return false))

(fn `IsMapSystemHideEnd`
  (returns (End :type Boolean))
  (return false))

(fn `IsMapSystemLevelLoadEnd`
  (params (MapID :type Integer) (Type :type "/Game/Blueprints/Common/Map/LevelCtrl/E_MAP_SYSTEMRESIDENT_ID Enum" :default "NewEnumerator0"))
  (returns (End :type Boolean))
  (return false))

(fn `IsMapSystemOnlyLoadEnd`
  (returns (End :type Boolean))
  (return false))

(fn `IsMapSystemUnloadEnd`
  (returns (End :type Boolean))
  (return false))

(fn `IsNextMapBGLoadEnd`
  (returns (end :type Boolean))
  (return false))

(fn `IsUnLoadMapArea`
  (returns (end :type Boolean))
  (return false))

(fn `SetMapEventPlaying`
  (params (IsMapEventPlaying :type Boolean))
  (returns (Dummy :type Boolean))
  (return false))

(fn `UserConstructionScript`)