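; BP_TitleMovieCtrl2 is a variant of a title-screen movie controller that stubs out much of its inherited interface.
; Starting the controller, seek completion on the Mana component, mouse visibility and pause setting are empty, and the end check always returns false.
; Lifecycle events, pause-movie events and the talk-part, pause and playback queries simply forward to the parent class.
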(event `self.ReceiveBeginPlay`
  (`parent.ReceiveBeginPlay`))

(event `self.ReceiveTick`
  (params (DeltaSeconds :type "Float (single-precision)"))
  (`parent.ReceiveTick` DeltaSeconds))

(event `self.ReceiveEndPlay`
  (params (EndPlayReason :type "EEndPlayReason Enum" :default "Destroyed"))
  (`parent.ReceiveEndPlay` EndPlayReason))

(event `/Game/Blueprints/Title/BPI_TitleMovieCtrl.StartTitleMovieCtrl`
  (params (IsFirstMovie :type Boolean)))

(event `self.StartPauseMovieEvent`
  (`parent.StartPauseMovieEvent`))

(event `self.EndPauseMovieEvent`
  (`parent.EndPauseMovieEvent`))

(event `self.PauseMovie`
  (`parent.PauseMovie`))

(event `private_SeekCompleteNext`
  (params (FrameNumber :type Integer) (ManaComponent :type "ManaComponent Object Reference")))

(fn `CheckPauseEvent`
  (returns (ReturnValue :type Boolean))
  (bind _returnvalue (`parent.CheckPauseEvent`))
  (return _returnvalue))

(fn `IsEndTitleMovieCtrl`
  (returns (IsEnd :type Boolean))
  (return false))

(fn `IsPauseMovieEvent`
  (returns (ReturnValue :type Boolean))
  (bind _returnvalue (`parent.IsPauseMovieEvent`))
  (return _returnvalue))

(fn `IsPlayingMovieEvent`
  (returns (ReturnValue :type Boolean))
  (bind _returnvalue (`parent.IsPlayingMovieEvent`))
  (return _returnvalue))

(fn `IsTalkPart`
  (returns (ReturnValue :type Boolean))
  (bind _returnvalue (`parent.IsTalkPart`))
  (return _returnvalue))

(fn `SetMyMouseVisibility`
  (params (Show :type Boolean)))

(fn `SetMyPause`
  (params (m_IsPause :type Boolean)))

(fn `UserConstructionScript`)