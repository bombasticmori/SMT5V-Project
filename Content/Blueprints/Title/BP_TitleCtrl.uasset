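; BP_TitleCtrl is a title screen controller actor, laid out to run the top menu, continue, options, difficulty select, convert and copyright screens.
; Its interface pairs per-screen tick-start and tick functions with spawners for sub-controllers, plus cursor, mouse, yes/no dialog and end-result functions.
; Function bodies here are empty or return fixed defaults, and the lifecycle events that do anything only call their parent.
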(event `self.ReceiveBeginPlay`
  (`parent.ReceiveBeginPlay`))

(event `self.ReceiveTick`
  (params (DeltaSeconds :type "Float (single-precision)"))
  (`parent.ReceiveTick` DeltaSeconds))

(event `OnLoaded_39B295964692A44CB6EAE6A93C776812`
  (params (Loaded :type "Object Class Reference")))

(event `OnLoaded_74EC4B344489C4AD2B7E65945E9C49A2`
  (params (Loaded :type "Object Class Reference")))

(event `OnLoaded_2D484EA94E42E2485BA45CAB3377E4D6`
  (params (Loaded :type "Object Class Reference")))

(event `OnLoaded_70DE6DFF41872028BF2E12927655FE49`
  (params (Loaded :type "Object Class Reference")))

(event `OnLoaded_F626ACB2404288A4FBFAD08736779276`
  (params (Loaded :type "Object Class Reference")))

(event `OnLoaded_73E854CA4A4A00CCF0276EAD888280E9`
  (params (Loaded :type "Object Class Reference")))

(event `self.ReceiveDestroyed`
  (`parent.ReceiveDestroyed`))

(event `/Game/Blueprints/Title/BPI_TitleCtrl.StartCtrl`)

(event `private_Initialize`)

(event `self.ReceiveEndPlay`
  (params (EndPlayReason :type "EEndPlayReason Enum" :default "Destroyed"))
  (`parent.ReceiveEndPlay` EndPlayReason))

(event `private_LoadHeader`)

(fn `ChangeTopCursor`
  (params (add :type Integer) (set :type Integer) (isLimitStop :type Boolean)))

(fn `DecideTopSelection`
  (params (Index :type Integer)))

(fn `DestroyCreatedObj`)

(fn `DialogCtrlInput`
  (returns (InputButtonNum :type Integer) (InputCursorNum :type Integer) (IsTriggerInput :type Boolean))
  (return 0 0 false))

(fn `DialogCtrlUpdate`
  (returns (SelectedYes :type Boolean) (SelectedNo :type Boolean))
  (return false false))

(fn `DispFunc_OnClickedMouse`
  (params (Index :type Integer)))

(fn `DispFunc_OnHoveredMouse`
  (params (Index :type Integer)))

(fn `EndCtrl`
  (params (in_EndType :type "/Game/Blueprints/Title/E_TitleEndType Enum" :default "NewEnumerator0") (in_NewGameType :type "/Game/Blueprints/Title/E_NewGameType Enum" :default "NewEnumerator3") (in_SaveDataID :type Integer)))

(fn `GetBenefitData`
  (returns (Data :type "BenefitData Structure"))
  (return))

(fn `GetDifficulty`
  (returns (Difficulty :type "E_GAME_DIFFICULTY Enum"))
  (return "E_GAME_EASY"))

(fn `GetEndType`
  (returns (Type :type "/Game/Blueprints/Title/E_TitleEndType Enum"))
  (return "NewEnumerator0"))

(fn `GetNewgameType`
  (returns (Type :type "/Game/Blueprints/Title/E_NewGameType Enum"))
  (return "NewEnumerator3"))

(fn `GetSaveDataIndex`
  (returns (ID :type Integer))
  (return 0))

(fn `HelpWindowExecutionClose`)

(fn `IsEndTitleCtrl`
  (returns (IsEnd :type Boolean))
  (return false))

(fn `OpenDialogYesNo`
  (params (InScriptMessageAsset :type "ScriptMessageAsset Object Reference") (DialogTextLabel :type Name) (InitCursorPosition :type Integer)))

(fn `SpawnBenefitSelectCtrl`)

(fn `SpawnConvertCtrl`)

(fn `SpawnCopyrightCtrl`)

(fn `SpawnDifficultySelectCtrl`)

(fn `SpawnItemMovieCtrl`)

(fn `SpawnOptionCtrl`)

(fn `TickFunc_Continue`)

(fn `TickFunc_Convert`)

(fn `TickFunc_Copyright`)

(fn `TickFunc_DifficultySelect`)

(fn `TickFunc_Initializing`)

(fn `TickFunc_Option`)

(fn `TickFunc_SelectEnd`)

(fn `TickFunc_TitleTop`
  (params (DeltaSeconds :type "Float (double-precision)")))

(fn `TickStartContinue`)

(fn `TickStartDifficultySelect`)

(fn `TickStartOption`)

(fn `TickStartOption_Convert`)

(fn `TickStartOption_Copyright`)

(fn `TickStartOption_SelectEnd`)

(fn `TickStartTitleTop`)

(fn `UpdateTopInput`
  (returns (ButtonNum :type Integer) (CursorNum :type Integer) (TriggerNum :type Boolean))
  (return 0 0 false))

(fn `UserConstructionScript`)