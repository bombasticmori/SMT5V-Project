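; BP_Result_TopCtrl is, by its naming, the top-level controller for the Result screen, covering UI, camera, page changes and transitions.
; Its functions outline a lifecycle of init mode, data setup, model load request, control start, UI close and transition out, with completion checks.
; Every function here is an empty stub or returns false; BeginPlay, Tick and EndPlay only call the parent.
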(event `self.ReceiveBeginPlay`
  (`parent.ReceiveBeginPlay`))

(event `self.ReceiveTick`
  (params (DeltaSeconds :type "Float (single-precision)"))
  (`parent.ReceiveTick` DeltaSeconds))

(event `self.ReceiveEndPlay`
  (params (EndPlayReason :type "EEndPlayReason Enum" :default "Destroyed"))
  (`parent.ReceiveEndPlay` EndPlayReason))

(fn `BindFunc_OnMovedScrollBarByMouse`
  (params (InScrollRate :type "Float (double-precision)")))

(fn `ButtonCheck`
  (returns (ReturnValue :type Boolean))
  (return false))

(fn `ChangeTopCamera`)

(fn `CloseUI`
  (params (Immediate :type Boolean))
  (returns (dummy :type Boolean))
  (return false))

(fn `DestroyUI`)

(fn `ImmediateInit`
  (returns (dummy :type Boolean))
  (return false))

(fn `IsEndCloseUI`
  (returns (IsEnd :type Boolean))
  (return false))

(fn `IsEndCtrl`
  (returns (IsEnd :type Boolean))
  (return false))

(fn `IsEndTransitionOut`
  (returns (IsEnd :type Boolean))
  (return false))

(fn `IsEndVIewCover`
  (returns (IsEnd :type Boolean))
  (return false))

(fn `IsInitialized`
  (returns (comp :type Boolean))
  (return false))

(fn `ModelLoadReq`
  (returns (Return :type Boolean))
  (return false))

(fn `PageChangeButton`
  (returns (ReturnValue :type Boolean))
  (return false))

(fn `PageChangeSeq`)

(fn `ReplaceFillScreen`
  (returns (success :type Boolean))
  (return false))

(fn `SetInitMode`
  (params (Battle :type Boolean) (Field :type Boolean))
  (returns (Dummy :type Boolean))
  (return false))

(fn `SetTopDataObj`
  (params (ResultTopDataObj :type "Object Object Reference"))
  (returns (Success :type Boolean))
  (return false))

(fn `StartCtrl`
  (params (FuncDispObj :type "Object Object Reference"))
  (returns (success :type Boolean))
  (return false))

(fn `StartTransitionOut`
  (params (White :type Boolean))
  (returns (Dummy :type Boolean))
  (return false))

(fn `UserConstructionScript`)