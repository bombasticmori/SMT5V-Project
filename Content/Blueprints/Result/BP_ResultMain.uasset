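; BP_ResultMain is a result-screen controller Blueprint, apparently for post-battle results given its FromBattle, currency and item inputs.
; BeginPlay and Hide Env Request both invoke CallDispHideEnv, which is defined outside this file.
; The remaining events and functions, covering initialization, level-up, environment spawning, widget cleanup and asset-load callbacks, are stubs that do nothing or return false, apart from Tick's parent call.
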(event `self.ReceiveBeginPlay`
  (`parent.ReceiveBeginPlay`)
  (`self.Disp_HideEnv`))

(event `self.ReceiveTick`
  (params (DeltaSeconds :type "Float (single-precision)"))
  (`parent.ReceiveTick` DeltaSeconds))

(event `OnLoaded_27939E0B40F528B0353C0BBDF3120BDF`
  (params (Loaded :type "Object Class Reference")))

(event `OnLoaded_5A30892A4E57C587DD48E2A1CB80FA41`
  (params (Loaded :type "Object Class Reference")))

(event `OnLoaded_FFB235B8426CC5BF55A5F7A71EE8107E`
  (params (Loaded :type "Object Class Reference")))

(event `OnLoaded_287509E74C0EDFCBA0D1BB880CBBC8A7`
  (params (Loaded :type "Object Class Reference")))

(event `OnLoaded_595AAE5C4A6524C0BF1213B778433B44`
  (params (Loaded :type "Object Class Reference")))

(event `OnLoaded_F460E84B40DD7CBF6B8D519A35AE3A21`
  (params (Loaded :type "Object Class Reference")))

(event `private_SpawnEnvironment`)

(event `EndAllEvent`)

(event `CalcLevelUp`)

(event `StartResult`)

(event `private_Init`)

(fn `AfterScreenIsCovered`
  (returns (Dummy :type Boolean))
  (return false))

(fn `ClearMsgText`)

(fn `ClearWidgetAndActor`
  (returns (Finished :type Boolean))
  (return false))

(fn `CloseHelpWindow`)

(fn `DestroyEventDataObject`)

(fn `GetIsEndInTransition`
  (returns (IsEnd :type Boolean))
  (return false))

(fn `Hide Env Request`
  (`self.Disp_HideEnv`))

(fn `Initialize`
  (params (FromBattle :type Boolean) (GetMakkaInResult :type Boolean) (GetItemInResult :type Boolean) (EndFadeOutWhite :type Boolean))
  (returns (Success :type Boolean))
  (return false))

(fn `IsEndResult`
  (returns (IsEnd :type Boolean))
  (return false))

(fn `IsInitialized`
  (returns (Complete :type Boolean))
  (return false))

(fn `SetOtherEnvWait`
  (params (m_OtherEnvEndWait :type Boolean)))

(fn `SpawnComplete`
  (returns (complete :type Boolean))
  (return false))

(fn `UpdateWidgetMode`)

(fn `UserConstructionScript`)