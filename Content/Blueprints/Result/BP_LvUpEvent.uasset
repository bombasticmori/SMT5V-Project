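; Level-up event Blueprint for the result flow, covering hero stat allocation and ally (Nkm) skill learning, discarding and gifts, with Garden, Camp and Unite variants.
; Function names outline an event state machine with paired Start and TickEvent steps, switched through SetNextEvent and EventChangeFunc.
; Helpers cover dialogs, messages, button and mouse input, voice and status camera.
; All bodies here are empty or return defaults, except parent BeginPlay, Tick and EndPlay calls.
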(event `self.ReceiveBeginPlay`
  (`parent.ReceiveBeginPlay`))

(event `self.ReceiveTick`
  (params (DeltaSeconds :type "Float (single-precision)"))
  (`parent.ReceiveTick` DeltaSeconds))

(event `OnLoaded_29F745DC45C64BF7A176EEA5E1FE8305`
  (params (Loaded :type "Object Object Reference")))

(event `self.ReceiveEndPlay`
  (params (EndPlayReason :type "EEndPlayReason Enum" :default "Destroyed"))
  (`parent.ReceiveEndPlay` EndPlayReason))

(event `Private_LoadDevilMessageAsset`)

(event `Private_EndLvUpProcess`)

(event `private_StartCtrl`)

(fn `AddDistParam`
  (params (Param :type Integer)))

(fn `BindFunc_OnClickedParamCursor`
  (params (add :type Integer)))

(fn `BindFunc_OnClickedSkillSlot`
  (params (Index :type Integer)))

(fn `BindFunc_OnHoveredParamPanel`
  (params (Index :type Integer)))

(fn `BindFunc_OnHoveredSkillSlot`
  (params (Index :type Integer)))

(fn `BindFunc_OnMovedRightScrollBarByMouse`
  (params (NewOffset :type Integer)))

(fn `BtnHelpUpdate`
  (params (ForceOpen :type Boolean)))

(fn `ButtonCheckAnyButton`)

(fn `ButtonCheckHeroParamUp`)

(fn `ButtonCheckNkmGetSkill`)

(fn `ButtonCheckSelectMsg`)

(fn `ButtonCheckShowParam`)

(fn `Calc Move Index by Wheel`
  (params (InOffset :type Integer) (InMove :type Integer))
  (returns (CursorDataIndex :type Integer) (ScrollStack :type Integer) (CurosrMoved :type Boolean))
  (return 0 0 false))

(fn `CharaChangeInit`)

(fn `Close Btn Help`
  (params (SkipAnimation :type Boolean)))

(fn `CloseDialog`)

(fn `CloseHelpWindowImmediate`)

(fn `CloseMessage`)

(fn `CloseMessageImmediate`)

(fn `CloseUI`
  (params (Immediate :type Boolean))
  (returns (dummy :type Boolean))
  (return false))

(fn `EndAllEvent`)

(fn `EventChangeFunc`)

(fn `G_TickEvent`)

(fn `GetCurrentSumParam`
  (returns (CurrentParam :type Integer))
  (return 0))

(fn `GetDistParam`
  (returns (Param :type Integer))
  (return 0))

(fn `GetEnableMouseCtrl`
  (returns (ReturnValue :type Boolean))
  (return false))

(fn `GetStatusObj`
  (returns (StatudDataObj :type "Object Object Reference"))
  (return null))

(fn `GotoNextCharacter`
  (returns (allEventEnd :type Boolean))
  (return false))

(fn `Grow Up For Camp Item`
  (params (nkmIndex :type Integer) (upLv :type Integer))
  (returns (ExistLvUpChara :type Boolean))
  (return false))

(fn `GrowUpFromResultData`
  (params (ResultData :type "ResultData Structure (by ref)"))
  (returns (ExistLvUpChara :type Boolean))
  (return false))

(fn `HW_SetGardenStartMessage`
  (params (InChangeAnime :type Boolean)))

(fn `HW_SetLvUpMessage`
  (params (InChangeAnime :type Boolean)))

(fn `HW_WindowClose`)

(fn `InitializeLvUpEvent`
  (params (CharaChanger :type "Actor Object Reference"))
  (returns (Success :type Boolean))
  (return false))

(fn `IsEmptySlotExist`
  (returns (Exist :type Boolean))
  (return false))

(fn `IsEnd`
  (returns (NewParam :type Boolean))
  (return false))

(fn `IsEndCloseUI`
  (returns (IsEnd :type Boolean))
  (return false))

(fn `IsEndLvUpEvent`
  (returns (IsEnd :type Boolean))
  (return false))

(fn `IStartEvent`
  (params (NewParam :type "LevelUpManager Object Reference")))

(fn `LvUpEventStart`
  (returns (dummy :type Boolean))
  (return false))

(fn `MW_CheckButtonNext`
  (params (SelectMenu :type Boolean))
  (returns (Return :type Boolean))
  (return false))

(fn `MW_InitAutoTime`)

(fn `MW_SetAutoTime`
  (params (msgCtrl :type "Object Object Reference")))

(fn `MW_UpdateAuto`
  (returns (IsAuto :type Boolean))
  (return false))

(fn `MW_UpdateSkip`
  (returns (Skip :type Boolean))
  (return false))

(fn `OpenDialog`
  (params (InScriptMessageAsset :type "ScriptMessageAsset Object Reference") (InLabel :type Name)))

(fn `OpenMessage`
  (params (argScriptMessageAsset :type "ScriptMessageAsset Object Reference") (DevilID :type Integer) (argLabel :type Name) (MsgSelectItemName :type "Array of Name (by ref)") (`Program 0 Text` :type String)))

(fn `PlayGardenFlashSE`)

(fn `PlaySE`
  (params (SE :type "ESystemSE Enum" :default "Cursor")))

(fn `Pre Init Garden Result`
  (params (gardenResultData :type "GardenResultData Structure") (gardenSystemMsg :type "ScriptMessageAsset Object Reference"))
  (returns (Success :type Boolean))
  (return false))

(fn `PreInitCampAllocateResult`
  (params (`M Hero Bonus Point` :type Integer))
  (returns (Success :type Boolean))
  (return false))

(fn `PreLoadModel`
  (returns (Dummy :type Boolean))
  (return false))

(fn `SetNextEvent`
  (params (NextEventType :type "E_LVUPMANAGER_GSTATUS Enum" :default "E_LVUPMANAGER_GSTATUS_EMPTY") (WaitDeltaSeconds :type "Float (double-precision)") (Immediate :type Boolean)))

(fn `SetSkillHelpMessage`)

(fn `StartCampAllocateEvent`
  (params (NewParam :type "LevelUpManager Object Reference")))

(fn `StartGardenEvent`
  (params (NewParam :type "LevelUpManager Object Reference")))

(fn `StartGardenHeroAllocateStartMess`)

(fn `StartGardenHeroParamDialog`)

(fn `StartGardenHeroParamNotYetMess`)

(fn `StartGardenHeroParamUp`)

(fn `StartGardenParamUpMess`)

(fn `StartGardenShowParam`)

(fn `StartGardenTekiseiUpMess`)

(fn `StartHeroAllocateStartMess`)

(fn `StartHeroCloseUI`)

(fn `StartHeroGetGodParam`)

(fn `StartHeroParamDialog`)

(fn `StartHeroParamNotYetMess`)

(fn `StartHeroParamUp`)

(fn `StartNewCharaIn`)

(fn `StartNkmCloseUI`)

(fn `StartNkmDiscardStartMess`)

(fn `StartNkmGetExSkill`)

(fn `StartNkmGetGift`)

(fn `StartNkmGetSkill`)

(fn `StartNkmGetSkillAkirame`)

(fn `StartNkmGetSkillDecide`)

(fn `StartNkmGetSkillMaeoki`)

(fn `StartNkmGiftSystemMess`)

(fn `StartNkmLearnSkillAnim`)

(fn `StartNkmNextSkillFlash`)

(fn `StartShowUpParam`)

(fn `StatusCameraEnd`
  (returns (Success :type Boolean))
  (return false))

(fn `StatusCameraStart`
  (params (CharaChanger :type "Actor Object Reference"))
  (returns (Success :type Boolean))
  (return false))

(fn `TickEventGardenHeroAllocateStartMess`)

(fn `TickEventGardenHeroParamDialog`)

(fn `TickEventGardenHeroParamNotYetMess`)

(fn `TickEventGardenHeroParamUp`)

(fn `TickEventGardenParamUpMess`)

(fn `TickEventGardenShowParam`)

(fn `TickEventGardenTekiseiUpMess`)

(fn `TickEventHeroAllocateStartMess`)

(fn `TickEventHeroGetGodParam`)

(fn `TickEventHeroParamDialog`)

(fn `TickEventHeroParamNotYetMess`)

(fn `TickEventHeroParamUp`)

(fn `TickEventNkmDiscardStartMess`)

(fn `TickEventNkmGetGift`)

(fn `TickEventNkmGetSkill`)

(fn `TickEventNkmGetSkillAkirame`)

(fn `TickEventNkmGetSkillDecide`)

(fn `TickEventNkmGetSkillMaeoki`)

(fn `TickEventNkmGiftSystemMess`)

(fn `TickEventNkmLearnSkillAnim`)

(fn `TickEventNkmNextSkillFlash`)

(fn `TickEventShowParam`)

(fn `TryCreateLvUpEvent_ForUnite`
  (params (resultNkmIndex :type Integer))
  (returns (HappenLvUpEvent :type Boolean))
  (return false))

(fn `UpdateButtonHelp`)

(fn `UserConstructionScript`)

(fn `VoiceRequest`
  (params (m_VoiceReq :type "EDevilVoiceType Enum" :default "EDevilVoiceType_None")))

(fn `WaitSystemAnimCheck`
  (returns (Complete :type Boolean))
  (return false))