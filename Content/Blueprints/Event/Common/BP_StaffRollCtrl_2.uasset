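; BP_StaffRollCtrl_2 is a staff roll controller whose graphs here are an empty skeleton.
; It declares functions for init by movie time or speed, playback, speed and slow-down, color fades, name and font changes, and widget removal, plus BI-prefixed counterparts for external control.
; All bodies are empty or return false or zero, except Tick, which only forwards to the parent.
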(event `self.ReceiveTick`
  (params (DeltaSeconds :type "Float (single-precision)"))
  (`parent.ReceiveTick` DeltaSeconds))

(event `/Game/Blueprints/Event/Common/BPI_StaffRollCtrl.BI_Init`
  (params (MovieTime :type "Float (single-precision)") (StartRate :type "Float (single-precision)") (StartFadeTime :type "Float (single-precision)") (EndFadeTime :type "Float (single-precision)") (FadeColor :type "LinearColor Structure") (UseSlowDown :type Boolean)))

(event `/Game/Blueprints/Event/Common/BPI_StaffRollCtrl.BI_Stop`
  (params (FadeTime :type "Float (single-precision)")))

(event `/Game/Blueprints/Event/Common/BPI_StaffRollCtrl.BI_Pause`)

(event `/Game/Blueprints/Event/Common/BPI_StaffRollCtrl.BI_Play`)

(event `/Game/Blueprints/Event/Common/BPI_StaffRollCtrl.BI_RemoveWidget`)

(fn `BI_GetIsFinished`
  (returns (IsFinished :type Boolean))
  (return false))

(fn `ChangeAllName`
  (params (Name :type String)))

(fn `ChangeFontSize`
  (params (FontSize :type Integer)))

(fn `FadeInColor`
  (params (FadeTime :type "Float (double-precision)") (FadeColor :type "LinearColor Structure")))

(fn `FadeOutColor`
  (params (FadeTime :type "Float (double-precision)") (FadeColor :type "LinearColor Structure")))

(fn `Get Is Finished`
  (returns (isFinished :type Boolean))
  (return false))

(fn `GetFadeFinished`
  (returns (FadeFinished :type Boolean))
  (return false))

(fn `GetIsPaused`
  (returns (isPaused :type Boolean))
  (return false))

(fn `GetIsPlaying`
  (returns (isPlaying :type Boolean))
  (return false))

(fn `GetIsSlowDown`
  (returns (isSlowDown :type Boolean))
  (return false))

(fn `GetNeedSlowDown`
  (returns (lastListAdded :type Boolean))
  (return false))

(fn `GetSpeed`
  (returns (ReturnSpeed :type "Float (double-precision)"))
  (return 0.0))

(fn `Init`
  (params (MovieTime :type "Float (double-precision)") (StartRate :type "Float (double-precision)") (StartFadeTime :type "Float (double-precision)") (EndFadeTime :type "Float (double-precision)") (FadeColor :type "LinearColor Structure") (UseSlowDown :type Boolean)))

(fn `InitBySpeed`
  (params (Speed :type "Float (double-precision)") (StartRate :type "Float (double-precision)") (StartFadeTime :type "Float (double-precision)") (EndFadeTime :type "Float (double-precision)") (FadeColor :type "LinearColor Structure") (UseSlowDown :type Boolean)))

(fn `InputCheck`)

(fn `Pause`)

(fn `Play`)

(fn `RemoveWidget`)

(fn `Set Speed Rate`
  (params (Rate :type Integer)))

(fn `SetParallelNum`
  (params (ParallelNum :type Integer)))

(fn `SetSpeed`
  (params (speed :type "Float (double-precision)")))

(fn `SlowDown`
  (params (SlowDownTime :type "Float (double-precision)")))

(fn `Stop`
  (params (FadeTime :type "Float (double-precision)")))

(fn `UserConstructionScript`)