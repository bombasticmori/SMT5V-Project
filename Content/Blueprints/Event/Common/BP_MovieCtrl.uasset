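; BP_MovieCtrl is a movie controller Blueprint under common event assets, exposing playback, pause, help and talk-part hooks.
; Pause-movie events, pause and playing-state checks, the talk-part check and Tick simply forward to the parent class.
; Playback, setup, help and start/end pause functions are empty stubs, and the prepare and end checks always return false, so this asset adds no behavior of its own.
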(event `self.ReceiveTick`
  (params (DeltaSeconds :type "Float (single-precision)"))
  (`parent.ReceiveTick` DeltaSeconds))

(event `PauseEvent`)

(event `self.PauseMovie`
  (`parent.PauseMovie`))

(event `self.StartPauseMovieEvent`
  (`parent.StartPauseMovieEvent`))

(event `self.EndPauseMovieEvent`
  (`parent.EndPauseMovieEvent`))

(fn `CheckPauseEvent`
  (returns (ReturnValue :type Boolean))
  (bind _returnvalue (`parent.CheckPauseEvent`))
  (return _returnvalue))

(fn `CloseHelp`)

(fn `EndPause`)

(fn `Finish`)

(fn `IsEnd`
  (returns (IsEnd :type Boolean))
  (return false))

(fn `IsPauseMovieEvent`
  (returns (ReturnValue :type Boolean))
  (bind _returnvalue (`parent.IsPauseMovieEvent`))
  (return _returnvalue))

(fn `IsPlayingMovieEvent`
  (returns (ReturnValue :type Boolean))
  (bind _returnvalue (`parent.IsPlayingMovieEvent`))
  (return _returnvalue))

(fn `IsPrepare`
  (returns (IsPrepare :type Boolean))
  (return false))

(fn `IsTalkPart`
  (returns (ReturnValue :type Boolean))
  (bind _returnvalue (`parent.IsTalkPart`))
  (return _returnvalue))

(fn `OpenHelp`)

(fn `Play`)

(fn `Prepare`)

(fn `Reset`)

(fn `SetData`
  (params (Texture :type "ManaTexture Object Reference") (Sound :type "SoundAtomCue Object Reference")))

(fn `StartPause`)

(fn `Stop`)

(fn `TickHelp`
  (params (DeltaTime :type "Float (double-precision)")))

(fn `UserConstructionScript`)