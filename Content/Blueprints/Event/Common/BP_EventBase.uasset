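; Base Blueprint for in-game story events and cutscenes, declaring a shared API for sequence playback, messages, choices, character motion, audio, screen effects and skipping.
; Nearly every function is an empty stub returning default values, including the BI_EB play-start and finish checks.
; Only lifecycle events, movie pause events and a few talk and movie state queries forward to the parent class.
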(event `self.ReceiveBeginPlay`
  (`parent.ReceiveBeginPlay`))

(event `self.ReceiveTick`
  (params (DeltaSeconds :type "Float (single-precision)"))
  (`parent.ReceiveTick` DeltaSeconds))

(event `self.ReceiveEndPlay`
  (params (EndPlayReason :type "EEndPlayReason Enum" :default "Destroyed"))
  (`parent.ReceiveEndPlay` EndPlayReason))

(event `AutoPlaySE`
  (params (SoundID :type String) (Volume :type "Float (double-precision)") (Pitch :type "Float (double-precision)") (Time :type "Float (double-precision)")))

(event `self.PauseMovie`
  (`parent.PauseMovie`))

(event `self.StartPauseMovieEvent`
  (`parent.StartPauseMovieEvent`))

(event `self.EndPauseMovieEvent`
  (`parent.EndPauseMovieEvent`))

(event `CE_DebugOutputTextTIme`)

(fn `_GetSelectionVoiceArray`
  (params (VoiceArray :type "Array of AtomSound Object Reference (by ref)"))
  (returns (Voice :type "AtomSound Object Reference"))
  (return null))

(fn `AddSelection`
  (params (Image :type "Image Object Reference") (LookAt :type "/Game/Blueprints/Event/Common/BP_EventLookAt Object Reference") (Facial :type Name) (Motion :type "AnimSequence Object Reference") (Emitter :type "Emitter Object Reference") (NextStep :type Integer) (InputKey :type "E_ACTION_MAPPING_TYPE Enum" :default "E_ACTION_MAPPING_ACTION") (VoiceSE :type "Array of AtomSound Object Reference (by ref)")))

(fn `AddVisibleLevel`
  (params (LevelName :type Name) (Visible :type Boolean)))

(fn `AttachMesh`
  (params (Tag :type Name) (SrcMesh :type Name) (DestMesh :type Name) (DestBone :type Name)))

(fn `AutoMotion`
  (params (Tag :type Name) (IsLoop :type Boolean) (BlendTime :type "Float (double-precision)") (OffsetTime :type "Float (double-precision)") (EventTime :type "Float (double-precision)")))

(fn `BI_EB_IsFinish`
  (returns (Finish :type Boolean))
  (return false))

(fn `BI_EB_PlayStart`
  (returns (NoUse :type Boolean))
  (return false))

(fn `ChangeColorFade`
  (params (FinalColor :type "LinearColor Structure") (Time :type "Float (double-precision)") (Additive :type Boolean)))

(fn `ChangeCueVolume`
  (params (Category :type "EOptionVolumeCategory Enum" :default "BGM") (Volume :type "Float (double-precision)")))

(fn `ChangeCueVolumeEase`
  (params (Category :type "EOptionVolumeCategory Enum" :default "BGM") (Volume :type "Float (double-precision)") (Time :type "Float (double-precision)")))

(fn `ChangeCueVolumeTime`
  (params (Category :type "EOptionVolumeCategory Enum" :default "BGM") (Volume :type "Float (double-precision)") (Time :type "Float (double-precision)")))

(fn `ChangeMapPostProcess`
  (params (Daath :type Integer) (DownIntensity :type "Float (double-precision)") (TopIntensity :type "Float (double-precision)")))

(fn `ChangeMapPostProcessEx`
  (params (PostProcessMaterial :type "MaterialInterface Object Reference") (ParameterName :type "Array of Name (by ref)") (Value :type "Array of Float (double-precision) (by ref)")))

(fn `ChangeMaterial`
  (params (Tag :type Name) (Table :type "DataTable Object Reference")))

(fn `ChangeMaterialCore`
  (params (Mesh :type "MeshComponent Object Reference") (DataTable :type "DataTable Object Reference") (UseColor :type Boolean) (Color :type "LinearColor Structure")))

(fn `ChangeMovieLanguage`
  (params (Culture :type String)))

(fn `ChangePlayRate`
  (params (PlayRate :type "Float (double-precision)")))

(fn `ChangeVolume`
  (params (Category :type "EGameVolumeCategory Enum" :default "BGM") (Volume :type "Float (double-precision)")))

(fn `CheckMovieText`)

(fn `CheckPauseEvent`
  (returns (ReturnValue :type Boolean))
  (bind _returnvalue (`parent.CheckPauseEvent`))
  (return _returnvalue))

(fn `CheckSkip`
  (returns (Return :type Boolean))
  (return false))

(fn `ClearBindingActors`
  (params (BindingActors :type "Array of Name (by ref)")))

(fn `ClearCharaForcedLOD`)

(fn `ClearMaterial`
  (params (Tag :type Name)))

(fn `ClearTemporaryText`)

(fn `ClearText`
  (params (VoiceOnlyStop :type Boolean)))

(fn `CutFinalize`
  (params (LevelSelf :type "Actor Object Reference")))

(fn `DebugAddSoundKey`)

(fn `DebugDrawSkip`)

(fn `DebugFlagControl`
  (params (Text :type Text) (Left :type Name) (L_Flag :type Boolean) (Right :type Name) (R_Flag :type Boolean) (Up :type Name) (U_Flag :type Boolean) (Down :type Name) (D_Flag :type Boolean))
  (returns (Next :type Boolean))
  (return false))

(fn `DebugForceFinish`)

(fn `DebugOpenWindow`)

(fn `DebugOutputTextTime`)

(fn `DebugPrintAperture`)

(fn `DebugPrintInfo`
  (params (UserData :type String)))

(fn `DebugPrintRate`)

(fn `DebugPrintTime`)

(fn `DebugSlomoFunc`)

(fn `DebugTextOff`)

(fn `DebugTextOn`
  (params (Text :type Text)))

(fn `DebugTextTime`)

(fn `DrawSelect`)

(fn `DrawTemporaryText`
  (params (MessageID :type Integer)))

(fn `DrawText`
  (params (MessageID :type Integer) (System :type Boolean) (CharaTag :type Name) (ForceAuto :type Boolean) (AutoDelay :type "Float (double-precision)")))

(fn `EndSequence`)

(fn `EnterSkip`)

(fn `EventFlagSetUp`
  (params (EventID :type String) (Last :type Boolean)))

(fn `Facial`
  (params (Tag :type Name) (Facial :type Name)))

(fn `FadeOutBattle`)

(fn `GetEventTableItem`
  (params (Table :type "Array of /Game/Blueprints/Event/Common/EventTableStrInt Structure (by ref)") (Object :type String))
  (returns (Find :type Boolean) (Value :type Integer))
  (return false 0))

(fn `GetFinish`
  (returns (IsFinish :type Boolean))
  (return false))

(fn `GetInput`
  (params (Action :type "E_ACTION_MAPPING_TYPE Enum" :default "E_ACTION_MAPPING_ACTION"))
  (returns (Return :type Boolean))
  (return false))

(fn `GetMessageWidget`
  (returns (MessageWidget :type "/Game/Blueprints/UI/Message/WB_Message Object Reference"))
  (return null))

(fn `GetNextMessageID`
  (returns (MessageID :type Integer) (SkipBlock :type Boolean) (system :type Boolean) (CharaTag :type Name) (ForceAuto :type Boolean) (AutoDelay :type "Float (double-precision)"))
  (return 0 false false "None" false 0.0))

(fn `GetNextMessageTime`
  (returns (NextTime :type "Float (double-precision)"))
  (return 0.0))

(fn `GetRate`
  (params (ObjectName :type String))
  (returns (Rate :type "Float (double-precision)"))
  (return 0.0))

(fn `GetTextFixTime`
  (params (Index :type Integer))
  (returns (FixTime :type "Float (double-precision)"))
  (return 0.0))

(fn `Initialize`
  (params (MessageAsset :type "ScriptMessageAsset Object Reference")))

(fn `InitMessage`)

(fn `InitPlayerPosition`
  (params (PositionActor :type "Actor Object Reference")))

(fn `InitSelection`
  (params (CharaTag :type Name) (BaseVoiceSE :type "AtomSound Object Reference")))

(fn `InitSelectionEx`
  (params (SelectType :type "/Game/Blueprints/Event/Common/E_EVENT_SELECTION_EX_TYPE Enum" :default "NewEnumerator0") (SelectMax :type Integer)))

(fn `InitSelectionLR`
  (params (Chara :type "/Game/Blueprints/Character/Base/CharaBase Object Reference") (LeftImage :type "Image Object Reference") (RightImage :type "Image Object Reference") (LeftLookAt :type "/Game/Blueprints/Event/Common/BP_EventLookAt Object Reference") (RightLookAt :type "/Game/Blueprints/Event/Common/BP_EventLookAt Object Reference") (LeftEffect :type "Emitter Object Reference") (RightEffect :type "Emitter Object Reference") (LeftGoToStep :type Integer) (RightGoToStep :type Integer) (LeftKey :type "E_ACTION_MAPPING_TYPE Enum" :default "E_ACTION_MAPPING_ACTION") (RightKey :type "E_ACTION_MAPPING_TYPE Enum" :default "E_ACTION_MAPPING_ACTION")))

(fn `InterpolationEvent`
  (params (Type :type Integer)))

(fn `IsEndSequence`
  (returns (End :type Boolean))
  (return false))

(fn `IsFinish`
  (returns (Finish :type Boolean))
  (return false))

(fn `IsNextMessage`
  (returns (Next :type Boolean))
  (return false))

(fn `IsNextSelect`
  (returns (return :type Boolean))
  (return false))

(fn `IsPauseMovieEvent`
  (returns (ReturnValue :type Boolean))
  (bind _returnvalue (`parent.IsPauseMovieEvent`))
  (return _returnvalue))

(fn `IsPlayingMovieEvent`
  (returns (ReturnValue :type Boolean))
  (bind _returnvalue (`parent.IsPlayingMovieEvent`))
  (return _returnvalue))

(fn `IsTalkPart`
  (returns (ReturnValue :type Boolean))
  (bind _returnvalue (`parent.IsTalkPart`))
  (return _returnvalue))

(fn `LookAtActor`
  (params (CharaTag :type Name) (TargetTag :type Name) (Immediately :type Boolean)))

(fn `LookAtChara`
  (params (CharaTag :type Name) (TargetTag :type Name) (Socket :type Name) (Immediately :type Boolean)))

(fn `MakeRateTable`)

(fn `MovieText`
  (params (MessageID :type Integer)))

(fn `OneSequencer`)

(fn `PlayBGM`
  (params (SoundID :type Name) (FadeTime :type "Float (double-precision)")))

(fn `PlayCue`
  (params (SoundID :type String) (Volume :type "Float (double-precision)") (Pitch :type "Float (double-precision)") (Time :type "Float (double-precision)")))

(fn `PlayCueBGM`
  (params (SoundID :type String) (Volume :type "Float (double-precision)") (Pitch :type "Float (double-precision)") (Time :type "Float (double-precision)")))

(fn `PlayCueENV`
  (params (SoundID :type String) (Volume :type "Float (double-precision)") (Pitch :type "Float (double-precision)") (Time :type "Float (double-precision)")))

(fn `PlayCueLoop`
  (params (SoundID :type String) (Volume :type "Float (double-precision)") (Pitch :type "Float (double-precision)")))

(fn `PlayDefaultBlink`
  (params (Tag :type Name)))

(fn `PlayMotion`
  (params (Tag :type Name) (AnimSequence :type Name) (IsLoop :type Boolean) (BlendTime :type "Float (double-precision)") (OffsetTime :type "Float (double-precision)") (EventTime :type "Float (double-precision)")))

(fn `PlayMotionConv`
  (params (Tag :type String) (AnimSequence :type String) (isLoop :type Boolean) (BlendTime :type "Float (double-precision)") (OffsetTime :type "Float (double-precision)") (EventTime :type "Float (double-precision)") (PlayRate :type "Float (double-precision)")))

(fn `PlayMotionID`
  (params (Tag :type Name) (AnimSequence :type "AnimSequenceBase Object Reference") (IsLoop :type Boolean) (BlendTime :type "Float (double-precision)") (OffsetTime :type "Float (double-precision)") (EventTime :type "Float (double-precision)")))

(fn `PlayMotionMob`
  (params (Tag :type String) (AnimSequence :type String) (IsLoop :type Boolean) (OffsetTime :type "Float (double-precision)") (EventTime :type "Float (double-precision)") (PlayRate :type "Float (double-precision)")))

(fn `PlayMotionProp`
  (params (Tag :type String) (AnimSequence :type String) (IsLoop :type Boolean) (OffsetTime :type "Float (double-precision)") (EventTime :type "Float (double-precision)") (PlayRate :type "Float (double-precision)")))

(fn `PlayPriorityBGM`
  (params (SoundID :type Name) (FadeTime :type "Float (double-precision)")))

(fn `PlaySE`
  (params (SoundID :type Name)))

(fn `PlaySelectionSoundEnter`
  (params (SoundFlag :type Boolean)))

(fn `PlaySelectionSoundSelect`
  (params (SoundFlag :type Boolean)))

(fn `PlaySequence`
  (params (Sequencer :type "LevelSequenceActor Object Reference") (CineCamera :type "CineCameraActor Object Reference") (BindID :type "MovieSceneObjectBindingID Structure") (FadeEnd :type Boolean))
  (returns (Play :type Boolean))
  (return false))

(fn `PlayShake`)

(fn `PlayStart`)

(fn `PlayVoice`
  (params (Voice :type Name) (CharaTag :type Name)))

(fn `ProcSelection`
  (params (DeltaSeconds :type "Float (double-precision)"))
  (returns (IsEnd :type Boolean) (Next :type Integer))
  (return false 0))

(fn `ProcSelectionEx`
  (params (SoundFlag :type Boolean))
  (returns (Return :type Integer) (Enter :type Boolean))
  (return 0 false))

(fn `ProcSelectionLR`
  (params (DeltaSeconds :type "Float (double-precision)"))
  (returns (IsEnd :type Boolean) (Next :type Integer))
  (return false 0))

(fn `Reflesh`)

(fn `ResetBlurInvalid`)

(fn `RevertMapPostProcess`)

(fn `SelectBranch`
  (params (Select1 :type Integer) (Select2 :type Integer) (Select3 :type Integer) (Select4 :type Integer))
  (returns (Return :type Integer))
  (return 0))

(fn `Set Activate`
  (params (Activate :type Boolean)))

(fn `Set Event Pause`
  (params (Puase :type Boolean) (Stop :type Boolean)))

(fn `Set Force End`)

(fn `SetBindingActors`
  (params (BindingActors :type "Array of Name (by ref)") (EventCtrl :type "Actor Object Reference")))

(fn `SetBlurInvalid`)

(fn `SetCharaForcedLOD`)

(fn `SetColorFade`
  (params (FirstColor :type "LinearColor Structure") (FinalColor :type "LinearColor Structure") (Time :type "Float (double-precision)") (Additive :type Boolean)))

(fn `SetDummyMessage`
  (params (StartTime :type "Float (double-precision)")))

(fn `SetFontAlpha`
  (params (Alpha :type "Float (double-precision)")))

(fn `SetIKEnable`
  (params (Type :type "/Game/Blueprints/Event/Common/E_IK_TYPE_LIST Enum" :default "NewEnumerator0") (Enable :type Boolean) (Immediately :type Boolean) (Tag :type Name)))

(fn `SetMessage`
  (params (MessageID :type Integer) (StartTime :type "Float (double-precision)") (SkipBlock :type Boolean) (System :type Boolean) (CharaTag :type Name) (ForceAuto :type Boolean) (AutoDelay :type "Float (double-precision)")))

(fn `SetMessageAsset`
  (params (NewParam :type "ScriptMessageAsset Object Reference")))

(fn `SetMotionBlur`
  (params (switch :type Boolean)))

(fn `SetNormalUnite`
  (params (`1stDevilID` :type Integer) (`2ndDevilID` :type Integer) (ResultID :type Integer) (Accident :type Boolean)))

(fn `SetPosition`
  (params (PositionActor :type "Actor Object Reference")))

(fn `SetRate`
  (params (ObjectName :type String) (Rate :type "Float (double-precision)")))

(fn `SetSearchAssetPath`
  (params (VoiceAssetPath :type Name) (LipAssetPath :type Name)))

(fn `SetSelectionLRVoiceBase`
  (params (Voice :type "AtomSound Object Reference")))

(fn `SetSelectionLRVoiceLeft`
  (params (Voice :type "AtomSound Object Reference")))

(fn `SetSelectionLRVoiceRight`
  (params (Voice :type "AtomSound Object Reference")))

(fn `SetSelectMessage`
  (params (MessageID_1 :type Integer) (MessageID_2 :type Integer) (MessageID_3 :type Integer) (MessageID_4 :type Integer)))

(fn `SetSkipEnable`
  (params (Enable :type Boolean)))

(fn `SetStaffSkip`
  (params (Use :type Boolean) (EventStaff :type "Actor Object Reference")))

(fn `SetUniteDevils`
  (params (Accident :type Boolean) (ResultDevil :type Integer) (`1st` :type Integer) (`2nd` :type Integer) (`3rd` :type Integer) (`4th` :type Integer)))

(fn `SetUniteSkip`
  (params (Use :type Boolean)))

(fn `SetVolumeCueLoop`
  (params (SoundID :type String) (Volume :type "Float (double-precision)")))

(fn `SimpleTextOff`)

(fn `SimpleTextOn`
  (params (Id :type Integer)))

(fn `StartChooseSE`
  (params (Sound :type "SoundAtomCue Object Reference")))

(fn `StepFinal`
  (params (IsFade :type Boolean) (AutoFadeOut :type Boolean) (NoResetVolume :type Boolean) (NoStopPrioBGM :type Boolean)))

(fn `StepFirst`
  (params (EventID :type String) (NoBGM :type Boolean) (NoChangeScene :type Boolean) (NoAutoFade :type Boolean) (PlayerHidden :type Boolean) (MaxFPS :type Integer))
  (returns (Next :type Boolean))
  (return false))

(fn `StopCueBGM`
  (params (FadeTime :type "Float (double-precision)") (NoBGM :type Boolean)))

(fn `StopCueENV`
  (params (FadeTime :type "Float (double-precision)") (NoBGM :type Boolean)))

(fn `StopCueLoop`
  (params (SoundID :type String)))

(fn `StopDefaultBlink`
  (params (Tag :type Name)))

(fn `StopPriorityBGM`
  (params (FadeTime :type "Float (double-precision)")))

(fn `StopShake`)

(fn `TerminateSE`)

(fn `TerminateVoice`)

(fn `UpdateVoice`)

(fn `UserConstructionScript`)

(fn `VisibleLevelFinal`)

(fn `VisibleLevelInit`)

(fn `WaitSequence`
  (params (PrintTime :type Boolean)))