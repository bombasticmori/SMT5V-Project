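; BP_EventScriptFade is an event script Blueprint whose function names describe screen fades to and from black or white.
; It declares color fade, SetFade and additive-mode functions, plus BI-prefixed counterparts and script spawn, delete and area-check hooks.
; All these bodies are empty or return false, so the file shows no working fade logic.
; BeginPlay, Tick and EndPlay only call the parent.
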(event `self.ReceiveBeginPlay`
  (`parent.ReceiveBeginPlay`))

(event `self.ReceiveTick`
  (params (DeltaSeconds :type "Float (single-precision)"))
  (`parent.ReceiveTick` DeltaSeconds))

(event `/Game/Blueprints/Event/Script/BPI_EventScript.CheckActive`)

(event `/Game/Blueprints/Event/Script/BPI_EventScript.DestroyKeyFree`)

(event `/Game/Blueprints/Event/Script/BPI_EventScript.CallDeactivate`)

(event `/Game/Blueprints/Event/Script/BPI_EventScript.PlayDeadMotion`
  (params (Active :type Boolean)))

(event `/Game/Blueprints/Event/Script/BPI_EventScript.BI_ChangeMaterialAlice`)

(event `/Game/Blueprints/Event/Script/BPI_EventScript.BI_RecalcOverlap`)

(event `self.ReceiveEndPlay`
  (params (EndPlayReason :type "EEndPlayReason Enum" :default "Destroyed"))
  (`parent.ReceiveEndPlay` EndPlayReason))

(fn `BI_CheckActiveArea`
  (returns (IsActive :type Boolean))
  (return false))

(fn `BI_DeleteScript`
  (returns (NoUse :type Boolean))
  (return false))

(fn `BI_FadeInBlack`
  (params (Time :type "Float (double-precision)"))
  (returns (ret :type Boolean))
  (return false))

(fn `BI_FadeInWhite`
  (params (Time :type "Float (double-precision)"))
  (returns (ret :type Boolean))
  (return false))

(fn `BI_FadeOutBlack`
  (params (Time :type "Float (double-precision)"))
  (returns (ret :type Boolean))
  (return false))

(fn `BI_FadeOutWhite`
  (params (Time :type "Float (double-precision)"))
  (returns (ret :type Boolean))
  (return false))

(fn `BI_SetInvalidWindow`
  (params (Invalid :type Boolean))
  (returns (NoUse :type Boolean))
  (return false))

(fn `BI_SpawnScript`
  (returns (NoUse :type Boolean))
  (return false))

(fn `FadeInBlack`
  (params (Time :type "Float (double-precision)")))

(fn `FadeInWhite`
  (params (Time :type "Float (double-precision)")))

(fn `FadeOutBlack`
  (params (Time :type "Float (double-precision)")))

(fn `FadeOutWhite`
  (params (Time :type "Float (double-precision)")))

(fn `ForceSpawnScript`
  (returns (NoUse :type Boolean))
  (return false))

(fn `SetAdditiveMode`
  (params (Additive :type Boolean)))

(fn `SetFade`
  (params (FirstColor :type "LinearColor Structure") (FinalColor :type "LinearColor Structure") (Time :type "Float (double-precision)")))

(fn `SpawnReflesh`
  (returns (NoUse :type Boolean))
  (return false))

(fn `UserConstructionScript`)