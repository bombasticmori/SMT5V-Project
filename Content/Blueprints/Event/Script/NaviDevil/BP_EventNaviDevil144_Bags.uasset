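; Navi Devil event actor 144 ("Bags"), a child Blueprint in the game's event script set.
; It adds no logic of its own: BeginPlay, QuestExecute, CheckActive, CallDeactivate and the BPI_CheckNaviDevil check all defer to the parent class.
; Its three asset OnLoaded handlers are empty, and its Tick and overlap events are disabled.
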(event `self.ReceiveBeginPlay`
  (`parent.ReceiveBeginPlay`))

(event `OnLoaded_113C03D44DBBB647C7ECA9AE813D10B5`
  (params (Loaded :type "Object Class Reference")))

(event `OnLoaded_823E54A649D9F357DE80D79A9C7629B6`
  (params (Loaded :type "Object Class Reference")))

(event `OnLoaded_EBE363AF48A425B496BADFB7A4AEAE94`
  (params (Loaded :type "Object Object Reference")))

(event `/Game/Blueprints/Event/Script/BP_EventMissionBaseCommon.QuestExecute`
  (`parent.QuestExecute`))

(event `/Game/Blueprints/Event/Script/BPI_EventScript.CheckActive`
  (`parent.CheckActive`))

(event `/Game/Blueprints/Event/Script/BPI_EventScript.CallDeactivate`
  (`parent.CallDeactivate`))

(fn `BPI_CheckNaviDevil`
  (returns (NaviDevil :type Boolean))
  (bind _navidevil (`parent.BPI_CheckNaviDevil`))
  (return _navidevil))

(fn `UserConstructionScript`
  (`parent.UserConstructionScript`))