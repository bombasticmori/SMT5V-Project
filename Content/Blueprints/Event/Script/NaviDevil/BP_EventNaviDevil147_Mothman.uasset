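; BP_EventNaviDevil147_Mothman is an event Blueprint for navi devil 147, Mothman, derived from a parent NaviDevil event class.
; BeginPlay, quest execution, active checks, deactivation, construction and the BPI_CheckNaviDevil check all pass straight through to the parent.
; It adds no logic of its own: its three async OnLoaded callbacks are empty, and its Tick and overlap events are disabled.
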(event `self.ReceiveBeginPlay`
  (`parent.ReceiveBeginPlay`))

(event `OnLoaded_113C03D44DBBB647C7ECA9AE621970D1`
  (params (Loaded :type "Object Class Reference")))

(event `OnLoaded_AE9E021B4E37B0B91A775EBF42B8F47D`
  (params (Loaded :type "Object Class Reference")))

(event `OnLoaded_EBE363AF48A425B496BADFB7478ACEF0`
  (params (Loaded :type "Object Object Reference")))

(event `/Game/Blueprints/Event/Script/BP_EventMissionBaseCommon.QuestExecute`
  (`parent.QuestExecute`))

(event `/Game/Blueprints/Event/Script/BPI_EventScript.CheckActive`
  (`parent.CheckActive`))

(event `/Game/Blueprints/Event/Script/BPI_EventScript.CallDeactivate`
  (`parent.CallDeactivate`))

(fn `BPI_CheckNaviDevil`
  (returns (NaviDevil :type Boolean))
  (bind _navidevil (`parent.BPI_CheckNaviDevil`))
  (return _navidevil))

(fn `UserConstructionScript`
  (`parent.UserConstructionScript`))