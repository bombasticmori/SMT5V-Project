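; Event Blueprint for navi devil 044, Agathion, a child variant of a parent navi devil event class.
; BeginPlay, the construction script, quest execution, active checks, deactivation and the BPI_CheckNaviDevil query only forward to the parent, so behavior is inherited.
; Three async load callbacks are empty, and Tick and overlap events are disabled, leaving no Agathion-specific logic in these graphs.
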(event `self.ReceiveBeginPlay`
  (`parent.ReceiveBeginPlay`))

(event `OnLoaded_113C03D44DBBB647C7ECA9AE345BD5F0`
  (params (Loaded :type "Object Class Reference")))

(event `OnLoaded_69CABD4E4C1F595C3E4C41ADFCA6396A`
  (params (Loaded :type "Object Class Reference")))

(event `OnLoaded_EBE363AF48A425B496BADFB711C86BD1`
  (params (Loaded :type "Object Object Reference")))

(event `/Game/Blueprints/Event/Script/BP_EventMissionBaseCommon.QuestExecute`
  (`parent.QuestExecute`))

(event `/Game/Blueprints/Event/Script/BPI_EventScript.CheckActive`
  (`parent.CheckActive`))

(event `/Game/Blueprints/Event/Script/BPI_EventScript.CallDeactivate`
  (`parent.CallDeactivate`))

(fn `BPI_CheckNaviDevil`
  (returns (NaviDevil :type Boolean))
  (bind _navidevil (`parent.BPI_CheckNaviDevil`))
  (return _navidevil))

(fn `UserConstructionScript`
  (`parent.UserConstructionScript`))