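; BP_EventScriptArea is a skeleton Blueprint for an event script area, with hooks for active-area checks, script spawn, refresh and deletion.
; It also exposes BI-prefixed hooks for screen fades, window invalidation, material change and overlap recalculation.
; Every function and event is an empty stub or returns false, except BeginPlay, which only calls its parent.
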(event `self.ReceiveBeginPlay`
  (`parent.ReceiveBeginPlay`))

(event `/Game/Blueprints/Event/Script/BPI_EventScript.CheckActive`)

(event `/Game/Blueprints/Event/Script/BPI_EventScript.DestroyKeyFree`)

(event `/Game/Blueprints/Event/Script/BPI_EventScript.CallDeactivate`)

(event `/Game/Blueprints/Event/Script/BPI_EventScript.PlayDeadMotion`
  (params (Active :type Boolean)))

(event `/Game/Blueprints/Event/Script/BPI_EventScript.BI_ChangeMaterialAlice`)

(event `/Game/Blueprints/Event/Script/BPI_EventScript.BI_RecalcOverlap`)

(event `BeginOverlap`)

(event `EndOverlap`)

(event `SpawnRefresh`)

(event `SpawnScriptSplit`)

(fn `BI_CheckActiveArea`
  (returns (IsActive :type Boolean))
  (return false))

(fn `BI_DeleteScript`
  (returns (NoUse :type Boolean))
  (return false))

(fn `BI_FadeInBlack`
  (params (Time :type "Float (double-precision)"))
  (returns (ret :type Boolean))
  (return false))

(fn `BI_FadeInWhite`
  (params (Time :type "Float (double-precision)"))
  (returns (ret :type Boolean))
  (return false))

(fn `BI_FadeOutBlack`
  (params (Time :type "Float (double-precision)"))
  (returns (ret :type Boolean))
  (return false))

(fn `BI_FadeOutWhite`
  (params (Time :type "Float (double-precision)"))
  (returns (ret :type Boolean))
  (return false))

(fn `BI_SetInvalidWindow`
  (params (Invalid :type Boolean))
  (returns (NoUse :type Boolean))
  (return false))

(fn `BI_SpawnScript`
  (returns (NoUse :type Boolean))
  (return false))

(fn `CheckActiveArea`
  (returns (IsActive :type Boolean))
  (return false))

(fn `DeleteScript`)

(fn `ForceSpawnScript`
  (returns (NoUse :type Boolean))
  (return false))

(fn `MakeActorList`)

(fn `SpawnReflesh`
  (returns (NoUse :type Boolean))
  (return false))

(fn `SpawnScript`)

(fn `UserConstructionScript`)