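; BP_EventMissionBase is a base Blueprint for event missions, declaring a shared set of hooks for scripted quest events.
; It stubs quest lifecycle, area and action enter/exit, screen fades, post-process loading and script spawning.
; BeginPlay, Tick and construction only call the parent.
; The other events and functions are empty or return false, so the file itself holds no mission logic.
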(event `self.ReceiveBeginPlay`
  (`parent.ReceiveBeginPlay`))

(event `self.ReceiveTick`
  (params (DeltaSeconds :type "Float (single-precision)"))
  (`parent.ReceiveTick` DeltaSeconds))

(event `Timeline_PostProcess_On__FinishedFunc`)

(event `Timeline_PostProcess_On__UpdateFunc`)

(event `OnLoaded_A168829F44F2BCD021419D82EF0C427F`
  (params (Loaded :type "Object Object Reference")))

(event `/Game/Blueprints/Event/Script/BPI_EventScript.CheckActive`)

(event `/Game/Blueprints/Event/Script/BPI_EventScript.DestroyKeyFree`)

(event `/Game/Blueprints/Event/Script/BPI_EventScript.PlayDeadMotion`
  (params (Active :type Boolean)))

(event `/Game/Blueprints/Event/Script/BPI_EventScript.BI_ChangeMaterialAlice`)

(event `/Game/Blueprints/Event/Script/BPI_EventScript.BI_RecalcOverlap`)

(event `StartQuest`)

(event `ReadyQuest`)

(event `AreaIn`)

(event `AreaOut`)

(event `/Game/Blueprints/Event/Script/BPI_EventScript.CallDeactivate`)

(event `Deactivate`)

(event `EndQuest`)

(event `ActionIn`)

(event `ActionOut`)

(event `SetInvalidWindow`
  (params (Invalid :type Boolean)))

(event `Activate_PP`)

(event `Deactivate_PP`)

(event `Remove_PP`
  (params (CameraActor :type "CameraActor Object Reference")))

(event `Load_PP`
  (params (Material :type "MaterialInstance Soft Object Reference") (CameraActor :type "CameraActor Object Reference")))

(event `ResetWindowType`
  (params (WindowType :type "E_AActionWindowType Enum" :default "E_AActionWindow_None")))

(fn `BI_CheckActiveArea`
  (returns (IsActive :type Boolean))
  (return false))

(fn `BI_DeleteScript`
  (returns (NoUse :type Boolean))
  (return false))

(fn `BI_FadeInBlack`
  (params (Time :type "Float (double-precision)"))
  (returns (ret :type Boolean))
  (return false))

(fn `BI_FadeInWhite`
  (params (Time :type "Float (double-precision)"))
  (returns (ret :type Boolean))
  (return false))

(fn `BI_FadeOutBlack`
  (params (Time :type "Float (double-precision)"))
  (returns (ret :type Boolean))
  (return false))

(fn `BI_FadeOutWhite`
  (params (Time :type "Float (double-precision)"))
  (returns (ret :type Boolean))
  (return false))

(fn `BI_SetInvalidWindow`
  (params (Invalid :type Boolean))
  (returns (NoUse :type Boolean))
  (return false))

(fn `BI_SpawnScript`
  (returns (NoUse :type Boolean))
  (return false))

(fn `ForceSpawnScript`
  (returns (NoUse :type Boolean))
  (return false))

(fn `SetPlayerLookAt`
  (params (Enable :type Boolean)))

(fn `SpawnReflesh`
  (returns (NoUse :type Boolean))
  (return false))

(fn `UserConstructionScript`
  (`parent.UserConstructionScript`))