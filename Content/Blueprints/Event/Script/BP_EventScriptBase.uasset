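; BP_EventScriptBase is a base Blueprint for event scripts, declaring a shared interface for script lifecycle, areas, actions, characters and messages.
; Nearly every event and function is an empty stub or returns a default, covering start/end, area in/out, spawning, deletion, fades, look-at and talk icons.
; Only BeginPlay, Tick, construction and the mission-event check forward to the parent; the overlap event is disabled.
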(event `self.ReceiveBeginPlay`
  (`parent.ReceiveBeginPlay`))

(event `self.ReceiveTick`
  (params (DeltaSeconds :type "Float (single-precision)"))
  (`parent.ReceiveTick` DeltaSeconds))

(event `OnLoaded_221B908D41E0B5F6EEA9618D90FADD7D`
  (params (Loaded :type "Object Object Reference")))

(event `OnLoaded_44E8C5904B9505DDBE91FBAD0D27188E`
  (params (Loaded :type "Object Object Reference")))

(event `/Game/Blueprints/Event/Script/BPI_EventScript.CheckActive`)

(event `/Game/Blueprints/Event/Script/BPI_EventScript.DestroyKeyFree`)

(event `/Game/Blueprints/Event/Script/BPI_EventScript.PlayDeadMotion`
  (params (Active :type Boolean)))

(event `/Game/Blueprints/Event/Script/BPI_EventScript.BI_ChangeMaterialAlice`)

(event `/Game/Blueprints/Event/Script/BPI_EventScript.BI_RecalcOverlap`)

(event `StartScript`)

(event `EndScript`)

(event `ReadyScript`)

(event `AreaIn`)

(event `AreaOut`)

(event `/Game/Blueprints/Event/Script/BPI_EventScript.CallDeactivate`)

(event `Deactivate`)

(event `ActionIn`)

(event `ActionOut`)

(event `SetInvalidWindow`
  (params (Invalid :type Boolean)))

(event `ToiletMark`
  (params (Type :type "/Game/Blueprints/Event/Script/E_EVENT_TOILETMARK_TYPE Enum" :default "NewEnumerator0") (Tag :type Name)))

(fn `AddCharacter`
  (params (Character :type "Actor Object Reference") (Tag :type Name)))

(fn `BI_CheckActiveArea`
  (returns (IsActive :type Boolean))
  (return false))

(fn `BI_DeleteScript`
  (returns (NoUse :type Boolean))
  (return false))

(fn `BI_FadeInBlack`
  (params (Time :type "Float (double-precision)"))
  (returns (ret :type Boolean))
  (return false))

(fn `BI_FadeInWhite`
  (params (Time :type "Float (double-precision)"))
  (returns (ret :type Boolean))
  (return false))

(fn `BI_FadeOutBlack`
  (params (Time :type "Float (double-precision)"))
  (returns (ret :type Boolean))
  (return false))

(fn `BI_FadeOutWhite`
  (params (Time :type "Float (double-precision)"))
  (returns (ret :type Boolean))
  (return false))

(fn `BI_SetInvalidWindow`
  (params (Invalid :type Boolean))
  (returns (NoUse :type Boolean))
  (return false))

(fn `BI_SpawnScript`
  (returns (NoUse :type Boolean))
  (return false))

(fn `BPI_CheckMissionEvent`
  (returns (MissionEvent :type Boolean))
  (bind _missionevent (`parent.BPI_CheckMissionEvent`))
  (return _missionevent))

(fn `Character`
  (params (Class :type "Actor Class Reference") (PosX :type "Float (double-precision)") (PosY :type "Float (double-precision)") (PosZ :type "Float (double-precision)") (RotZ :type "Float (double-precision)") (Tag :type Name))
  (returns (SpawnActor :type "Actor Object Reference"))
  (return null))

(fn `ForceSpawnScript`
  (returns (NoUse :type Boolean))
  (return false))

(fn `GetActive`
  (returns (IsActive :type Boolean))
  (return false))

(fn `Initialize`
  (params (PlayerCamera :type Boolean) (PlayerVisible :type Boolean)))

(fn `RegisterTalkIcon`
  (params (`3DCharacter` :type "Actor Object Reference")))

(fn `SetDataTable`
  (params (DataTable :type "DataTable Object Reference")))

(fn `SetLookAt`
  (params (lookAt :type Boolean)))

(fn `SetMessage`
  (params (MessageAsset :type "ScriptMessageAsset Object Reference")))

(fn `SetPlayerLookAt`
  (params (Enable :type Boolean)))

(fn `SpawnReflesh`
  (returns (NoUse :type Boolean))
  (return false))

(fn `UserConstructionScript`
  (`parent.UserConstructionScript`))