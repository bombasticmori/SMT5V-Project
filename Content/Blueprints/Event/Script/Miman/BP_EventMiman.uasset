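; BP_EventMiman is a quest-event actor for Miman, mostly a skeleton in which begin play, quest execution, activation checks, deactivation and action input defer to its parent.
; Show, hide and icon-update interface events, montage-end handling, found-count check and garden-point award are all empty stubs.
; The Miman interface check returns the parent's result, while the camera-shift and minimap-row functions return fixed negative results.
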(event `self.ReceiveBeginPlay`
  (`parent.ReceiveBeginPlay`))

(event `/Game/Blueprints/Event/Script/BP_EventMissionBaseCommon.QuestExecute`
  (`parent.QuestExecute`))

(event `/Game/Blueprints/Event/Script/BPI_EventScript.CheckActive`
  (`parent.CheckActive`))

(event `/Game/Blueprints/Event/Script/BPI_EventScript.CallDeactivate`
  (`parent.CallDeactivate`))

(event `/Game/Blueprints/Event/Script/Miman/BPI_EventMiman.BPI_ShowAgainMiman`)

(event `/Game/Blueprints/Event/Script/Miman/BPI_EventMiman.BPI_HideMiman`)

(event `/Game/Blueprints/Event/Script/Miman/BPI_EventMiman.BPI_UpdateIconView`)

(event `Func2`)

(event `Func3`)

(event `self.ActionIn`
  (`parent.ActionIn`))

(event `Func1`)

(event `Func4`)

(event `Func5`)

(event `OnMontageEnded_`
  (params (Montage :type "AnimMontage Object Reference") (bInterrupted :type Boolean)))

(fn `AddGardenPoint`)

(fn `BPI_CheckMiman`
  (returns (Miman :type Boolean))
  (bind _miman (`parent.BPI_CheckMiman`))
  (return _miman))

(fn `CheckMimanFoundNum`)

(fn `SetMinimapIconTableRow`
  (params (Index :type Integer))
  (returns (OutRow :type "MinimapIconTableRow Structure") (NeedToAddMore :type Boolean))
  (return (struct) false))

(fn `ShiftCameraCheck`
  (returns (Shift :type Boolean) (Rotate :type "Rotator Structure"))
  (return false))

(fn `UserConstructionScript`
  (`parent.UserConstructionScript`))