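; BP_EventMiman_Answer is a quest event Blueprint for a Miman conversation, and currently holds only scaffolding.
; BeginPlay, QuestExecute, CheckActive and CallDeactivate simply forward to the parent class, which supplies any actual behavior.
; Named events for talk start, end and cancel, five OpenDaath variants, OpenMiman and NoMakka are empty stubs.
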(event `self.ReceiveBeginPlay`
  (`parent.ReceiveBeginPlay`))

(event `/Game/Blueprints/Event/Script/BP_EventMissionBaseCommon.QuestExecute`
  (`parent.QuestExecute`))

(event `/Game/Blueprints/Event/Script/BPI_EventScript.CheckActive`
  (`parent.CheckActive`))

(event `/Game/Blueprints/Event/Script/BPI_EventScript.CallDeactivate`
  (`parent.CallDeactivate`))

(event `TalkStart`)

(event `OpenDaath1`)

(event `OpenDaath2`)

(event `OpenDaath3`)

(event `OpenDaath4`)

(event `EndTalk`)

(event `OpenMiman`)

(event `NoMakka`)

(event `CancelTalk`)

(event `OpenDaath5`)

(fn `UserConstructionScript`
  (`parent.UserConstructionScript`))