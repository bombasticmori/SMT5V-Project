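; Base-style actor for map event areas, declaring hooks for event flow, map icons and interface queries.
; Its functions cover event start, end and fades, camera hand shake, activation, Tokyo large-map mission and talk icons, and 3D POI icons.
; BPI functions expose mission, Miman and navi-devil checks, event ID, hit box size and icon location.
; Every graph here is an empty stub or returns a default value.
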(fn `ActivateBase`)

(fn `Add3DIconToStaticPOI`
  (params (POIType :type "E_MINIMAP_POI_TYPE Enum" :default "E_MINIMAP_POI_TYPE_NONE") (DataId :type Integer) (AreaId :type Integer) (Owner :type "Actor Object Reference")))

(fn `AddTokyoLargeMapIconMission`
  (params (ActorLocation :type "Vector Structure") (MissionId :type Integer)))

(fn `AddTokyoLargeMapIconTalk`
  (params (ActorLocation :type "Vector Structure") (InactiveFlag :type Name)))

(fn `BPI_CheckMiman`
  (returns (Miman :type Boolean))
  (return false))

(fn `BPI_CheckMissionEvent`
  (returns (MissionEvent :type Boolean))
  (return false))

(fn `BPI_CheckNaviDevil`
  (returns (NaviDevil :type Boolean))
  (return false))

(fn `BPI_GetDebugMemo`
  (returns (Memo :type Text))
  (return ""))

(fn `BPI_GetHitBoxSize`
  (returns (Size :type "Vector Structure"))
  (return (0.0 0.0 0.0)))

(fn `BPI_GetMapEventId`
  (returns (MapEventId :type Integer))
  (return 0))

(fn `BPI_Map3DIconGetShouldBeRendered`
  (returns (ShouldBeRendered :type Boolean) (Unknown :type Boolean))
  (return false false))

(fn `BPI_Map3DIconGetWorldLocation`
  (returns (WorldLocation :type "Vector Structure"))
  (return (0.0 0.0 0.0)))

(fn `DeactivateBase`)

(fn `Delete3DIconFromStaticPOI`)

(fn `DeleteTokyoLargeMapIcon`)

(fn `EndMapEvent`
  (returns (Dummy :type Boolean))
  (return false))

(fn `EndMapEventAfterBattle`
  (returns (Dummy :type Boolean))
  (return false))

(fn `FadeInMapEvent`
  (returns (Delay :type "Float (double-precision)"))
  (return 0.0))

(fn `FadeOutMapEvent`
  (returns (Delay :type "Float (double-precision)"))
  (return 0.0))

(fn `HandShakeStart`
  (params (ShakeClass :type "MatineeCameraShake Class Reference") (ShakeScale :type "Float (double-precision)")))

(fn `HandShakeStartEx`
  (params (ShakeScale :type "Float (double-precision)")))

(fn `HandShakeStop`
  (params (bImmediately :type Boolean)))

(fn `Map3DIconGetWorldLocation`
  (returns (ReturnValue :type "Vector Structure"))
  (return (0.0 0.0 0.0)))

(fn `SetEndMapEventParam`
  (returns (Dummy :type Boolean))
  (return false))

(fn `StartMapEvent`
  (params (PlayerVisible :type Boolean) (NoStopPrioBGM :type Boolean) (PlayerCameraEnable :type Boolean) (NoStopQuestBGM :type Boolean))
  (returns (Dummy :type Boolean))
  (return false))

(fn `UserConstructionScript`)