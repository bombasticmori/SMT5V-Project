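; BP_es617_m085_01 is an event script Blueprint for es617_m085 that adds no logic of its own.
; BeginPlay, CheckActive, BIRecalcOverlap and the construction script only forward to the parent class, which supplies any actual behavior.
; The overlap and Tick events are disabled stubs, and an OnLoaded event is present but empty.
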(event `self.ReceiveBeginPlay`
  (`parent.ReceiveBeginPlay`))

(event `OnLoaded_0E38A2EA4724D2AEB4E20FBD4D29AEC2`
  (params (Loaded :type "Object Object Reference")))

(event `/Game/Blueprints/Event/Script/BPI_EventScript.CheckActive`
  (`parent.CheckActive`))

(event `/Game/Blueprints/Event/Script/BPI_EventScript.BI_RecalcOverlap`
  (`parent.BI_RecalcOverlap`))

(fn `UserConstructionScript`
  (`parent.UserConstructionScript`))