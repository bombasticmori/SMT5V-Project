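; BP_EventMissionBase_HitAction is an event-mission Blueprint, named as a base for hit-triggered quest actions.
; It declares hooks for quest lifecycle, area and action enter/exit, and hit handling, all left empty.
; BI_-prefixed functions for area checks, script spawn/delete, screen fades and window invalidation are stubs, returning false where they have a result.
; Only BeginPlay, Tick and the construction script do anything, forwarding to the parent.
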(event `self.ReceiveBeginPlay`
  (`parent.ReceiveBeginPlay`))

(event `self.ReceiveTick`
  (params (DeltaSeconds :type "Float (single-precision)"))
  (`parent.ReceiveTick` DeltaSeconds))

(event `/Game/Blueprints/Event/Script/BPI_EventScript.CheckActive`)

(event `/Game/Blueprints/Event/Script/BPI_EventScript.DestroyKeyFree`)

(event `/Game/Blueprints/Event/Script/BPI_EventScript.PlayDeadMotion`
  (params (Active :type Boolean)))

(event `/Game/Blueprints/Event/Script/BPI_EventScript.BI_ChangeMaterialAlice`)

(event `/Game/Blueprints/Event/Script/BPI_EventScript.BI_RecalcOverlap`)

(event `StartQuestAction`)

(event `ReadyQuest`)

(event `AreaIn`)

(event `AreaOut`)

(event `/Game/Blueprints/Event/Script/BPI_EventScript.CallDeactivate`)

(event `Deactivate`)

(event `EndQuest`)

(event `StartQuestHit`)

(event `ActionIn`)

(event `ActionOut`)

(event `SetInvalidWindow`
  (params (Invalid :type Boolean)))

(fn `BI_CheckActiveArea`
  (returns (IsActive :type Boolean))
  (return false))

(fn `BI_DeleteScript`
  (returns (NoUse :type Boolean))
  (return false))

(fn `BI_FadeInBlack`
  (params (Time :type "Float (double-precision)"))
  (returns (ret :type Boolean))
  (return false))

(fn `BI_FadeInWhite`
  (params (Time :type "Float (double-precision)"))
  (returns (ret :type Boolean))
  (return false))

(fn `BI_FadeOutBlack`
  (params (Time :type "Float (double-precision)"))
  (returns (ret :type Boolean))
  (return false))

(fn `BI_FadeOutWhite`
  (params (Time :type "Float (double-precision)"))
  (returns (ret :type Boolean))
  (return false))

(fn `BI_SetInvalidWindow`
  (params (Invalid :type Boolean))
  (returns (NoUse :type Boolean))
  (return false))

(fn `BI_SpawnScript`
  (returns (NoUse :type Boolean))
  (return false))

(fn `ForceSpawnScript`
  (returns (NoUse :type Boolean))
  (return false))

(fn `QuestFunctionHit`)

(fn `SetPlayerLookAt`
  (params (Enable :type Boolean)))

(fn `SpawnReflesh`
  (returns (NoUse :type Boolean))
  (return false))

(fn `UserConstructionScript`
  (`parent.UserConstructionScript`))