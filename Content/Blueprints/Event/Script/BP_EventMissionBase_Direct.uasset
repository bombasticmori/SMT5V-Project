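; BP_EventMissionBase_Direct is an event mission script Blueprint, apparently a base class, that currently holds no logic of its own.
; Its interface-style events and functions for quest start/end, screen fades, script spawning and deletion, and area checks are empty or return false.
; Only the construction script and EndMapEvent forward to the parent; BeginPlay, overlap and Tick are disabled placeholders.
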(event `/Game/Blueprints/Event/Script/BPI_EventScript.CheckActive`)

(event `/Game/Blueprints/Event/Script/BPI_EventScript.DestroyKeyFree`)

(event `/Game/Blueprints/Event/Script/BPI_EventScript.CallDeactivate`)

(event `/Game/Blueprints/Event/Script/BPI_EventScript.PlayDeadMotion`
  (params (Active :type Boolean)))

(event `/Game/Blueprints/Event/Script/BPI_EventScript.BI_ChangeMaterialAlice`)

(event `/Game/Blueprints/Event/Script/BPI_EventScript.BI_RecalcOverlap`)

(event `StartQuest`)

(event `EndQuest`)

(fn `BI_CheckActiveArea`
  (returns (IsActive :type Boolean))
  (return false))

(fn `BI_DeleteScript`
  (returns (NoUse :type Boolean))
  (return false))

(fn `BI_FadeInBlack`
  (params (Time :type "Float (double-precision)"))
  (returns (ret :type Boolean))
  (return false))

(fn `BI_FadeInWhite`
  (params (Time :type "Float (double-precision)"))
  (returns (ret :type Boolean))
  (return false))

(fn `BI_FadeOutBlack`
  (params (Time :type "Float (double-precision)"))
  (returns (ret :type Boolean))
  (return false))

(fn `BI_FadeOutWhite`
  (params (Time :type "Float (double-precision)"))
  (returns (ret :type Boolean))
  (return false))

(fn `BI_SetInvalidWindow`
  (params (Invalid :type Boolean))
  (returns (NoUse :type Boolean))
  (return false))

(fn `BI_SpawnScript`
  (returns (NoUse :type Boolean))
  (return false))

(fn `EndMapEvent`
  (returns (Dummy :type Boolean))
  (bind _dummy (`parent.EndMapEvent`))
  (return _dummy))

(fn `ForceSpawnScript`
  (returns (NoUse :type Boolean))
  (return false))

(fn `SpawnReflesh`
  (returns (NoUse :type Boolean))
  (return false))

(fn `UserConstructionScript`
  (`parent.UserConstructionScript`))