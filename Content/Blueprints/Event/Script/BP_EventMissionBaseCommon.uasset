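; BP_EventMissionBaseCommon is a Blueprint layer for mission event scripts, exposing functions for map events, quests, characters, message windows and icons.
; StartMapEvent, EndMapEvent and BPI_CheckMissionEvent forward to their parent implementations and return the results.
; The other functions, including the Ex and Ryuketsu map-event variants, are stubs that do nothing or return false.
; BeginPlay, overlap and Tick are disabled, and the construction script only calls the parent.
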(fn `AddCharacter`
  (params (Character :type "Actor Object Reference") (Tag :type Name)))

(fn `BPI_CheckMissionEvent`
  (returns (MissionEvent :type Boolean))
  (bind _missionevent (`parent.BPI_CheckMissionEvent`))
  (return _missionevent))

(fn `Character`
  (params (Class :type "Actor Class Reference") (PosX :type "Float (double-precision)") (PosY :type "Float (double-precision)") (PosZ :type "Float (double-precision)") (RotZ :type "Float (double-precision)") (Tag :type Name)))

(fn `CreateMessageWindow`
  (params (Scene :type "EBgmScene Enum" :default "Map")))

(fn `DeleteMessageWindow`)

(fn `EndMapEvent`
  (returns (Dummy :type Boolean))
  (bind _dummy (`parent.EndMapEvent`))
  (return _dummy))

(fn `EndMapEventEx`
  (params (BGMScene :type "EBgmScene Enum" :default "Map"))
  (returns (Dummy :type Boolean))
  (return false))

(fn `EndMapEventRyuketsu`
  (params (RyuketsuIndex :type Integer)))

(fn `GetActive`
  (returns (IsActive :type Boolean))
  (return false))

(fn `IsPlayerLooking`
  (returns (IsLooking :type Boolean))
  (return false))

(fn `QuestExecute`)

(fn `RegisterMissionIcon`
  (params (`3DCharacter` :type "Actor Object Reference")))

(fn `SetLookAt`
  (params (lookAt :type Boolean)))

(fn `StartMapEvent`
  (params (PlayerVisible :type Boolean) (NoStopPrioBGM :type Boolean) (PlayerCameraEnable :type Boolean) (NoStopQuestBGM :type Boolean))
  (returns (Dummy :type Boolean))
  (bind _dummy (`parent.StartMapEvent` PlayerVisible NoStopPrioBGM PlayerCameraEnable NoStopQuestBGM))
  (return _dummy))

(fn `StartMapEventEx`
  (params (PlayerVisible :type Boolean) (BGMCue :type "SoundAtomCue Object Reference") (NoStopPrioBGM :type Boolean) (PlayerCameraEnable :type Boolean))
  (returns (Dummy :type Boolean))
  (return false))

(fn `ToiletMark`
  (params (Type :type "/Game/Blueprints/Event/Script/E_EVENT_TOILETMARK_TYPE Enum" :default "NewEnumerator0") (Tag :type Name))
  (returns (SpawnedActor :type "StaticMeshActor Object Reference"))
  (return null))

(fn `UserConstructionScript`
  (`parent.UserConstructionScript`))