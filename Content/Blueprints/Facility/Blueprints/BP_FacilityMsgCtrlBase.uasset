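; BP_FacilityMsgCtrlBase is a base Blueprint defining the interface for message window control in facilities.
; It declares functions for setup and teardown, window in/out, message requests by label, index or tag value, page input, auto and fast buttons, voice, lip sync and button help.
; Nearly all are empty stubs returning false or defaults, apparently for child classes to override; only Tick and EndPlay forward to the parent.
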(event `self.ReceiveTick`
  (params (DeltaSeconds :type "Float (single-precision)"))
  (`parent.ReceiveTick` DeltaSeconds))

(event `self.ReceiveEndPlay`
  (params (EndPlayReason :type "EEndPlayReason Enum" :default "Destroyed"))
  (`parent.ReceiveEndPlay` EndPlayReason))

(event `ReqOutWindw`)

(fn `ApplyMessage`
  (returns (bOk :type Boolean))
  (return false))

(fn `ApplyMessageComplete`
  (returns (bOk :type Boolean))
  (return false))

(fn `CheckButtonAuto`
  (returns (ReturnValue :type Boolean))
  (return false))

(fn `CheckButtonFast`
  (returns (ReturnValue :type Boolean))
  (return false))

(fn `CheckButtonNext`
  (params (bSelectMenu :type Boolean))
  (returns (ReturnValue :type Boolean))
  (return false))

(fn `CheckStopLipSync`)

(fn `CheckVoice`
  (returns (IsEnd :type Boolean))
  (return false))

(fn `ClearButtonHelpAppearance`)

(fn `ClearLipSync`)

(fn `ClearRequestMessage`)

(fn `ClearStateInfo`)

(fn `DestoryLipSyncActor`)

(fn `EndCtrl`
  (returns (bOk :type Boolean))
  (return false))

(fn `GetMsgCtrlActor`
  (returns (MsgCtrlActor :type "Actor Object Reference"))
  (return null))

(fn `GetMsgScriptAsset`
  (returns (MsgScriptAsset :type "ScriptMessageAsset Object Reference"))
  (return null))

(fn `GetNowMsgIndex`
  (returns (NowMsgIndex :type Integer))
  (return 0))

(fn `InitCtrl`
  (params (ScriptAsset :type "ScriptMessageAsset Object Reference"))
  (returns (bOK :type Boolean))
  (return false))

(fn `InWindow`
  (params (bExecution :type Boolean)))

(fn `IsCompletedMsg`
  (returns (bFinished :type Boolean))
  (return false))

(fn `IsDispMessage`
  (returns (ReturnValue :type Boolean))
  (return false))

(fn `IsOpenWindow`
  (returns (bOpen :type Boolean))
  (return false))

(fn `IsRequestMessage`
  (returns (ReturnValue :type Boolean))
  (return false))

(fn `IsRunningMsg`
  (returns (bRunning :type Boolean))
  (return false))

(fn `IsRunningWindowAnim`
  (returns (ReturnValue :type Boolean))
  (return false))

(fn `IsValidCtrl`
  (returns (bValid :type Boolean))
  (return false))

(fn `OutWindow`
  (params (bExecution :type Boolean)))

(fn `RequestCloseMessage`
  (params (Excution :type Boolean))
  (returns (bOk :type Boolean))
  (return false))

(fn `RequestCompleMessage`
  (returns (bOk :type Boolean))
  (return false))

(fn `RequestMessage`
  (params (Label :type Name) (bExecution :type Boolean) (bNextIcon :type Boolean) (bSystemMsg :type Boolean) (SpeakingActor :type "Actor Object Reference") (ButtonFastToneDown :type Boolean))
  (returns (bOk :type Boolean))
  (return false))

(fn `RequestMessageIndex`
  (params (Index :type Integer) (bExecution :type Boolean) (bNextIcon :type Boolean) (bSystemMsg :type Boolean) (SpeakingActor :type "Actor Object Reference") (ButtonFastToneDown :type Boolean))
  (returns (bOk :type Boolean))
  (return false))

(fn `RequestMessageTagValue`
  (params (Label :type Name) (TagInfo :type "Array of /Game/Blueprints/Facility/Blueprints/FacilityMsgTagInfo Structure (by ref)") (bExecution :type Boolean) (bNextIcon :type Boolean) (bSystemMsg :type Boolean) (SpeakingActor :type "Actor Object Reference") (ButtonFastToneDown :type Boolean))
  (returns (bOk :type Boolean))
  (return false))

(fn `SetButtonhelpFunction`
  (params (Is :type Boolean)))

(fn `StartLipSync`)

(fn `StopLipSync`)

(fn `UpdateButtonHelpAppearance`)

(fn `UpdateMessageInput`
  (params (bPlaySE :type Boolean) (bSelectMenu :type Boolean))
  (returns (bRunningMsg :type Boolean) (bCompleteMsg :type Boolean) (bReqCompleteMsg :type Boolean) (bReqNextPage :type Boolean) (bMW_Off :type Boolean))
  (return false false false false false))