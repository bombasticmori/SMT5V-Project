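; BP_FacilityMenuCtrlBase is a base controller for facility menus, defining the interface for select menus, yes/no prompts and their message windows.
; It declares functions to request, apply, close and clear menus, poll wait state, handle input with sound flags, and read or move the cursor.
; These functions are empty stubs returning false or zero, presumably for subclasses to override.
; InitCtrl, EndCtrl and Tick only call the parent implementation.
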(event `self.ReceiveTick`
  (params (DeltaSeconds :type "Float (single-precision)"))
  (`parent.ReceiveTick` DeltaSeconds))

(fn `ApplyRequestYesNoMenu`
  (returns (bOk :type Boolean))
  (return false))

(fn `ApplyReuestSelectMenu`
  (returns (bReq :type Boolean))
  (return false))

(fn `CheckRequestWait`
  (returns (bWait :type Boolean))
  (return false))

(fn `ClearRequestSeletMenuInfo`)

(fn `ClearSeletMenuInfo`)

(fn `EndCtrl`
  (returns (bOk :type Boolean))
  (bind _bok (`parent.EndCtrl`))
  (return _bok))

(fn `GetSelectMenuCursorPos`
  (returns (CursorPos :type Integer))
  (return 0))

(fn `InitCtrl`
  (params (ScriptAsset :type "ScriptMessageAsset Object Reference"))
  (returns (bOK :type Boolean))
  (bind _bok (`parent.InitCtrl` ScriptAsset))
  (return _bok))

(fn `IsOpenSelectMenu`
  (returns (bOpen :type Boolean))
  (return false))

(fn `MoveMouseSelectCursor`
  (params (InPosition :type Integer))
  (returns (OutIndex :type Integer))
  (return 0))

(fn `RequestCloseSelectMenu`
  (params (bWindowClose :type Boolean) (bWindowExcution :type Boolean))
  (returns (bOk :type Boolean))
  (return false))

(fn `RequestSelectMenu`
  (params (MenuName :type "Array of Name (by ref)") (MenuCursorPos :type Integer) (MenuNewIocn :type "Array of Boolean (by ref)") (MenuOpenDelay :type "Float (double-precision)") (bMenuWaitMsg :type Boolean) (WindowMessage :type Name) (bWindowExcution :type Boolean) (bWindowSystemMsg :type Boolean) (SpeakingActor :type "Actor Object Reference") (ButtonFastToneDown :type Boolean))
  (returns (bOk :type Boolean))
  (return false))

(fn `RequestSelectMenuBase`
  (params (MenuName :type "Array of Name (by ref)") (MenuCursorPos :type Integer) (MenuNewIocn :type "Array of Boolean (by ref)") (MenuOpenDelay :type "Float (double-precision)") (bMenuWaitMsg :type Boolean) (bWindowExcution :type Boolean) (WindowMessage :type Name) (bWindowNextIcon :type Boolean) (bWindowSystemMsg :type Boolean) (SpeakingActor :type "Actor Object Reference") (ButtonFastToneDown :type Boolean))
  (returns (bOk :type Boolean))
  (return false))

(fn `RequestSelectMenuMultiMsg`
  (params (MenuName :type "Array of Name (by ref)") (MenuCursorPos :type Integer) (MenuNewIocn :type "Array of Boolean (by ref)") (MenuOpenDelay :type "Float (double-precision)") (bMenuWaitMsg :type Boolean) (WindowMessageList :type "Array of Name (by ref)") (bWindowExcution :type Boolean) (bWindowSystemMsg :type Boolean) (ButtonFastToneDown :type Boolean))
  (returns (bOk :type Boolean))
  (return false))

(fn `RequestSelectMenuTagValue`
  (params (MenuName :type "Array of Name (by ref)") (MenuCursorPos :type Integer) (MenuNewIocn :type "Array of Boolean (by ref)") (MenuOpenDelay :type "Float (double-precision)") (bMenuWaitMsg :type Boolean) (WindowMessage :type Name) (WindowTagInfo :type "Array of /Game/Blueprints/Facility/Blueprints/FacilityMsgTagInfo Structure (by ref)") (bWindowExcution :type Boolean) (bWindowSystemMsg :type Boolean) (ButtonFastToneDown :type Boolean))
  (returns (bOk :type Boolean))
  (return false))

(fn `RequestYesNoMenu`
  (params (MenuOpenDelay :type "Float (double-precision)") (WindowMessage :type Name) (bWindowExcution :type Boolean) (bWindowSystemMsg :type Boolean) (SpeakingActor :type "Actor Object Reference"))
  (returns (bOk :type Boolean))
  (return false))

(fn `RequestYesNoMenuTagValue`
  (params (MenuOpenDelay :type "Float (double-precision)") (WindowMessage :type Name) (WindowTagInfo :type "Array of /Game/Blueprints/Facility/Blueprints/FacilityMsgTagInfo Structure (by ref)") (bWindowExcution :type Boolean) (bWindowSystemMsg :type Boolean) (SpeakingActor :type "Actor Object Reference"))
  (returns (bOk :type Boolean))
  (return false))

(fn `UpdateSelectMenuInput`
  (params (bPlayActionSE :type Boolean) (bPlayCancelSE :type Boolean) (bPlayCursorSE :type Boolean) (bPlayMessageSE :type Boolean))
  (returns (bAction :type Boolean) (bCancel :type Boolean) (bMoveCursor :type Boolean) (bSkipMessage :type Boolean))
  (return false false false false))