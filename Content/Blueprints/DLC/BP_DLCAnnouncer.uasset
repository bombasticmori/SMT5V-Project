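; BP_DLCAnnouncer is an actor whose interface names indicate it reflects mounted DLC into system data and announces it to the player.
; Interface entry points cover reflect-and-announce, reflect-only, announce-only and task status, alongside a mount-complete event.
; Functions are declared for DLC enable/disable lists and tag-to-name or tutorial-enum conversion.
; All custom bodies here are empty stubs; BeginPlay, Tick and EndPlay only call the parent.
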(event `self.ReceiveBeginPlay`
  (`parent.ReceiveBeginPlay`))

(event `self.ReceiveTick`
  (params (DeltaSeconds :type "Float (single-precision)"))
  (`parent.ReceiveTick` DeltaSeconds))

(event `/Game/Blueprints/DLC/BPI_DLCAnnouncer.BPI_StartTask_DlcReflectAndAnnounce`
  (params (IsBoot :type Boolean)))

(event `/Game/Blueprints/DLC/BPI_DLCAnnouncer.BPI_StartTask_OnlyDlcReflect`
  (params (IsBoot :type Boolean)))

(event `/Game/Blueprints/DLC/BPI_DLCAnnouncer.BPI_StartTask_OnlyAnnounce`)

(event `DLC_OnMountComplete`)

(event `self.ReceiveEndPlay`
  (params (EndPlayReason :type "EEndPlayReason Enum" :default "Destroyed"))
  (`parent.ReceiveEndPlay` EndPlayReason))

(fn `BPI_GetDelegateCheckActor`
  (returns (OutActor :type "/Game/Blueprints/DLC/BP_DLCAnnouncer_DelegateChecker Object Reference"))
  (return null))

(fn `BPI_IsActiveAnnounceTask`
  (returns (IsActiveTask :type Boolean))
  (return false))

(fn `ConvDLC_TagToName`
  (params (InTagList :type "Array of Name (by ref)"))
  (returns (DLC_NameList :type "Array of Name"))
  (return))

(fn `ConvDLC_TagToTutorialEnum`
  (params (InTagList :type "Array of Name (by ref)"))
  (returns (EnumList :type "Array of E_TUTORIAL_WINDOW_MESSAGE_TYPE Enum"))
  (return))

(fn `DLC_AddDisableList`
  (params (In_DLC_Name :type Name)))

(fn `DLC_AddEnableList`
  (params (In_DLC_Name :type Name)))

(fn `DLC_ClearList`)

(fn `RefrectDLC_SystemData`)

(fn `ResetParam`
  (params (ClearList :type Boolean)))

(fn `UserConstructionScript`)