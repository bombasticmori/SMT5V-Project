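; BP_RailActor is a rail actor for the battle camera rig, exposing a camera interface for spline playback, spring arm attachment and command camera info.
; BeginPlay, ResetTransform and the construction script only forward to the parent class, which is not shown here.
; Every other function is an empty stub or returns a default, including spline location queries, arrival checks, play rate, camera side and camera factory accessors.
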(event `self.ReceiveBeginPlay`
  (`parent.ReceiveBeginPlay`))

(event `self.Reset Transform`
  (`parent.Reset Transform`))

(fn `AttachToSpringArm`
  (params (Target :type "Actor Object Reference") (SpringArmName :type Name))
  (returns (IsAttached :type Boolean))
  (return false))

(fn `DbgPrintSplinePoint`)

(fn `DetachToSpringArm`)

(fn `GetCameraSideType`
  (returns (BF_Type :type "E_CAMERA_SIDE_BF_TYPE Enum") (LR_Type :type "E_CAMERA_SIDE_LR_TYPE Enum"))
  (return "E_BF_CAMERA_BACK" "E_LR_CAMERA_LEFT"))

(fn `GetCamFactory`
  (returns (Factory :type "/Game/Blueprints/Battle/FrameWork/Actors/BPI_BattleCamActorFactory Interface"))
  (return null))

(fn `GetCurrentLocationAndRotation`
  (params (length :type "Float (double-precision)") (loop :type Boolean))
  (returns (retLocation :type "Vector Structure") (retDirection :type "Vector Structure") (retRotation :type "Rotator Structure"))
  (return (0.0 0.0 0.0) (0.0 0.0 0.0)))

(fn `GetPlayInfo`
  (returns (m_PlayInfo :type "RigRailPlayInfo Structure"))
  (return))

(fn `GetPlayRate`
  (returns (PlayRate :type "Float (double-precision)"))
  (return 0.0))

(fn `GetSplinePointNum`
  (returns (retValue :type Integer))
  (return 0))

(fn `IsArrived`
  (params (length :type "Float (double-precision)"))
  (returns (retValue :type Boolean))
  (return false))

(fn `IsAttachToSpringArm`
  (returns (IsAttached :type Boolean))
  (return false))

(fn `IsSameCommandCamInfo`
  (params (CommandTargetIndex :type Integer) (SelectedIndex :type Integer) (TargetType :type "E_SKILL_TARGET Enum" :default "E_SKILL_TARGET_INV_SIDE_ONE") (IsSeletingTarget :type Boolean))
  (returns (IsSame :type Boolean))
  (return false))

(fn `ResetTransformImpl`)

(fn `SetCamFactory`
  (params (Factory :type "/Game/Blueprints/Battle/FrameWork/Actors/BPI_BattleCamActorFactory Interface")))

(fn `SetCommandCamInfo`
  (params (CommandTargetIndex :type Integer) (SelectedIndex :type Integer) (TargetType :type "E_SKILL_TARGET Enum" :default "E_SKILL_TARGET_INV_SIDE_ONE") (IsSelectingTarget :type Boolean)))

(fn `SetPlayRate`
  (params (PlayRate :type "Float (double-precision)")))

(fn `UserConstructionScript`
  (`parent.UserConstructionScript`))