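; BP_RailMoveComponent is a component in the battle camera rig folder that declares the interface for moving along a spline rail while looking at a target.
; It exposes playback, distance and speed control, looping or return options, and target tracking with socket override and offset.
; All functions here are empty stubs or return defaults, and Tick only calls the parent, so no movement logic is implemented.
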(event `self.ReceiveTick`
  (params (DeltaSeconds :type "Float (single-precision)"))
  (`parent.ReceiveTick` DeltaSeconds))

(event `Update`
  (params (DeltaSec :type "Float (double-precision)")))

(fn `AddMoveDistance`
  (params (addDistance :type "Float (double-precision)")))

(fn `CalcTargetLocation with Offset`
  (params (TargetLocation :type "Vector Structure") (IsValidTargetLocation :type Boolean) (IsOverrideTargetSocket :type Boolean))
  (returns (ReturnValue :type "Vector Structure"))
  (return (0.0 0.0 0.0)))

(fn `ForceMove`
  (returns (ReturnValue :type "Transform Structure"))
  (return))

(fn `GetFirstTransform`
  (returns (ReturnValue :type "Transform Structure"))
  (return))

(fn `GetSplineLength`
  (returns (retValue :type "Float (double-precision)"))
  (return 0.0))

(fn `IsArrived`
  (returns (retValue :type Boolean))
  (return false))

(fn `IsPlaying`
  (returns (retValue :type Boolean))
  (return false))

(fn `Pause`
  (params (isPause :type Boolean)))

(fn `Play`)

(fn `Reculc Camera Look At`)

(fn `ResetOverrideTarget`)

(fn `SetMoveDistance`
  (params (inDistance :type "Float (double-precision)")))

(fn `SetMoveSpeed`)

(fn `SetOverrideTarget`
  (params (SocketName :type Name)))

(fn `SetPlayInfo`
  (params (isLoop :type Boolean) (isReturn :type Boolean) (target :type "Vector Structure") (isLockTarget :type Boolean) (changeSpeedPoint :type "Float (double-precision)") (firstSpeed :type "Float (double-precision)") (secondSpeed :type "Float (double-precision)") (IsPanCamera :type Boolean)))

(fn `SetSpline`
  (params (inRail :type "/Game/Blueprints/Battle/Blueprint/CamRigRail/BP_RailActor Object Reference")))

(fn `SetTargetActor`
  (params (Target :type "Actor Object Reference")))

(fn `Stop`)

(fn `UpdateMoveDistance`
  (params (tick :type "Float (double-precision)")))

(fn `UpdateTargetLocation`)

(fn `VectorToOrientationRotate`
  (params (inVec :type "Vector Structure") (inUp :type "Vector Structure"))
  (returns (retValue :type "Rotator Structure"))
  (return))