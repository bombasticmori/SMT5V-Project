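; Base Blueprint for battle field checkers, declaring the interface for validating a battle location's angles, origin, ceiling and bottom.
; It declares stub events for trace stages, success, failure and per-check errors, plus helper functions for ground traces, normals, encounter data, visibility and debug logging.
; Apart from a parent BeginPlay call, every event is empty and every function returns defaults or nothing, so no checking logic lives here.
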(event `self.ReceiveBeginPlay`
  (`parent.ReceiveBeginPlay`))

(event `StartTrace`)

(event `Evt_TraceAngle`)

(event `Evt_Failed`)

(event `Evt_TraceCeiling`)

(event `Evt_TraceBottom`)

(event `Evt_Success`)

(event `Evt_AboutAngle`)

(event `Evt_Err_PFAngle`
  (params (angle :type "Float (double-precision)")))

(event `Evt_Err_EFAngle`
  (params (angle :type "Float (double-precision)")))

(event `Evt_Err_Origin`)

(event `Evt_Err_ChipAngle`
  (params (inMesh :type "Object Object Reference") (angle :type "Float (double-precision)")))

(event `Evt_ChipAngleFinished`)

(event `Evt_Err_Celling`
  (params (inMesh :type "Object Object Reference") (ErrorObject :type "Object Object Reference")))

(event `Evt_CellingFinished`)

(event `Evt_Err_Bottom`
  (params (inMesh :type "Object Object Reference")))

(event `Evt_BattleFinished`)

(fn `ApplyEncountPostData`
  (returns (IsDone :type Boolean))
  (return false))

(fn `AroundSearch`)

(fn `ChipNormal`
  (params (inChip :type "SceneComponent Object Reference"))
  (returns (hit :type Boolean) (location :type "Vector Structure") (normal :type "Vector Structure"))
  (return false (0.0 0.0 0.0) (0.0 0.0 0.0)))

(fn `ChipTraceGround`
  (params (chipLocationPoint :type "Array of SceneComponent Object Reference (by ref)") (upVector :type "Vector Structure"))
  (returns (hit :type Boolean) (location :type "Vector Structure") (normal :type "Vector Structure"))
  (return false (0.0 0.0 0.0) (0.0 0.0 0.0)))

(fn `DebugLog`
  (params (str :type String)))

(fn `DisableMeshCollision`)

(fn `GetEncountIDStr`
  (params (inValue :type Integer))
  (returns (retValue :type String))
  (return ""))

(fn `HiddenObject`
  (params (actor :type "Actor Object Reference (by ref)")))

(fn `Initialize`)

(fn `SetAllVisibility`
  (params (sw :type Boolean)))

(fn `TraceGroundObject`
  (params (Base :type "Vector Structure") (Direction :type "Vector Structure") (Length :type "Float (double-precision)") (Radius :type "Float (double-precision)") (DrawDebugType :type "EDrawDebugTrace Enum" :default "None"))
  (returns (Hit :type Boolean) (Location :type "Vector Structure") (Normal :type "Vector Structure") (Surface :type "EPhysicalSurface Enum") (HitActor :type "Actor Object Reference") (HitComponent :type "PrimitiveComponent Object Reference"))
  (return false (0.0 0.0 0.0) (0.0 0.0 0.0) "SurfaceType_Default" null null))

(fn `TriNormal`
  (params (v0 :type "Vector Structure") (v1 :type "Vector Structure") (v2 :type "Vector Structure"))
  (returns (ReturnValue :type "Vector Structure"))
  (return (0.0 0.0 0.0)))

(fn `UserConstructionScript`)