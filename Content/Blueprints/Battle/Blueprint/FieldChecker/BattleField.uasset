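; BattleField is a battle field Blueprint that declares the hooks for setting up an encounter, with every body left as an empty stub or default return.
; Its functions cover field collision, player and enemy side creation, encounter application, added-post and command box lookups, and player replacement, partly through BI_-prefixed variants.
; A PrepareRenzokuBattle event, enemy getter and completion check outline consecutive (renzoku) battles.
; BeginPlay and construction only call the parent.
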(event `self.ReceiveBeginPlay`
  (`parent.ReceiveBeginPlay`))

(event `/Game/Blueprints/Battle/Blueprint/FieldChecker/BPI_BattleField.PrepareRenzokuBattle`
  (params (EncountID :type Integer) (IsEvent :type Boolean) (EnemyIDs :type "Array of Integer (by ref)") (OnlyApplyEncountPostData :type Boolean)))

(fn `ApplyEncount`)

(fn `BI_GetAddPost`
  (params (Index :type Integer))
  (returns (Output :type "SceneComponent Object Reference"))
  (return null))

(fn `BI_GetCommandBoxTransform`
  (returns (Trans :type "Transform Structure"))
  (return))

(fn `BI_GetPlayerReplaceResult`
  (returns (TransformMap :type "Map of Integer to Transform Structure"))
  (return))

(fn `BI_IsReplaceFinished`
  (returns (IsFinished :type Boolean))
  (return false))

(fn `BI_ReplacePlayer`
  (params (InDevilList :type "Array of Integer (by ref)"))
  (returns (NoUse :type Boolean))
  (return false))

(fn `GetAddPost`
  (params (index :type Integer))
  (returns (Output :type "SceneComponent Object Reference"))
  (return null))

(fn `GetCommandBoxTransform`
  (returns (retValue :type "Transform Structure"))
  (return))

(fn `GetRenzokuBattleEnemy`
  (returns (Enemy :type "Array of /Game/Blueprints/Character/Base/CharaBase Object Reference") (EncountID :type Integer))
  (return _ 0))

(fn `IsEndPrepareRenzokuBattle`
  (returns (IsDone :type Boolean))
  (return false))

(fn `MakeEnemySide`
  (params (symbolActor :type "/Game/Blueprints/Character/Base/CharaBase Object Reference") (aroundDevil :type "Array of /Game/Blueprints/Character/Base/CharaBase Object Reference (by ref)") (SpawnIDList :type "Array of Integer (by ref)") (IsRenzokuEncount :type Boolean)))

(fn `MakeEnemySideNoLoad`
  (params (enemyList :type "Array of /Game/Blueprints/Character/Base/CharaBase Object Reference (by ref)")))

(fn `MakePlayerSide`
  (params (isJump :type Boolean)))

(fn `SetFieldCollisionEnable`
  (params (sw :type Boolean)))

(fn `UserConstructionScript`
  (`parent.UserConstructionScript`))