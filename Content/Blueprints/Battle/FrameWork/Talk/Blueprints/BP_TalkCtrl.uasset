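; BP_TalkCtrl is the controller actor for demon negotiation in battle, covering scouting, questions, quizzes, begging for life, mercy and myth talk.
; It declares an event per talk step, plus timelines for hero/demon movement and quiz effects, and async load callbacks.
; Helpers cover tone-based messages, talk/battle cameras, character placement, motion, voice and UI.
; Only BeginPlay and EndPlay do work, calling their parents; everything else is empty or returns defaults.
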(event `self.ReceiveBeginPlay`
  (`parent.ReceiveBeginPlay`))

(event `QuizCharaBlackenEnd__FinishedFunc`)

(event `QuizCharaBlackenEnd__UpdateFunc`)

(event `QuizCharaBlackenEnd__Switch__EventFunc`)

(event `QuizWipeScaleUp1__FinishedFunc`)

(event `QuizWipeScaleUp1__UpdateFunc`)

(event `QuizWipeScaleDown1__FinishedFunc`)

(event `QuizWipeScaleDown1__UpdateFunc`)

(event `QuizWipeScaleDown2__FinishedFunc`)

(event `QuizWipeScaleDown2__UpdateFunc`)

(event `QuizWipeScaleUp2__FinishedFunc`)

(event `QuizWipeScaleUp2__UpdateFunc`)

(event `Timeline_HeroMove__FinishedFunc`)

(event `Timeline_HeroMove__UpdateFunc`)

(event `Timeline_DevilMove__FinishedFunc`)

(event `Timeline_DevilMove__UpdateFunc`)

(event `OnLoaded_741E43CC490ADF7DD89B53ABEF4B0ABF`
  (params (Loaded :type "Object Class Reference")))

(event `OnLoaded_761DA75E441C41587A9750B1D5F1C094`
  (params (Loaded :type "Object Object Reference")))

(event `OnLoaded_741E43CC490ADF7DD89B53AB6619A97F`
  (params (Loaded :type "Object Class Reference")))

(event `OnLoaded_761DA75E441C41587A9750B15CA36354`
  (params (Loaded :type "Object Object Reference")))

(event `OnLoaded_741E43CC490ADF7DD89B53AB846A41FD`
  (params (Loaded :type "Object Class Reference")))

(event `OnLoaded_761DA75E441C41587A9750B1BED08BD6`
  (params (Loaded :type "Object Object Reference")))

(event `OnLoaded_741E43CC490ADF7DD89B53AB5F6202FE`
  (params (Loaded :type "Object Class Reference")))

(event `OnLoaded_761DA75E441C41587A9750B165D8C8D5`
  (params (Loaded :type "Object Object Reference")))

(event `OnLoaded_741E43CC490ADF7DD89B53AB66A6FE94`
  (params (Loaded :type "Object Class Reference")))

(event `OnLoaded_761DA75E441C41587A9750B15C1C34BF`
  (params (Loaded :type "Object Object Reference")))

(event `OnLoaded_741E43CC490ADF7DD89B53ABAA07768C`
  (params (Loaded :type "Object Class Reference")))

(event `OnLoaded_761DA75E441C41587A9750B190BDBCA7`
  (params (Loaded :type "Object Object Reference")))

(event `OnLoaded_18FAE4904585CCCFC8DBDA928F723BF6`
  (params (Loaded :type "Object Object Reference")))

(event `OnLoaded_B56F8E0A4087071A01A318948B471DC5`
  (params (Loaded :type "Object Object Reference")))

(event `OnLoaded_58C4F3A344E087E21CF022AE0F7992D0`
  (params (Loaded :type "Object Object Reference")))

(event `OnLoaded_8A43E0E34A09FF2BD22DEF97D37BA0EA`
  (params (Loaded :type "Object Object Reference")))

(event `OnLoaded_33A06C84454230A0AF018496357EBD8F`
  (params (Loaded :type "Object Class Reference")))

(event `OnLoaded_E060ACA34EE950C8F482EFA05F326ED6`
  (params (Loaded :type "Object Class Reference")))

(event `OnLoaded_853A0F8D4A75D88EE001D69CB60C398D`
  (params (Loaded :type "Object Class Reference")))

(event `OnLoaded_956CDAE3404572E86E1930BBBCB3B75A`
  (params (Loaded :type "Object Object Reference")))

(event `OnLoaded_8E5A00544AC4BCD3F46BB1B58EB058A6`
  (params (Loaded :type "Object Object Reference")))

(event `EvtOpenMsgbyLabel`
  (params (Label :type Name) (IsDevil :type Boolean) (CameraType :type "/Game/Blueprints/Battle/FrameWork/Talk/Enums/E_TalkCamera Enum" :default "NewEnumerator4")))

(event `EvtOpenToneMsgById`
  (params (MsgId :type Integer) (IsDevilSpeak :type Boolean) (CameraType :type "/Game/Blueprints/Battle/FrameWork/Talk/Enums/E_TalkCamera Enum" :default "NewEnumerator4")))

(event `EvtOpenSysMsg`
  (params (Label :type Name) (CameraType :type "/Game/Blueprints/Battle/FrameWork/Talk/Enums/E_TalkCamera Enum" :default "NewEnumerator4")))

(event `Evt_WantPartStart`)

(event `Evt_WantChoice`)

(event `Evt_WantAcCard`)

(event `Evt_WantReaction`)

(event `Evt_WantReactionTutorial`)

(event `Evt_QuizStart`)

(event `Evt_QuizSummon`)

(event `Evt_QuizQuestion`)

(event `Evt_QuizAnswer`)

(event `Evt_TalkNG`
  (params (NGType :type "E_TALK_NG_TYPE Enum" :default "E_NONE")))

(event `Evt_MercyTalkStart`)

(event `Evt_MercyTalkLoopStart`)

(event `Evt_MercyTalkYes`)

(event `Evt_MercyTalkEndMercy`)

(event `Evt_MercyTalkNo`)

(event `Evt_MercyTalkEndNo`)

(event `Evt_MythSpawnDevil`
  (params (DevilId :type Integer)))

(event `Evt_MythMessage`)

(event `Evt_MythEnd`)

(event `Evt_MythBegin`)

(event `Evt_MythEnemyTurn`)

(event `Evt_BeglifeBegin`)

(event `Evt_BeglifeMoney`)

(event `Evt_BeglifeChoice`)

(event `Evt_BeglifeDie`)

(event `Evt_BeglifeNkm`)

(event `Evt_BeglifeMoneyLoop`)

(event `Evt_BeglifeSuccessEnd`)

(event `Evt_BeglifeSoul`)

(event `Evt_BeglifeIncense`)

(event `Evt_ChangeMotionDelay`
  (params (MotionId :type "E_CHARA_MOTION_ID Enum" :default "NONE") (Delay :type "Float (double-precision)")))

(event `Evt_DebugCmd_ChangeTone`)

(event `Evt_ShowItemPanel`
  (params (ItemId :type Integer) (Add :type Integer)))

(event `Evt_ShowMoneyPanel`
  (params (MoneyAdd :type Integer)))

(event `Evt_HeroMove`
  (params (StartTransform :type "Transform Structure") (TargetTransform :type "Transform Structure")))

(event `Evt_DevilMove`
  (params (StartTransform :type "Transform Structure") (TargetTransform :type "Transform Structure")))

(event `Evt_SetAddMoneyPanel`
  (params (MoneyAdd :type Integer)))

(event `Evt_UniqueSkillDevilDisappear`)

(event `Evt_ScoutFirst`)

(event `Evt_ScoutMythBranch`)

(event `Evt_TalkQuestion`)

(event `Evt_ScoutSuccess`)

(event `Evt_ScoutFail`)

(event `Evt_ScoutNothing`)

(event `Evt_EndScout`)

(event `Evt_QuestionBranch`)

(event `Evt_QuestionLotReaction`)

(event `Evt_ScoutFailAnimation`)

(event `Evt_BeginChoice`)

(event `Evt_CancelTalk`)

(event `Evt_Cancel1`)

(event `Evt_Cancel2`)

(event `Evt_QuestionReactionProc`)

(event `Evt_ScoutLeaveAnimation`)

(event `Evt_ScoutEnemyTurnAnimation`)

(event `Evt_MoonTemperBranch`)

(event `Evt_FriendTalk`)

(event `Evt_LevelWaitFlag`)

(event `Evt_MoonTemperGood`)

(event `Evt_ScoutSafetyQuestion`)

(event `Evt_ScoutNkmUnconditional`)

(event `Evt_ScoutSafetyWant`)

(event `Evt_StockWaitFlag`)

(event `Evt_HeroBadStatus`)

(event `Evt_YoroCameraCheck`)

(event `Evt_ApologyWaitFlag`)

(event `Evt_LotQuiz`)

(event `self.ReceiveEndPlay`
  (params (EndPlayReason :type "EEndPlayReason Enum" :default "Destroyed"))
  (`parent.ReceiveEndPlay` EndPlayReason))

(event `Evt_InitScene`)

(event `Evt_TalkStartBranch`)

(event `Evt_TalkEnd`)

(fn `ApplyDistance`
  (params (Distance :type "Float (double-precision)")))

(fn `BackModelView`)

(fn `ChangeBtlCamera`)

(fn `ChangeMotion`
  (params (MotionID :type "E_CHARA_MOTION_ID Enum" :default "NONE")))

(fn `ChangeTalkCamera`)

(fn `CheckMotion`
  (returns (MotionType :type "E_CHARA_MOTION_ID Enum") (Check :type Boolean))
  (return "NONE" false))

(fn `CheckPadAction`
  (returns (Success :type Boolean))
  (return false))

(fn `CheckTalkEnd`
  (returns (IsEnd :type Boolean))
  (return false))

(fn `DebugCameraOff`)

(fn `DebugCmd_ChangeTone`)

(fn `DebugStartInfo`)

(fn `FindDevilUnit`
  (returns (Unit :type "/Game/Blueprints/Character/Base/CharaBase Object Reference"))
  (return null))

(fn `FindHeroUnit`
  (returns (Unit :type "/Game/Blueprints/Character/Base/CharaBase Object Reference"))
  (return null))

(fn `FindLookAtRotation_Daath`
  (params (Start :type "Vector Structure") (Target :type "Vector Structure") (ZOnly :type Boolean))
  (returns (ReturnValue :type "Rotator Structure"))
  (return))

(fn `GetBIMainWork`
  (returns (BPI :type "/Game/Blueprints/Battle/FrameWork/Actors/BPI_BattleMain Interface"))
  (return null))

(fn `GetBIPartySystem`
  (returns (ret :type "/Game/Blueprints/Battle/FrameWork/Actors/BPI_BattleParty Interface"))
  (return null))

(fn `GetBISoundManager`
  (returns (ret :type "/Game/Blueprints/Battle/FrameWork/Actors/BPI_BattleSoundManager Interface"))
  (return null))

(fn `GetDefaultTone`
  (returns (Tone :type "E_TALK_TONE_TYPE Enum"))
  (return "E_NONE"))

(fn `GetDevilBase`
  (returns (DevilBase :type "/Game/Blueprints/Character/Base/DevilBase Object Reference"))
  (return null))

(fn `GetDevilCharaBase`
  (returns (CharaBase :type "/Game/Blueprints/Character/Base/CharaBase Object Reference"))
  (return null))

(fn `GetDevilMesh`
  (returns (Mesh :type "SkeletalMeshComponent Object Reference"))
  (return null))

(fn `GetDevilTransform`
  (returns (Transform :type "Transform Structure"))
  (return))

(fn `GetHeroCamTarget`
  (returns (CamTarget :type "Transform Structure"))
  (return))

(fn `GetHeroCharaBase`
  (returns (CharaBase :type "/Game/Blueprints/Character/Base/CharaBase Object Reference"))
  (return null))

(fn `GetHeroTransform`
  (returns (Transform :type "Transform Structure"))
  (return))

(fn `GetMsgText_ById`
  (params (MsgId :type Integer) (IsDevil :type Boolean))
  (returns (Text :type Text))
  (return ""))

(fn `GetMsgText_ByLabel`
  (params (Label :type Name) (IsDevil :type Boolean))
  (returns (Text :type Text))
  (return ""))

(fn `GetMsgTextList_ByIdList`
  (params (IdList :type "Array of Integer (by ref)") (IsDevil :type Boolean))
  (returns (TextList :type "Array of Text"))
  (return))

(fn `GetQuizGlowRadiusModify`
  (returns (Modify :type "Float (double-precision)"))
  (return 0.0))

(fn `GetShortcutLabel`
  (returns (Label :type Name))
  (return "None"))

(fn `GetTalkAssetInfo`
  (params (Tone :type "E_TALK_TONE_TYPE Enum" :default "E_NONE"))
  (returns (AssetInfo :type "/Game/Blueprints/Battle/FrameWork/Talk/Blueprints/TalkAssetInfo Structure"))
  (return))

(fn `GetTalkCameraOffsetTable`
  (params (DevilID :type Integer))
  (returns (CameraOffset :type "/Game/Blueprints/Camp/Status/ST_TalkCameraOffset Structure"))
  (return))

(fn `GetText_ByLabel`
  (params (B :type Name))
  (returns (Item :type Text))
  (return ""))

(fn `GetToneMsgAsset_Soft`
  (params (Index :type "E_TALK_TONE_TYPE Enum" :default "E_NONE"))
  (returns (ReturnValue :type "ScriptMessageAsset Soft Object Reference"))
  (return null))

(fn `GetToneTable_Soft`
  (params (Tone :type "E_TALK_TONE_TYPE Enum" :default "E_NONE"))
  (returns (Asset :type "Object Soft Object Reference"))
  (return null))

(fn `GetWantReacCardLabel`
  (returns (CardLabel :type Name))
  (return "None"))

(fn `HideBtlUI`)

(fn `InitChara`)

(fn `IsBGMChanged`
  (returns (Changed :type Boolean))
  (return false))

(fn `IsMagatsukaEncount`
  (returns (IsMagatsuka :type Boolean))
  (return false))

(fn `IsModelVisible`
  (params (Chara :type "/Game/Blueprints/Character/Base/CharaBase Object Reference"))
  (returns (IsVisible :type Boolean))
  (return false))

(fn `IsMoveCameraForMsg`
  (returns (Move :type Boolean))
  (return false))

(fn `IsMythMode`
  (returns (IsMythMode :type Boolean))
  (return false))

(fn `LotQuestionEx`)

(fn `MakeUpToneTable`)

(fn `MoveHero`
  (params (IsTalk :type Boolean) (isMoving :type Boolean)))

(fn `OnlyModelView`)

(fn `PlayReactionVoice`)

(fn `PlaySe`
  (params (Type :type Integer)))

(fn `PlayVoice`
  (params (TalkVoice :type "EDevilTalkVoice Enum" :default "None") (DontAttachToTalker :type Boolean)))

(fn `PrintCamera`)

(fn `PrintCameraTable`)

(fn `ResetPlayerGaze`)

(fn `SaveStartTransform`)

(fn `SetBattleTransform`)

(fn `SetSword`
  (params (On :type Boolean)))

(fn `SetTagValue`
  (params (ValueIndex :type Integer) (Value :type Integer)))

(fn `SetupQuizChara`
  (params (QuizChara :type "/Game/Blueprints/Character/Base/DevilBase Object Reference")))

(fn `ShowBtlUI`)

(fn `ShowHero`
  (params (IsShow :type Boolean)))

(fn `StartGaze`)

(fn `UserConstructionScript`)