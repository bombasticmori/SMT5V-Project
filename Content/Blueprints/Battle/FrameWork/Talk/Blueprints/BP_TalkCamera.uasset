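; BP_TalkCamera is the camera for battle talk scenes, framing the player, enemy demon and friend models.
; Its interface covers eased moves by camera type, table index or target, plus status, quiz and unique-skill shots with per-demon lookups.
; Helpers handle eye/look offsets, model scale, ground clearance, unit hiding, shake and debug.
; Function bodies here are empty stubs; only BeginPlay, Tick and EndPlay call their parent implementations.
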(event `self.ReceiveBeginPlay`
  (`parent.ReceiveBeginPlay`))

(event `self.ReceiveTick`
  (params (DeltaSeconds :type "Float (single-precision)"))
  (`parent.ReceiveTick` DeltaSeconds))

(event `Timeline_Camera__FinishedFunc`)

(event `Timeline_Camera__UpdateFunc`)

(event `Evt_MoveCameraCore`
  (params (Start :type "Transform Structure") (Target :type "Transform Structure") (Time :type "Float (double-precision)") (IsEase :type Boolean) (ModelHide :type "E_TALK_CAMERA_MODEL_HIDE Enum" :default "E_NONE")))

(event `self.ReceiveEndPlay`
  (params (EndPlayReason :type "EEndPlayReason Enum" :default "Destroyed"))
  (`parent.ReceiveEndPlay` EndPlayReason))

(fn `AboveGround`
  (params (InLocation :type "Vector Structure"))
  (returns (OutLocation :type "Vector Structure"))
  (return (0.0 0.0 0.0)))

(fn `ApplyDebug`)

(fn `ApplyModelHide`
  (params (ModelHide :type "E_TALK_CAMERA_MODEL_HIDE Enum" :default "E_NONE")))

(fn `CalcBaseLocationStatus`)

(fn `CalcCameraTransform`
  (params (CameraParam :type "TalkCameraParam Structure (by ref)") (CameraType :type "/Game/Blueprints/Battle/FrameWork/Talk/Enums/E_TalkCamera Enum" :default "NewEnumerator4"))
  (returns (OutTransform :type "Transform Structure"))
  (return))

(fn `CalcCameraTransformOfTable`
  (params (TableIndex :type Integer) (IsDebug :type Boolean))
  (returns (Out :type "Transform Structure"))
  (return))

(fn `CheckCameraAnim`
  (returns (IsMove :type Boolean))
  (return false))

(fn `FindLookAtRocation_Daath`
  (params (Start :type "Vector Structure (by ref)") (Target :type "Vector Structure (by ref)") (ZOnly :type Boolean))
  (returns (ReturnValue :type "Rotator Structure"))
  (return))

(fn `GetCameraEye_Normal`
  (params (ToEnemyRate :type "Float (double-precision)") (Distance :type "Float (double-precision)") (Height :type "Float (double-precision)"))
  (returns (Eye :type "Vector Structure"))
  (return (0.0 0.0 0.0)))

(fn `GetCameraLook_Normal`
  (params (ToEnemyRate :type "Float (double-precision)") (HeightOffset :type "Float (double-precision)"))
  (returns (Look :type "Vector Structure"))
  (return (0.0 0.0 0.0)))

(fn `GetCameraParam_MythFriendUp`
  (returns (Eye :type "Vector Structure") (Look :type "Vector Structure"))
  (return (0.0 0.0 0.0) (0.0 0.0 0.0)))

(fn `GetCameraParam_Yoro`
  (returns (Eye :type "Vector Structure") (Look :type "Vector Structure"))
  (return (0.0 0.0 0.0) (0.0 0.0 0.0)))

(fn `GetCameraTransform`
  (params (CameraType :type "/Game/Blueprints/Battle/FrameWork/Talk/Enums/E_TalkCamera Enum" :default "NewEnumerator4"))
  (returns (Transform :type "Transform Structure"))
  (return))

(fn `GetEyeOffset_MythFriendUp`
  (returns (EyeOffset :type "Vector Structure"))
  (return (0.0 0.0 0.0)))

(fn `GetEyeOffset_Status`
  (returns (EyeOffset :type "Vector Structure"))
  (return (0.0 0.0 0.0)))

(fn `GetEyeOffset_Yoro`
  (returns (EyeOffset :type "Vector Structure"))
  (return (0.0 0.0 0.0)))

(fn `GetLookOffset_MythFriendUp`
  (returns (LookOffset :type "Vector Structure"))
  (return (0.0 0.0 0.0)))

(fn `GetLookOffset_Status`
  (returns (LookOffset :type "Vector Structure"))
  (return (0.0 0.0 0.0)))

(fn `GetLookOffset_Yoro`
  (returns (LookOffset :type "Vector Structure"))
  (return (0.0 0.0 0.0)))

(fn `GetTargetHeight`
  (returns (Out :type "Float (double-precision)"))
  (return 0.0))

(fn `IsCameraReverse`
  (params (T1 :type "Transform Structure") (T2 :type "Transform Structure"))
  (returns (IsReverse :type Boolean))
  (return false))

(fn `ModifyEyeFromCameraScale`
  (params (Eye :type "Vector Structure") (Look :type "Vector Structure") (CameraScale :type "Float (double-precision)"))
  (returns (ModifiedEye :type "Vector Structure"))
  (return (0.0 0.0 0.0)))

(fn `MoveCamera`
  (params (Target :type "Transform Structure") (Time :type "Float (double-precision)") (IsEase :type Boolean)))

(fn `MoveCamera_ByTable`
  (params (Time :type "Float (double-precision)") (TableIndex :type Integer) (ModelHide :type Boolean)))

(fn `MoveCamera_ByType`
  (params (CameraType :type "/Game/Blueprints/Battle/FrameWork/Talk/Enums/E_TalkCamera Enum" :default "NewEnumerator4") (Time :type "Float (double-precision)") (ForceMove :type Boolean) (Ease :type Boolean)))

(fn `MoveCamera_Quiz`
  (params (Time :type "Float (double-precision)") (IsEase :type Boolean) (StatusModel :type "/Game/Blueprints/Character/Base/CharaBase Object Reference") (DevilId :type Integer)))

(fn `MoveCamera_Status`
  (params (Time :type "Float (double-precision)") (IsEase :type Boolean) (StatusModel :type "/Game/Blueprints/Character/Base/CharaBase Object Reference") (DevilId :type Integer)))

(fn `MoveCamera_UniqueSkill`
  (params (Time :type "Float (double-precision)") (IsEase :type Boolean) (UniqueSkillModel :type "/Game/Blueprints/Character/Base/CharaBase Object Reference") (DevilId :type Integer)))

(fn `PrintInfo`)

(fn `ResetDebug`)

(fn `SearchQuizTable`
  (params (DevilId :type Integer))
  (returns (QuizTableRow :type "TalkQuizCameraTableRow Structure"))
  (return))

(fn `SearchTalkCameraOffsetTable`
  (params (DevilId :type Integer))
  (returns (CameraOffset :type "/Game/Blueprints/Camp/Status/ST_TalkCameraOffset Structure"))
  (return))

(fn `SetCameraTransform`
  (params (CameraType :type "/Game/Blueprints/Battle/FrameWork/Talk/Enums/E_TalkCamera Enum" :default "NewEnumerator4") (Transform :type "Transform Structure (by ref)")))

(fn `SetParam`
  (params (BaseCameraTransform :type "Transform Structure") (PlayerFace :type "Transform Structure (by ref)") (PlayerChest :type "Transform Structure (by ref)") (EnemyFace :type "Transform Structure (by ref)") (EnemyBody :type "Transform Structure (by ref)") (HeroTalkTransform :type "Transform Structure") (PlayerCameraScale :type "Float (double-precision) (by ref)") (EnemyCameraScale :type "Float (double-precision) (by ref)") (PlayerLocationOffset :type "Vector Structure") (MythMode :type "Boolean (by ref)") (UpVector :type "Vector Structure") (FriendModel :type "/Game/Blueprints/Character/Base/CharaBase Object Reference (by ref)") (EnemyModel :type "/Game/Blueprints/Character/Base/CharaBase Object Reference (by ref)") (EyeOffsetYoro :type "Vector Structure") (LookOffsetYoro :type "Vector Structure")))

(fn `SetQuizTable`
  (params (DevilId :type Integer) (InTableRow :type "TalkQuizCameraTableRow Structure")))

(fn `SetShakeParam`
  (params (IsMythMode :type Boolean)))

(fn `SetTableDataIndex`
  (params (index :type Integer)))

(fn `SetUnitVisibility`
  (params (Chara :type "/Game/Blueprints/Character/Base/CharaBase Object Reference") (Visible :type Boolean)))

(fn `ShakeCameraReset`)

(fn `ShakeCameraRestart`)

(fn `ShakeCameraStart`)

(fn `ShakeCameraStop`)

(fn `UpdateCameraTransform`)

(fn `UpdateShake`
  (params (DeltaSeconds :type "Float (double-precision)")))

(fn `UserConstructionScript`)