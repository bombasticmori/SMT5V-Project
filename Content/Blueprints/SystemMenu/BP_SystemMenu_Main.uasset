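; BP_SystemMenu_Main is an actor Blueprint for the game's system menu, mostly an empty skeleton in this file.
; It declares stub events for init, menu start and end, blur in/out completion, level-load completion and player locking.
; Menu step functions outline a start/end state flow with a Top step, but only ChangeMenuStep has logic, forwarding to its parent.
; BeginPlay, Tick and the construction script also just call the parent.
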(event `self.ReceiveBeginPlay`
  (`parent.ReceiveBeginPlay`))

(event `self.ReceiveTick`
  (params (DeltaSeconds :type "Float (single-precision)"))
  (`parent.ReceiveTick` DeltaSeconds))

(event `StartSystemMenu`)

(event `EndBlurIn`)

(event `Evdis_EndLevelLoad_イベント_0`)

(event `EndSystemMenu`)

(event `Evdis_EndBlurOut_イベント_0`)

(event `SetPlayerLock`
  (params (IsLock :type Boolean)))

(event `Init`)

(fn `ChangeMenuStep`
  (params (NextStep :type "/Game/Blueprints/SystemMenu/E_SYSMENU_STEP Enum" :default "NewEnumerator0"))
  (returns (ret :type Boolean))
  (bind _ret (`parent.ChangeMenuStep` NextStep))
  (return _ret))

(fn `EndMenuStep`
  (params (Step :type "/Game/Blueprints/SystemMenu/E_SYSMENU_STEP Enum" :default "NewEnumerator0")))

(fn `EndMenuStep_Top`)

(fn `GetCompornent`
  (params (Index :type "/Game/Blueprints/SystemMenu/E_SYSMENU_STEP Enum" :default "NewEnumerator0"))
  (returns (ActCompornent :type "/Game/Blueprints/SystemMenu/Actor/SysMenu_CompornentBase Object Reference"))
  (return null))

(fn `StartMenuStep`
  (params (Step :type "/Game/Blueprints/SystemMenu/E_SYSMENU_STEP Enum" :default "NewEnumerator0")))

(fn `StartMenuStep_Top`)

(fn `UserConstructionScript`
  (`parent.UserConstructionScript`))